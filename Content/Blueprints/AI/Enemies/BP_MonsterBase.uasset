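; Base alien enemy Character that holds AI state (seen player, chasing flag, patrol route) and maps movement states to walk speeds.
; Pawn sensing records the seen pawn, and getters and setters expose that state.
; A box overlap repeatedly applies randomized timed damage until the overlap ends.
; Incoming damage is reported as an AI sense event and reduces AlienHP, triggering ragdoll death and disabled movement at zero.
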(event `/Game/Blueprints/Interfaces/BPI_EnemyAI.SetSeenPlayer`
  (params (SeenPlayer :type "Pawn Object Reference"))
  (set `self.SeenPlayer` SeenPlayer))

(event `Attack`
  (`self.Jump`)
  (`KismetSystemLibrary.PrintString` "Attacking Player"))

(event `Local_EventDamage`
  (params (Damage :type "Float (double-precision)") (`Damage Type` :type "DamageType Object Reference") (`Instigated By` :type "Controller Object Reference") (`Damage By` :type "Actor Object Reference"))
  ; Alien Death Sequence
  (`AISense_Damage.ReportDamageEvent` self `Instigated By` Damage (`self.K2_GetActorLocation`))
  (bind _output_get (set `self.AlienHP` (- (`self.AlienHP`) Damage)))
  (`KismetSystemLibrary.PrintString` (`KismetStringLibrary.Conv_DoubleToString` _output_get))
  (if (<= (`self.AlienHP`) 0.0)
    (`self.AlienDeath`)))

(event `self.ReceiveAnyDamage`
  (params (Damage :type "Float (single-precision)") (DamageType :type "DamageType Object Reference") (InstigatedBy :type "Controller Object Reference") (DamageCauser :type "Actor Object Reference"))
  (`self.Local_EventDamage` Damage DamageType InstigatedBy DamageCauser))

(event `AlienDeath`
  (`PrimitiveComponent.SetSimulatePhysics` (`self.Mesh`) true)
  (`CharacterMovementComponent.DisableMovement` (`self.CharacterMovement`)))

(event `self.Box.OnComponentBeginOverlap`
  (params (OverlappedComponent :type "PrimitiveComponent Object Reference") (OtherActor :type "Actor Object Reference") (OtherComp :type "PrimitiveComponent Object Reference") (OtherBodyIndex :type Integer) (bFromSweep :type Boolean) (SweepResult :type "HitResult Structure (by ref)"))
  (set `self.Attacking?` true)
  (`GameplayStatics.ApplyDamage` OtherActor (`KismetMathLibrary.Conv_IntToDouble` (`KismetMathLibrary.Round` (`KismetMathLibrary.RandomFloatInRange` 25.0 35.0))) null self :!label _label)
  (`KismetSystemLibrary.Delay` 1.5)
  (if (`self.Attacking?`)
    (goto _label)))

(event `/Game/Blueprints/Interfaces/BPI_EnemyAI.SetIsChasing`
  (params (Chasing :type Boolean))
  (set `self.ChasingPlayer?` Chasing))

(event `self.PawnSensing.OnSeePawn`
  (params (Pawn :type "Pawn Object Reference"))
  (set `self.SeenPlayer` Pawn))

(event `self.Box.OnComponentEndOverlap`
  (params (OverlappedComponent :type "PrimitiveComponent Object Reference") (OtherActor :type "Actor Object Reference") (OtherComp :type "PrimitiveComponent Object Reference") (OtherBodyIndex :type Integer))
  (set `self.Attacking?` false))

(fn `GetISChasing`
  (returns (Chasing :type Boolean))
  (return (`self.ChasingPlayer?`)))

(fn `GetPatrolRoute`
  (returns (PatrolRoute :type "/Game/Blueprints/AI/BP_PatrolRoute Object Reference"))
  (return (`self.PatrolRoute`)))

(fn `GetSeenPlayer`
  (returns (SeenPlayer :type "Pawn Object Reference"))
  (return (`self.SeenPlayer`)))

(fn `SetMovementSpeed`
  (params (Speed :type "/Game/Blueprints/AI/AIv2/E_MovementSpeed Enum" :default "NewEnumerator0"))
  (returns (SpeedValue :type "Float (double-precision)"))
  (bind _output_get (set `CharacterMovementComponent.MaxWalkSpeed` (select `/Game/Blueprints/AI/AIv2/E_MovementSpeed` Speed :`NewEnumerator1` 150.0 :`NewEnumerator2` 300.0 :`NewEnumerator3` 500.0 :!type "Float (single-precision)") (`self.CharacterMovement`)))
  (return _output_get))

(fn `UserConstructionScript`)