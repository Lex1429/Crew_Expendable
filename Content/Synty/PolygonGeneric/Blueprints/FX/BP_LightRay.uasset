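; BP_LightRay is a placeable light ray effect that stretches a cube or round ray mesh along a spline.
; The construction script adds a manually attached spline mesh, picks its mesh from LightRayType, and bends it between the first two LightSpline points using world-space positions and tangents.
; BaseSize and TargetSize set the uniform start and end cross-section scales, allowing the ray to taper or widen.
; The event graph has no runtime logic.
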(fn `UserConstructionScript`
  (bind _lightspline (`self.LightSpline`))
  (bind _basesize (`self.BaseSize`))
  (bind _targetsize (`self.TargetSize`))
  (bind _returnvalue (`AddComponent|NODE_AddSplineMeshComponent-0` :`bManualAttachment` true))
  (`StaticMeshComponent.SetStaticMesh` _returnvalue (select `byte` (`self.LightRayType`) :`0` "/Game/Synty/PolygonGeneric/Meshes/FX/SM_LightRay_Cube_01.SM_LightRay_Cube_01" :`1` "/Game/Synty/PolygonGeneric/Meshes/FX/SM_LightRay_Round_01.SM_LightRay_Round_01" :!type "StaticMesh Object Reference"))
  (`SplineMeshComponent.SetStartAndEnd` _returnvalue (`SplineComponent.GetLocationAtSplinePoint` _lightspline 0 "World") (`SplineComponent.GetTangentAtSplinePoint` _lightspline 0 "World") (`SplineComponent.GetLocationAtSplinePoint` _lightspline 1 "World") (`SplineComponent.GetTangentAtSplinePoint` _lightspline 1 "World") false)
  (`SplineMeshComponent.SetStartScale` _returnvalue (`KismetMathLibrary.MakeVector2D` _basesize _basesize) false)
  (`SplineMeshComponent.SetEndScale` _returnvalue (`KismetMathLibrary.MakeVector2D` _targetsize _targetsize) true))