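; BP_Hallway2 is a modular hallway building piece with supports, legs and an overhead light.
; Its construction script applies MasterMaterial to the hallway, support and leg meshes and sets both legs' height offset from LegLegnth.
; It also copies its RoomTag into the OverheadLight1 child actor, a BP_LampBase.
; The event graph holds no active logic.
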(fn `UserConstructionScript`
  (bind _leglegnth (`self.LegLegnth`))
  (`PrimitiveComponent.SetMaterial` (`self.Hallway`) 0 (`self.MasterMaterial`))
  (`PrimitiveComponent.SetMaterial` (`self.Support1`) 0 (`self.MasterMaterial`))
  (`PrimitiveComponent.SetMaterial` (`self.Leg1`) 0 (`self.MasterMaterial`))
  (`PrimitiveComponent.SetMaterial` (`self.Support2`) 0 (`self.MasterMaterial`))
  (`PrimitiveComponent.SetMaterial` (`self.Leg2`) 0 (`self.MasterMaterial`))
  (`SceneComponent.K2_SetRelativeLocation` (`self.Leg1`) (`KismetMathLibrary.MakeVector` 0.0 155.0 _leglegnth) false false)
  (`SceneComponent.K2_SetRelativeLocation` (`self.Leg2`) (`KismetMathLibrary.MakeVector` 0.0 155.0 _leglegnth) false false)
  (bind _asbp_lamp_base (cast `/Game/Blueprints/Interactables/CealingLights/BP_LampBase` (`ChildActorComponent.ChildActor` (`self.OverheadLight1`))))
  (set `/Game/Blueprints/Interactables/CealingLights/BP_LampBase.RoomTag` (`self.RoomTag`) _asbp_lamp_base))