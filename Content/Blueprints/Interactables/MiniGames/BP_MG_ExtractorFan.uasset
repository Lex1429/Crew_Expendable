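; Minigame extractor fan that starts spinning and clears the station smoke post-process effect once its linked AC vent is repaired.
; Binds to the vent's repaired event, which plays the FanRotation timeline to rotate the blades.
; Each timeline update also spawns an attached fan sound and zeroes Opacity in the post-process parameter collection.
; A dynamic smoke material is created at BeginPlay but not used afterwards.
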(event `self.ReceiveBeginPlay`
  (add `/Game/Blueprints/Interactables/MiniGames/BP_MG_AirVent_v2.ACRepaired` (`self.ACVentRef`) (delegate `ACRepaired`))
  (bind _returnvalue (`KismetMaterialLibrary.CreateDynamicMaterialInstance` "/Game/Materials/PostProccess/PPMI_StationSmoke.PPMI_StationSmoke"))
  (set `self.SmokeRef` _returnvalue))

(event `ACRepaired`
  (`self.FanTimer`))

(event `FanTimer`
  (bind (_direction _newtrack_0) (`Timeline|FanRotation`)
    (:`Update`
      (`SceneComponent.K2_SetRelativeRotation` (`self.SM_Prop_Extractor_Fan_01_Blades_01`) (`KismetMathLibrary.RLerp` (struct) (struct :`Pitch` 360.0) _newtrack_0) false false)
      (`GameplayStatics.SpawnSoundAttached` "/Game/SFX/EnviromentSounds/Fan-Continue_001.Fan-Continue_001" (`self.SM_Prop_Extractor_Fan_01`) "None" (0.0 0.0 0.0) (struct) "KeepRelativeOffset" false 1.0 1.0 0.0 "/Game/MBLS/Assets/Audio/Classes/SA_Short.SA_Short" null)
      (`KismetMaterialLibrary.SetScalarParameterValue` "/Game/Materials/PostProccess/MPC_PostProccess.MPC_PostProccess" "Opacity"))))

(fn `UserConstructionScript`)