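; Base Blueprint for in-world mini-game screens, with overridable action, exit and camera-blend events for specific games.
; Enabling or disabling swaps the screen between idle and offline dynamic materials.
; Overlap checks record the player, and a looping timer compares facing against the arrow to toggle the idle material's key prompt.
; It also filters axis input by gamepad sensitivity and adds research points to the game state on success.
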(event `EnableMiniGame`
  ;[1 1 1] Init
  (`PrimitiveComponent.SetMaterial` (`self.MiniGameScreen`) 0 (`self.DMI_Idle`) :!label _label)
  (set `self.MiniGameEnabled` true))

(event `self.ReceiveBeginPlay`
  ;[1 1 1] Init
  (bind _returnvalue (`KismetSystemLibrary.K2_SetTimer` null "CheckPlayerDirection" 0.15 true))
  (set `self.CheckPlayerDirectionHandle` _returnvalue)
  (set `self.PlayerOverlapped` false)
  (set `self.PlayerDetected` false)
  (set `self.IsMiniGameActivated` false)
  (set `self.InputEnable` true)
  (set `self.RightAxis` 0.0)
  (set `self.ForwardAxis` 0.0)
  ;;[1 1 1] Idle material
  (bind _returnvalue_2 (`KismetMaterialLibrary.CreateDynamicMaterialInstance` "/Game/MiniGames2/Materials/MI_MiniGamesIdle_Inst.MI_MiniGamesIdle_Inst"))
  (set `self.DMI_Idle` _returnvalue_2)
  ;;[1 1 1] Offline material
  (bind _returnvalue_3 (`KismetMaterialLibrary.CreateDynamicMaterialInstance` "/Game/MiniGames2/Materials/MI_MiniGameOffline_Inst.MI_MiniGameOffline_Inst"))
  (set `self.DMI_Offline` _returnvalue_3)
  (if (`self.MiniGameEnabled`)
    (goto _label)
    (else
      (`PrimitiveComponent.SetMaterial` (`self.MiniGameScreen`) 0 (`self.DMI_Offline`) :!label _label_2)
      (set `self.MiniGameEnabled` false))))

(event `DisableMiniGame`
  ;[1 1 1] Init
  (goto _label_2))

(event `Server_DisableMiniGame`
  ;[1 1 1] Init
  (`self.DisableMiniGame`))

(event `InputAxis|MoveForward` :consume false
  (params (AxisValue :type "Float (single-precision)")))

(event `EnhancedInput|/Game/Blueprints/Inputs/IA_NextCamera`
  (params (ActionValue :type "Float (double-precision)") (ElapsedSeconds :type "Float (double-precision)") (TriggeredSeconds :type "Float (double-precision)") (InputAction :type "InputAction Object Reference" :default "/Game/Blueprints/Inputs/IA_NextCamera.IA_NextCamera"))
  (:`Triggered`
    ;[1 1 1] Controls
    (if (>= (`KismetMathLibrary.Abs` ActionValue) (`self.GamepadSensitivity`))
      (set `self.ForwardAxis` ActionValue)
      (else
        (set `self.ForwardAxis` 0.0)))))

(event `CheckBeginOverlap`
  (params (Actor :type "Actor Object Reference"))
  (bind _playerpawn (`self.PlayerPawn`))
  ;[1 1 1] Check overlapped Player
  (if (`KismetSystemLibrary.IsValid` _playerpawn)
    (if (== Actor _playerpawn)
      (set `self.PlayerDetected` true :!label _label_3)
      (set `self.OverlappedActor` Actor))
    (else
      (goto _label_3))))

(event `InputAxis|MoveRight` :consume false
  (params (AxisValue :type "Float (single-precision)")))

(event `EnhancedInput|/Game/Blueprints/Inputs/IA_PreviousCamera`
  (params (ActionValue :type "Float (double-precision)") (ElapsedSeconds :type "Float (double-precision)") (TriggeredSeconds :type "Float (double-precision)") (InputAction :type "InputAction Object Reference" :default "/Game/Blueprints/Inputs/IA_PreviousCamera.IA_PreviousCamera"))
  (:`Triggered`
    ;[1 1 1] Controls
    (if (>= (`KismetMathLibrary.Abs` ActionValue) (`self.GamepadSensitivity`))
      (set `self.RightAxis` ActionValue)
      (else
        (set `self.RightAxis` 0.0)))))

(event `CheckEndOverlap`
  (params (Actor :type "Actor Object Reference"))
  ;[1 1 1] Check overlapped Player
  (if (`self.PlayerDetected`)
    (if (== Actor (`self.OverlappedActor`))
      (set `self.PlayerDetected` false)
      (set `self.PlayerOverlapped` false)
      (set `self.OverlappedActor` null)
      (`MaterialInstanceDynamic.SetScalarParameterValue` (`self.DMI_Idle`) "ShowKey" 0.0))))

(event `Server_Cancel`
  (`self.Owner_Cancel`))

(event `Owner_Cancel`
  ;[1 1 1] Exit (Cancel) game
  (if (`self.MiniGameEnabled`)
    (if (`self.IsMiniGameActivated`)
      (`PrimitiveComponent.SetMaterial` (`self.MiniGameScreen`) 0 (`self.DMI_Idle`))
      (`self.ForceExit`))))

(event `CheckPlayerDirection`
  (bind _overlappedactor (`self.OverlappedActor`))
  (bind _dmi_idle (`self.DMI_Idle`))
  ;[1 1 1] Check if player oriented to Mini Game screen
  (if (`self.PlayerDetected`)
    (`/Engine/EditorBlueprintResources/StandardMacros.IsValid` _overlappedactor
      (:`Is Valid`
        (if (<= (`KismetMathLibrary.DegAcos` (`KismetMathLibrary.Dot_VectorVector` (`SceneComponent.GetForwardVector` (`self.Arrow`)) (`self.GetActorForwardVector` _overlappedactor))) (`self.DetectionAngle`))
          (set `self.PlayerOverlapped` true)
          (`MaterialInstanceDynamic.SetScalarParameterValue` _dmi_idle "ShowKey" 1.0)
          (else
            (set `self.PlayerOverlapped` false)
            (`MaterialInstanceDynamic.SetScalarParameterValue` _dmi_idle "ShowKey" 0.0)))))))

(event `/Game/Blueprints/Interfaces/BPI_Interact.MiniGameComplete`
  (`self.Server_Cancel`))

(event `BlendCameraFromPlayerToGame`
  (params (MiniGame :type "Actor Object Reference") (Player :type "Actor Object Reference"))
  ;[1 1 1] Camera transition from Player to Mini Game
  (`self.DisableInput` Player null))

(event `ForceAction`
  ;[0 0.3254 1] Overwritable events
)

(event `SetOfflineMaterial`
  ;[1 1 1] Set Offline material for the screen
  (`PrimitiveComponent.SetMaterial` (`self.MiniGameScreen`) 0 (`self.DMI_Offline`)))

(event `self.InteractionBoundBox.OnComponentBeginOverlap`
  (params (OverlappedComponent :type "PrimitiveComponent Object Reference") (OtherActor :type "Actor Object Reference") (OtherComp :type "PrimitiveComponent Object Reference") (OtherBodyIndex :type Integer) (bFromSweep :type Boolean) (SweepResult :type "HitResult Structure (by ref)")))

(event `BlendCameraFromGameToPlayer`
  (params (Player :type "Actor Object Reference"))
  ;[1 1 1] Camera Transition from Mini Game to Player
)

(event `ForceExit`
  ;[0 0.3254 1] Overwritable events
)

(event `Success`
  (bind _returnvalue (`GameplayStatics.GetGameState`))
  ;[0 0 1] Success Event
  (bind _researchpoints (message `/Game/Blueprints/Interfaces/BPI_Stats.GetResearchPoints` _returnvalue))
  (message `/Game/Blueprints/Interfaces/BPI_Stats.SetResearchPoints` _returnvalue (+ _researchpoints (`self.ResearchPointGrant`))))

(fn `GetCanBePickedUp`
  (returns (CanBePickedUp :type Boolean))
  (return false))

(fn `GetItemToSpawn`
  (returns (Item :type "/Game/Blueprints/Interactables/Weapons/BP_WeaponComponentMaster Class Reference"))
  (return null))

(fn `UserConstructionScript`)