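; Interactable breaker panel that toggles power for one tagged sector, with a sign mesh showing the sector number.
; Interact routes through a server event that, if the reactor is on, updates every BP_RoomSwitch with a matching sector tag.
; Power-off also triggers each switch's light toggle; the lever timeline and sign material follow power state per matching switch.
; SetPanelStatus shows reactor readiness on the sign, and box overlap outlines the panel.
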(event `self.ReceiveBeginPlay`
  (`|SwitchGameplayTagContainer` (`self.SectorTag`)
    (:`(GameplayTags=((TagName="Sector1")))`
      (`StaticMeshComponent.SetStaticMesh` (`self.SectorSign`) "/Game/PolygonSciFiSpace/Meshes/Signs/SM_SignBorder_Number_01.SM_SignBorder_Number_01"))
    (:`(GameplayTags=((TagName="Sector2")))`
      (`StaticMeshComponent.SetStaticMesh` (`self.SectorSign`) "/Game/PolygonSciFiSpace/Meshes/Signs/SM_SignBorder_Number_02.SM_SignBorder_Number_02"))
    (:`(GameplayTags=((TagName="Sector3")))`
      (`StaticMeshComponent.SetStaticMesh` (`self.SectorSign`) "/Game/PolygonSciFiSpace/Meshes/Signs/SM_SignBorder_Number_03.SM_SignBorder_Number_03"))
    (:`(GameplayTags=((TagName="Sector4")))`
      (`StaticMeshComponent.SetStaticMesh` (`self.SectorSign`) "/Game/PolygonSciFiSpace/Meshes/Signs/SM_SignBorder_Number_04.SM_SignBorder_Number_04"))
    (:`(GameplayTags=((TagName="Sector5")))`
      (`StaticMeshComponent.SetStaticMesh` (`self.SectorSign`) "/Game/PolygonSciFiSpace/Meshes/Signs/SM_SignBorder_Number_05.SM_SignBorder_Number_05"))))

(event `Local_SectorPower`
  (bind _reactoron_ (message `/Game/Blueprints/Interfaces/BPI_Stats.GetReactorOn` (`GameplayStatics.GetGameState`)))
  (if _reactoron_
    (if (`self.SectorPowerOn?`)
      (set `self.SectorPowerOn?` false)
      (else
        (set `self.SectorPowerOn?` true)))
    (bind _outactors (`GameplayStatics.GetAllActorsOfClass` "/Game/Blueprints/Interactables/Buttons/BP_RoomSwitch.BP_RoomSwitch_C"))
    (for _array_element _outactors
      (if (== (`/Game/Blueprints/Interactables/Buttons/BP_RoomSwitch.SectorTag` _array_element) (`self.SectorTag`))
        (if (`self.SectorPowerOn?`)
          (set `/Game/Blueprints/Interactables/Buttons/BP_RoomSwitch.SectorPowered` true _array_element)
          (bind (_direction _newtrack_0) (`Timeline|Lever` :!label _label)
            (:`Update`
              (`SceneComponent.K2_SetRelativeRotation` (`self.SM_Lever_4_Lever`) (`KismetMathLibrary.RLerp` (struct) (struct :`Pitch` -170.0) _newtrack_0) false false)
              (`PrimitiveComponent.SetMaterial` (`self.SectorSign`) 0 "/Game/PolygonSciFiSpace/Materials/Misc/MI_SignOn.MI_SignOn")))
          (else
            (set `/Game/Blueprints/Interactables/Buttons/BP_RoomSwitch.SectorPowered` false _array_element)
            (`/Game/Blueprints/Interactables/Buttons/BP_RoomSwitch.Server_LightSwitch` _array_element)
            (`PrimitiveComponent.SetMaterial` (`self.SectorSign`) 0 "/Game/PolygonSciFiSpace/Materials/Misc/MI_SignReady.MI_SignReady")
            (goto _label :!via `Reverse`)))))))

(event `self.Interact`
  (params (Character :type "/Game/Blueprints/Characters/BP_BaseCharacter Object Reference"))
  (`self.Server_SectorPower`))

(event `Server_SectorPower`
  (`self.Local_SectorPower`))

(event `self.Box.OnComponentBeginOverlap`
  (params (OverlappedComponent :type "PrimitiveComponent Object Reference") (OtherActor :type "Actor Object Reference") (OtherComp :type "PrimitiveComponent Object Reference") (OtherBodyIndex :type Integer) (bFromSweep :type Boolean) (SweepResult :type "HitResult Structure (by ref)"))
  (`MeshComponent.SetOverlayMaterial` (`self.PanelSwitch`) "/Game/Materials/M_Outline.M_Outline"))

(event `self.Box.OnComponentEndOverlap`
  (params (OverlappedComponent :type "PrimitiveComponent Object Reference") (OtherActor :type "Actor Object Reference") (OtherComp :type "PrimitiveComponent Object Reference") (OtherBodyIndex :type Integer))
  (`MeshComponent.SetOverlayMaterial` (`self.PanelSwitch`) null))

(fn `SetPanelStatus`
  (bind _reactoron_ (message `/Game/Blueprints/Interfaces/BPI_Stats.GetReactorOn` (`GameplayStatics.GetGameState`)))
  (if _reactoron_
    (`PrimitiveComponent.SetMaterial` (`self.SectorSign`) 0 "/Game/PolygonSciFiSpace/Materials/Misc/MI_SignReady.MI_SignReady")
    (else
      (`PrimitiveComponent.SetMaterial` (`self.SectorSign`) 0 "/Game/PolygonSciFiSpace/Materials/Misc/MI_PolygonSciFiSpace_Signs_01_A.MI_PolygonSciFiSpace_Signs_01_A"))))

(fn `UserConstructionScript`)