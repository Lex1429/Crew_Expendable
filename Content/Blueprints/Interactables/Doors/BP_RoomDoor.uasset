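; BP_RoomDoor is an interactable sliding door that toggles open and closed.
; Interact routes through server and local open events, which play a hydraulic sound at the arch and flip IsDoorOpen.
; The SlideDoor timeline plays or reverses to lerp the door mesh's relative location sideways.
; Actor overlap applies an outline overlay material to the arch and clears it when overlap ends.
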(event `/Game/Blueprints/Interfaces/BPI_Interact.Interact`
  (params (Character :type "/Game/Blueprints/Characters/BP_BaseCharacter Object Reference"))
  (`self.Server_OpenDoor`))

(event `Server_OpenDoor`
  (`self.Local_OpenDoor`))

(event `Local_OpenDoor`
  (`GameplayStatics.PlaySoundAtLocation` "/Game/SFX/echoey_hatch-hydrolic.echoey_hatch-hydrolic" (`SceneComponent.K2_GetComponentLocation` (`self.Arch`)) (struct) 0.4 1.0 0.0 "/Game/SFX/SA_Test.SA_Test" null null null)
  (if (not (`self.IsDoorOpen?`))
    (set `self.IsDoorOpen?` true)
    (bind (_direction _slidetrack) (`Timeline|SlideDoor` :!label _label)
      (:`Update`
        (`SceneComponent.K2_SetRelativeLocation` (`self.Door`) (`KismetMathLibrary.VLerp` (90.0 0.0 0.0) (240.0 0.0 0.0) _slidetrack) false true)))
    (else
      (set `self.IsDoorOpen?` false)
      (goto _label :!via `Reverse`))))

(event `self.Box.OnComponentBeginOverlap`
  (params (OverlappedComponent :type "PrimitiveComponent Object Reference") (OtherActor :type "Actor Object Reference") (OtherComp :type "PrimitiveComponent Object Reference") (OtherBodyIndex :type Integer) (bFromSweep :type Boolean) (SweepResult :type "HitResult Structure (by ref)")))

(event `self.ReceiveActorBeginOverlap`
  (params (OtherActor :type "Actor Object Reference"))
  (`MeshComponent.SetOverlayMaterial` (`self.Arch`) "/Game/Materials/M_Outline.M_Outline"))

(event `self.ReceiveActorEndOverlap`
  (params (OtherActor :type "Actor Object Reference"))
  (`MeshComponent.SetOverlayMaterial` (`self.Arch`) null))

(fn `UserConstructionScript`)