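; BP_RoomSwitch is an interactable light switch that toggles every BP_LampBase sharing its RoomTag.
; Interact calls a server event that runs the local toggle, turning each matching lamp on or off, or always off when SectorPowered is false.
; The Switch timeline plays or reverses with the toggle to rotate the lever mesh.
; Box overlap and interact-focus events set or clear outline overlay materials on TouchPanel.
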(event `Local_Lightswitch`
  (bind _outactors (`GameplayStatics.GetAllActorsOfClass` "/Game/Blueprints/Interactables/CealingLights/BP_LampBase.BP_LampBase_C"))
  (for _array_element _outactors
    (if (== (`/Game/Blueprints/Interactables/CealingLights/BP_LampBase.RoomTag` _array_element) (`self.RoomTag`))
      (if (`self.SectorPowered`)
        (if (`/Game/Blueprints/Interactables/CealingLights/BP_LampBase.IsLightOn?` _array_element)
          (`/Game/Blueprints/Interactables/CealingLights/BP_LampBase.Server_LightOff` _array_element :!label _label)
          (bind (_direction _newtrack_0) (`Timeline|Switch` :!via `Reverse` :!label _label_2)
            (:`Update`
              (`SceneComponent.K2_SetRelativeRotation` (`self.SM_Lever_1_Lever`) (`KismetMathLibrary.RLerp` (struct :`Pitch` -45.0) (struct :`Pitch` 35.0) _newtrack_0) false false)))
          (else
            (`/Game/Blueprints/Interactables/CealingLights/BP_LampBase.Server_LightOn` _array_element)
            (goto _label_2)))
        (else
          (goto _label))))))

(event `Server_LightSwitch`
  (`self.Local_Lightswitch`))

(event `self.Interact`
  (params (Character :type "/Game/Blueprints/Characters/BP_BaseCharacter Object Reference"))
  (`self.Server_LightSwitch`))

(event `self.Box.OnComponentBeginOverlap`
  (params (OverlappedComponent :type "PrimitiveComponent Object Reference") (OtherActor :type "Actor Object Reference") (OtherComp :type "PrimitiveComponent Object Reference") (OtherBodyIndex :type Integer) (bFromSweep :type Boolean) (SweepResult :type "HitResult Structure (by ref)"))
  (`MeshComponent.SetOverlayMaterial` (`self.TouchPanel`) "/Game/Materials/M_Outline.M_Outline"))

(event `self.Box.OnComponentEndOverlap`
  (params (OverlappedComponent :type "PrimitiveComponent Object Reference") (OtherActor :type "Actor Object Reference") (OtherComp :type "PrimitiveComponent Object Reference") (OtherBodyIndex :type Integer))
  (`MeshComponent.SetOverlayMaterial` (`self.TouchPanel`) null))

(event `/Game/Blueprints/Interfaces/BPI_Interact.OverlapInteract`
  (params (Character :type "PlayerController Object Reference"))
  (`MeshComponent.SetOverlayMaterial` (`self.TouchPanel`) "/Game/Materials/MI_Outline_Test.MI_Outline_Test"))

(event `/Game/Blueprints/Interfaces/BPI_Interact.AwayFromInteract`
  (params (Character :type "PlayerController Object Reference") (InteractPrompt :type "/Game/UI/WB_InteractRing Object Reference"))
  (`MeshComponent.SetOverlayMaterial` (`self.TouchPanel`) null))

(fn `UserConstructionScript`)