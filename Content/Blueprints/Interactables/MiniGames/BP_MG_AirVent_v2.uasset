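; Interactable air vent minigame in which players repair an AC unit by inserting cooling and heating filters.
; BeginPlay spawns a pickup for each filter type.
; Interacting with a repaired filter held flags that type, clears it from the player's hands and spawns it at the vent, with a server path for clients.
; Once both are in, the ACRepaired RepNotify loops the animation, stops Niagara, swaps the coil material and signals the repair.
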(event `self.ReceiveBeginPlay`
  (bind _heaterspawn (`self.HeaterSpawn`))
  (bind _coolerspawn (`self.CoolerSpawn`))
  (`|SpawnActorFromClass` "/Game/Blueprints/EquipmentSystem/BP_CoreEquipmentPickup.BP_CoreEquipmentPickup_C" (`KismetMathLibrary.MakeTransform` (`SceneComponent.K2_GetComponentLocation` _coolerspawn) (`SceneComponent.K2_GetComponentRotation` _coolerspawn)) "AdjustIfPossibleButAlwaysSpawn" "MultiplyWithRoot" null "5" null)
  (`|SpawnActorFromClass` "/Game/Blueprints/EquipmentSystem/BP_CoreEquipmentPickup.BP_CoreEquipmentPickup_C" (`KismetMathLibrary.MakeTransform` (`SceneComponent.K2_GetComponentLocation` _heaterspawn) (`SceneComponent.K2_GetComponentRotation` _heaterspawn)) "AdjustIfPossibleButAlwaysSpawn" "MultiplyWithRoot" null "7" null))

(event `Server_InsertFilter`
  (bind _returnvalue (select `int` (`self.SelectedFilter`) :`0` (`self.CoolerSpawn`) :`1` (`self.HeaterSlot`) :!type "SceneComponent Object Reference"))
  (`|SpawnActorFromClass` "/Game/Blueprints/EquipmentSystem/BP_CoreEquipmentPickup.BP_CoreEquipmentPickup_C" (`KismetMathLibrary.MakeTransform` (`SceneComponent.K2_GetComponentLocation` _returnvalue) (`SceneComponent.K2_GetComponentRotation` _returnvalue)) "AdjustIfPossibleButAlwaysSpawn" "MultiplyWithRoot" null (`self.FilterID`) null :!label _label)
  (`self.Local_Insert Filter`))

(event `/Game/Blueprints/Interfaces/BPI_Interact.Interact`
  (params (Character :type "/Game/Blueprints/Characters/BP_BaseCharacter Object Reference") (PlayerCharacter :type "/Game/Blueprints/Characters/BP_PlayerCharacterCore Object Reference"))
  (bind _output_get (set `self.PlayerRef` PlayerCharacter))
  (switch `name` (`/Game/Blueprints/Characters/BP_PlayerCharacterCore.CurrentEquipmentHeld` _output_get)
    (:`6`
      (set `self.CoolingFilterRepaired?` true)
      (set `self.FilterID` "6")
      (set `self.SelectedFilter` 0))
    (:`8`
      (set `self.HeatingFilterRepaired?` true)
      (set `self.FilterID` "8")
      (set `self.SelectedFilter` 1)))
  (`self.Owner_InsertFilter` _output_get)
  (`/Engine/EditorBlueprintResources/ActorMacros.Switch Has Authority`
    (:`Authority`
      (goto _label))
    (:`Remote`
      (`self.Server_InsertFilter`))))

(event `Owner_InsertFilter`
  (params (Player :type "/Game/Blueprints/Characters/BP_PlayerCharacterCore Object Reference"))
  (`/Game/Blueprints/Characters/BP_PlayerCharacterCore.RemoveItemFromInventory` Player)
  (`/Game/Blueprints/Characters/BP_PlayerCharacterCore.Server_SetHeldEquipment` Player "1"))

(event `Local_Insert Filter`
  (if (and (`self.CoolingFilterRepaired?`) (`self.HeatingFilterRepaired?`))
    (set `self.ACRepaired?` true)))

(fn `GetCanBePickedUp`
  (returns (CanBePickedUp :type Boolean))
  (return false))

(fn `GetItemToSpawn`
  (returns (Item :type "/Game/Blueprints/Interactables/Weapons/BP_WeaponComponentMaster Class Reference"))
  (return null))

(fn `OnRep_ACRepaired?`
  (if (`self.ACRepaired?`)
    (`SkeletalMeshComponent.PlayAnimation` (`self.AC`) "/Game/Assets/VentMiniGameParts/vent_mini_game_Anim.vent_mini_game_Anim" true)
    (`ActorComponent.Deactivate` (`self.Niagara`))
    (`self.ACRepaired`)
    (`PrimitiveComponent.SetMaterialByName` (`self.AC`) "CoilCenter" "/Game/Assets/VentMiniGameParts/ACStatusMats/MI_ACFunctional.MI_ACFunctional")))

(fn `UserConstructionScript`)