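; BP_ItemSpawner is an interactable physics pickup in the inventory system, with its mesh set from ItemData at construction.
; SetFocused shows the widget and hides it through a short retriggerable delay, so it stays visible while focus calls repeat.
; Interact passes ItemData to the player character's pickup message, then destroys the actor through ServerDestroy.
; QueryAsset exposes ItemData, while GetCanBePickedUp returns false and GetItemToSpawn returns nothing.
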(event `self.ReceiveBeginPlay`
  (bind _foundwidgets (`WidgetBlueprintLibrary.GetAllWidgetsOfClass` null))
  (set `self.InteractWidgetRed` (`|GetArrayItem` _foundwidgets)))

(event `/Game/Blueprints/Interfaces/BPI_Interact.SetFocused`
  (`SceneComponent.SetVisibility` (`self.Widget`) true false)
  (`KismetSystemLibrary.RetriggerableDelay` 0.1)
  (`SceneComponent.SetVisibility` (`self.Widget`) false false))

(event `/Game/Blueprints/Interfaces/BPI_Interact.Interact`
  (params (Character :type "/Game/Blueprints/Characters/BP_BaseCharacter Object Reference") (PlayerCharacter :type "/Game/Blueprints/Characters/BP_PlayerCharacterCore Object Reference"))
  (message `/Game/Blueprints/Interfaces/BPI_Equipables.PickedUpObject` PlayerCharacter (`self.ItemData`))
  (`self.ServerDestroy`))

(event `ServerDestroy`
  (`self.K2_DestroyActor`))

(fn `GetCanBePickedUp`
  (returns (CanBePickedUp :type Boolean))
  (return false))

(fn `GetItemToSpawn`
  (returns (Item :type "/Game/Blueprints/Interactables/Weapons/BP_WeaponComponentMaster Class Reference"))
  (return null))

(fn `QueryAsset`
  (returns (Asset :type "/Game/Blueprints/InventorySystem/Pickups/Data/PDA_Items Object Reference"))
  (return (`self.ItemData`)))

(fn `UserConstructionScript`
  (bind _staticmesh (`self.StaticMesh`))
  (`StaticMeshComponent.SetStaticMesh` _staticmesh (`/Game/Blueprints/InventorySystem/Pickups/Data/PDA_Items.ObjectMesh` (`self.ItemData`)))
  (`PrimitiveComponent.SetSimulatePhysics` _staticmesh true))