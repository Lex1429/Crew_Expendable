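; Mini-game event controller that tallies mini-game completions and reports a phase to the game state.
; AddCompletion increments CompletionCounter and, once it equals the length of MGComponentRef, calls SetPhaseMessage on the game state with the Phase variable.
; The mission ID, phase and mission details getters return only placeholder or empty values, and BeginPlay is empty.
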(event `self.ReceiveBeginPlay`)

(event `AddCompletion`
  (bind _result (`/Engine/EditorBlueprintResources/StandardMacros.IncrementInt` (`self.CompletionCounter`))
    (:`  `
      (if (== _result (`KismetArrayLibrary.Array_Length` (`self.MGComponentRef`)))
        (message `/Game/Blueprints/Interfaces/BPI_MissionLog.SetPhase` (`GameplayStatics.GetGameState`) (`self.Phase`))))))

(fn `GetCurrentMissionID`
  (returns (MissionID :type Name))
  (return "None"))

(fn `GetMissionDetails`
  (returns (Mission :type "/Game/Blueprints/MissionLog/S_Missions Structure"))
  (return))

(fn `GetPhase`
  (returns (Phase :type "/Game/Blueprints/MissionLog/Enum_Phases Enum"))
  (return "NewEnumerator0"))

(fn `UserConstructionScript`)