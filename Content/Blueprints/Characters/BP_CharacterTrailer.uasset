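; BP_CharacterTrailer is a character Blueprint, apparently for staging trailer shots, with a child-actor gun shown or hidden by CanSeeGun in the construction script.
; On BeginPlay, a DoN and Delay loop spawns a limited burst of Niagara muzzle flashes attached to the gun.
; Disconnected chains hold alternative staged actions that never run: ragdoll with blood, a "Traitor" pistol animation sequence, and AI movement to a Destination actor.
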(event `self.ReceiveBeginPlay`
  (bind _childactor (`self.ChildActor`))
  (`/Engine/EditorBlueprintResources/StandardMacros.Do N` 10 :!label _label
    (:`Exit`
      (`NiagaraFunctionLibrary.SpawnSystemAttached` "/Game/MuzzleFlashesVol1/Particles/NiagaraSystems/NS_MuzzleFlash_v04.NS_MuzzleFlash_v04" _childactor "AssaultRifleMuzzle" (+ (`SceneComponent.RelativeLocation` _childactor) (0.0 80.0 10.0)) (struct) "KeepRelativeOffset")
      (`KismetSystemLibrary.Delay` 0.5)
      (goto _label))))

(fn `UserConstructionScript`
  (`SceneComponent.SetVisibility` (`self.ChildActor`) (`self.CanSeeGun`) false))