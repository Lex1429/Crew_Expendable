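; BP_TunnelVentControl is a manager actor that tracks the level's BP_TunnelVent actors and the currently selected vent route.
; On BeginPlay and ReRollVents it fills VentsArray from every BP_TunnelVent in the world, with no shuffling.
; RemoveVent ignores its index and only counts calls, resetting and triggering ReRollVents on the third.
; SetActiveRoute stores the vent at the given route number as SelectedVentRef.
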(event `ReRollVents`
  (bind _outactors (`GameplayStatics.GetAllActorsOfClass` "/Game/Blueprints/Interactables/LevelProps/BP_TunnelVent.BP_TunnelVent_C" :!label _label))
  (for (_array_element _array_index) _outactors
    (`KismetArrayLibrary.Array_Set` (`self.VentsArray`) _array_index _array_element)))

(event `self.ReceiveBeginPlay`
  (goto _label))

(event `RemoveVent`
  (params (ArrayInt :type Integer))
  (bind _result (`/Engine/EditorBlueprintResources/StandardMacros.IncrementInt` (`self.VentCounter`))
    (:`  `
      (if (== _result 3)
        (set `self.VentCounter` 0)
        (`self.ReRollVents`)))))

(event `SetActiveRoute`
  (params (RouteNumber :type Integer))
  (set `self.SelectedVentRef` (`|GetArrayItem` (`self.VentsArray`) RouteNumber)))

(fn `UserConstructionScript`)