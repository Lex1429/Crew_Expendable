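; Game instance that holds session-wide state such as player counts, player skin, menu status and camera inversion, exposed through simple getters.
; On init it starts audio setup, which loads and applies saved audio settings after a short delay.
; Network and travel failures cache their failure type as a string, then share one path that destroys the player's session.
; The server creator and server search getters are empty stubs.
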(event `self.ReceiveInit`
  (`self.Initialize_AudioSettings`))

(event `Initialize_AudioSettings`
  (`KismetSystemLibrary.Delay` 0.2)
  (`/Game/MBLS/Blueprints/FunctionLibrary/BP_FL_General.Load/Set_AudioSettings`))

(event `self.HandleNetworkError`
  (params (FailureType :type "ENetworkFailure Enum" :default "NetDriverAlreadyExists") (bIsServer :type Boolean))
  (set `self.Cached_Network_Error` (`|GetEnumeratorNameAsString` FailureType))
  (`DestroySessionCallbackProxy.DestroySession` (`GameplayStatics.GetPlayerController` 0) :!label _label))

(event `self.HandleTravelError`
  (params (FailureType :type "ETravelFailure Enum" :default "NoLevel"))
  (set `self.Cached_Travel_Error` (`|GetEnumeratorNameAsString` FailureType))
  (goto _label))

(fn `GetLivePlayers`
  (returns (LivePalyerCount :type Integer))
  (return (`self.LivePlayers`)))

(fn `GetMenuUp`
  (returns (MenuUp :type Boolean))
  (return (`self.MenuUp`)))

(fn `GetMouseInversion`
  (returns (MouseInverted :type Boolean))
  (return (`self.CameraInverted?`)))

(fn `GetPlayerCount`
  (returns (PlayerCount :type Integer))
  (return (`self.ServerPlayerCount`)))

(fn `GetPlayerSkin`
  (returns (PlayerSkin :type "MaterialInstance Object Reference"))
  (return (`self.PlayerSkin`)))

(fn `GetServerCreator`
  (returns (Creator :type Text))
  (return ""))

(fn `GetServerSearch`
  (returns (SearchResult :type "BlueprintSessionResult Structure"))
  (return))