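; Inventory component for the player character that manages equipment slots holding items by name, with one slot selected at a time.
; Mouse up/down events cycle three slots with wraparound and SwapSlot jumps directly, updating the HUD equipment overlay and the character's held equipment.
; Add, query and remove functions act only on the current slot.
; BeginPlay caches owner and controller after a delay, for locally controlled players only.
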(event `self.ReceiveBeginPlay`
  (`KismetSystemLibrary.Delay` 2.0)
  (if (`Pawn.IsLocallyControlled` (`Actor.Instigator` (`self.GetOwner`)))
    (bind _asbp_player_character_core (cast `/Game/Blueprints/Characters/BP_PlayerCharacterCore` (`self.GetOwner`)))
    (set `self.OwnerRef` _asbp_player_character_core)
    (`/Game/UI/WB_EquipmentOverlay.SelectSlot` (`/Game/UI/WB_PlayerUI.WB_EquipmentOverlay` (`/Game/MBLS/Blueprints/Core/Gameplay/Player/BP_PC_Gameplay.HUDRef` (`/Game/Blueprints/Characters/BP_PlayerCharacterCore.Gameplay Controller Ref` (`self.OwnerRef`)))) 0)
    (bind _asbp_pc_gameplay (cast `/Game/MBLS/Blueprints/Core/Gameplay/Player/BP_PC_Gameplay` (`GameplayStatics.GetPlayerController` 0)))
    (set `self.ControllerRef` _asbp_pc_gameplay)))

(event `MouseUpSelect`
  (bind _currentslotindex (`self.CurrentSlotIndex`))
  (`/Game/UI/WB_EquipmentOverlay.UnselectSlot` (`/Game/UI/WB_PlayerUI.WB_EquipmentOverlay` (`/Game/MBLS/Blueprints/Core/Gameplay/Player/BP_PC_Gameplay.HUDRef` (`/Game/Blueprints/Characters/BP_PlayerCharacterCore.Gameplay Controller Ref` (`self.OwnerRef`)))) _currentslotindex)
  (bind _output_get (set `self.CurrentSlotIndex` (+ _currentslotindex 1)))
  (if (>= _output_get 3)
    (bind _output_get_2 (set `self.CurrentSlotIndex` 0))
    (`/Game/UI/WB_EquipmentOverlay.SelectSlot` (`/Game/UI/WB_PlayerUI.WB_EquipmentOverlay` (`/Game/MBLS/Blueprints/Core/Gameplay/Player/BP_PC_Gameplay.HUDRef` (`self.ControllerRef`))) _output_get_2)
    (else
      (`/Game/UI/WB_EquipmentOverlay.SelectSlot` (`/Game/UI/WB_PlayerUI.WB_EquipmentOverlay` (`/Game/MBLS/Blueprints/Core/Gameplay/Player/BP_PC_Gameplay.HUDRef` (`/Game/Blueprints/Characters/BP_PlayerCharacterCore.Gameplay Controller Ref` (`self.OwnerRef`)))) (`self.CurrentSlotIndex`))))
  (`self.ChangeSlotMesh` :!label _label))

(event `MouseDownSelect`
  (bind _currentslotindex (`self.CurrentSlotIndex`))
  (`/Game/UI/WB_EquipmentOverlay.UnselectSlot` (`/Game/UI/WB_PlayerUI.WB_EquipmentOverlay` (`/Game/MBLS/Blueprints/Core/Gameplay/Player/BP_PC_Gameplay.HUDRef` (`/Game/Blueprints/Characters/BP_PlayerCharacterCore.Gameplay Controller Ref` (`self.OwnerRef`)))) _currentslotindex)
  (bind _output_get (set `self.CurrentSlotIndex` (- _currentslotindex 1)))
  (if (<= _output_get -1)
    (bind _output_get_2 (set `self.CurrentSlotIndex` 2))
    (`/Game/UI/WB_EquipmentOverlay.SelectSlot` (`/Game/UI/WB_PlayerUI.WB_EquipmentOverlay` (`/Game/MBLS/Blueprints/Core/Gameplay/Player/BP_PC_Gameplay.HUDRef` (`/Game/Blueprints/Characters/BP_PlayerCharacterCore.Gameplay Controller Ref` (`self.OwnerRef`)))) _output_get_2)
    (goto _label)
    (else
      (`/Game/UI/WB_EquipmentOverlay.SelectSlot` (`/Game/UI/WB_PlayerUI.WB_EquipmentOverlay` (`/Game/MBLS/Blueprints/Core/Gameplay/Player/BP_PC_Gameplay.HUDRef` (`/Game/Blueprints/Characters/BP_PlayerCharacterCore.Gameplay Controller Ref` (`self.OwnerRef`)))) (`self.CurrentSlotIndex`))
      (goto _label))))

(fn `ChangeSlot`
  (returns (SlotIndex :type Integer) (Icon :type "Texture2D Object Reference") (`SlotEmpty?` :type Boolean)))

(fn `ChangeSlotMesh`
  (bind _output (`|GetArrayItem` (`self.EquipmentSlots`) (`self.CurrentSlotIndex`)))
  (`/Game/Blueprints/Characters/BP_PlayerCharacterCore.ChangeHeldEquipment` (`self.OwnerRef`) (select `bool` (== _output "None") :`false` _output)))

(fn `GetPickedUpDetails`
  (returns (AnimType :type "/Game/Blueprints/EquipmentSystem/E_EquipmentState Enum") (SocketName :type Name) (SkeletalMesh :type "SkeletalMesh Object Reference"))
  (return "NewEnumerator0" "None" null))

(fn `IsSlotFree?`
  (params (Equipment :type Name))
  (returns (`SlotFree?` :type Boolean))
  (if (== (`|GetArrayItem` (`self.EquipmentSlots`) (`self.CurrentSlotIndex`)) "None")
    (`KismetArrayLibrary.Array_Set` (`self.EquipmentSlots`) (`self.CurrentSlotIndex`) Equipment)
    ; Get Data table to plug in icon.
    (`/Game/UI/WB_EquipmentOverlay.SlotChange` (`/Game/UI/WB_PlayerUI.WB_EquipmentOverlay` (`/Game/MBLS/Blueprints/Core/Gameplay/Player/BP_PC_Gameplay.HUDRef` (`self.ControllerRef`))) (`self.CurrentSlotIndex`) null false)
    (return true)
    (else
      (`/Game/UI/WB_EquipmentOverlay.SlotChange` (`/Game/UI/WB_PlayerUI.WB_EquipmentOverlay` (`/Game/MBLS/Blueprints/Core/Gameplay/Player/BP_PC_Gameplay.HUDRef` (`self.ControllerRef`))) (`self.CurrentSlotIndex`) null true)
      (return false))))

(fn `QueryInventory`
  (returns (SlotNotEmpty :type Boolean) (ObjectyName :type Name))
  (bind _output (`|GetArrayItem` (`self.EquipmentSlots`) (`self.CurrentSlotIndex`)))
  (if (== _output "None")
    (return false "None")
    (else
      (return true _output))))

(fn `RemoveFromInventory`
  (`KismetArrayLibrary.Array_Set` (`self.EquipmentSlots`) (`self.CurrentSlotIndex`))
  (`/Game/UI/WB_EquipmentOverlay.SlotChange` (`/Game/UI/WB_PlayerUI.WB_EquipmentOverlay` (`/Game/MBLS/Blueprints/Core/Gameplay/Player/BP_PC_Gameplay.HUDRef` (`self.ControllerRef`))) (`self.CurrentSlotIndex`) null true))

(fn `SwapSlot`
  (params (SlotIndex :type Integer))
  (`/Game/UI/WB_EquipmentOverlay.UnselectSlot` (`/Game/UI/WB_PlayerUI.WB_EquipmentOverlay` (`/Game/MBLS/Blueprints/Core/Gameplay/Player/BP_PC_Gameplay.HUDRef` (`/Game/Blueprints/Characters/BP_PlayerCharacterCore.Gameplay Controller Ref` (`self.OwnerRef`)))) (`self.CurrentSlotIndex`))
  (bind _output_get (set `self.CurrentSlotIndex` SlotIndex))
  (`/Game/UI/WB_EquipmentOverlay.SelectSlot` (`/Game/UI/WB_PlayerUI.WB_EquipmentOverlay` (`/Game/MBLS/Blueprints/Core/Gameplay/Player/BP_PC_Gameplay.HUDRef` (`/Game/Blueprints/Characters/BP_PlayerCharacterCore.Gameplay Controller Ref` (`self.OwnerRef`)))) _output_get)
  (`self.ChangeSlotMesh`))