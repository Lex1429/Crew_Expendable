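; AI controller that starts the BT_SAL_AI behavior tree two seconds after possessing a pawn.
; AI Perception events feed the blackboard, setting Target to player characters from batch updates, or to any actor from per-target updates.
; Per-target updates and forgotten events each set a different AIState, and forgetting writes that actor to Target instead of clearing it.
; When the blackboard initializes, its AIMovement value is copied into AIMovementState.
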(event `self.ReceivePossess`
  (params (PossessedPawn :type "Pawn Object Reference"))
  (`KismetSystemLibrary.Delay` 2.0)
  (`self.RunBehaviorTree` "/Game/Blueprints/AI/AIv2/BT_SAL_AI.BT_SAL_AI"))

(event `self.AIPerception.OnPerceptionUpdated`
  (params (UpdatedActors :type "Array of Actor Object Reference (by ref)"))
  (for _array_element UpdatedActors
    (bind _asbp_player_character_core (cast `/Game/Blueprints/Characters/BP_PlayerCharacterCore` _array_element))
    (`BlackboardComponent.SetValueAsObject` (`AIBlueprintHelperLibrary.GetBlackboard` null) "Target" _asbp_player_character_core)))

(event `self.OnUsingBlackBoard`
  (params (BlackboardComp :type "BlackboardComponent Object Reference") (BlackboardAsset :type "BlackboardData Object Reference"))
  (set `self.AIMovementState` (cast `/Game/Blueprints/Enums/AIEnums/E_SAL_Movement` (`BlackboardComponent.GetValueAsEnum` BlackboardComp "AIMovement"))))

(event `self.AIPerception.OnTargetPerceptionUpdated`
  (params (Actor :type "Actor Object Reference") (Stimulus :type "AIStimulus Structure"))
  (bind _returnvalue (`AIBlueprintHelperLibrary.GetBlackboard` null))
  (`BlackboardComponent.SetValueAsObject` _returnvalue "Target" Actor)
  (`BlackboardComponent.SetValueAsEnum` _returnvalue "AIState" (enumliteral `/Game/Blueprints/Enums/AIEnums/E_SALState` "NewEnumerator5")))

(event `self.AIPerception.OnTargetPerceptionForgotten`
  (params (Actor :type "Actor Object Reference"))
  (bind _returnvalue (`AIBlueprintHelperLibrary.GetBlackboard` null))
  (`BlackboardComponent.SetValueAsObject` _returnvalue "Target" Actor)
  (`BlackboardComponent.SetValueAsEnum` _returnvalue "AIState" (enumliteral `/Game/Blueprints/Enums/AIEnums/E_SALState` "NewEnumerator3")))

(fn `UserConstructionScript`)