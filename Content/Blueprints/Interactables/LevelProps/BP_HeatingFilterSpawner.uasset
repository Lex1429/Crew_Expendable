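; Level prop cabinet that dispenses a replacement heating filter when the linked disposal reports that a filter was disposed of.
; The disposal event calls a server event that, on authority, spawns a core equipment pickup at the spawner point and sets a replicated flag.
; The flag's OnRep updates the game state's cooler filter status, clears the AC vent's filter ID and swings the cabinet door open with a timeline.
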(event `Server_HeaterReady`
  (`/Engine/EditorBlueprintResources/ActorMacros.Switch Has Authority`
    (:`Authority`
      (`|SpawnActorFromClass` "/Game/Blueprints/EquipmentSystem/BP_CoreEquipmentPickup.BP_CoreEquipmentPickup_C" (`KismetMathLibrary.MakeTransform` (`SceneComponent.K2_GetComponentLocation` (`self.FilterSpawner`)) (struct :`Yaw` 180.0)) "AdjustIfPossibleButAlwaysSpawn" "MultiplyWithRoot" null "8" null)
      (set `self.FilterSpawned?` true))
    (:`Remote`
      (`self.Server_HeaterReady`))))

(event `Local_HeaterReady`
  (bind (_direction _newtrack_0) (`Timeline|CabinetDoor`)
    (:`Update`
      (`SceneComponent.K2_SetRelativeRotation` (`self.SM_Prop_Cabinet_03_Door`) (`KismetMathLibrary.RLerp` (struct) (struct :`Yaw` -120.0) _newtrack_0 true) false false))))

(event `self.ReceiveBeginPlay`
  (add `/Game/Blueprints/Interactables/LevelProps/BP_FilterDisposal.HeatingFilterDispossed` (`self.DisposalRef`) (delegate `SpawnHeater`)))

(event `SpawnHeater`
  (`self.Server_HeaterReady`))

(fn `GetCanBePickedUp`
  (returns (CanBePickedUp :type Boolean))
  (return false))

(fn `GetCoolerFilterStatus`
  (returns (`InAC?` :type Boolean) (`InDispenser?` :type Boolean) (`Broken?` :type Boolean))
  (return false false false))

(fn `GetItemToSpawn`
  (returns (Item :type "/Game/Blueprints/Interactables/Weapons/BP_WeaponComponentMaster Class Reference"))
  (return null))

(fn `OnRep_FilterSpawned?`
  (if (`self.FilterSpawned?`)
    (message `/Game/Blueprints/Interfaces/BPI_FilterStats.SetCoolerFilterStatus` (`GameplayStatics.GetGameState`) false true false)
    (set `/Game/Blueprints/Interactables/MiniGames/BP_MG_AirVent_v2.FilterID` "None" (`self.ACVentRef`))
    (`self.Local_HeaterReady`)))

(fn `UserConstructionScript`)