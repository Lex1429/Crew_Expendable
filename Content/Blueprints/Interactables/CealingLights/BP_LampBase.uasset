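; Base ceiling lamp Blueprint that switches a spotlight and its light panel's material glow on or off.
; BeginPlay applies the starting state and, if flagged, a flicker light function material.
; Lamps that start off and are flagged broken show an electric loop effect with randomized range parameters.
; Server on/off events forward to local events that set spotlight intensity, panel LightStrength and the IsLightOn state.
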(event `self.ReceiveBeginPlay`
  (bind _n_electricloop (`self.N_ElectricLoop`))
  (if (`self.LightFlicker?`)
    (`LightComponent.SetLightFunctionMaterial` (`self.SpotLight`) "/Game/Materials/M_LightFlicker.M_LightFlicker"))
  (if (`self.IsLightOn?`)
    (`LightComponent.SetIntensity` (`self.SpotLight`) 100.0)
    (set `self.IsLightOn?` true)
    (`MeshComponent.SetScalarParameterValueOnMaterials` (`self.SM_Prop_Light_Panel_02`) "LightStrength" 2.0)
    (else
      (`LightComponent.SetIntensity` (`self.SpotLight`) 0.0)
      (set `self.IsLightOn?` false)
      (`MeshComponent.SetScalarParameterValueOnMaterials` (`self.SM_Prop_Light_Panel_02`) "LightStrength" 0.0)
      (if (`self.BrokenLight?`)
        (`SceneComponent.SetVisibility` _n_electricloop true false)
        (`FXSystemComponent.SetFloatParameter` _n_electricloop "MinRandom" (`KismetMathLibrary.RandomFloatInRange` (`self.RandomMin`) 3.0))
        (`FXSystemComponent.SetFloatParameter` _n_electricloop "MaxRandom" (`KismetMathLibrary.RandomFloatInRange` 4.0 (`self.RandomMax`)))))))

(event `Local_LightOn`
  (`LightComponent.SetIntensity` (`self.SpotLight`) 100.0)
  (set `self.IsLightOn?` true)
  (`MeshComponent.SetScalarParameterValueOnMaterials` (`self.SM_Prop_Light_Panel_02`) "LightStrength" 5.0))

(event `Local_LightOff`
  (`LightComponent.SetIntensity` (`self.SpotLight`) 0.0)
  (set `self.IsLightOn?` false)
  (`MeshComponent.SetScalarParameterValueOnMaterials` (`self.SM_Prop_Light_Panel_02`) "LightStrength" 0.0))

(event `Server_LightOn`
  (`self.Local_LightOn`))

(event `Server_LightOff`
  (`self.Local_LightOff`))

(fn `UserConstructionScript`)