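; BP_SkinSelect is an interactable lobby prop, a hanging suit that lets a character equip its skin.
; The suit mesh displays the Skin material on BeginPlay and gains an outline overlay material while something overlaps its box.
; Interact passes the character to a server select event, which applies the skin through SetSkinColor and plays an equip sound at that character's mesh.
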(event `self.ReceiveBeginPlay`
  (`PrimitiveComponent.SetMaterial` (`self.SM_Prop_Suit_Hanging_01`) 0 (`self.Skin`))
  (bind _asbp_base_character (cast `/Game/Blueprints/Characters/BP_BaseCharacter` (`GameplayStatics.GetPlayerCharacter` 0)))
  (set `self.CharacterRef` _asbp_base_character))

(event `self.Box.OnComponentBeginOverlap`
  (params (OverlappedComponent :type "PrimitiveComponent Object Reference") (OtherActor :type "Actor Object Reference") (OtherComp :type "PrimitiveComponent Object Reference") (OtherBodyIndex :type Integer) (bFromSweep :type Boolean) (SweepResult :type "HitResult Structure (by ref)"))
  (`MeshComponent.SetOverlayMaterial` (`self.SM_Prop_Suit_Hanging_01`) "/Game/Materials/M_Outline.M_Outline"))

(event `self.Box.OnComponentEndOverlap`
  (params (OverlappedComponent :type "PrimitiveComponent Object Reference") (OtherActor :type "Actor Object Reference") (OtherComp :type "PrimitiveComponent Object Reference") (OtherBodyIndex :type Integer))
  (`MeshComponent.SetOverlayMaterial` (`self.SM_Prop_Suit_Hanging_01`) null))

(event `Server_SelectSkin`
  (params (Player :type "/Game/Blueprints/Characters/BP_BaseCharacter Object Reference"))
  (bind _skin (`self.Skin`))
  (`/Game/Blueprints/Characters/BP_BaseCharacter.SetSkinColor` Player _skin _skin)
  (`GameplayStatics.PlaySoundAtLocation` "/Game/SFX/SuitEquip/SC_SuitEquip.SC_SuitEquip" (`SceneComponent.K2_GetComponentLocation` (`Character.Mesh` Player)) (struct) 1.0 1.0 0.0 null null null null))

(event `/Game/Blueprints/Interfaces/BPI_Interact.Interact`
  (params (Character :type "/Game/Blueprints/Characters/BP_BaseCharacter Object Reference"))
  (`self.Server_SelectSkin` Character))

(fn `UserConstructionScript`)