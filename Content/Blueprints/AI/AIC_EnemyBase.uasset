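; Base enemy AI controller that runs BT_EnemyBase and switches its blackboard state between Passive, Investigating and Attacking.
; AI Perception updates route sight and damage to attacking the sensed actor and hearing to investigating its location, without interrupting an existing attack.
; Sighting a dead actor resets to Passive.
; A looping timer checks for seen actors that perception has forgotten, returning to Passive if the attack target is lost.
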(event `self.ReceivePossess`
  (params (PossessedPawn :type "Pawn Object Reference"))
  (`self.RunBehaviorTree` "/Game/Blueprints/AI/BT_EnemyBase.BT_EnemyBase")
  (`self.SetStateAsPassive`)
  (bind _returnvalue (`KismetSystemLibrary.K2_SetTimerDelegate` (`|CreateDelegate` :!event `CheckIfForgottenSeenActor`) 0.5 true))
  (set `self.CheckForgottenActorsTimer` _returnvalue))

(event `Event On UnPossess`
  (`KismetSystemLibrary.K2_ClearAndInvalidateTimerHandle` (`self.CheckForgottenActorsTimer`)))

(event `self.AIPerception.OnTargetPerceptionUpdated`
  (params (Actor :type "Actor Object Reference") (Stimulus :type "AIStimulus Structure"))
  (`|ExecutionSequence`
    (:`then_0`
      (bind _sensed (`self.CanSenseActor` Actor "NewEnumerator1"))
      (if _sensed
        (`self.HandleSensedSight` Actor)))
    (:`then_1`
      (bind (_sensed_2 _stimulus) (`self.CanSenseActor` Actor "NewEnumerator2"))
      (if _sensed_2
        (`self.HandleSensedSound` (`.StimulusLocation` (break `AIStimulus` _stimulus)))))
    (:`then_2`
      (bind _sensed_3 (`self.CanSenseActor` Actor "NewEnumerator3"))
      (if _sensed_3
        (`self.HandleSensedDamage` Actor)))))

(event `CheckIfForgottenSeenActor`
  (if (!= (`KismetArrayLibrary.Array_Length` (`self.KnownSceneActors`)) (`KismetArrayLibrary.Array_Length` (`AIPerceptionComponent.GetKnownPerceivedActors` (`self.AIPerception`) null)))
    (for _array_element (`self.KnownSceneActors`)
      (if (== (`KismetArrayLibrary.Array_Find` (`AIPerceptionComponent.GetKnownPerceivedActors` (`self.AIPerception`) null) _array_element) -1)
        (`self.HandleForgotActor` _array_element)))))

(fn `CanSenseActor`
  (params (Actor :type "Actor Object Reference") (Sense :type "/Game/Blueprints/Enums/E_AISense Enum" :default "NewEnumerator0"))
  (returns (Sensed :type Boolean) (Stimulus :type "AIStimulus Structure") (Output_Get :type "Actor Object Reference"))
  (bind _info (`AIPerceptionComponent.GetActorsPerception` (`self.AIPerception`) Actor))
  (bind (_target _lastsensedstimuli) (break `ActorPerceptionBlueprintInfo` _info))
  (bind _output_get (set `self.AttackTarget` _target))
  (for (_array_element _array_index) _lastsensedstimuli
    (set `self.PerceievedPlayer` _array_index)
    (bind _returnvalue (`AIPerceptionSystem.GetSenseClassForStimulus` _array_element))
    (if (== _returnvalue (select `/Game/Blueprints/Enums/E_AISense` Sense :`NewEnumerator1` "/Script/AIModule.AISense_Sight" :`NewEnumerator2` "/Script/AIModule.AISense_Hearing" :`NewEnumerator3` "/Script/AIModule.AISense_Damage" :!type "Object Class Reference"))
      (return (`.bSuccessfullySensed` (break `AIStimulus` _array_element)) _array_element _output_get))))

(fn `GetCurrentState`
  (returns (State :type "/Game/Blueprints/Enums/E_AIState Enum"))
  (return (cast `/Game/Blueprints/Enums/E_AIState` (`BlackboardComponent.GetValueAsEnum` (`self.Blackboard`) (`self.StateKeyName`)))))

(fn `HandleForgotActor`
  (params (Actor :type "Actor Object Reference"))
  (`KismetArrayLibrary.Array_RemoveItem` (`self.KnownSceneActors`))
  (if (== Actor (`self.AttackTarget`))
    (`self.SetStateAsPassive`)))

(fn `HandleSensedDamage`
  (params (Actor :type "Actor Object Reference"))
  (bind _state (`self.GetCurrentState`))
  (switch `/Game/Blueprints/Enums/E_AIState` _state
    (:`NewEnumerator0`
      _)
    (:`NewEnumerator3`
      _))
  (`self.SetStateAsAttacking` Actor))

(fn `HandleSensedSight`
  (params (Actor :type "Actor Object Reference"))
  (bind _isdead (message `/Game/Blueprints/Interfaces/BPI_Stats.GetIsDead` Actor))
  (if _isdead
    (`self.SetStateAsPassive`)
    (else
      (`KismetArrayLibrary.Array_AddUnique` (`self.KnownSceneActors`) Actor)
      (bind _state (`self.GetCurrentState`))
      (switch `/Game/Blueprints/Enums/E_AIState` _state
        (:`NewEnumerator0`
          _)
        (:`NewEnumerator3`
          _))
      (`self.SetStateAsAttacking` Actor))))

(fn `HandleSensedSound`
  (params (Location :type "Vector Structure"))
  (bind _state (`self.GetCurrentState`))
  (switch `/Game/Blueprints/Enums/E_AIState` _state
    (:`NewEnumerator0`
      _)
    (:`NewEnumerator3`
      _))
  (`self.SetStateAsInvestigating` Location))

(fn `SetStateAsAttacking`
  (params (AttackTarget :type "Actor Object Reference"))
  (bind _output_get (set `self.AttackTarget` AttackTarget))
  (`BlackboardComponent.SetValueAsObject` (`self.Blackboard`) (`self.AttackTargetKeyName`) _output_get)
  (`BlackboardComponent.SetValueAsEnum` (`self.Blackboard`) (`self.StateKeyName`) (enumliteral `/Game/Blueprints/Enums/E_AIState` "NewEnumerator1")))

(fn `SetStateAsInvestigating`
  (params (Location :type "Vector Structure"))
  (`BlackboardComponent.SetValueAsEnum` (`self.Blackboard`) (`self.StateKeyName`) (enumliteral `/Game/Blueprints/Enums/E_AIState` "NewEnumerator3"))
  (`BlackboardComponent.SetValueAsVector` (`self.Blackboard`) (`self.PointOfInterestKeyName`) Location))

(fn `SetStateAsPassive`
  (bind _blackboard (`self.Blackboard`))
  (`BlackboardComponent.SetValueAsEnum` _blackboard (`self.StateKeyName`) (enumliteral `/Game/Blueprints/Enums/E_AIState` "NewEnumerator0"))
  (bind _output_get (set `self.AttackTarget` null))
  (`BlackboardComponent.SetValueAsObject` _blackboard (`self.AttackTargetKeyName`) _output_get))

(fn `UserConstructionScript`)