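; Interactable locker cabinet whose door swings open and closed, optionally gated by a keycard.
; Interact passes through a server event to a local event, which plays or reverses a timeline that rotates the door.
; Timeline updates also clear the interacting character's keycard flag, even when no keycard is required.
; Box overlap adds an outline and shows the unlocked material for keycard holders; leaving restores the locked look.
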(event `/Game/Blueprints/Interfaces/BPI_Interact.Interact`
  (params (Character :type "/Game/Blueprints/Characters/BP_BaseCharacter Object Reference"))
  (`self.Server_CabinetInteract` Character))

(event `Server_CabinetInteract`
  (params (Character :type "/Game/Blueprints/Characters/BP_BaseCharacter Object Reference"))
  (`self.Local_CabinetInteract` Character))

(event `Local_CabinetInteract`
  (params (Character :type "/Game/Blueprints/Characters/BP_BaseCharacter Object Reference"))
  (if (`self.RequireKeycard?`)
    (bind _haskeycard (message `/Game/Blueprints/Interfaces/BPI_SelectedWeapons.GetHasKeycard` Character))
    (if _haskeycard
      (if (`self.IsCabinetOpen?`) :!label _label
        (set `self.IsCabinetOpen?` false)
        (bind (_direction _newtrack_0) (`Timeline|Cabinet` :!via `Reverse` :!label _label_2)
          (:`Update`
            (`SceneComponent.K2_SetRelativeRotation` (`self.SM_Prop_Locker_01_Door_01`) (`KismetMathLibrary.RLerp` (struct) (struct :`Yaw` -125.0) _newtrack_0) false false)
            (message `/Game/Blueprints/Interfaces/BPI_SelectedWeapons.SetHasKeycard` Character false)))
        (else
          (set `self.IsCabinetOpen?` true)
          (goto _label_2)))
      (elif (`self.IsCabinetOpen?`)
        (goto _label_2 :!via `Reverse`)))
    (else
      (goto _label))))

(event `self.Box.OnComponentBeginOverlap`
  (params (OverlappedComponent :type "PrimitiveComponent Object Reference") (OtherActor :type "Actor Object Reference") (OtherComp :type "PrimitiveComponent Object Reference") (OtherBodyIndex :type Integer) (bFromSweep :type Boolean) (SweepResult :type "HitResult Structure (by ref)"))
  (`MeshComponent.SetOverlayMaterial` (`self.SM_Prop_Locker_01_Door_01`) "/Game/Materials/M_Outline.M_Outline")
  (bind _haskeycard (message `/Game/Blueprints/Interfaces/BPI_SelectedWeapons.GetHasKeycard` OtherActor))
  (if _haskeycard
    (`PrimitiveComponent.SetMaterial` (`self.SM_Prop_Locker_01_Door_01`) 0 "/Game/Materials/Cabinets/M_CabinetUnlocked.M_CabinetUnlocked")))

(event `self.Box.OnComponentEndOverlap`
  (params (OverlappedComponent :type "PrimitiveComponent Object Reference") (OtherActor :type "Actor Object Reference") (OtherComp :type "PrimitiveComponent Object Reference") (OtherBodyIndex :type Integer))
  (`MeshComponent.SetOverlayMaterial` (`self.SM_Prop_Locker_01_Door_01`) null)
  (`PrimitiveComponent.SetMaterial` (`self.SM_Prop_Locker_01_Door_01`) 0 "/Game/Materials/Cabinets/M_CabinetLocked.M_CabinetLocked"))

(fn `UserConstructionScript`)