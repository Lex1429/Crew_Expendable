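; Test alien AI character that can sense pawns, attack the player and die.
; AttackPlayer plays the attack montage and signals attack end whether it completes or is interrupted.
; PawnSensing stores the last seen pawn in SensedPawn.
; A server death event calls the local death logic, which plays a non-looping dying animation and disables movement.
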(event `AttackPlayer`
  (`|PlayMontage` (`self.Mesh`) "/Game/Animations/TempAlien/AM_TestAlienAttack.AM_TestAlienAttack" 1.0 0.0 "None" false
    (:`OnCompleted`
      _)
    (:`OnInterrupted`
      _))
  (`self.OnAttackEnd`))

(event `self.PawnSensing.OnSeePawn`
  (params (Pawn :type "Pawn Object Reference"))
  (set `self.SensedPawn` Pawn))

(event `Local_AIDeath`
  (`SkeletalMeshComponent.PlayAnimation` (`self.Mesh`) "/Game/Animations/TempAlien/Dying.Dying" false)
  (`CharacterMovementComponent.DisableMovement` (`self.CharacterMovement`)))

(event `Server_AIDeath`
  (`self.Local_AIDeath`))

(fn `UserConstructionScript`
  (`parent.UserConstructionScript`))