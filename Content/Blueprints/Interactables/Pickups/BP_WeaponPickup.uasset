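; Weapon pickup interactable that gives the interacting character a weapon.
; Interact passes the character and the pickup's SpawnWeapon variable to a server-named event, which calls SpawnWeapon on that character and then destroys the pickup actor.
; BeginPlay, overlap and Tick are disabled stubs, so the pickup acts only through Interact.
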(event `/Game/Blueprints/Interfaces/BPI_Interact.Interact`
  (params (Character :type "/Game/Blueprints/Characters/BP_BaseCharacter Object Reference"))
  (`self.Server_SpawnWeapon` Character (`self.SpawnWeapon`)))

(event `Server_SpawnWeapon`
  (params (Character :type "/Game/Blueprints/Characters/BP_BaseCharacter Object Reference") (Weapon :type "/Game/Blueprints/Interactables/Weapons/BP_WeaponComponentMaster Class Reference"))
  (`/Game/Blueprints/Characters/BP_BaseCharacter.SpawnWeapon` Character Weapon)
  (`self.K2_DestroyActor`))

(fn `UserConstructionScript`
  (`parent.UserConstructionScript`))