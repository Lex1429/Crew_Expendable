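; BP_CrewActivateTest is an interactable button that starts server travel to the MidgardStation map.
; Overlapping its InteractRadius shows a widget prompt and sets AbleToStart; leaving hides the widget and clears the flag.
; On Interact, if AbleToStart is set and it runs on the server, it calls ServerTravel, then sets the game state's live players message from its player count message.
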(event `self.InteractRadius.OnComponentBeginOverlap`
  (params (OverlappedComponent :type "PrimitiveComponent Object Reference") (OtherActor :type "Actor Object Reference") (OtherComp :type "PrimitiveComponent Object Reference") (OtherBodyIndex :type Integer) (bFromSweep :type Boolean) (SweepResult :type "HitResult Structure (by ref)"))
  (`SceneComponent.SetVisibility` (`self.Widget`) true false)
  (set `self.AbleToStart?` true))

(event `self.InteractRadius.OnComponentEndOverlap`
  (params (OverlappedComponent :type "PrimitiveComponent Object Reference") (OtherActor :type "Actor Object Reference") (OtherComp :type "PrimitiveComponent Object Reference") (OtherBodyIndex :type Integer))
  (`SceneComponent.SetVisibility` (`self.Widget`) false false)
  (set `self.AbleToStart?` false))

(event `/Game/Blueprints/Interfaces/BPI_Interact.Interact`
  (params (Character :type "/Game/Blueprints/Characters/BP_BaseCharacter Object Reference"))
  (bind _returnvalue (`GameplayStatics.GetGameState`))
  (if (`self.AbleToStart?`)
    (if (`KismetSystemLibrary.IsServer`)
      (`AdvancedSessionsLibrary.ServerTravel` "MidgardStation")
      (bind _playercount (message `/Game/Blueprints/Interfaces/BPI_Server.GetPlayerCount` _returnvalue))
      (message `/Game/Blueprints/Interfaces/BPI_Server.SetLivePlayers` _returnvalue _playercount))))

(fn `UserConstructionScript`)