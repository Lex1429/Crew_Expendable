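; Base pickup actor for salvage items that shows an interaction prompt and a proximity highlight, with no collection logic of its own.
; Shortly after BeginPlay it caches the player UI widget and looks up its name and value in the salvage DataTable by PickupName.
; Viewing shows or resets the "Pick Up" prompt with that data.
; InRange briefly flashes an outline overlay material on the pickup object when true.
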(event `self.ReceiveBeginPlay`
  (`KismetSystemLibrary.Delay` 2.0)
  (`|ExecutionSequence`
    (:`then_0`
      (bind _foundwidgets (`WidgetBlueprintLibrary.GetAllWidgetsOfClass` "/Game/UI/WB_PlayerUI.WB_PlayerUI_C"))
      (set `self.PlayerUIRef` (`|GetArrayItem` _foundwidgets)))
    (:`then_1`
      (bind _returnvalue (`|GetDataTableRow` "/Game/Blueprints/Salvage/DT_SalvageList.DT_SalvageList" (`self.PickupName`))
        (:`then`
          (bind (_name _value) (break `/Game/Blueprints/Salvage/S_Salvage` _returnvalue))
          (set `self.Name` _name)
          (set `self.Value` _value))))))

(event `/Game/Blueprints/Interfaces/BPI_Interact.Viewing`
  (params (State :type Boolean))
  (bind _playeruiref (`self.PlayerUIRef`))
  (if State
    (message `/Game/Blueprints/Interfaces/BPI_CombatUI.InteractElement` _playeruiref (`KismetTextLibrary.Conv_NameToText` (`self.Name`)) (`KismetTextLibrary.Conv_IntToText` (`self.Value`)) "Pick Up" true)
    (else
      (message `/Game/Blueprints/Interfaces/BPI_CombatUI.InteractElement` _playeruiref "" "" "" false))))

(event `/Game/Blueprints/Interfaces/BPI_Interact.InRange`
  (params (State :type Boolean))
  (bind _pickupobject (`self.PickupObject`))
  (if State
    (`MeshComponent.SetOverlayMaterial` _pickupobject "/Game/Materials/M_Outline.M_Outline")
    (`KismetSystemLibrary.Delay` 1.5)
    (`MeshComponent.SetOverlayMaterial` _pickupobject null)))

(fn `UserConstructionScript`)