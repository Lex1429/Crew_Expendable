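; BP_Intersection1 is a modular building hub piece with three optional end caps, each paired with a window.
; All logic runs in the Construction Script, which applies a shared building material to the hub and caps and passes its RoomTag to the child-actor overhead lamp.
; Per-cap booleans then toggle visibility and collision for each cap and window pair.
; The lamp cast gates these toggles, so they are skipped if it fails.
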(fn `UserConstructionScript`
  (bind _endcap1 (`self.EndCap1`))
  (`PrimitiveComponent.SetMaterial` (`self.SM_Bld_Pod_Hub_02`) 0 (`self.BuildingMaterial`))
  (`PrimitiveComponent.SetMaterial` (`self.EndCap1`) 0 (`self.BuildingMaterial`))
  (`PrimitiveComponent.SetMaterial` (`self.EndCap2`) 0 (`self.BuildingMaterial`))
  (`PrimitiveComponent.SetMaterial` (`self.EndCap3`) 0 (`self.BuildingMaterial`))
  (bind _asbp_lamp_base (cast `/Game/Blueprints/Interactables/CealingLights/BP_LampBase` (`ChildActorComponent.ChildActor` (`self.OverheadLight1`))))
  (set `/Game/Blueprints/Interactables/CealingLights/BP_LampBase.RoomTag` (`self.RoomTag`) _asbp_lamp_base)
  (`|ExecutionSequence`
    (:`then_0`
      (if (`self.Endcap1On?`)
        (`SceneComponent.SetVisibility` (`self.EndCap1`) true false)
        (`SceneComponent.SetVisibility` (`self.Window1`) true false)
        (`PrimitiveComponent.SetCollisionEnabled` (`self.Window1`) "QueryAndPhysics")
        (`PrimitiveComponent.SetCollisionEnabled` (`self.EndCap1`) "QueryAndPhysics")
        (else
          (`SceneComponent.SetVisibility` _endcap1 false false)
          (`SceneComponent.SetVisibility` (`self.Window1`) false false)
          (`PrimitiveComponent.SetCollisionEnabled` _endcap1 "NoCollision")
          (`PrimitiveComponent.SetCollisionEnabled` (`self.Window1`) "NoCollision"))))
    (:`then_1`
      (if (`self.Endcap2On?`)
        (`SceneComponent.SetVisibility` (`self.Window2`) true false)
        (`SceneComponent.SetVisibility` (`self.EndCap2`) true false)
        (`PrimitiveComponent.SetCollisionEnabled` (`self.EndCap2`) "QueryAndPhysics")
        (`PrimitiveComponent.SetCollisionEnabled` (`self.Window2`) "QueryAndPhysics")
        (else
          (`SceneComponent.SetVisibility` (`self.Window2`) false false)
          (`SceneComponent.SetVisibility` (`self.EndCap2`) false false)
          (`PrimitiveComponent.SetCollisionEnabled` (`self.EndCap2`) "NoCollision")
          (`PrimitiveComponent.SetCollisionEnabled` (`self.Window2`) "NoCollision"))))
    (:`then_2`
      (if (`self.Endcap3On?`)
        (`SceneComponent.SetVisibility` (`self.Window3`) true false)
        (`SceneComponent.SetVisibility` (`self.EndCap3`) true false)
        (`PrimitiveComponent.SetCollisionEnabled` (`self.EndCap3`) "QueryAndPhysics")
        (`PrimitiveComponent.SetCollisionEnabled` (`self.Window3`) "QueryAndPhysics")
        (else
          (`SceneComponent.SetVisibility` (`self.Window3`) false false)
          (`SceneComponent.SetVisibility` (`self.EndCap3`) false false)
          (`PrimitiveComponent.SetCollisionEnabled` (`self.EndCap3`) "NoCollision")
          (`PrimitiveComponent.SetCollisionEnabled` (`self.Window3`) "NoCollision"))))))