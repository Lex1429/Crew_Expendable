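; Base Blueprint for in-world mini-game screens that switch between idle and offline materials as the game is enabled or disabled.
; A looping timer compares the detected player's facing to an arrow, revealing a key prompt and allowing interact or exit input.
; Child classes override ForceAction and ForceExit, using stored move axes and transition events that only toggle player input, as camera blends are disconnected.
; Completion is reported to BP_PS_Gameplay.
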(event `EnableMiniGame`
  ;[1 1 1] Init
  (`PrimitiveComponent.SetMaterial` (`self.MiniGameScreen`) 0 (`self.DMI_Idle`) :!label _label)
  (set `self.MiniGameEnabled` true))

(event `self.ReceiveBeginPlay`
  ;[1 1 1] Init
  (bind _returnvalue (`KismetSystemLibrary.K2_SetTimer` null "CheckPlayerDirection" 0.15 true))
  (set `self.CheckPlayerDirectionHandle` _returnvalue)
  (set `self.PlayerOverlapped` false)
  (set `self.PlayerDetected` false)
  (set `self.IsMiniGameActivated` false)
  (set `self.InputEnable` true)
  (set `self.RightAxis` 0.0)
  (set `self.ForwardAxis` 0.0)
  ;;[1 1 1] Idle material
  (bind _returnvalue_2 (`KismetMaterialLibrary.CreateDynamicMaterialInstance` "/Game/MiniGames3/Materials/MI_MiniGamesIdle_Inst.MI_MiniGamesIdle_Inst"))
  (set `self.DMI_Idle` _returnvalue_2)
  ;;[1 1 1] Offline material
  (bind _returnvalue_3 (`KismetMaterialLibrary.CreateDynamicMaterialInstance` "/Game/MiniGames3/Materials/MI_MiniGameOffline_Inst.MI_MiniGameOffline_Inst"))
  (set `self.DMI_Offline` _returnvalue_3)
  (if (`self.MiniGameEnabled`)
    (goto _label)
    (else
      (`PrimitiveComponent.SetMaterial` (`self.MiniGameScreen`) 0 (`self.DMI_Offline`) :!label _label_2)
      (set `self.MiniGameEnabled` false))))

(event `DisableMiniGame`
  ;[1 1 1] Init
  (goto _label_2))

(event `EnhancedInput|/Game/Blueprints/Inputs/IA_Move`
  (params (ActionValue :type "Vector2D Structure") (ElapsedSeconds :type "Float (double-precision)") (TriggeredSeconds :type "Float (double-precision)") (InputAction :type "InputAction Object Reference" :default "/Game/Blueprints/Inputs/IA_Move.IA_Move"))
  (bind _gamepadsensitivity (`self.GamepadSensitivity`))
  ;[1 0.3624 0.09625 1 24] Please note!
  ; Default Action mapping specified inside of  IMC_Default (/Demo/Input/IMC_Default.uasset)
  ;;[1 1 1] Controls
  (:`Triggered`
    (`|ExecutionSequence` :!label _label_3
      (:`then_0`
        (if (>= (`KismetMathLibrary.Abs` ActionValue_Y) _gamepadsensitivity)
          (set `self.ForwardAxis` ActionValue_Y)
          (else
            (set `self.ForwardAxis` 0.0))))
      (:`then_1`
        (if (>= (`KismetMathLibrary.Abs` ActionValue_X) _gamepadsensitivity)
          (set `self.RightAxis` ActionValue_X)
          (else
            (set `self.RightAxis` 0.0))))))
  (:`Completed`
    (goto _label_3)))

(event `CheckBeginOverlap`
  (params (Actor :type "Actor Object Reference"))
  (bind _playerpawn (`self.PlayerPawn`))
  ;[1 1 1] Check overlapped Player
  (if (`KismetSystemLibrary.IsValid` _playerpawn)
    (if (== Actor _playerpawn)
      (set `self.PlayerDetected` true :!label _label_4)
      (set `self.OverlappedActor` Actor))
    (else
      (goto _label_4))))

(event `CheckEndOverlap`
  (params (Actor :type "Actor Object Reference"))
  ;[1 1 1] Check overlapped Player
  (if (`self.PlayerDetected`)
    (if (== Actor (`self.OverlappedActor`))
      (set `self.PlayerDetected` false)
      (set `self.PlayerOverlapped` false)
      (set `self.OverlappedActor` null)
      (`MaterialInstanceDynamic.SetScalarParameterValue` (`self.DMI_Idle`) "ShowKey" 0.0))))

(event `EnhancedInput|/Game/Blueprints/Inputs/IA_Interact`
  (params (ActionValue :type Boolean) (ElapsedSeconds :type "Float (double-precision)") (TriggeredSeconds :type "Float (double-precision)") (InputAction :type "InputAction Object Reference" :default "/Game/Blueprints/Inputs/IA_Interact.IA_Interact"))
  ;[1 0.3624 0.09625 1 24] Please note!
  ; Default Action mapping specified inside of  IMC_Default (/Demo/Input/IMC_Default.uasset)
  ;;[1 1 1] Start mini game or Action key in the mini game
  (:`Triggered`
    (if (`self.MiniGameEnabled`) :!label _label_5
      (if (`self.PlayerOverlapped`)
        (`self.ForceAction` null))))
  (:`Started`
    (goto _label_5)))

(event `CheckPlayerDirection`
  (bind _overlappedactor (`self.OverlappedActor`))
  (bind _dmi_idle (`self.DMI_Idle`))
  ;[1 1 1] Check if player oriented to Mini Game screen
  (if (`self.PlayerDetected`)
    (`/Engine/EditorBlueprintResources/StandardMacros.IsValid` _overlappedactor
      (:`Is Valid`
        (if (<= (`KismetMathLibrary.DegAcos` (`KismetMathLibrary.Dot_VectorVector` (`SceneComponent.GetForwardVector` (`self.Arrow`)) (`self.GetActorForwardVector` _overlappedactor))) (`self.DetectionAngle`))
          (set `self.PlayerOverlapped` true)
          (`MaterialInstanceDynamic.SetScalarParameterValue` _dmi_idle "ShowKey" 1.0)
          (else
            (set `self.PlayerOverlapped` false)
            (`MaterialInstanceDynamic.SetScalarParameterValue` _dmi_idle "ShowKey" 0.0)))))))

(event `EnhancedInput|/Game/MiniGames3/Demo/Input/Actions/IA_MiniGameExit`
  (params (ActionValue :type Boolean) (ElapsedSeconds :type "Float (double-precision)") (TriggeredSeconds :type "Float (double-precision)") (InputAction :type "InputAction Object Reference" :default "/Game/MiniGames3/Demo/Input/Actions/IA_MiniGameExit.IA_MiniGameExit"))
  ;[1 0.3624 0.09625 1 24] Please note!
  ; Default Action mapping specified inside of  IMC_Default (/Demo/Input/IMC_Default.uasset)
  ;;[1 1 1] Exit for mini game
  (:`Triggered`
    (if (`self.MiniGameEnabled`)
      (if (`self.PlayerOverlapped`)
        (if (`self.IsMiniGameActivated`)
          (`PrimitiveComponent.SetMaterial` (`self.MiniGameScreen`) 0 (`self.DMI_Idle`))
          (`self.ForceExit`))))))

(event `BlendCameraFromPlayerToGame`
  (params (MiniGame :type "Actor Object Reference") (Player :type "Actor Object Reference"))
  ;[1 1 1] Camera transition from Player to Mini Game
  (`self.DisableInput` Player (`GameplayStatics.GetPlayerController` 0)))

(event `ForceAction`
  (params (Player :type "/Game/Blueprints/Characters/BP_PlayerCharacterCore Object Reference"))
  ;[0 0.3254 1] Overwritable events
)

(event `SetOfflineMaterial`
  ;[1 1 1] Set Offline material for the screen
  (`PrimitiveComponent.SetMaterial` (`self.MiniGameScreen`) 0 (`self.DMI_Offline`)))

(event `ForceExit`
  ;[0 0.3254 1] Overwritable events
)

(event `BlendCameraFromGameToPlayer`
  (params (Player :type "Actor Object Reference"))
  ;[1 1 1] Camera Transition from Mini Game to Player
  (`self.EnableInput` Player (`GameplayStatics.GetPlayerController` 0)))

(event `GameCompleted`
  (params (Minigame :type "/Game/MiniGames3/Blueprints/Data/BP_MiniGamesBase2 Object Reference"))
  (bind _asbp_ps_gameplay (cast `/Game/MBLS/Blueprints/Core/Gameplay/Player/BP_PS_Gameplay` (`GameplayStatics.GetPlayerState` 0)))
  (`/Game/MBLS/Blueprints/Core/Gameplay/Player/BP_PS_Gameplay.MiniGame1Test` _asbp_ps_gameplay Minigame))

(fn `GetCanBePickedUp`
  (returns (CanBePickedUp :type Boolean))
  (return false))

(fn `GetItemToSpawn`
  (returns (Item :type "/Game/Blueprints/Interactables/Weapons/BP_WeaponComponentMaster Class Reference"))
  (return null))

(fn `UserConstructionScript`)