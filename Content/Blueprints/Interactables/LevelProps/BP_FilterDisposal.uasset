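; Interactable disposal bin that accepts held cooling or heating filters and rejects any other equipment with error lights and a deny sound.
; Interact clears the player's held item, then routes through authority or a server event to fire the matching filter-disposed dispatcher and play staged sounds and an electric effect.
; Box overlap slides the lid via timeline and resets the lights on exit, while range and view events drive an outline and UI prompt.
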(event `self.ReceiveBeginPlay`
  (`|ExecutionSequence`
    (:`then_0`
      (`KismetSystemLibrary.Delay` 2.0)
      (bind _foundwidgets (`WidgetBlueprintLibrary.GetAllWidgetsOfClass` "/Game/UI/WB_PlayerUI.WB_PlayerUI_C"))
      (set `self.PlayerUIRef` (`|GetArrayItem` _foundwidgets)))))

(event `/Game/Blueprints/Interfaces/BPI_Interact.Interact`
  (params (Character :type "Object Object Reference") (PlayerCharacter :type "/Game/Blueprints/Characters/BP_PlayerCharacterCore Object Reference"))
  (switch `name` (`/Game/Blueprints/Characters/BP_PlayerCharacterCore.CurrentEquipmentHeld` PlayerCharacter)
    (:`Default`
      (`PrimitiveComponent.SetMaterial` (`self.light_left`) 0 "/Game/Assets/VentMiniGameParts/TrashCan/MI_LightError.MI_LightError")
      (`PrimitiveComponent.SetMaterial` (`self.light_right`) 0 "/Game/Assets/VentMiniGameParts/TrashCan/MI_LightError.MI_LightError")
      (`GameplayStatics.SpawnSoundAttached` "/Game/SFX/MinigameSounds/ACVent/WDU-Deny-Item.WDU-Deny-Item" (`self.SM_Prop_TrashBin_01`) "None" (0.0 0.0 0.0) (struct) "KeepRelativeOffset" false 1.0 1.0 0.0 "/Game/MBLS/Assets/Audio/Classes/SA_Short.SA_Short" null))
    (:`5`
      (set `self.DroppedItem` "5")
      (`self.Owner_DropOff` PlayerCharacter)
      (`/Engine/EditorBlueprintResources/ActorMacros.Switch Has Authority`
        (:`Authority`
          (`self.CoolingFilterDispossed`)
          (`self.Local_DropOff` PlayerCharacter :!label _label))
        (:`Remote`
          (`self.Server_DropOff` PlayerCharacter))))
    (:`7`
      (set `self.DroppedItem` "7")
      (`self.Owner_DropOff` PlayerCharacter)
      (`/Engine/EditorBlueprintResources/ActorMacros.Switch Has Authority`
        (:`Authority`
          (`self.HeatingFilterDispossed`)
          (goto _label))
        (:`Remote`
          (`self.Server_DropOff` PlayerCharacter))))))

(event `Owner_DropOff`
  (params (Player :type "/Game/Blueprints/Characters/BP_PlayerCharacterCore Object Reference"))
  (`/Game/Blueprints/Characters/BP_PlayerCharacterCore.RemoveItemFromInventory` Player)
  (`/Game/Blueprints/Characters/BP_PlayerCharacterCore.Server_SetHeldEquipment` Player "1"))

(event `Server_DropOff`
  (params (Player :type "/Game/Blueprints/Characters/BP_PlayerCharacterCore Object Reference"))
  (switch `name` (`self.DroppedItem`)
    (:`5`
      (`self.CoolingFilterDispossed`))
    (:`7`
      (`self.HeatingFilterDispossed`)))
  (`self.Local_DropOff` Player))

(event `Local_DropOff`
  (params (Player :type "/Game/Blueprints/Characters/BP_PlayerCharacterCore Object Reference"))
  (bind _itemspawnpoint (`self.ItemSpawnPoint`))
  (`GameplayStatics.SpawnSoundAttached` "/Game/SFX/MinigameSounds/ACVent/Tossed-item-in-bin.Tossed-item-in-bin" (`self.SM_Prop_TrashBin_01`) "None" (0.0 0.0 0.0) (struct) "KeepRelativeOffset" false 1.0 1.0 0.0 "/Game/MBLS/Assets/Audio/Classes/SA_Short.SA_Short" null)
  (`KismetSystemLibrary.Delay` 0.5)
  (`GameplayStatics.SpawnSoundAttached` "/Game/SFX/MinigameSounds/ACVent/WDU-Accept-Item.WDU-Accept-Item" (`self.SM_Prop_TrashBin_01`) "None" (0.0 0.0 0.0) (struct) "KeepRelativeOffset" false 1.0 1.0 0.0 "/Game/MBLS/Assets/Audio/Classes/SA_Short.SA_Short" null)
  (`KismetSystemLibrary.Delay` 0.7)
  (`GameplayStatics.SpawnSoundAttached` "/Game/SFX/MinigameSounds/ACVent/Item-Processing.Item-Processing" (`self.SM_Prop_TrashBin_01`) "None" (0.0 0.0 0.0) (struct) "KeepRelativeOffset" false 1.0 1.0 0.0 "/Game/MBLS/Assets/Audio/Classes/SA_Short.SA_Short" null)
  (`NiagaraFunctionLibrary.SpawnSystemAttached` "/Game/AllShadesofVFXBundle/EnvironmentVFX/VFX/Electricity/Systems/N_ElectricExplosion2.N_ElectricExplosion2" _itemspawnpoint "None" (`SceneComponent.RelativeLocation` _itemspawnpoint) (`SceneComponent.RelativeRotation` _itemspawnpoint) "SnapToTarget" true))

(event `self.InRange`
  (params (State :type Boolean))
  (bind _sm_prop_trashbin_01 (`self.SM_Prop_TrashBin_01`))
  (if State
    (`MeshComponent.SetOverlayMaterial` _sm_prop_trashbin_01 "/Game/Materials/M_Outline.M_Outline")
    (`KismetSystemLibrary.Delay` 1.5)
    (`MeshComponent.SetOverlayMaterial` _sm_prop_trashbin_01 null)))

(event `self.Viewing`
  (params (State :type Boolean))
  (bind _playeruiref (`self.PlayerUIRef`))
  (if State
    (message `/Game/Blueprints/Interfaces/BPI_CombatUI.InteractElement` _playeruiref "Disposal" "" "Activate" true "")
    (else
      (message `/Game/Blueprints/Interfaces/BPI_CombatUI.InteractElement` _playeruiref "" "" "" false ""))))

(event `self.Box.OnComponentBeginOverlap`
  (params (OverlappedComponent :type "PrimitiveComponent Object Reference") (OtherActor :type "Actor Object Reference") (OtherComp :type "PrimitiveComponent Object Reference") (OtherBodyIndex :type Integer) (bFromSweep :type Boolean) (SweepResult :type "HitResult Structure (by ref)"))
  (`GameplayStatics.SpawnSoundAttached` "/Game/SFX/MinigameSounds/ACVent/WDU-Lid-Open.WDU-Lid-Open" (`self.SM_Prop_TrashBin_01`) "None" (0.0 0.0 0.0) (struct) "KeepRelativeOffset" false 1.0 1.0 0.0 "/Game/MBLS/Assets/Audio/Classes/SA_Short.SA_Short" null)
  (bind (_direction _newtrack_0) (`Timeline|LidOpening` :!label _label_2)
    (:`Update`
      (`SceneComponent.K2_SetRelativeLocation` (`self.opening_panel`) (`KismetMathLibrary.VLerp` (0.0 0.0 0.0) (0.0 -37.0 23.0) _newtrack_0) false false))))

(event `self.Box.OnComponentEndOverlap`
  (params (OverlappedComponent :type "PrimitiveComponent Object Reference") (OtherActor :type "Actor Object Reference") (OtherComp :type "PrimitiveComponent Object Reference") (OtherBodyIndex :type Integer))
  (`PrimitiveComponent.SetMaterial` (`self.light_left`) 0 "/Game/Assets/VentMiniGameParts/TrashCan/MI_TrashOn.MI_TrashOn")
  (`PrimitiveComponent.SetMaterial` (`self.light_right`) 0 "/Game/Assets/VentMiniGameParts/TrashCan/MI_TrashOn.MI_TrashOn")
  (goto _label_2 :!via `Reverse`))

(fn `GetCanBePickedUp`
  (returns (CanBePickedUp :type Boolean))
  (return false))

(fn `GetItemToSpawn`
  (returns (Item :type "/Game/Blueprints/Interactables/Weapons/BP_WeaponComponentMaster Class Reference"))
  (return null))

(fn `OnRep_CoolingFilterDeposit?`)

(fn `UserConstructionScript`)