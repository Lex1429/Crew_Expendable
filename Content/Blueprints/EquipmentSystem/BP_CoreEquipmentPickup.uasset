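; Base world pickup for equipment, taking its mesh and display name from the DT_EquipmentDetails row matching WeaponID.
; InView briefly shows the widget, with a retriggerable delay hiding it once calls stop.
; PickupObject sets DestroyObject, whose OnRep destroys the actor.
; QueryItem returns WeaponID, while GetCanBePickedUp returns false and GetItemToSpawn and QueryAsset are empty.
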(event `self.ReceiveBeginPlay`
  (`parent.ReceiveBeginPlay`)
  (`|ExecutionSequence`
    (:`then_0`
      (`self.SetUpPickUp`))
    (:`then_1`
      (`KismetSystemLibrary.Delay` 0.3)
      (bind _foundwidgets (`WidgetBlueprintLibrary.GetAllWidgetsOfClass` "/Game/UI/InteractPromptWidgets/WB_InteractPickup.WB_InteractPickup_C"))
      (set `self.InteractWidgetRef` (`|GetArrayItem` _foundwidgets)))))

(event `/Game/Blueprints/Interfaces/BPI_Pickup.InView`
  (bind _widget (`self.Widget`))
  (`SceneComponent.SetVisibility` _widget true false)
  (`KismetSystemLibrary.RetriggerableDelay` 0.1)
  (`SceneComponent.SetVisibility` _widget false false))

(event `/Game/Blueprints/Interfaces/BPI_Pickup.PickupObject`
  (params (PlayerRef :type "/Game/Blueprints/Characters/BP_PlayerCharacterCore Object Reference"))
  (set `self.DestroyObject` true))

(fn `GetCanBePickedUp`
  (returns (CanBePickedUp :type Boolean))
  (return false))

(fn `GetItemToSpawn`
  (returns (Item :type "/Game/Blueprints/Interactables/Weapons/BP_WeaponComponentMaster Class Reference"))
  (return null))

(fn `OnRep_DestroyObject`
  (`self.K2_DestroyActor`))

(fn `QueryAsset`
  (returns (Asset :type "/Game/Blueprints/InventorySystem/Pickups/Data/PDA_Items Object Reference"))
  (return null))

(fn `QueryItem`
  (returns (Item :type Name))
  (return (`self.WeaponID`)))

(fn `SetUpPickUp`
  (`parent.UserConstructionScript`)
  (bind _returnvalue (`|GetDataTableRow` "/Game/Blueprints/EquipmentSystem/DT_EquipmentDetails.DT_EquipmentDetails" (`self.WeaponID`))
    (:`then`
      (bind (_dispalyname _animationtype _equipmenttag _startingammo _rateoffire _firerange _throwingrange _damage _staticmesh) (break `/Game/Blueprints/EquipmentSystem/ST_Equipment` _returnvalue))
      (`StaticMeshComponent.SetStaticMesh` (`self.ObjectPickUp`) _staticmesh)
      (set `self.Dispaly Name` _dispalyname))))

(fn `UserConstructionScript`
  (message `/Game/Blueprints/Interfaces/BPI_CombatUI.InteractElement` (`self.InteractWidgetRef`) "" "" "Pick Up" true "")
  (`self.SetUpPickUp`))