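; BP_SAL is an AI enemy character with a patrol route and a repeating melee attack.
; A front hitbox overlap applies damage and plays the attack animation, repeating on a delay until overlap end clears IsAttacking.
; Patrol route accessors and an enum-to-walk-speed setter expose movement control, while Attack, GetISChasing and GetSeenPlayer are stubs.
; The construction script hides the mesh's wing bones.
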(event `Attack`)

(event `/Game/Blueprints/Interfaces/BPI_EnemyAI.SetPatrolRoute`
  (params (PatrolRoute :type "/Game/Blueprints/AI/BP_PatrolRoute Object Reference"))
  (set `self.NavPoint` PatrolRoute))

(event `self.FrontHitBox.OnComponentBeginOverlap`
  (params (OverlappedComponent :type "PrimitiveComponent Object Reference") (OtherActor :type "Actor Object Reference") (OtherComp :type "PrimitiveComponent Object Reference") (OtherBodyIndex :type Integer) (bFromSweep :type Boolean) (SweepResult :type "HitResult Structure (by ref)"))
  (set `self.IsAttacking?` true)
  (`GameplayStatics.ApplyDamage` OtherActor 25.0 null self :!label _label)
  (`SkeletalMeshComponent.PlayAnimation` (`self.Mesh`) "/Game/Animations/SAL_Animations/Basic_Attack.Basic_Attack" false)
  (`KismetSystemLibrary.Delay` 3.0)
  (if (`self.IsAttacking?`)
    (goto _label)))

(event `self.FrontHitBox.OnComponentEndOverlap`
  (params (OverlappedComponent :type "PrimitiveComponent Object Reference") (OtherActor :type "Actor Object Reference") (OtherComp :type "PrimitiveComponent Object Reference") (OtherBodyIndex :type Integer))
  (set `self.IsAttacking?` false))

(fn `GetISChasing`
  (returns (Chasing :type Boolean))
  (return false))

(fn `GetPatrolRoute`
  (returns (PatrolRoute :type "/Game/Blueprints/AI/BP_PatrolRoute Object Reference"))
  (return (`self.NavPoint`)))

(fn `GetSeenPlayer`
  (returns (SeenPlayer :type "Pawn Object Reference"))
  (return null))

(fn `SetMovementSpeed`
  (params (Speed :type "/Game/Blueprints/AI/AIv2/E_MovementSpeed Enum" :default "NewEnumerator0"))
  (returns (SpeedValue :type "Float (double-precision)"))
  (bind _output_get (set `CharacterMovementComponent.MaxWalkSpeed` (select `/Game/Blueprints/AI/AIv2/E_MovementSpeed` Speed :`NewEnumerator1` 150.0 :`NewEnumerator2` 300.0 :`NewEnumerator3` 200.0 :`NewEnumerator4` 200.0 :!type "Float (single-precision)") (`self.CharacterMovement`)))
  (return _output_get))

(fn `UserConstructionScript`
  (bind _mesh (`self.Mesh`))
  (`SkinnedMeshComponent.HideBoneByName` _mesh "BigWing_L" "PBO_None")
  (`SkinnedMeshComponent.HideBoneByName` _mesh "BigWing_R" "PBO_None")
  (`SkinnedMeshComponent.HideBoneByName` _mesh "LittleWing_L" "PBO_None")
  (`SkinnedMeshComponent.HideBoneByName` _mesh "LittleWing_R" "PBO_None"))