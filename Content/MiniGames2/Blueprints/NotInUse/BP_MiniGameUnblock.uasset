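; Unblock mini-game: a symbol-matching puzzle on an in-world screen, where the player finds four hidden pairs on an eight-slot ring.
; Looping timers poll directional input to move the selector and randomize decor; the action button reveals picks.
; A match lights a block, while a mismatch flashes, spins the ring and shifts the symbol array to reposition symbols.
; One dynamic material renders everything through parameters, with timelines driving animation.
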(event `self.ReceiveBeginPlay`
  ;[1 1 1] Init
  (`parent.ReceiveBeginPlay`)
  (bind _returnvalue (`KismetMaterialLibrary.CreateDynamicMaterialInstance` "/Game/MiniGames2/Materials/MI_MiniGameUnblock_Inst.MI_MiniGameUnblock_Inst"))
  (set `self.DMI` _returnvalue)
  (bind _returnvalue_2 (`KismetSystemLibrary.K2_SetTimer` null "CheckContorls" 0.05 true))
  (set `self.ControlsTimeHandle` _returnvalue_2)
  (bind _returnvalue_3 (`KismetSystemLibrary.K2_SetTimer` null "UpdateDecor" 0.1 true))
  (set `self.DecorTimeHandle` _returnvalue_3)
  (set `self.IsMiniGameActivated` false)
  (set `self.InputEnable` false))

(event `InitGame`
  (bind _symbolindices (`self.SymbolIndices`))
  (bind _dmi (`self.DMI`))
  (bind _symbolindices_2 (`self.SymbolIndices`))
  ;[1 1 1] ReInit game
  (set `self.IsRotation` false)
  (set `self.SolvedCounter` 0)
  (set `self.SelectorIndex` 0)
  (set `self.SelectorCounter` 0)
  (set `self.Symbol1_Index` -1)
  (set `self.Symbol2_Index` -1)
  (set `self.RotAngle` 0.0)
  (`self.ResetSymbols`)
  (`MaterialInstanceDynamic.SetScalarParameterValue` (`self.DMI`) "SelectorIndex" (`KismetMathLibrary.Conv_IntToDouble` (`self.SelectorIndex`)))
  (`MaterialInstanceDynamic.SetVectorParameterValue` _dmi "SelectorColor" (`self.SelectorColor`))
  (`MaterialInstanceDynamic.SetVectorParameterValue` _dmi "SymbolColor" (`self.SymbolColor`))
  (`KismetArrayLibrary.Array_Clear` (`self.SymbolIndices`))
  (`MaterialInstanceDynamic.SetVectorParameterValue` (`self.DMI`) "Blk1_Color" (`self.DisabledColor`))
  (`MaterialInstanceDynamic.SetVectorParameterValue` (`self.DMI`) "Blk2_Color" (`self.DisabledColor`))
  (`MaterialInstanceDynamic.SetVectorParameterValue` (`self.DMI`) "Blk3_Color" (`self.DisabledColor`))
  (`MaterialInstanceDynamic.SetVectorParameterValue` (`self.DMI`) "Blk4_Color" (`self.DisabledColor`))
  (for _index (range 1 9)
    (`MaterialInstanceDynamic.SetVectorParameterValue` (`self.DMI`) (`KismetStringLibrary.Conv_StringToName` (`KismetStringLibrary.Concat_StrStr` "Ring" (`KismetStringLibrary.Conv_IntToString` _index) "_Color")) (`self.NormalColor`)))
  (for _index_2 (range 4)
    (`KismetArrayLibrary.Array_Add` _symbolindices _index_2)
    (`KismetArrayLibrary.Array_Add` _symbolindices _index_2))
  (for _ (range 6)
    ;;[1 0.07657 0] For Nativization compatibility
    (set `self.Ind1` (`KismetMathLibrary.RandomIntegerInRange` 0 7))
    (set `self.Ind2` (`KismetMathLibrary.RandomIntegerInRange` 0 7))
    (set `self.Value1` (`|GetArrayItem` _symbolindices_2 (`self.Ind1`)))
    (set `self.Value2` (`|GetArrayItem` _symbolindices_2 (`self.Ind2`)))
    (`KismetArrayLibrary.Array_Set` _symbolindices_2 (`self.Ind1`) (`self.Value2`))
    (`KismetArrayLibrary.Array_Set` _symbolindices_2 (`self.Ind2`) (`self.Value1`))))

(event `self.ReceiveTick`
  (params (DeltaSeconds :type "Float (single-precision)"))
  (`parent.ReceiveTick` DeltaSeconds))

(event `UpdateDecor`
  (bind _dmi (`self.DMI`))
  ;[1 1 1] Update Decor
  (if (`self.IsMiniGameActivated`)
    (`MaterialInstanceDynamic.SetScalarParameterValue` _dmi "DecorText4" (`KismetMathLibrary.Conv_IntToDouble` (`KismetMathLibrary.RandomIntegerInRange` 0 31)))
    (if (`self.IsRotation`)
      (`MaterialInstanceDynamic.SetScalarParameterValue` _dmi "DecorText1" (`KismetMathLibrary.Conv_IntToDouble` (`KismetMathLibrary.RandomIntegerInRange` 0 31)))
      (`MaterialInstanceDynamic.SetScalarParameterValue` _dmi "DecorText2" (`KismetMathLibrary.Conv_IntToDouble` (`KismetMathLibrary.RandomIntegerInRange` 0 31)))
      (`MaterialInstanceDynamic.SetScalarParameterValue` _dmi "DecorText3" (`KismetMathLibrary.Conv_IntToDouble` (`KismetMathLibrary.RandomIntegerInRange` 0 31))))))

(event `ResetSymbols`
  (bind _dmi (`self.DMI`))
  ;[1 1 1] Reset symbols
  (`MaterialInstanceDynamic.SetScalarParameterValue` _dmi "Sel1_Sym1" 0.0)
  (`MaterialInstanceDynamic.SetScalarParameterValue` _dmi "Sel1_Sym2" 0.0)
  (`MaterialInstanceDynamic.SetScalarParameterValue` _dmi "Sel1_Sym3" 0.0)
  (`MaterialInstanceDynamic.SetScalarParameterValue` _dmi "Sel1_Sym4" 0.0)
  (`MaterialInstanceDynamic.SetScalarParameterValue` _dmi "Sel2_Sym1" 0.0)
  (`MaterialInstanceDynamic.SetScalarParameterValue` _dmi "Sel2_Sym2" 0.0)
  (`MaterialInstanceDynamic.SetScalarParameterValue` _dmi "Sel2_Sym3" 0.0)
  (`MaterialInstanceDynamic.SetScalarParameterValue` _dmi "Sel2_Sym4" 0.0)
  (`MaterialInstanceDynamic.SetScalarParameterValue` _dmi "Sym1_Scale" 0.0)
  (`MaterialInstanceDynamic.SetScalarParameterValue` _dmi "Sym2_Scale" 0.0))

(event `UpdateSelector`
  ;[1 1 1] Controls
  (`MaterialInstanceDynamic.SetScalarParameterValue` (`self.DMI`) "SelectorIndex" (`KismetMathLibrary.Conv_IntToDouble` (`self.SelectorIndex`)) :!label _label))

(event `CheckContorls`
  (bind _rightaxis (`self.RightAxis`))
  (bind _forwardaxis (`self.ForwardAxis`))
  (bind _output (`|GetArrayItem` (`self.SymbolIndices`) (`self.TempIndex`)))
  ;[1 1 1] Controls
  (if (`self.InputEnable`)
    (if (`self.IsMiniGameActivated`)
      (if (or (!= (`self.RightAxis`) 0.0) (!= (`self.ForwardAxis`) 0.0))
        (if (and (!= (`self.PrevRightAxis`) 0.0) (!= (`self.PrevForwAxis`) 0.0))
          (if (and (!= (`self.RightAxis`) 0.0) (!= (`self.ForwardAxis`) 0.0))
            (set `self.PrevRightAxis` (`self.RightAxis`) :!label _label_2)
            (set `self.PrevForwAxis` (`self.ForwardAxis`))
            (if (and (> (`self.ForwardAxis`) 0.0) (< (`self.RightAxis`) 0.0))
              (set `self.TempIndex` 7)
              (else
                (set `self.TempIndex` (/ (+ (`KismetMathLibrary.SelectInt` 2 0 (> _rightaxis 0.0)) (`KismetMathLibrary.SelectInt` 6 0 (< _rightaxis 0.0)) (`KismetMathLibrary.SelectInt` 0 0 (> _forwardaxis 0.0)) (`KismetMathLibrary.SelectInt` 4 0 (< _forwardaxis 0.0))) (+ (`KismetMathLibrary.SelectInt` 1 0 (!= (`self.RightAxis`) 0.0)) (`KismetMathLibrary.SelectInt` 1 0 (!= (`self.ForwardAxis`) 0.0)))))))
            (`KismetSystemLibrary.PrintString` (`KismetStringLibrary.Concat_StrStr` "Symbol index: " (`KismetStringLibrary.Conv_IntToString` _output)) false false (struct :`G` 1.0 :`A` 1.0))
            (if (>= _output 0)
              (if (== (`self.SelectorCounter`) 1)
                (if (!= (`self.Selector_Index1`) (`self.TempIndex`))
                  (set `self.SelectorIndex` (`self.TempIndex`) :!label _label_3)
                  (goto _label))
                (else
                  (goto _label_3)))))
          (else
            (goto _label_2)))
        (else
          (set `self.PrevRightAxis` 0.0)
          (set `self.PrevForwAxis` 0.0))))))

(event `self.InteractionBoundBox.OnComponentBeginOverlap`
  (params (OverlappedComponent :type "PrimitiveComponent Object Reference") (OtherActor :type "Actor Object Reference") (OtherComp :type "PrimitiveComponent Object Reference") (OtherBodyIndex :type Integer) (bFromSweep :type Boolean) (SweepResult :type "HitResult Structure (by ref)"))
  ;[1 1 1] Player overlapping
  (`self.CheckBeginOverlap` OtherActor))

(event `self.ForceExit`
  ;[1 1 1] Cancel
  (if (and (`self.MiniGameEnabled`) (`self.IsMiniGameActivated`))
    (set `self.IsMiniGameActivated` false)
    (set `self.InputEnable` false)
    (`self.OnMiniGameCanceled`)
    (`self.BlendCameraFromGameToPlayer` (`self.OverlappedActor`))))

(event `self.InteractionBoundBox.OnComponentEndOverlap`
  (params (OverlappedComponent :type "PrimitiveComponent Object Reference") (OtherActor :type "Actor Object Reference") (OtherComp :type "PrimitiveComponent Object Reference") (OtherBodyIndex :type Integer))
  ;[1 1 1] Player overlapping
  (`self.CheckEndOverlap` OtherActor))

(event `self.ForceAction`
  (params (Player :type "/Game/Blueprints/Characters/BP_PlayerCharacterCore Object Reference"))
  (bind _dmi (`self.DMI`))
  (bind _dmi_2 (`self.DMI`))
  (bind _selectorcounter (`self.SelectorCounter`))
  (bind _selectorindex (`self.SelectorIndex`))
  (bind _symbolindices (`self.SymbolIndices`))
  (bind _dmi_3 (`self.DMI`))
  (bind _disabledcolor (`self.DisabledColor`))
  (bind _dmi_4 (`self.DMI`))
  (bind _output (`|GetArrayItem` (`self.SymbolIndices`) (`self.SelectorIndex`)))
  ;[1 1 1] Action button
  (if (`self.PlayerOverlapped`)
    (if (`self.IsMiniGameActivated`)
      (if (`self.InputEnable`)
        (if (== (`self.SelectorCounter`) 1)
          (if (!= (`self.SelectorIndex`) (`self.Selector_Index1`))
            (set `self.InputEnable` false :!label _label_4)
            (bind _result (`/Engine/EditorBlueprintResources/StandardMacros.IncrementInt` (`self.SelectorCounter`))
              (:`  `
                (if (== _result 1)
                  (set `self.Symbol1_Index` _output)
                  (set `self.Selector_Index1` _selectorindex)
                  (else
                    (set `self.Symbol2_Index` _output)
                    (set `self.Selector_Index2` _selectorindex)))
                (`MaterialInstanceDynamic.SetScalarParameterValue` _dmi_4 (`KismetStringLibrary.Conv_StringToName` (`KismetStringLibrary.Concat_StrStr` "Sel" (`KismetStringLibrary.Conv_IntToString` _selectorcounter) "_Sym" (`KismetStringLibrary.Conv_IntToString` (+ (select `int` _selectorcounter :`0` 0 :`1` (`self.Symbol1_Index`) :`2` (`self.Symbol2_Index`)) 1)))) 1.0)
                (`MaterialInstanceDynamic.SetVectorParameterValue` _dmi_4 (`KismetStringLibrary.Conv_StringToName` (`KismetStringLibrary.Concat_StrStr` "Ring" (`KismetStringLibrary.Conv_IntToString` (+ (`self.SelectorIndex`) 1)) "_Color")) (`self.SelectColor`))
                (bind (_direction _newtrack_0) (`Timeline|Timeline_0` :!via `PlayFromStart`)
                  (:`Update`
                    (`MaterialInstanceDynamic.SetScalarParameterValue` _dmi_2 (`KismetStringLibrary.Conv_StringToName` (`KismetStringLibrary.Concat_StrStr` "Sym" (`KismetStringLibrary.Conv_IntToString` (`self.SelectorCounter`)) "_Scale")) _newtrack_0)
                    (`MaterialInstanceDynamic.SetVectorParameterValue` _dmi_2 "SymbolColor" (`self.SymbolColor`)))
                  (:`Finished`
                    (if (< (`self.SelectorCounter`) 2)
                      (set `self.InputEnable` true)
                      (elif (== (`self.Symbol1_Index`) (`self.Symbol2_Index`))
                        (`KismetSystemLibrary.Delay` 0.5)
                        (`MaterialInstanceDynamic.SetVectorParameterValue` _dmi_3 (`KismetStringLibrary.Conv_StringToName` (`KismetStringLibrary.Concat_StrStr` "Ring" (`KismetStringLibrary.Conv_IntToString` (+ (`self.Selector_Index1`) 1)) "_Color")) _disabledcolor)
                        (`MaterialInstanceDynamic.SetVectorParameterValue` _dmi_3 (`KismetStringLibrary.Conv_StringToName` (`KismetStringLibrary.Concat_StrStr` "Ring" (`KismetStringLibrary.Conv_IntToString` (+ (`self.Selector_Index2`) 1)) "_Color")) _disabledcolor)
                        (`self.ResetSymbols`)
                        (`|VariableSetRef` (`|GetArrayItem` _symbolindices (`self.Selector_Index1`)) -1)
                        (`|VariableSetRef` (`|GetArrayItem` _symbolindices (`self.Selector_Index2`)) -1)
                        (bind _result_2 (`/Engine/EditorBlueprintResources/StandardMacros.IncrementInt` (`self.SolvedCounter`))
                          (:`  `
                            (`MaterialInstanceDynamic.SetVectorParameterValue` (`self.DMI`) (`KismetStringLibrary.Conv_StringToName` (`KismetStringLibrary.Concat_StrStr` "Blk" (`KismetStringLibrary.Conv_IntToString` _result_2) "_Color")) (`self.SelectColor`))
                            (if (>= _result_2 4)
                              ;;[1 1 1] Success
                              (set `self.MiniGameEnabled` false)
                              (set `self.IsMiniGameActivated` false)
                              (set `self.InputEnable` false)
                              (`MaterialInstanceDynamic.SetScalarParameterValue` (`self.DMI`) "ShowUnblocked" 1.0)
                              (`KismetSystemLibrary.Delay` (`self.DelayTimeWhenComplete`))
                              (`self.SetOfflineMaterial`)
                              (`self.OnMiniGameSuccess`)
                              (`self.BlendCameraFromGameToPlayer` (`self.OverlappedActor`))
                              (else
                                (for (_array_element _array_index) (`self.SymbolIndices`) :!label _label_5
                                  (if (>= _array_element 0)
                                    (break)))
                                (set `self.SelectorIndex` _array_index)
                                (set `self.SelectorCounter` 0)
                                (`self.UpdateSelector`)
                                (set `self.InputEnable` true)))))
                        (else
                          ;;[1 1 1] Error
                          (bind (_direction_2 _newtrack_0_2) (`Timeline|Timeline_1` :!via `PlayFromStart`)
                            (:`Update`
                              (bind _returnvalue (`KismetMathLibrary.LinearColorLerp` (`self.FailedColor1`) (`self.FaildedColor2`) _newtrack_0_2))
                              (`MaterialInstanceDynamic.SetVectorParameterValue` _dmi (`KismetStringLibrary.Conv_StringToName` (`KismetStringLibrary.Concat_StrStr` "Ring" (`KismetStringLibrary.Conv_IntToString` (+ (`self.Selector_Index1`) 1)) "_Color")) _returnvalue)
                              (`MaterialInstanceDynamic.SetVectorParameterValue` _dmi (`KismetStringLibrary.Conv_StringToName` (`KismetStringLibrary.Concat_StrStr` "Ring" (`KismetStringLibrary.Conv_IntToString` (+ (`self.Selector_Index2`) 1)) "_Color")) _returnvalue)
                              (`MaterialInstanceDynamic.SetVectorParameterValue` _dmi "SymbolColor" _returnvalue))
                            (:`Finished`
                              (`self.ResetSymbols`)
                              (bind _output_get (set `self.Iterations` (`KismetMathLibrary.RandomIntegerInRange` 1 3)))
                              (set `self.ToAngle` (+ (`self.RotAngle`) (* _output_get 0.125)))
                              (set `self.IsRotation` true)
                              (`self.ShiftArray` (`self.Iterations`))
                              (bind (_direction_3 _newtrack_0_3) (`Timeline|Timeline_2` :!via `PlayFromStart`)
                                (:`Update`
                                  (`MaterialInstanceDynamic.SetScalarParameterValue` (`self.DMI`) "Rotation" (`KismetMathLibrary.FInterpEaseInOut` 0.0 (`self.ToAngle`) _newtrack_0_3 2.0)))
                                (:`Finished`
                                  (set `self.IsRotation` false)
                                  (for (_array_element_2 _array_index_2) (`self.SymbolIndices`)
                                    (`MaterialInstanceDynamic.SetVectorParameterValue` (`self.DMI`) (`KismetStringLibrary.Conv_StringToName` (`KismetStringLibrary.Concat_StrStr` "Ring" (`KismetStringLibrary.Conv_IntToString` (+ _array_index_2 1)) "_Color")) (`KismetMathLibrary.SelectColor` (`self.NormalColor`) (`self.DisabledColor`) (>= _array_element_2 0)))
                                    (`MaterialInstanceDynamic.SetScalarParameterValue` (`self.DMI`) "Rotation" 0.0))
                                  (goto _label_5)))))))))))))
          (else
            (goto _label_4))))
      (else
        (`self.InitGame`)
        (`PrimitiveComponent.SetMaterial` (`self.MiniGameScreen`) 0 (`self.DMI`))
        (`self.BlendCameraFromPlayerToGame` self (`self.OverlappedActor`))
        (set `self.IsMiniGameActivated` true)
        (set `self.InputEnable` true)))))

(fn `ShiftArray`
  (params (Steps :type Integer))
  (locals (LastValue :type Integer) (Val1 :type Integer))
  (bind _symbolindices (`self.SymbolIndices`))
  ;[1 1 1] Shift array from low to height index
  (for _ (range Steps)
    (set `local.LastValue` (`|GetArrayItem` (`self.SymbolIndices`) 7))
    (for _index (range 7)
      (bind _returnvalue (- 6 _index))
      (`|VariableSetRef` (`|GetArrayItem` _symbolindices (+ _returnvalue 1)) (`|GetArrayItem` _symbolindices _returnvalue)))
    (`|VariableSetRef` (`|GetArrayItem` _symbolindices) (`local.LastValue`))))

(fn `UserConstructionScript`
  (`parent.UserConstructionScript`))