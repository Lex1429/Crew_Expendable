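; BP_AutoDoorLrg is a large automatic sliding door triggered when something begins overlapping its Box.
; The overlap calls a server-named open event, which forwards to a local event that toggles IsDoorOpen and plays or reverses the SlideDoor timeline.
; The timeline lerps the Door's relative location along X without sweeping.
; Each new overlap toggles the door, as there is no end-overlap handling or actor filter.
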(event `Server_OpenDoor`
  (`self.Local_OpenDoor`))

(event `Local_OpenDoor`
  (if (not (`self.IsDoorOpen?`))
    (set `self.IsDoorOpen?` true)
    (bind (_direction _slidetrack) (`Timeline|SlideDoor` :!label _label)
      (:`Update`
        (`SceneComponent.K2_SetRelativeLocation` (`self.Door`) (`KismetMathLibrary.VLerp` (90.0 0.0 0.0) (240.0 0.0 0.0) _slidetrack) false true)))
    (else
      (set `self.IsDoorOpen?` false)
      (goto _label :!via `Reverse`))))

(event `self.Box.OnComponentBeginOverlap`
  (params (OverlappedComponent :type "PrimitiveComponent Object Reference") (OtherActor :type "Actor Object Reference") (OtherComp :type "PrimitiveComponent Object Reference") (OtherBodyIndex :type Integer) (bFromSweep :type Boolean) (SweepResult :type "HitResult Structure (by ref)"))
  (`self.Server_OpenDoor`))

(fn `UserConstructionScript`)