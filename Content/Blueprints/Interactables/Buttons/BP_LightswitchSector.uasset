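; Interactable sector light switch that toggles every BP_LightSource sharing its RoomTag and can be destroyed by damage.
; Interact routes through a server event to the toggle, which flips each light by its own state, swaps the case material and drives the lever timeline.
; When HP runs out it spawns an electric effect and stops working.
; It also feeds a player UI prompt when viewed and briefly outlines when in range.
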(event `Local_Lightswitch`
  (if (not (`self.Broken?`))
    (bind _outactors (`GameplayStatics.GetAllActorsOfClass` "/Game/Blueprints/Interactables/CealingLights/BP_LightSource.BP_LightSource_C"))
    (for _array_element _outactors
      (if (== (`/Game/Blueprints/Interactables/CealingLights/BP_LightSource.RoomTag` _array_element) (`self.RoomTag`))
        (if (`/Game/Blueprints/Interactables/CealingLights/BP_LightSource.IsLightOn?` _array_element)
          (`/Game/Blueprints/Interactables/CealingLights/BP_LightSource.Server_LightOff` _array_element)
          (`PrimitiveComponent.SetMaterial` (`self.SwitchCase`) 0 "/Game/Synty/PolygonSciFiHorror/Materials/Alts/SkinAlts/MI_PolygonSciFiHorror_01_A.MI_PolygonSciFiHorror_01_A")
          (`self.LightSwitchToggle` false)
          (bind (_direction _newtrack_0) (`Timeline|Switch` :!via `Reverse` :!label _label)
            (:`Update`
              (`SceneComponent.K2_SetRelativeLocation` (`self.SM_Prop_Lever_02_Handle`) (`KismetMathLibrary.VLerp` (-7.0 20.0 15.0) (-7.0 20.0 -23.0) _newtrack_0) false false)))
          (else
            (`/Game/Blueprints/Interactables/CealingLights/BP_LightSource.Server_LightOn` _array_element)
            (`PrimitiveComponent.SetMaterial` (`self.SwitchCase`) 0 "/Game/Synty/PolygonSciFiHorror/Materials/Alts/Blinking/MI_SciFiHorror_04_B_Blinking.MI_SciFiHorror_04_B_Blinking")
            (`self.LightSwitchToggle` true)
            (goto _label)))))))

(event `Server_LightSwitch`
  (`self.Local_Lightswitch`))

(event `self.Interact`
  (params (Character :type "/Game/Blueprints/Characters/BP_BaseCharacter Object Reference") (PlayerCharacter :type "/Game/Blueprints/Characters/BP_PlayerCharacterCore Object Reference"))
  (`self.Server_LightSwitch`))

(event `self.ReceiveAnyDamage`
  (params (Damage :type "Float (single-precision)") (DamageType :type "DamageType Object Reference") (InstigatedBy :type "Controller Object Reference") (DamageCauser :type "Actor Object Reference"))
  (bind _output_get (set `self.HP` (- (`self.HP`) Damage)))
  (if (<= _output_get 0.0)
    (`NiagaraFunctionLibrary.SpawnSystemAtLocation` "/Game/AllShadesofVFXBundle/EnvironmentVFX/VFX/Electricity/Systems/N_ElectricLoop.N_ElectricLoop" (`SceneComponent.K2_GetComponentLocation` (`self.SwitchCase`)) (struct) (1.0 1.0 1.0) false)
    (set `self.Broken?` true)))

(event `self.ReceiveBeginPlay`
  (`KismetSystemLibrary.Delay` 2.0)
  (bind _foundwidgets (`WidgetBlueprintLibrary.GetAllWidgetsOfClass` "/Game/UI/WB_PlayerUI.WB_PlayerUI_C"))
  (set `self.PlayerUIRef` (`|GetArrayItem` _foundwidgets)))

(event `self.Viewing`
  (params (State :type Boolean))
  (bind _playeruiref (`self.PlayerUIRef`))
  (if State
    (message `/Game/Blueprints/Interfaces/BPI_CombatUI.InteractElement` _playeruiref "Light Switch" "0" "Toggle" true "See the light, or embrace the dark.")
    (else
      (message `/Game/Blueprints/Interfaces/BPI_CombatUI.InteractElement` _playeruiref "" "" "" false ""))))

(event `self.InRange`
  (params (State :type Boolean))
  (bind _switchcase (`self.SwitchCase`))
  (if State
    (`MeshComponent.SetOverlayMaterial` _switchcase "/Game/Materials/M_Outline.M_Outline")
    (`KismetSystemLibrary.Delay` 1.5)
    (`MeshComponent.SetOverlayMaterial` _switchcase null)))

(fn `GetCanBePickedUp`
  (returns (CanBePickedUp :type Boolean))
  (return false))

(fn `GetItemToSpawn`
  (returns (Item :type "/Game/Blueprints/Interactables/Weapons/BP_WeaponComponentMaster Class Reference"))
  (return null))

(fn `UserConstructionScript`)