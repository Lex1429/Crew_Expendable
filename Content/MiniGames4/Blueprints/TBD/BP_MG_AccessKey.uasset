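; Access-key minigame in which the player matches a Lissajous figure to a moving target figure on a screen.
; Action cycles the curve type while axis input adjusts phase and scale; the target rotates, rescales at intervals and periodically switches shape.
; CalculatePoints packs two curve points per Material Parameter Collection vector for the screen material to display.
; Matching shape, phase and scale within tolerance triggers success and returns the camera to the player.
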(event `self.ReceiveBeginPlay`
  ;[1 1 1] Begin play
  (`parent.ReceiveBeginPlay`)
  (bind _returnvalue (`KismetMaterialLibrary.CreateDynamicMaterialInstance` "/Game/MiniGames4/Materials/MI_MG_AccessKey_Inst.MI_MG_AccessKey_Inst"))
  (set `self.DMI` _returnvalue))

(event `InitGame`
  (bind _returnvalue (- (`KismetArrayLibrary.Array_Length` (`self.Config`)) 1))
  ;[1 1 1] Init game
  (`MaterialInstanceDynamic.SetScalarParameterValue` (`self.DMI`) "ShowEnabled" 0.0)
  (set `self.SolverIndex` (`KismetMathLibrary.RandomIntegerInRange` 0 _returnvalue))
  (set `self.CurrIndex` (`KismetMathLibrary.RandomIntegerInRange` 0 _returnvalue))
  (set `self.SolverDelta` (`KismetMathLibrary.RandomFloatInRange` (* (`KismetMathLibrary.GetPI`) -1.0) (`KismetMathLibrary.GetPI`)))
  (bind _output_get (set `self.SolverTargetScale` (`KismetMathLibrary.RandomFloatInRange` 0.5 1.0)))
  (set `self.SolverCurrentScale` _output_get)
  (set `self.StartScaleTime` (`KismetSystemLibrary.GetGameTimeInSeconds`))
  (set `self.ScaleCounter` 0)
  (set `self.SignFactor` (`KismetMathLibrary.RandomBool`)))

(event `self.InteractionBoundBox.OnComponentBeginOverlap`
  (params (OverlappedComponent :type "PrimitiveComponent Object Reference") (OtherActor :type "Actor Object Reference") (OtherComp :type "PrimitiveComponent Object Reference") (OtherBodyIndex :type Integer) (bFromSweep :type Boolean) (SweepResult :type "HitResult Structure (by ref)"))
  ;[1 1 1] Overlapping events
  (`self.CheckBeginOverlap` OtherActor))

(event `CheckControls`
  (bind _rightaxis (`self.RightAxis`))
  (bind _forwardaxis (`self.ForwardAxis`))
  ;[1 1 1] Controls
  (if (`self.IsMiniGameActivated`)
    (if (!= _rightaxis 0.0)
      (bind _result (`self.ClampDelta` (+ (`self.DeltaS`) (`KismetMathLibrary.SelectFloat` 0.02 -0.02 (> _rightaxis 0.0)))))
      (set `self.DeltaS` _result))
    (if (!= _forwardaxis 0.0)
      (set `self.Scale` (`KismetMathLibrary.FClamp` (+ (`self.Scale`) (`KismetMathLibrary.SelectFloat` 0.01 -0.01 (> _forwardaxis 0.0))) 0.5)))))

(event `self.InteractionBoundBox.OnComponentEndOverlap`
  (params (OverlappedComponent :type "PrimitiveComponent Object Reference") (OtherActor :type "Actor Object Reference") (OtherComp :type "PrimitiveComponent Object Reference") (OtherBodyIndex :type Integer))
  ;[1 1 1] Overlapping events
  (`self.CheckEndOverlap` OtherActor))

(event `self.ReceiveTick`
  (params (DeltaSeconds :type "Float (single-precision)"))
  ;[1 0 0] Tick
  (bind _output_get (set `self.DeltaTime` DeltaSeconds))
  (`parent.ReceiveTick` _output_get)
  (if (`self.IsMiniGameActivated`)
    ;[1 1 1] Sample figure
    (`self.CalculatePoints` 1 (`self.DeltaS`) (`self.Scale`) (`self.CurrIndex`))
    ;[1 1 1] Solver figure
    (`self.CalculatePoints` 25 (`self.SolverDelta`) (`self.SolverCurrentScale`) (`self.SolverIndex`))
    (`self.CheckControls`)
    (bind _result (`self.ClampDelta` (+ (`self.SolverDelta`) (* (/ (`self.SolverRotationSpeed`) 1000.0) (`KismetMathLibrary.SelectFloat` 1.0 -1.0 (`self.SignFactor`))))))
    (set `self.SolverDelta` _result)
    (set `self.SolverCurrentScale` (`KismetMathLibrary.FInterpTo` (`self.SolverCurrentScale`) (`self.SolverTargetScale`) (`self.DeltaTime`) 2.0))
    (if (and (== (`self.CurrIndex`) (`self.SolverIndex`)) (`KismetMathLibrary.NearlyEqual_FloatFloat` (`self.SolverCurrentScale`) (`self.Scale`) 0.08) (`KismetMathLibrary.NearlyEqual_FloatFloat` (`self.DeltaS`) (`self.SolverDelta`) 0.05))
      ;[1 1 1] Success
      (set `self.MiniGameEnabled` false)
      (set `self.IsMiniGameActivated` false)
      (set `self.InputEnable` false)
      (`MaterialInstanceDynamic.SetScalarParameterValue` (`self.DMI`) "ShowEnabled" 1.0)
      (`KismetSystemLibrary.Delay` (`self.DelayTimeWhenComplete`))
      (`self.SetOfflineMaterial`)
      (`self.OnMiniGameSuccess`)
      (`self.BlendCameraFromGameToPlayer` (`self.OverlappedActor`))
      (else
        ;[1 1 1] Get new sample figure
        (if (>= (- (`KismetSystemLibrary.GetGameTimeInSeconds`) (`self.StartScaleTime`)) (`self.ScaleIntervalTime`))
          (set `self.StartScaleTime` (`KismetSystemLibrary.GetGameTimeInSeconds`))
          (set `self.SolverTargetScale` (`KismetMathLibrary.RandomFloatInRange` 0.5 1.0))
          (bind _result_2 (`/Engine/EditorBlueprintResources/StandardMacros.IncrementInt` (`self.ScaleCounter`))
            (:`  `
              (if (>= _result_2 (`self.SwitchFigureSteps`))
                (set `self.SolverIndex` (`KismetMathLibrary.RandomIntegerInRange` 0 (- (`KismetArrayLibrary.Array_Length` (`self.Config`)) 1)))
                (set `self.ScaleCounter` 0)
                (set `self.SignFactor` (`KismetMathLibrary.RandomBool`))))))))))

(event `self.ForceExit`
  ;[1 1 1] Cancel
  (if (and (`self.MiniGameEnabled`) (`self.IsMiniGameActivated`))
    (set `self.IsMiniGameActivated` false)
    (set `self.InputEnable` false)
    (`self.OnMiniGameCanceled`)
    (`self.BlendCameraFromGameToPlayer` (`self.OverlappedActor`))))

(event `self.ForceAction`
  (params (Player :type "/Game/Blueprints/Characters/BP_PlayerCharacterCore Object Reference"))
  (bind _returnvalue (+ (`self.CurrIndex`) 1))
  ;[1 1 1] Action
  (if (`self.PlayerOverlapped`)
    (if (`self.IsMiniGameActivated`)
      (set `self.CurrIndex` (`KismetMathLibrary.SelectInt` 0 _returnvalue (>= _returnvalue (`KismetArrayLibrary.Array_Length` (`self.Config`)))))
      (else
        (`self.InitGame`)
        (`PrimitiveComponent.SetMaterial` (`self.MiniGameScreen`) 0 (`self.DMI`))
        (`self.BlendCameraFromPlayerToGame` self (`self.OverlappedActor`))
        (set `self.IsMiniGameActivated` true)
        (set `self.InputEnable` true)))))

(fn `CalculatePoints`
  (params (MPCIndex :type Integer) (Delta :type "Float (double-precision)") (Scale :type "Float (double-precision)") (ConfigIndex :type Integer))
  (locals (Rvalue :type "Float (double-precision)") (Gvalue :type "Float (double-precision)") (MPC_Index :type Integer) (S :type "Float (double-precision)") (S2 :type "Float (double-precision)") (Scale_Local :type "Float (double-precision)") (Config_index :type Integer))
  (bind _scale_local (`local.Scale_Local`))
  (bind (_output_param1 _output_param2) (break `/Game/MiniGames4/Blueprints/Data/F_MG_AccessKeyData` (`|GetArrayItem` (`self.Config`) (`local.Config_index`))))
  (bind _returnvalue (* (`KismetMathLibrary.Cos` (`local.S`)) _scale_local))
  (bind _returnvalue_2 (* (`KismetMathLibrary.Sin` (`local.S2`)) _scale_local))
  ;[1 1 1] Calculating Lissajous curve points and pass data into a material
  (set `local.MPC_Index` MPCIndex)
  (set `local.S` Delta)
  (set `local.Scale_Local` Scale)
  (set `local.Config_index` ConfigIndex)
  (set `local.S2` 0.0)
  (for _index (range 48)
    (if (== (mod (+ _index 1) 2) 0)
      (`KismetMaterialLibrary.SetVectorParameterValue` "/Game/MiniGames4/Materials/MPC_MG_AccessKey.MPC_MG_AccessKey" (`KismetStringLibrary.Conv_StringToName` (`KismetStringLibrary.Concat_StrStr` "Vector" (`KismetStringLibrary.Conv_IntToString` (`local.MPC_Index`)))) (make `LinearColor` (`local.Rvalue`) (`local.Gvalue`) _returnvalue _returnvalue_2))
      (`/Engine/EditorBlueprintResources/StandardMacros.IncrementInt` (`local.MPC_Index`)
        (:`  `
          _))
      (else
        (set `local.Rvalue` _returnvalue)
        (set `local.Gvalue` _returnvalue_2)))
    (set `local.S` (+ (`local.S`) (* (/ (`KismetMathLibrary.GetPI`) 24.0) _output_param1)))
    (set `local.S2` (+ (`local.S2`) (* (/ (`KismetMathLibrary.GetPI`) 24.0) _output_param2)))))

(fn `ClampDelta`
  (params (Value :type "Float (double-precision)"))
  (returns (Result :type "Float (double-precision)"))
  (bind _returnvalue (* (`KismetMathLibrary.GetPI`) 2.0))
  ;[1 1 1] Clamp value 0 to 2*PI
  (return (`KismetMathLibrary.SelectFloat` (- Value _returnvalue) (`KismetMathLibrary.SelectFloat` (+ Value _returnvalue) Value (< Value 0.0)) (> Value _returnvalue))))

(fn `UserConstructionScript`
  (`parent.UserConstructionScript`))