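; Modular cold storage pod building piece whose exterior or interior material follows the state of a linked light switch.
; The construction script passes RoomTag to the child overhead lamp, applies the building material, and shows or hides an optional emergency door, also moving its panel.
; At BeginPlay it binds to the light switch's toggle event, then swaps the pod's material to an on or off variant chosen by RoomTag for Sector 3 Cultures or Sector 5 Cold Storage.
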(event `self.ReceiveBeginPlay`
  (bind _lightswitchref (`self.LightSwitchRef`))
  (`/Engine/EditorBlueprintResources/StandardMacros.IsValid` _lightswitchref
    (:`Is Valid`
      (add `/Game/Blueprints/Interactables/Buttons/BP_Lightswitch.LightSwitchToggle` _lightswitchref (`|CreateDelegate` :!event `LightSwitchToggle`)))))

(event `LightSwitchToggle`
  (params (`IsOn?` :type Boolean))
  (bind _sm_bld_pod_hab_small_04 (`self.SM_Bld_Pod_Hab_Small_04`))
  (if `IsOn?`
    (`|SwitchGameplayTagContainer` (`self.RoomTag`)
      (:`(GameplayTags=((TagName="Sector3.Cultures")))`
        (`PrimitiveComponent.SetMaterial` _sm_bld_pod_hab_small_04 0 "/Game/Materials/CustomTextures/V1Materials/M_Sector3_On.M_Sector3_On"))
      (:`(GameplayTags=((TagName="Sector5.ColdStorage")))`
        (`PrimitiveComponent.SetMaterial` _sm_bld_pod_hab_small_04 0 "/Game/Materials/CustomTextures/V1Materials/M_Sector5_On.M_Sector5_On")))
    (else
      (`|SwitchGameplayTagContainer` (`self.RoomTag`)
        (:`(GameplayTags=((TagName="Sector3.Cultures")))`
          (`PrimitiveComponent.SetMaterial` _sm_bld_pod_hab_small_04 0 "/Game/Materials/CustomTextures/V1Materials/M_Sector3_Off.M_Sector3_Off"))
        (:`(GameplayTags=((TagName="Sector5.ColdStorage")))`
          (`PrimitiveComponent.SetMaterial` _sm_bld_pod_hab_small_04 0 "/Game/Materials/CustomTextures/V1Materials/M_Sector5_Off.M_Sector5_Off"))))))

(fn `UserConstructionScript`
  (bind _asbp_lamp_base (cast `/Game/Blueprints/Interactables/CealingLights/BP_LampBase` (`ChildActorComponent.ChildActor` (`self.OverheadLight1`))))
  (set `/Game/Blueprints/Interactables/CealingLights/BP_LampBase.RoomTag` (`self.RoomTag`) _asbp_lamp_base)
  (`PrimitiveComponent.SetMaterial` (`self.SM_Bld_Pod_Hab_Small_04`) 0 (`self.BuildingMaterial`))
  (if (`self.EmergencyDoor?`)
    (`SceneComponent.SetVisibility` (`self.SM_Bld_Door_Single_01`) true false)
    (`SceneComponent.SetVisibility` (`self.SM_Bld_Door_Single_01_Door_01`) true false)
    (`SceneComponent.K2_SetRelativeLocation` (`self.SM_Bld_Door_Single_01_Door_01`) (-70.0 0.0 0.0) false false)
    (else
      (`SceneComponent.SetVisibility` (`self.SM_Bld_Door_Single_01`) false false)
      (`SceneComponent.SetVisibility` (`self.SM_Bld_Door_Single_01_Door_01`) false false)
      (`SceneComponent.K2_SetRelativeLocation` (`self.SM_Bld_Door_Single_01_Door_01`) (-70.0 0.0 400.0) false false))))