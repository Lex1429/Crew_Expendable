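; Salvage drop-off bin that converts the interacting character's held weapon into salvage value.
; Interact looks up the item name in DT_SalvageList and, if found, adds its value to the GameState's SalvageAmountMessage.
; It then swaps the weapon for a scaled-down, gravity-free pickup at the spawn point, destroyed after an electric-explosion effect and short delay.
; Box overlap toggles the bin's outline and an interact-ring widget.
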(event `self.Interact`
  (params (Character :type "/Game/Blueprints/Characters/BP_BaseCharacter Object Reference"))
  (bind _returnvalue (`GameplayStatics.GetGameState`))
  (bind _currentweapon (`/Game/Blueprints/Characters/BP_BaseCharacter.GetCurrentWeapon` Character))
  (`/Engine/EditorBlueprintResources/StandardMacros.IsValid` _currentweapon
    (:`Is Valid`
      (bind _output_get (set `self.DroppedItem` (`/Game/Blueprints/Interactables/Weapons/BP_WeaponComponentMaster.ItemName` _currentweapon)))
      (bind _returnvalue_2 (`|GetDataTableRow` "/Game/Blueprints/Salvage/DT_SalvageList.DT_SalvageList" _output_get)
        (:`then`
          (bind _salvage (message `/Game/Blueprints/Interfaces/BPI_Stats.GetSalvageAmount` _returnvalue))
          (message `/Game/Blueprints/Interfaces/BPI_Stats.SetSalvageAmount` _returnvalue (+ _salvage (`.Value_15_F222FCC64FCAB1A8F20AACB203483459` (break `/Game/Blueprints/Salvage/S_Salvage` _returnvalue_2))))
          (`self.Local_DropOff` Character))))))

(event `Local_DropOff`
  (params (Character :type "/Game/Blueprints/Characters/BP_BaseCharacter Object Reference"))
  (bind _itemspawnpoint (`self.ItemSpawnPoint`))
  (bind _returnvalue (`|SpawnActorFromClass` (`/Game/Blueprints/Interactables/Weapons/BP_WeaponComponentMaster.PickupClass` (`/Game/Blueprints/Characters/BP_BaseCharacter.GetCurrentWeapon` Character)) (`KismetMathLibrary.MakeTransform` (`SceneComponent.K2_GetComponentLocation` (`self.ItemSpawnPoint`)) (struct) (0.5 0.5 0.5)) "Undefined" "MultiplyWithRoot" null null))
  (`/Game/Blueprints/Characters/BP_BaseCharacter.DestroyCurrentItem` Character)
  (`PrimitiveComponent.SetEnableGravity` (`/Game/Blueprints/Interactables/Pickups/BP_PickupMaster.PickupObject` _returnvalue) false)
  (`NiagaraFunctionLibrary.SpawnSystemAttached` "/Game/AllShadesofVFXBundle/EnvironmentVFX/VFX/Electricity/Systems/N_ElectricExplosion2.N_ElectricExplosion2" _itemspawnpoint "None" (`SceneComponent.RelativeLocation` _itemspawnpoint) (`SceneComponent.RelativeRotation` _itemspawnpoint) "SnapToTarget" true)
  (`KismetSystemLibrary.Delay` 1.0)
  (`self.K2_DestroyActor` _returnvalue))

(event `self.Box.OnComponentBeginOverlap`
  (params (OverlappedComponent :type "PrimitiveComponent Object Reference") (OtherActor :type "Actor Object Reference") (OtherComp :type "PrimitiveComponent Object Reference") (OtherBodyIndex :type Integer) (bFromSweep :type Boolean) (SweepResult :type "HitResult Structure (by ref)"))
  (bind _widget (`self.Widget`))
  (`MeshComponent.SetOverlayMaterial` (`self.SM_Prop_TrashBin_01`) "/Game/Materials/M_Outline.M_Outline")
  (bind _returnvalue (`|CreateWidget` "/Game/UI/WB_InteractRing.WB_InteractRing_C" null "Salvager" "" "Toggle"))
  (`WidgetComponent.SetWidget` _widget _returnvalue)
  (`SceneComponent.SetVisibility` _widget true false))

(event `self.Box.OnComponentEndOverlap`
  (params (OverlappedComponent :type "PrimitiveComponent Object Reference") (OtherActor :type "Actor Object Reference") (OtherComp :type "PrimitiveComponent Object Reference") (OtherBodyIndex :type Integer))
  (`MeshComponent.SetOverlayMaterial` (`self.SM_Prop_TrashBin_01`) null)
  (`SceneComponent.SetVisibility` (`self.Widget`) false false)
  (`Widget.RemoveFromParent` (stale `self.Box.OnComponentBeginOverlap` _returnvalue)))

(fn `UserConstructionScript`)