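; Base interactable door that toggles open and closed and plays a sound at the door unless it is locked.
; Flags pick one of three Timelines: vertical slide, rotating swing or small-door swing, each lerping the Door component between closed and open transforms and reversing to close.
; Server-named events forward to Local events for opening and for toggling the lock.
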(event `Server_OpenDoor`
  (`self.Local_OpenDoor`))

(event `Local_OpenDoor`
  (if (not (`self.IsDoorLocked?`))
    (`GameplayStatics.PlaySoundAtLocation` null (`SceneComponent.K2_GetComponentLocation` (`self.Door`)) (struct) 1.0 1.0 0.0 null null null null)
    (if (not (`self.IsRotatingDoor?`))
      (if (not (`self.IsDoorOpen?`))
        (set `self.IsDoorOpen?` true)
        (bind (_direction _newtrack_0) (`Timeline|DoorMovementVert` :!label _label)
          (:`Update`
            (`SceneComponent.K2_SetRelativeLocation` (`self.Door`) (`KismetMathLibrary.VLerp` (`self.VertClosedPosition`) (`self.VertOpenPosition`) _newtrack_0) false true)))
        (else
          (set `self.IsDoorOpen?` false)
          (goto _label :!via `Reverse`)))
      (elif (not (`self.SmallDoor?`))
        (if (not (`self.IsDoorOpen?`))
          (set `self.IsDoorOpen?` true)
          (bind (_direction_2 _newtrack_0_2) (`Timeline|RotatingDoor` :!label _label_2)
            (:`Update`
              (`SceneComponent.K2_SetRelativeRotation` (`self.Door`) (`KismetMathLibrary.RLerp` (`self.RotatingClosedPos`) (`self.RotatingOpenPos`) _newtrack_0_2) false true)))
          (else
            (set `self.IsDoorOpen?` false)
            (goto _label_2 :!via `Reverse`)))
        (elif (not (`self.IsDoorOpen?`))
          (set `self.IsDoorOpen?` true)
          (bind (_direction_3 _newtrack_0_3) (`Timeline|SmallDoor` :!label _label_3)
            (:`Update`
              (`SceneComponent.K2_SetRelativeRotation` (`self.Door`) (`KismetMathLibrary.RLerp` (`self.RotatingClosedPos`) (`self.RotatingOpenPos`) _newtrack_0_3) false true)))
          (else
            (set `self.IsDoorOpen?` false)
            (goto _label_3 :!via `Reverse`)))))))

(event `Server_LockStatus`
  (`self.Local_LockStatus`))

(event `Local_LockStatus`
  (if (not (`self.IsDoorLocked?`))
    (set `self.IsDoorLocked?` true)
    (else
      (set `self.IsDoorLocked?` false))))

(fn `UserConstructionScript`)