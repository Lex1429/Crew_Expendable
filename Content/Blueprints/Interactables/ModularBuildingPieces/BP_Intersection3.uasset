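; Modular hallway intersection piece with three optional end caps with windows, an optional corridor connector, and an overhead lamp.
; The construction script applies the building material, passes RoomTag to the child lamp, and toggles each optional part's visibility, moving disabled caps and connector upward.
; At BeginPlay it binds to the referenced light switch, whose toggle swaps the hub mesh to the on or off material of its Hallways sector, chosen by RoomTag.
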(event `self.ReceiveBeginPlay`
  (bind _lightswitchref (`self.LightSwitchRef`))
  (`/Engine/EditorBlueprintResources/StandardMacros.IsValid` _lightswitchref
    (:`Is Valid`
      (add `/Game/Blueprints/Interactables/Buttons/BP_Lightswitch.LightSwitchToggle` _lightswitchref (`|CreateDelegate` :!event `LightSwitchToggle`)))))

(event `LightSwitchToggle`
  (params (`IsOn?` :type Boolean))
  (bind _sm_bld_pod_hub_02 (`self.SM_Bld_Pod_Hub_02`))
  (bind _sm_bld_pod_hub_02_2 (`self.SM_Bld_Pod_Hub_02`))
  (if `IsOn?`
    (`|SwitchGameplayTagContainer` (`self.RoomTag`)
      (:`(GameplayTags=((TagName="Sector1.Hallways")))`
        (`PrimitiveComponent.SetMaterial` _sm_bld_pod_hub_02_2 0 "/Game/Materials/CustomTextures/V1Materials/M_Sector1_On.M_Sector1_On"))
      (:`(GameplayTags=((TagName="Sector2.Hallways")))`
        (`PrimitiveComponent.SetMaterial` _sm_bld_pod_hub_02_2 0 "/Game/Materials/CustomTextures/V1Materials/M_Sector2_On.M_Sector2_On"))
      (:`(GameplayTags=((TagName="Sector3.Hallways")))`
        (`PrimitiveComponent.SetMaterial` _sm_bld_pod_hub_02_2 0 "/Game/Materials/CustomTextures/V1Materials/M_Sector3_On.M_Sector3_On"))
      (:`(GameplayTags=((TagName="Sector4.Hallways")))`
        (`PrimitiveComponent.SetMaterial` _sm_bld_pod_hub_02_2 0 "/Game/Materials/CustomTextures/V1Materials/M_Sector4_On.M_Sector4_On"))
      (:`(GameplayTags=((TagName="Sector5.Hallways")))`
        (`PrimitiveComponent.SetMaterial` _sm_bld_pod_hub_02_2 0 "/Game/Materials/CustomTextures/V1Materials/M_Sector5_On.M_Sector5_On")))
    (else
      (`|SwitchGameplayTagContainer` (`self.RoomTag`)
        (:`(GameplayTags=((TagName="Sector1.Hallways")))`
          (`PrimitiveComponent.SetMaterial` _sm_bld_pod_hub_02 0 "/Game/Materials/CustomTextures/V1Materials/M_Sector1_Off.M_Sector1_Off"))
        (:`(GameplayTags=((TagName="Sector2.Hallways")))`
          (`PrimitiveComponent.SetMaterial` _sm_bld_pod_hub_02 0 "/Game/Materials/CustomTextures/V1Materials/M_Sector2_Off.M_Sector2_Off"))
        (:`(GameplayTags=((TagName="Sector3.Hallways")))`
          (`PrimitiveComponent.SetMaterial` _sm_bld_pod_hub_02 0 "/Game/Materials/CustomTextures/V1Materials/M_Sector3_Off.M_Sector3_Off"))
        (:`(GameplayTags=((TagName="Sector4.Hallways")))`
          (`PrimitiveComponent.SetMaterial` _sm_bld_pod_hub_02 0 "/Game/Materials/CustomTextures/V1Materials/M_Sector4_Off.M_Sector4_Off"))
        (:`(GameplayTags=((TagName="Sector5.Hallways")))`
          (`PrimitiveComponent.SetMaterial` _sm_bld_pod_hub_02 0 "/Game/Materials/CustomTextures/V1Materials/M_Sector5_Off.M_Sector5_Off"))))))

(fn `UserConstructionScript`
  (bind _endcap1 (`self.EndCap1`))
  (bind _sm_bld_pod_corridor_switch_connector_01 (`self.SM_Bld_Pod_Corridor_Switch_Connector_01`))
  (bind _sm_bld_pod_corridor_switch_connector_01_2 (`self.SM_Bld_Pod_Corridor_Switch_Connector_01`))
  (bind _endcap1_2 (`self.EndCap1`))
  (`PrimitiveComponent.SetMaterial` (`self.SM_Bld_Pod_Hub_02`) 0 (`self.BuildingMaterial`))
  (`PrimitiveComponent.SetMaterial` (`self.EndCap1`) 0 (`self.BuildingMaterial`))
  (`PrimitiveComponent.SetMaterial` (`self.EndCap2`) 0 (`self.BuildingMaterial`))
  (`PrimitiveComponent.SetMaterial` (`self.EndCap3`) 0 (`self.BuildingMaterial`))
  (bind _asbp_lamp_base (cast `/Game/Blueprints/Interactables/CealingLights/BP_LampBase` (`ChildActorComponent.ChildActor` (`self.OverheadLight1`))))
  (set `/Game/Blueprints/Interactables/CealingLights/BP_LampBase.RoomTag` (`self.RoomTag`) _asbp_lamp_base)
  (`|ExecutionSequence`
    (:`then_0`
      (if (`self.Endcap1On?`)
        (`SceneComponent.SetVisibility` _endcap1 true false)
        (`SceneComponent.SetVisibility` (`self.Window1`) true false)
        (`SceneComponent.K2_SetRelativeLocation` _endcap1 (0.0 470.0 0.0) false false)
        (else
          (`SceneComponent.SetVisibility` _endcap1_2 false false)
          (`SceneComponent.SetVisibility` (`self.Window1`) false false)
          (`SceneComponent.K2_SetRelativeLocation` _endcap1_2 (0.0 470.0 400.0) false false))))
    (:`then_1`
      (if (`self.Endcap2On?`)
        (`SceneComponent.SetVisibility` (`self.Window2`) true false)
        (`SceneComponent.SetVisibility` (`self.EndCap2`) true false)
        (`SceneComponent.K2_SetRelativeLocation` (`self.EndCap2`) (0.0 -470.0 0.0) false false)
        (else
          (`SceneComponent.SetVisibility` (`self.Window2`) false false)
          (`SceneComponent.SetVisibility` (`self.EndCap2`) false false)
          (`SceneComponent.K2_SetRelativeLocation` (`self.EndCap2`) (0.0 -470.0 400.0) false false))))
    (:`then_2`
      (if (`self.Endcap3On?`)
        (`SceneComponent.SetVisibility` (`self.Window3`) true false)
        (`SceneComponent.SetVisibility` (`self.EndCap3`) true false)
        (`SceneComponent.K2_SetRelativeLocation` (`self.EndCap3`) (-470.0 0.0 0.0) false false)
        (else
          (`SceneComponent.SetVisibility` (`self.Window3`) false false)
          (`SceneComponent.SetVisibility` (`self.EndCap3`) false false)
          (`SceneComponent.K2_SetRelativeLocation` (`self.EndCap3`) (-470.0 0.0 400.0) false false))))
    (:`then_3`
      (if (`self.ConnectorOn?`)
        (`SceneComponent.SetVisibility` _sm_bld_pod_corridor_switch_connector_01 true false)
        (`SceneComponent.K2_SetRelativeLocation` _sm_bld_pod_corridor_switch_connector_01 (570.0 0.0 0.0) false false)
        (else
          (`SceneComponent.SetVisibility` _sm_bld_pod_corridor_switch_connector_01_2 false false)
          (`SceneComponent.K2_SetRelativeLocation` _sm_bld_pod_corridor_switch_connector_01_2 (570.0 0.0 400.0) false false))))))