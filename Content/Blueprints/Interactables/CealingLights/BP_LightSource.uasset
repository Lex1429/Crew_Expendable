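; Switchable ceiling light actor with a point light and a fixture mesh, placed with configurable color, material and starting on/off state.
; The construction script applies those settings, and BeginPlay reapplies intensity plus an optional flicker light function.
; Server on/off events call local ones that set intensity and mesh emissive.
; Switching on always flickers briefly, then clears the light function after a delay.
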(event `self.ReceiveBeginPlay`
  (if (`self.LightFlicker?`)
    (`LightComponent.SetLightFunctionMaterial` (`self.PointLight`) "/Game/Materials/M_LightFlicker.M_LightFlicker"))
  (if (`self.IsLightOn?`)
    (`LightComponent.SetIntensity` (`self.PointLight`) (`self.LightIntensityOn`))
    (set `self.IsLightOn?` true)
    (else
      (`LightComponent.SetIntensity` (`self.PointLight`) (`self.LightIntensityOff`))
      (set `self.IsLightOn?` false))))

(event `Local_LightOn`
  (`LightComponent.SetIntensity` (`self.PointLight`) (`self.LightIntensityOn`))
  (set `self.IsLightOn?` true)
  (`MeshComponent.SetScalarParameterValueOnMaterials` (`self.SM_Bld_Light_06`) "Emissive_Color" 10.0)
  (`LightComponent.SetLightFunctionMaterial` (`self.PointLight`) "/Game/Materials/M_LightFlicker.M_LightFlicker")
  (`KismetSystemLibrary.Delay` 1.5)
  (`LightComponent.SetLightFunctionMaterial` (`self.PointLight`) null))

(event `Local_LightOff`
  (`LightComponent.SetIntensity` (`self.PointLight`) (`self.LightIntensityOff`))
  (set `self.IsLightOn?` false)
  (`MeshComponent.SetScalarParameterValueOnMaterials` (`self.SM_Bld_Light_06`) "Emissive_Color" 0.0))

(event `Server_LightOn`
  (`self.Local_LightOn`))

(event `Server_LightOff`
  (`self.Local_LightOff`))

(fn `UserConstructionScript`
  (`|ExecutionSequence`
    (:`then_0`
      (if (`self.IsLightOn?`)
        (`LightComponent.SetIntensity` (`self.PointLight`) (`self.LightIntensityOn`))
        (set `self.IsLightOn?` true)
        (else
          (`LightComponent.SetIntensity` (`self.PointLight`) (`self.LightIntensityOff`))
          (set `self.IsLightOn?` false))))
    (:`then_1`
      (`LightComponent.SetLightColor` (`self.PointLight`) (`self.LightColor`) true))
    (:`then_2`
      (`PrimitiveComponent.SetMaterial` (`self.SM_Bld_Light_06`) 0 (`self.Material`)))))