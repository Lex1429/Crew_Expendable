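; BP_MiniFast is an in-world screen timing minigame where the player stops a moving marker on random targets across two to four bars.
; An overlap box plus timed facing check gates interaction, which starts the game or judges a press.
; Tick advances the marker, drawn with bars through dynamic material parameters.
; Hits advance a bar, misses flash and step back one, and clearing all fires success and destroys the screen.
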(event `EnableMiniGame`
  ; Base Code
  ;;[1 1 1] Init
  (`PrimitiveComponent.SetMaterial` (`self.MiniGameScreen`) 0 (`self.DMI_Idle`) :!label _label)
  (set `self.MiniGameEnabled` true))

(event `self.ReceiveBeginPlay`
  ; Base Code
  ;;[1 1 1] Init
  (`|ExecutionSequence`
    (:`then_0`
      (bind _asbp_pc_base (cast `/Game/MBLS/Blueprints/Core/Base/Player/BP_PC_Base` (`GameplayStatics.GetPlayerController` 0)))
      (set `self.BaseControlRef` _asbp_pc_base)
      (bind _returnvalue (`KismetSystemLibrary.K2_SetTimer` null "CheckPlayerDirection" 0.15 true))
      (set `self.CheckPlayerDirectionHandle` _returnvalue)
      (set `self.PlayerOverlapped` false)
      (set `self.PlayerDetected` false)
      (set `self.IsMiniGameActivated` false)
      (set `self.InputEnable` true)
      (set `self.RightAxis` 0.0)
      (set `self.ForwardAxis` 0.0)
      ;;;[1 1 1] Idle material
      (bind _returnvalue_2 (`KismetMaterialLibrary.CreateDynamicMaterialInstance` "/Game/MiniGames2/Materials/MI_MiniGamesIdle_Inst.MI_MiniGamesIdle_Inst"))
      (set `self.DMI_Idle` _returnvalue_2)
      ;;;[1 1 1] Offline material
      (bind _returnvalue_3 (`KismetMaterialLibrary.CreateDynamicMaterialInstance` "/Game/MiniGames2/Materials/MI_MiniGameOffline_Inst.MI_MiniGameOffline_Inst"))
      (set `self.DMI_Offline` _returnvalue_3)
      (if (`self.MiniGameEnabled`)
        (goto _label)
        (else
          (`PrimitiveComponent.SetMaterial` (`self.MiniGameScreen`) 0 (`self.DMI_Offline`) :!label _label_2)
          (set `self.MiniGameEnabled` false))))
    (:`then_1`
      (bind _asbp_gs_base (cast `/Game/MBLS/Blueprints/Core/Base/Core/BP_GS_Base` (`GameplayStatics.GetGameState`)))
      (set `self.As BP GS Base` _asbp_gs_base))
    (:`then_2`
      (set `self.IsMiniGameActivated` false)
      (set `self.InputEnable` false)
      (bind _returnvalue_4 (`KismetMaterialLibrary.CreateDynamicMaterialInstance` "/Game/MiniGames2/Materials/MI_MiniGamesFast_Inst.MI_MiniGamesFast_Inst"))
      (set `self.DMI` _returnvalue_4))))

(event `DisableMiniGame`
  ; Base Code
  ;;[1 1 1] Init
  (goto _label_2))

(event `Server_DisableMiniGame`
  ; Base Code
  (`self.DisableMiniGame`))

(event `InputAxis|MoveForward` :consume false
  (params (AxisValue :type "Float (single-precision)"))
  ; Base Code
  ;;[1 1 1] Controls
  (if (>= (`KismetMathLibrary.Abs` AxisValue) (`self.GamepadSensitivity`))
    (set `self.ForwardAxis` AxisValue)
    (else
      (set `self.ForwardAxis` 0.0))))

(event `CheckBeginOverlap`
  (params (Actor :type "Actor Object Reference"))
  (bind _playerpawn (`self.PlayerPawn`))
  ; Base Code
  ;;[1 1 1] Check overlapped Player
  (if (`KismetSystemLibrary.IsValid` _playerpawn)
    (if (== Actor _playerpawn)
      (set `self.PlayerDetected` true :!label _label_3)
      (set `self.OverlappedActor` Actor))
    (else
      (goto _label_3))))

(event `InputAxis|MoveRight` :consume false
  (params (AxisValue :type "Float (single-precision)"))
  ; Base Code
  ;;[1 1 1] Controls
  (if (>= (`KismetMathLibrary.Abs` AxisValue) (`self.GamepadSensitivity`))
    (set `self.RightAxis` AxisValue)
    (else
      (set `self.RightAxis` 0.0))))

(event `CheckEndOverlap`
  (params (Actor :type "Actor Object Reference"))
  ; Base Code
  ;;[1 1 1] Check overlapped Player
  (if (`self.PlayerDetected`)
    (if (== Actor (`self.OverlappedActor`))
      (set `self.PlayerDetected` false)
      (set `self.PlayerOverlapped` false)
      (set `self.OverlappedActor` null)
      (`MaterialInstanceDynamic.SetScalarParameterValue` (`self.DMI_Idle`) "ShowKey" 0.0))))

(event `/Game/Blueprints/Interfaces/BPI_Interact.Interact`
  (params (Character :type "/Game/Blueprints/Characters/BP_BaseCharacter Object Reference"))
  ; Base Code
  (`self.Server_GameStart`))

(event `Server_GameStart`
  ; Base Code
  (`self.Owning_GameStart`))

(event `Owning_GameStart`
  ; Base Code
  ;;[1 1 1] Action
  (if (`self.MiniGameEnabled`)
    (if (`self.PlayerOverlapped`)
      (bind _isdead (message `/Game/Blueprints/Interfaces/BPI_Stats.GetIsDead` (`GameplayStatics.GetPlayerCharacter` 0)))
      (if (not _isdead)
        (`self.ForceAction`)))))

(event `Server_Cancel`
  ; Base Code
  (`self.Owner_Cancel`))

(event `Owner_Cancel`
  ; Base Code
  ;;[1 1 1] Exit (Cancel) game
  (if (`self.MiniGameEnabled`)
    (if (`self.IsMiniGameActivated`)
      (`PrimitiveComponent.SetMaterial` (`self.MiniGameScreen`) 0 (`self.DMI_Idle`))
      (`self.ForceExit`))))

(event `CheckPlayerDirection`
  (bind _dmi_idle (`self.DMI_Idle`))
  (bind _overlappedactor (`self.OverlappedActor`))
  ; Base Code
  ;;[1 1 1] Check if player oriented to Mini Game screen
  (if (`self.PlayerDetected`)
    (`/Engine/EditorBlueprintResources/StandardMacros.IsValid` _overlappedactor
      (:`Is Valid`
        (if (<= (`KismetMathLibrary.DegAcos` (`KismetMathLibrary.Dot_VectorVector` (`SceneComponent.GetForwardVector` (`self.Arrow`)) (`self.GetActorForwardVector` _overlappedactor))) (`self.DetectionAngle`))
          (set `self.PlayerOverlapped` true)
          (`MaterialInstanceDynamic.SetScalarParameterValue` _dmi_idle "ShowKey" 1.0)
          (else
            (set `self.PlayerOverlapped` false)
            (`MaterialInstanceDynamic.SetScalarParameterValue` _dmi_idle "ShowKey" 0.0)))))))

(event `/Game/Blueprints/Interfaces/BPI_Interact.MiniGameComplete`
  ; Base Code
  (`self.Server_Cancel`))

(event `Success`
  ; Base Code
  ;;[0 0 1] Success Event
  (`ActorComponent.K2_DestroyComponent` (`self.MiniGameScreen`))
  (`KismetSystemLibrary.PrintString` "Success"))

(event `SetOfflineMaterial`
  ; Base Code
  ;;[1 1 1] Set Offline material for the screen
  (`PrimitiveComponent.SetMaterial` (`self.MiniGameScreen`) 0 (`self.DMI_Offline`)))

(event `self.InteractionBoundBox.OnComponentBeginOverlap`
  (params (OverlappedComponent :type "PrimitiveComponent Object Reference") (OtherActor :type "Actor Object Reference") (OtherComp :type "PrimitiveComponent Object Reference") (OtherBodyIndex :type Integer) (bFromSweep :type Boolean) (SweepResult :type "HitResult Structure (by ref)"))
  ; Base Code
  (`self.CheckBeginOverlap` OtherActor))

(event `Server_Success`
  ; Base Code
  (`self.Success`))

(event `self.InteractionBoundBox.OnComponentEndOverlap`
  (params (OverlappedComponent :type "PrimitiveComponent Object Reference") (OtherActor :type "Actor Object Reference") (OtherComp :type "PrimitiveComponent Object Reference") (OtherBodyIndex :type Integer))
  ; Base Code
  (`self.CheckEndOverlap` OtherActor))

(event `Server_ForceAction`
  ; Base Code
  (`self.ForceAction`))

(event `Server_ForceExit`
  ; Base Code
  (`self.ForceExit`))

(event `self.ReceiveTick`
  (params (DeltaSeconds :type "Float (single-precision)"))
  (bind _moverposition (`self.MoverPosition`))
  ; Update Mover
  (if (`self.CanMove`)
    (bind _output_get (set `self.MoverPosition` (`KismetMathLibrary.FClamp` (+ DeltaSeconds (`self.MoverPosition`) (* 0.0 (`self.MoverSpeed`) (`self.MoverDirection`))))))
    (`MaterialInstanceDynamic.SetScalarParameterValue` (`self.DMI`) "Mover_Xpos" _output_get)
    (if (or (<= _moverposition 0.0) (>= _moverposition 1.0))
      (set `self.MoverDirection` (* (`self.MoverDirection`) -1.0)))))

(event `ForceExit`
  ; Cancel Game
  (if (and (`self.MiniGameEnabled`) (`self.IsMiniGameActivated`))
    (set `self.InputEnable` false)
    (set `self.IsMiniGameActivated` false)
    (`self.OnMiniGameCanceled`)
    (`KismetSystemLibrary.PrintString` "Canceled")))

(event `SetupMover`
  (bind _currentbarindex (`self.CurrentBarIndex`))
  (bind _dmi (`self.DMI`))
  ; Set Mover Position Depend On Current Bar Index
  (`MaterialInstanceDynamic.SetScalarParameterValue` (`self.DMI`) "Mover_Xpos" 0.0)
  (switch `/Game/MiniGames2/Blueprints/Data/E_MG_FastCount` (`self.BarsCount`)
    (:`NewEnumerator0`
      (switch `int` _currentbarindex
        (:`0`
          (`MaterialInstanceDynamic.SetScalarParameterValue` _dmi "Mover_Ypos" 0.3)
          (set `self.MoverSpeed` (`self.Bar1_Speed`) :!label _label_4))
        (:`1`
          (`MaterialInstanceDynamic.SetScalarParameterValue` _dmi "Mover_Ypos" 0.2)
          (set `self.MoverSpeed` (`self.Bar2_Speed`) :!label _label_5))))
    (:`NewEnumerator1`
      (switch `int` _currentbarindex
        (:`0`
          (`MaterialInstanceDynamic.SetScalarParameterValue` _dmi "Mover_Ypos" 0.35)
          (goto _label_4))
        (:`1`
          (`MaterialInstanceDynamic.SetScalarParameterValue` _dmi "Mover_Ypos" 0.25)
          (goto _label_5))
        (:`2`
          (`MaterialInstanceDynamic.SetScalarParameterValue` _dmi "Mover_Ypos" 0.15)
          (set `self.MoverSpeed` (`self.Bar3_Speed`) :!label _label_6))))
    (:`NewEnumerator2`
      (switch `int` _currentbarindex
        (:`0`
          (`MaterialInstanceDynamic.SetScalarParameterValue` _dmi "Mover_Ypos" 0.4)
          (goto _label_4))
        (:`1`
          (`MaterialInstanceDynamic.SetScalarParameterValue` _dmi "Mover_Ypos" 0.3)
          (goto _label_5))
        (:`2`
          (`MaterialInstanceDynamic.SetScalarParameterValue` _dmi "Mover_Ypos" 0.2)
          (goto _label_6))
        (:`3`
          (`MaterialInstanceDynamic.SetScalarParameterValue` _dmi "Mover_Ypos" 0.1)
          (set `self.MoverSpeed` (`self.Bar4_Speed`)))))))

(event `SetTarget`
  (params (`Bar Number` :type Integer) (`Use Half` :type Boolean))
  (bind _dmi (`self.DMI`))
  (bind _targetpos (`self.TargetPos`))
  (bind _returnvalue (`KismetStringLibrary.Conv_IntToString` (+ `Bar Number` 1)))
  ; Set Target Based on Target Params
  (bind _output_get (set `self.TargetPos` (`KismetMathLibrary.RandomIntegerInRange` 0 7)))
  (switch `int` `Bar Number`
    (:`0`
      (set `self.Bar1_TargetIndex` _targetpos)
      (set `self.Bar1_Half` `Use Half`))
    (:`1`
      (set `self.Bar2_TargetIndex` _targetpos)
      (set `self.Bar2_Half` `Use Half`))
    (:`2`
      (set `self.Bar3_TargetIndex` _targetpos)
      (set `self.Bar3_Half` `Use Half`))
    (:`3`
      (set `self.Bar4_TargetIndex` _targetpos)
      (set `self.Bar4_Half` `Use Half`)))
  (`MaterialInstanceDynamic.SetScalarParameterValue` _dmi (`KismetStringLibrary.Conv_StringToName` (`KismetStringLibrary.Concat_StrStr` "Bar" _returnvalue "_" "Target" (`KismetStringLibrary.Conv_IntToString` (+ _output_get 1)))) 1.0)
  (`MaterialInstanceDynamic.SetScalarParameterValue` _dmi (`KismetStringLibrary.Conv_StringToName` (`KismetStringLibrary.Concat_StrStr` "Bar" _returnvalue "_" "Usehalf")) (`KismetMathLibrary.SelectFloat` 1.0 0.0 `Use Half`)))

(event `ResetBar`
  (params (BarNumber :type Integer) (State :type "Float (double-precision)") (UseHalf :type "Float (double-precision)") (Color :type "LinearColor Structure"))
  (bind _dmi (`self.DMI`))
  (bind _returnvalue (`KismetStringLibrary.Conv_IntToString` (+ BarNumber 1)))
  ; Reset Bar To Default State
  (for _index (range 1 9)
    (`MaterialInstanceDynamic.SetScalarParameterValue` _dmi (`KismetStringLibrary.Conv_StringToName` (`KismetStringLibrary.Concat_StrStr` "Bar" _returnvalue "_" "Target" (`KismetStringLibrary.Conv_IntToString` _index))) State)
    (`MaterialInstanceDynamic.SetScalarParameterValue` _dmi (`KismetStringLibrary.Conv_StringToName` (`KismetStringLibrary.Concat_StrStr` "Bar" _returnvalue "_" "Usehalf")) UseHalf)
    (`MaterialInstanceDynamic.SetVectorParameterValue` _dmi (`KismetStringLibrary.Conv_StringToName` (`KismetStringLibrary.Concat_StrStr` "Bar" _returnvalue "_" "StatusColor")) Color)))

(event `ReInitFailedBars`
  (bind _currentbarindex (`self.CurrentBarIndex`))
  ; REInt Solved Bars If Current Bar Is Failed
  (`self.ReInitBar` _currentbarindex)
  (if (> _currentbarindex 0)
    (bind _output_get (set `self.CurrentBarIndex` (- _currentbarindex 1)))
    (`self.ReInitBar` _output_get))
  (set `self.MoverPosition` 0.0)
  (`self.SetupMover`)
  (`MaterialInstanceDynamic.SetScalarParameterValue` (`self.DMI`) (`KismetStringLibrary.Conv_StringToName` (`KismetStringLibrary.Concat_StrStr` "Bar" (`KismetStringLibrary.Conv_IntToString` (+ (`self.CurrentBarIndex`) 1)) "_Vis")) 1.0)
  (set `self.CanMove` true))

(event `ReInitBar`
  (params (BarIndex :type Integer))
  ; ReInt Bar Based On Bar Index
  (`self.ResetBar` BarIndex 0.0 0.0 (`self.BarColorNormal`))
  (switch `int` BarIndex
    (:`0`
      (set `self.UseHalf` (`self.Bar1_Half`)))
    (:`1`
      (set `self.UseHalf` (`self.Bar2_Half`)))
    (:`2`
      (set `self.UseHalf` (`self.Bar3_Half`)))
    (:`3`
      (set `self.UseHalf` (`self.Bar4_Half`))))
  (`self.SetTarget` BarIndex (`self.UseHalf`)))

(event `InitGame`
  (bind _dmi (`self.DMI`))
  (bind _dmi_2 (`self.DMI`))
  (bind _barcolornormal (`self.BarColorNormal`))
  ; ReInit Game
  (`self.ResetBar` 0 0.0 0.0 _barcolornormal)
  (`self.ResetBar` 1 0.0 0.0 _barcolornormal)
  (`self.ResetBar` 2 0.0 0.0 _barcolornormal)
  (`self.ResetBar` 3 0.0 0.0 _barcolornormal)
  (switch `/Game/MiniGames2/Blueprints/Data/E_MG_FastCount` (`self.BarsCount`)
    (:`NewEnumerator0`
      (`MaterialInstanceDynamic.SetScalarParameterValue` _dmi_2 "Bar3_Vis" 0.0)
      (`MaterialInstanceDynamic.SetScalarParameterValue` _dmi_2 "Bar4_Vis" 0.0)
      (`MaterialInstanceDynamic.SetScalarParameterValue` _dmi_2 "Bar1_OY" 0.3)
      (`MaterialInstanceDynamic.SetScalarParameterValue` _dmi_2 "Bar2_OY" 0.2))
    (:`NewEnumerator1`
      (`MaterialInstanceDynamic.SetScalarParameterValue` _dmi_2 "Bar3_Vis" 1.0)
      (`MaterialInstanceDynamic.SetScalarParameterValue` _dmi_2 "Bar4_Vis" 0.0)
      (`MaterialInstanceDynamic.SetScalarParameterValue` _dmi_2 "Bar1_OY" 0.35)
      (`MaterialInstanceDynamic.SetScalarParameterValue` _dmi_2 "Bar2_OY" 0.25)
      (`MaterialInstanceDynamic.SetScalarParameterValue` _dmi_2 "Bar3_OY" 0.15))
    (:`NewEnumerator2`
      (`MaterialInstanceDynamic.SetScalarParameterValue` _dmi_2 "Bar3_Vis" 1.0)
      (`MaterialInstanceDynamic.SetScalarParameterValue` _dmi_2 "Bar4_Vis" 1.0)
      (`MaterialInstanceDynamic.SetScalarParameterValue` _dmi_2 "Bar1_OY" 0.4)
      (`MaterialInstanceDynamic.SetScalarParameterValue` _dmi_2 "Bar2_OY" 0.3)
      (`MaterialInstanceDynamic.SetScalarParameterValue` _dmi_2 "Bar3_OY" 0.2)
      (`MaterialInstanceDynamic.SetScalarParameterValue` _dmi_2 "Bar4_OY" 0.1)))
  (`self.SetTarget` 0 (`self.Bar1_UseHalf`))
  (`self.SetTarget` 1 (`self.Bar2_UseHalf`))
  (`self.SetTarget` 2 (`self.Bar3_UseHalf`))
  (`self.SetTarget` 3 (`self.Bar4_UseHalf`))
  (set `self.CurrentBarIndex` 0)
  (set `self.MoverPosition` 0.0)
  (set `self.MoverDirection` 1.0)
  (`MaterialInstanceDynamic.SetScalarParameterValue` _dmi "Mover_Xpos" 0.0)
  (`self.SetupMover`)
  (`MaterialInstanceDynamic.SetScalarParameterValue` _dmi "ShowActivated" 0.0)
  (`MaterialInstanceDynamic.SetScalarParameterValue` _dmi "Bar1_Vis" 1.0)
  (`MaterialInstanceDynamic.SetScalarParameterValue` _dmi "Bar2_Vis" 1.0)
  (`MaterialInstanceDynamic.SetScalarParameterValue` _dmi "MoverVis" 1.0)
  (set `self.CanMove` true))

(event `ForceAction`
  (bind _errorsound (`self.ErrorSound`))
  (bind _usehalf (`self.UseHalf`))
  (bind _moverposition (`self.MoverPosition`))
  (bind _dmi (`self.DMI`))
  ; Button Action
  (if (`self.PlayerOverlapped`)
    (if (`self.IsMiniGameActivated`)
      (set `self.CanMove` false)
      (switch `int` (`self.CurrentBarIndex`)
        (:`0`
          (set `self.TargetPos` (`self.Bar1_TargetIndex`))
          (set `self.UseHalf` (`self.Bar1_Half`)))
        (:`1`
          (set `self.TargetPos` (`self.Bar2_TargetIndex`))
          (set `self.UseHalf` (`self.Bar2_Half`)))
        (:`2`
          (set `self.TargetPos` (`self.Bar3_TargetIndex`))
          (set `self.UseHalf` (`self.Bar3_Half`)))
        (:`3`
          (set `self.TargetPos` (`self.Bar4_TargetIndex`))
          (set `self.UseHalf` (`self.Bar4_Half`))))
      (switch `int` (`self.TargetPos`)
        (:`0`
          (set `self.Target_From` (`KismetMathLibrary.SelectFloat` (`self.Target1_FromHalf`) (`self.Target1_From`) _usehalf))
          (set `self.Target_To` (`self.Target1_To`)))
        (:`1`
          (set `self.Target_From` (`KismetMathLibrary.SelectFloat` (`self.Target2_FromHalf`) (`self.Target2_From`) _usehalf))
          (set `self.Target_To` (`self.Target2_To`)))
        (:`2`
          (set `self.Target_From` (`KismetMathLibrary.SelectFloat` (`self.Target3_FromHalf`) (`self.Target3_From`) _usehalf))
          (set `self.Target_To` (`self.Target3_To`)))
        (:`3`
          (set `self.Target_From` (`KismetMathLibrary.SelectFloat` (`self.Target4_FromHalf`) (`self.Target4_From`) _usehalf))
          (set `self.Target_To` (`self.Target4_To`)))
        (:`4`
          (set `self.Target_From` (`KismetMathLibrary.SelectFloat` (`self.Target5_FromHalf`) (`self.Target5_From`) _usehalf))
          (set `self.Target_To` (`self.Target5_To`)))
        (:`5`
          (set `self.Target_From` (`KismetMathLibrary.SelectFloat` (`self.Target6_FromHalf`) (`self.Target6_From`) _usehalf))
          (set `self.Target_To` (`self.Target6_To`)))
        (:`6`
          (set `self.Target_From` (`KismetMathLibrary.SelectFloat` (`self.Target7_FromHalf`) (`self.Target7_From`) _usehalf))
          (set `self.Target_To` (`self.Target7_To`)))
        (:`7`
          (set `self.Target_From` (`self.Target8_From`))
          (set `self.Target_To` (`KismetMathLibrary.SelectFloat` (`self.Target8_ToHalf`) (`self.Target8_To`) (`self.UseHalf`)))))
      (if (and (>= _moverposition (`self.Target_From`)) (<= _moverposition (`self.Target_To`)))
        (bind _result (`/Engine/EditorBlueprintResources/StandardMacros.IncrementInt` (`self.CurrentBarIndex`))
          (:`  `
            (`MaterialInstanceDynamic.SetScalarParameterValue` (`self.DMI`) (`KismetStringLibrary.Conv_StringToName` (`KismetStringLibrary.Concat_StrStr` "Bar" (`KismetStringLibrary.Conv_IntToString` _result) "_Vis")) 0.0)
            (if (== _result (select `/Game/MiniGames2/Blueprints/Data/E_MG_FastCount` (`self.BarsCount`) :`NewEnumerator0` 2 :`NewEnumerator1` 3 :`NewEnumerator2` 4))
              ;;[1 1 1] Success
              (set `self.MiniGameEnabled` false)
              (set `self.IsMiniGameActivated` false)
              (set `self.InputEnable` false)
              (`MaterialInstanceDynamic.SetScalarParameterValue` _dmi "ShowActivated" 1.0)
              (`MaterialInstanceDynamic.SetScalarParameterValue` _dmi "MoverVis" 0.0)
              (`KismetSystemLibrary.Delay` (`self.DelayTimeWhenComplete`))
              (`self.OnMiniGameSuccess`)
              (`self.Server_Success`)
              (else
                (`self.SetupMover`)
                (set `self.MoverPosition` 0.0)
                (set `self.CanMove` true)))))
        (else
          ;;[1 1 1] Error
          (`self.ResetBar` (`self.CurrentBarIndex`) 1.0 0.0 (`self.BarColorFailed1`))
          (`/Engine/EditorBlueprintResources/StandardMacros.IsValid` _errorsound
            (:`Is Valid`
              (`GameplayStatics.PlaySoundAtLocation` _errorsound (`self.K2_GetActorLocation` self) (struct) 1.0 1.0 0.0 null null null null)
              (bind (_direction _newtrack_0) (`Timeline|MoverTimeline` :!via `PlayFromStart` :!label _label_7)
                (:`Update`
                  (`MaterialInstanceDynamic.SetVectorParameterValue` (`self.DMI`) (`KismetStringLibrary.Conv_StringToName` (`KismetStringLibrary.Concat_StrStr` "Bar" (`KismetStringLibrary.Conv_IntToString` (+ (`self.CurrentBarIndex`) 1)) "_StatusColor")) (`KismetMathLibrary.LinearColorLerp` (`self.BarColorFailed1`) (`self.BarColorFailed2`) _newtrack_0)))
                (:`Finished`
                  (`self.ReInitFailedBars`))))
            (:`Is Not Valid`
              (goto _label_7 :!via `PlayFromStart`)))))
      (else
        (`self.InitGame`)
        (`PrimitiveComponent.SetMaterial` (`self.MiniGameScreen`) 0 (`self.DMI`))
        (set `self.IsMiniGameActivated` true)
        (set `self.InputEnable` true)))))

(fn `OnRep_Spent`)

(fn `UserConstructionScript`)