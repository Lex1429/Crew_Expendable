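; BP_BaseProjectile is a base projectile that damages what it hits and destroys itself after a short lifetime.
; On hit, only the authority applies damage, prints the result, spawns a Niagara effect at the impact point and destroys the actor.
; Damage is always credited to player controller 0, and the effect is spawned directly in the authority branch with no multicast.
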(event `self.ReceiveBeginPlay`
  (`KismetSystemLibrary.Delay` 2.0)
  (`self.K2_DestroyActor`))

(event `self.ReceiveHit`
  (params (MyComp :type "PrimitiveComponent Object Reference") (Other :type "Actor Object Reference") (OtherComp :type "PrimitiveComponent Object Reference") (bSelfMoved :type Boolean) (HitLocation :type "Vector Structure") (HitNormal :type "Vector Structure") (NormalImpulse :type "Vector Structure") (Hit :type "HitResult Structure (by ref)"))
  (`/Engine/EditorBlueprintResources/ActorMacros.Switch Has Authority`
    (:`Authority`
      (set `self.Hit` Hit)
      (bind _returnvalue (`GameplayStatics.ApplyDamage` (`.HitActor` (`GameplayStatics.BreakHitResult` Hit)) (`self.Damage`) (`GameplayStatics.GetPlayerController` 0) self))
      (`KismetSystemLibrary.PrintString` (`KismetStringLibrary.Conv_DoubleToString` _returnvalue))
      (`NiagaraFunctionLibrary.SpawnSystemAtLocation` (`self.System Template`) HitLocation)
      (`self.K2_DestroyActor`))))

(fn `UserConstructionScript`)