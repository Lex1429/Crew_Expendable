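; Inventory component for the player character that tracks a currently selected equipment slot and mirrors it to the HUD equipment overlay.
; After short delays on BeginPlay, the locally controlled owner caches itself and highlights the first slot.
; Scroll events wrap through three slots, while SwapSlot jumps directly; all call ChangeSlotMesh, currently an empty stub.
; Helpers store, query or clear the current slot's item, with removal also destroying the owner's equipment component.
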(event `self.ReceiveBeginPlay`
  (`KismetSystemLibrary.Delay` 0.3)
  (if (`Pawn.IsLocallyControlled` (`Actor.Instigator` (`self.GetOwner`)))
    (bind _asbp_player_character_core (cast `/Game/Blueprints/Characters/BP_PlayerCharacterCore` (`self.GetOwner`)))
    (set `self.OwnerRef` _asbp_player_character_core)
    (`KismetSystemLibrary.Delay` 0.7)
    (`/Game/UI/WB_EquipmentOverlay.SelectSlot` (`/Game/UI/WB_PlayerUI.WB_EquipmentOverlay` (`/Game/MBLS/Blueprints/Core/Gameplay/Player/BP_PC_Gameplay.HUDRef` (`/Game/Blueprints/Characters/BP_PlayerCharacterCore.Gameplay Controller Ref` (`self.OwnerRef`)))) 0)))

(event `MouseUpSelect`
  (bind _currentslotindex (`self.CurrentSlotIndex`))
  (`/Game/UI/WB_EquipmentOverlay.UnselectSlot` (`/Game/UI/WB_PlayerUI.WB_EquipmentOverlay` (`/Game/MBLS/Blueprints/Core/Gameplay/Player/BP_PC_Gameplay.HUDRef` (`/Game/Blueprints/Characters/BP_PlayerCharacterCore.Gameplay Controller Ref` (`self.OwnerRef`)))) _currentslotindex)
  (bind _output_get (set `self.CurrentSlotIndex` (+ _currentslotindex 1)))
  (if (>= _output_get 3)
    (bind _output_get_2 (set `self.CurrentSlotIndex` 0))
    (`/Game/UI/WB_EquipmentOverlay.SelectSlot` (`/Game/UI/WB_PlayerUI.WB_EquipmentOverlay` (`/Game/MBLS/Blueprints/Core/Gameplay/Player/BP_PC_Gameplay.HUDRef` (`/Game/Blueprints/Characters/BP_PlayerCharacterCore.Gameplay Controller Ref` (`self.OwnerRef`)))) _output_get_2)
    (else
      (`/Game/UI/WB_EquipmentOverlay.SelectSlot` (`/Game/UI/WB_PlayerUI.WB_EquipmentOverlay` (`/Game/MBLS/Blueprints/Core/Gameplay/Player/BP_PC_Gameplay.HUDRef` (`/Game/Blueprints/Characters/BP_PlayerCharacterCore.Gameplay Controller Ref` (`self.OwnerRef`)))) (`self.CurrentSlotIndex`))))
  (`self.ChangeSlotMesh` :!label _label))

(event `MouseDownSelect`
  (bind _currentslotindex (`self.CurrentSlotIndex`))
  (`/Game/UI/WB_EquipmentOverlay.UnselectSlot` (`/Game/UI/WB_PlayerUI.WB_EquipmentOverlay` (`/Game/MBLS/Blueprints/Core/Gameplay/Player/BP_PC_Gameplay.HUDRef` (`/Game/Blueprints/Characters/BP_PlayerCharacterCore.Gameplay Controller Ref` (`self.OwnerRef`)))) _currentslotindex)
  (bind _output_get (set `self.CurrentSlotIndex` (- _currentslotindex 1)))
  (if (<= _output_get -1)
    (bind _output_get_2 (set `self.CurrentSlotIndex` 2))
    (`/Game/UI/WB_EquipmentOverlay.SelectSlot` (`/Game/UI/WB_PlayerUI.WB_EquipmentOverlay` (`/Game/MBLS/Blueprints/Core/Gameplay/Player/BP_PC_Gameplay.HUDRef` (`/Game/Blueprints/Characters/BP_PlayerCharacterCore.Gameplay Controller Ref` (`self.OwnerRef`)))) _output_get_2)
    (goto _label)
    (else
      (`/Game/UI/WB_EquipmentOverlay.SelectSlot` (`/Game/UI/WB_PlayerUI.WB_EquipmentOverlay` (`/Game/MBLS/Blueprints/Core/Gameplay/Player/BP_PC_Gameplay.HUDRef` (`/Game/Blueprints/Characters/BP_PlayerCharacterCore.Gameplay Controller Ref` (`self.OwnerRef`)))) (`self.CurrentSlotIndex`))
      (goto _label))))

(fn `ChangeSlotMesh`)

(fn `IsSlotFree?`
  (params (Item :type "/Game/Blueprints/InventorySystem/Pickups/Data/PDA_Items Object Reference"))
  (returns (`SlotFree?` :type Boolean))
  (if (== (`|GetArrayItem` (`self.InventorySlots`) (`self.CurrentSlotIndex`)) null)
    (`KismetArrayLibrary.Array_Set` (`self.InventorySlots`) (`self.CurrentSlotIndex`) Item)
    (`/Game/UI/WB_EquipmentOverlay.SlotChange` (`/Game/UI/WB_PlayerUI.WB_EquipmentOverlay` (`/Game/MBLS/Blueprints/Core/Gameplay/Player/BP_PC_Gameplay.HUDRef` (`/Game/Blueprints/Characters/BP_PlayerCharacterCore.Gameplay Controller Ref` (`self.OwnerRef`)))) (`self.CurrentSlotIndex`) (`/Game/Blueprints/InventorySystem/Pickups/Data/PDA_Items.ObjectIcon` Item) false)
    (return true)
    (else
      (return false))))

(fn `QueryInventory`
  (returns (SlotNotEmpty :type Boolean) (ObjectClass :type "/Game/Blueprints/InventorySystem/Pickups/Data/PDA_Items Object Reference"))
  (bind _output (`|GetArrayItem` (`self.InventorySlots`) (`self.CurrentSlotIndex`)))
  (if (== _output null)
    (return false null)
    (else
      (return true _output))))

(fn `RemoveFromInventory`
  (`KismetArrayLibrary.Array_Set` (`self.InventorySlots`) (`self.CurrentSlotIndex`))
  (`/Game/UI/WB_EquipmentOverlay.SlotChange` (`/Game/UI/WB_PlayerUI.WB_EquipmentOverlay` (`/Game/MBLS/Blueprints/Core/Gameplay/Player/BP_PC_Gameplay.HUDRef` (`/Game/Blueprints/Characters/BP_PlayerCharacterCore.Gameplay Controller Ref` (`self.OwnerRef`)))) (`self.CurrentSlotIndex`) null true)
  (`self.K2_DestroyComponent` (`Actor.GetComponentByClass` (`self.GetOwner`) "/Game/Blueprints/EquipmentSystem/BPC_CoreEquipmentComponent.BPC_CoreEquipmentComponent_C")))

(fn `SwapSlot`
  (params (SlotIndex :type Integer))
  (`/Game/UI/WB_EquipmentOverlay.UnselectSlot` (`/Game/UI/WB_PlayerUI.WB_EquipmentOverlay` (`/Game/MBLS/Blueprints/Core/Gameplay/Player/BP_PC_Gameplay.HUDRef` (`/Game/Blueprints/Characters/BP_PlayerCharacterCore.Gameplay Controller Ref` (`self.OwnerRef`)))) (`self.CurrentSlotIndex`))
  (bind _output_get (set `self.CurrentSlotIndex` SlotIndex))
  (`/Game/UI/WB_EquipmentOverlay.SelectSlot` (`/Game/UI/WB_PlayerUI.WB_EquipmentOverlay` (`/Game/MBLS/Blueprints/Core/Gameplay/Player/BP_PC_Gameplay.HUDRef` (`/Game/Blueprints/Characters/BP_PlayerCharacterCore.Gameplay Controller Ref` (`self.OwnerRef`)))) _output_get)
  (`self.ChangeSlotMesh`))