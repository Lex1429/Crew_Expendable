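; Large bio dome modular building piece, configured in the editor through its construction script, with no active runtime logic.
; Applies one master material to the building, dome, legs and end caps.
; Places the eight legs at fixed positions around the structure, sharing an adjustable leg height.
; Three toggles show or hide each end cap with its window, also disabling collision on the hidden pairs.
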(fn `UserConstructionScript`
  (bind _window2 (`self.Window2`))
  (bind _window3 (`self.Window3`))
  (bind _legheight (`self.LegHeight`))
  (bind _endcap1 (`self.EndCap1`))
  (`PrimitiveComponent.SetMaterial` (`self.Building`) 0 (`self.MasterMaterial`))
  (`PrimitiveComponent.SetMaterial` (`self.Leg1`) 0 (`self.MasterMaterial`))
  (`PrimitiveComponent.SetMaterial` (`self.Leg2`) 0 (`self.MasterMaterial`))
  (`PrimitiveComponent.SetMaterial` (`self.Leg3`) 0 (`self.MasterMaterial`))
  (`PrimitiveComponent.SetMaterial` (`self.Leg4`) 0 (`self.MasterMaterial`))
  (`PrimitiveComponent.SetMaterial` (`self.Leg5`) 0 (`self.MasterMaterial`))
  (`PrimitiveComponent.SetMaterial` (`self.Leg6`) 0 (`self.MasterMaterial`))
  (`PrimitiveComponent.SetMaterial` (`self.Leg7`) 0 (`self.MasterMaterial`))
  (`PrimitiveComponent.SetMaterial` (`self.Leg8`) 0 (`self.MasterMaterial`))
  (`PrimitiveComponent.SetMaterial` (`self.Dome`) 0 (`self.MasterMaterial`))
  (`PrimitiveComponent.SetMaterial` (`self.EndCap1`) 0 (`self.MasterMaterial`))
  (`PrimitiveComponent.SetMaterial` (`self.EndCap2`) 0 (`self.MasterMaterial`))
  (`PrimitiveComponent.SetMaterial` (`self.EndCap3`) 0 (`self.MasterMaterial`))
  (`SceneComponent.K2_SetRelativeLocation` (`self.Leg1`) (`KismetMathLibrary.MakeVector` -1614.0 -937.0 _legheight) false false)
  (`SceneComponent.K2_SetRelativeLocation` (`self.Leg2`) (`KismetMathLibrary.MakeVector` -935.0 -1613.0 _legheight) false false)
  (`SceneComponent.K2_SetRelativeLocation` (`self.Leg3`) (`KismetMathLibrary.MakeVector` 929.0 -1611.0 _legheight) false false)
  (`SceneComponent.K2_SetRelativeLocation` (`self.Leg4`) (`KismetMathLibrary.MakeVector` 1607.0 -931.0 _legheight) false false)
  (`SceneComponent.K2_SetRelativeLocation` (`self.Leg5`) (`KismetMathLibrary.MakeVector` 1615.0 931.0 _legheight) false false)
  (`SceneComponent.K2_SetRelativeLocation` (`self.Leg6`) (`KismetMathLibrary.MakeVector` 933.0 1617.0 _legheight) false false)
  (`SceneComponent.K2_SetRelativeLocation` (`self.Leg7`) (`KismetMathLibrary.MakeVector` -1616.0 937.0 _legheight) false false)
  (`SceneComponent.K2_SetRelativeLocation` (`self.Leg8`) (`KismetMathLibrary.MakeVector` -932.0 1618.0 _legheight) false false)
  (`|ExecutionSequence`
    (:`then_0`
      (if (`self.Endcap1?`)
        (`SceneComponent.SetVisibility` (`self.EndCap1`) true false)
        (`SceneComponent.SetVisibility` (`self.Window1`) true false)
        (else
          (`SceneComponent.SetVisibility` _endcap1 false false)
          (`SceneComponent.SetVisibility` (`self.Window1`) false false)
          (`PrimitiveComponent.SetCollisionEnabled` _endcap1 "NoCollision")
          (`PrimitiveComponent.SetCollisionEnabled` (`self.Window1`) "NoCollision"))))
    (:`then_1`
      (if (`self.Endcap2?`)
        (`SceneComponent.SetVisibility` (`self.Window2`) true false)
        (`SceneComponent.SetVisibility` (`self.EndCap2`) true false)
        (else
          (`SceneComponent.SetVisibility` _window2 false false)
          (`SceneComponent.SetVisibility` (`self.EndCap2`) false false)
          (`PrimitiveComponent.SetCollisionEnabled` _window2 "NoCollision")
          (`PrimitiveComponent.SetCollisionEnabled` (`self.EndCap2`) "NoCollision"))))
    (:`then_2`
      (if (`self.Endcap3?`)
        (`SceneComponent.SetVisibility` (`self.Window3`) true false)
        (`SceneComponent.SetVisibility` (`self.EndCap3`) true false)
        (else
          (`SceneComponent.SetVisibility` _window3 false false)
          (`SceneComponent.SetVisibility` (`self.EndCap3`) false false)
          (`PrimitiveComponent.SetCollisionEnabled` _window3 "NoCollision")
          (`PrimitiveComponent.SetCollisionEnabled` (`self.EndCap3`) "NoCollision"))))))