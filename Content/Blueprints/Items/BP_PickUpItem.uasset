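; Salvage pickup actor that the player can focus on to see its name and value, then interact with to collect it.
; ItemName selects the DT_SalvageList row that sets mesh and value, in construction and at BeginPlay.
; Focus shows a WB_PlayerUI prompt, cleared by a short retriggerable delay once focus calls stop.
; Interact passes the item name to the player's HandlePickupMessage, destroys the actor and clears the prompt.
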(event `self.ReceiveBeginPlay`
  (`self.SetUpMesh`)
  (`KismetSystemLibrary.Delay` 0.5)
  (bind _foundwidgets (`WidgetBlueprintLibrary.GetAllWidgetsOfClass` "/Game/UI/WB_PlayerUI.WB_PlayerUI_C"))
  (set `self.PlayerUIRef` (`|GetArrayItem` _foundwidgets)))

(event `/Game/Blueprints/Interfaces/BPI_Interact.Interact`
  (params (Character :type "/Game/Blueprints/Characters/BP_BaseCharacter Object Reference") (PlayerCharacter :type "/Game/Blueprints/Characters/BP_PlayerCharacterCore Object Reference"))
  (message `/Game/Blueprints/Interfaces/BPI_Equipables.HandlePickup` PlayerCharacter (`KismetStringLibrary.Conv_NameToString` (`self.ItemName`)))
  (`self.K2_DestroyActor`)
  (message `/Game/Blueprints/Interfaces/BPI_CombatUI.InteractElement` (`self.PlayerUIRef`) "" "" "" false ""))

(event `/Game/Blueprints/Interfaces/BPI_Interact.SetFocused`
  (bind _playeruiref (`self.PlayerUIRef`))
  (message `/Game/Blueprints/Interfaces/BPI_CombatUI.InteractElement` _playeruiref (`KismetTextLibrary.Conv_NameToText` (`self.ItemName`)) (`KismetTextLibrary.Conv_IntToText` (`self.Value`)) "Pick Up" true "")
  (`KismetSystemLibrary.RetriggerableDelay` 0.1)
  (message `/Game/Blueprints/Interfaces/BPI_CombatUI.InteractElement` _playeruiref "" "" "" false ""))

(fn `GetCanBePickedUp`
  (returns (CanBePickedUp :type Boolean))
  (return false))

(fn `GetItemToSpawn`
  (returns (Item :type "/Game/Blueprints/Interactables/Weapons/BP_WeaponComponentMaster Class Reference"))
  (return null))

(fn `SetUpMesh`
  (bind _returnvalue (`|GetDataTableRow` "/Game/Blueprints/Salvage/DT_SalvageList.DT_SalvageList" (`self.ItemName`))
    (:`then`
      (bind (_itemid _itemname _value _missioncritical _objectclass _slotimage _description _staticmesh) (break `/Game/Blueprints/Salvage/S_Salvage` _returnvalue))
      (`StaticMeshComponent.SetStaticMesh` (`self.StaticMesh`) _staticmesh)
      (set `self.Item Name` _itemname)
      (set `self.Value` _value))))

(fn `UserConstructionScript`
  (`self.SetUpMesh`))