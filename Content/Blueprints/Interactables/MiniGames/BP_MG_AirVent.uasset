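; Interactable air vent mini-game where players pull and insert the AC's cooling filter, starting on a looping broken animation.
; InView briefly shows Take or Insert prompts from the GameState filter status.
; PickupObject clears the inserted flag or inserts a filter, splitting owner-side inventory changes from mesh, animation, Niagara and material updates.
; The CoolingFilterInserted RepNotify updates visuals and writes filter status back to GameState.
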(event `/Game/Blueprints/Interfaces/BPI_Pickup.InView`
  (bind _insertwidget (`self.InsertWidget`))
  (bind _takewidget (`self.TakeWidget`))
  ;[0 0 1] Interact Messages based on Filter State [Cooling]
  (bind (_inac_ _indispenser_ _broken_) (message `/Game/Blueprints/Interfaces/BPI_FilterStats.GetCoolerFilterStatus` (`GameplayStatics.GetGameState`)))
  (if (and _inac_ (not _broken_))
    _
    (elif (and _inac_ _broken_)
      (`SceneComponent.SetVisibility` _takewidget true false)
      (`KismetSystemLibrary.RetriggerableDelay` 0.1)
      (`SceneComponent.SetVisibility` _takewidget false false)
      (elif (not _broken_)
        (`SceneComponent.SetVisibility` _insertwidget true false)
        (`KismetSystemLibrary.RetriggerableDelay` 0.1)
        (`SceneComponent.SetVisibility` _insertwidget false false)))))

(event `self.ReceiveBeginPlay`
  ;[0 1 0] Setup
  (`|ExecutionSequence`
    (:`then_0`
      (`SkeletalMeshComponent.PlayAnimation` (`self.AC`) "/Game/Assets/VentMiniGameParts/vent_mini_game_Broken.vent_mini_game_Broken" true))
    (:`then_1`
      (bind _foundwidgets (`WidgetBlueprintLibrary.GetAllWidgetsOfClass` "/Game/UI/WB_PlayerUI.WB_PlayerUI_C"))
      (set `self.PlayerUIRef` (`|GetArrayItem` _foundwidgets)))))

(event `/Game/Blueprints/Interfaces/BPI_Pickup.PickupObject`
  (params (PlayerRef :type "/Game/Blueprints/Characters/BP_PlayerCharacterCore Object Reference"))
  ;[0 0 1] Filter Pull/Insert
  ;; Filter Pull/Insert Handled by server
  (bind (_inac_ _indispenser_ _broken_) (message `/Game/Blueprints/Interfaces/BPI_FilterStats.GetCoolerFilterStatus` (`GameplayStatics.GetGameState`)))
  (if (and _inac_ (not _broken_))
    _
    (elif (== (`/Game/Blueprints/Characters/BP_PlayerCharacterCore.CurrentEquipmentHeld` PlayerRef) "6")
      (set `self.FilterState` "1" :!label _label)
      (`self.Owner_InsertFilter` PlayerRef)
      (`self.Local_InsertFilter` PlayerRef)
      (elif (`self.CoolingFilterInserted?`)
        (set `self.CoolingFilterInserted?` false)
        (else
          (goto _label))))))

(event `Local_InsertFilter`
  (params (Player :type "/Game/Blueprints/Characters/BP_PlayerCharacterCore Object Reference"))
  ;[0 0 1] Filter Pull/Insert
  ;; Server has Mesh and animation changes multicast and sets Gamestate status of filter
  (`SceneComponent.SetVisibility` (`self.CoolingFilter`) true false)
  (message `/Game/Blueprints/Interfaces/BPI_FilterStats.SetCoolerFilterStatus` (`GameplayStatics.GetGameState`) true false false)
  (`SkeletalMeshComponent.PlayAnimation` (`self.AC`) "/Game/Assets/VentMiniGameParts/vent_mini_game_Anim.vent_mini_game_Anim" true)
  (`ActorComponent.Deactivate` (`self.Niagara`))
  (`StaticMeshComponent.SetStaticMesh` (`self.CoolingFilter`) "/Game/Assets/VentMiniGameParts/Cooling_On.Cooling_On")
  (`PrimitiveComponent.SetMaterialByName` (`self.AC`) "CoilCenter" "/Game/Assets/VentMiniGameParts/ACStatusMats/MI_ACFunctional.MI_ACFunctional"))

(event `Owner_InsertFilter`
  (params (Player :type "/Game/Blueprints/Characters/BP_PlayerCharacterCore Object Reference"))
  ;[0 0 1] Filter Pull/Insert
  ;; Has Owning client handle own Equipment Set
  (`/Game/Blueprints/Characters/BP_PlayerCharacterCore.RemoveItemFromInventory` Player)
  (`/Game/Blueprints/Characters/BP_PlayerCharacterCore.Server_SetHeldEquipment` Player "1"))

(fn `GetCanBePickedUp`
  (returns (CanBePickedUp :type Boolean))
  (return false))

(fn `GetItemToSpawn`
  (returns (Item :type "/Game/Blueprints/Interactables/Weapons/BP_WeaponComponentMaster Class Reference"))
  (return null))

(fn `GiveFilter`
  (params (Player :type "/Game/Blueprints/Characters/BP_PlayerCharacterCore Object Reference"))
  (locals (NewLocalVar :type Name :default "5"))
  (bind _slotnotempty (`/Game/Blueprints/Characters/BP_PlayerCharacterCore.CheckInventory` Player))
  (if _slotnotempty
    (bind _slot_free_ (`/Game/Blueprints/Characters/BP_PlayerCharacterCore.CheckFreeSlot?` Player (`local.NewLocalVar`)))
    (if _slot_free_
      (`/Game/Blueprints/Characters/BP_PlayerCharacterCore.Server_SetHeldEquipment` Player "5"))))

(fn `OnRep_CoolingFilterInserted?`
  (if (`self.CoolingFilterInserted?`)
    (`SceneComponent.SetVisibility` (`self.CoolingFilter`) true false)
    (message `/Game/Blueprints/Interfaces/BPI_FilterStats.SetCoolerFilterStatus` (`GameplayStatics.GetGameState`) true false false)
    (`SkeletalMeshComponent.PlayAnimation` (`self.AC`) "/Game/Assets/VentMiniGameParts/vent_mini_game_Anim.vent_mini_game_Anim" true)
    (`ActorComponent.Deactivate` (`self.Niagara`))
    (`StaticMeshComponent.SetStaticMesh` (`self.CoolingFilter`) "/Game/Assets/VentMiniGameParts/Cooling_On.Cooling_On")
    (else
      (`SceneComponent.SetVisibility` (`self.CoolingFilter`) false false)
      (message `/Game/Blueprints/Interfaces/BPI_FilterStats.SetCoolerFilterStatus` (`GameplayStatics.GetGameState`) false false true)
      (`PrimitiveComponent.SetMaterialByName` (`self.AC`) "CoilCenter" "/Game/Assets/VentMiniGameParts/ACStatusMats/MI_ACError.MI_ACError"))))

(fn `QueryAsset`
  (returns (Asset :type "/Game/Blueprints/InventorySystem/Pickups/Data/PDA_Items Object Reference"))
  (return null))

(fn `QueryItem`
  (returns (Item :type Name))
  (return (`self.FilterState`)))

(fn `UserConstructionScript`)