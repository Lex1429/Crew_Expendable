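; BP_SALRoute is an AI route actor that exposes the points of a spline as world locations.
; A PathPoint index tracks the current point, and the NextSpline event increments it with no bounds or wrap check.
; Despite its name, SetSplinePoints only returns the world location at that index.
; BeginPlay prints the spline's point count for debugging.
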(event `self.ReceiveBeginPlay`
  (`KismetSystemLibrary.PrintString` (`KismetStringLibrary.Conv_IntToString` (`SplineComponent.GetNumberOfSplinePoints` (`self.Spline`))) true true (struct :`R` 1.0 :`B` 1.0 :`A` 1.0)))

(event `NextSpline`
  (`/Engine/EditorBlueprintResources/StandardMacros.IncrementInt` (`self.PathPoint`)))

(fn `SetSplinePoints`
  (returns (PointLocation :type "Vector Structure"))
  (return (`SplineComponent.GetLocationAtSplinePoint` (`self.Spline`) (`self.PathPoint`) "World")))

(fn `UserConstructionScript`)