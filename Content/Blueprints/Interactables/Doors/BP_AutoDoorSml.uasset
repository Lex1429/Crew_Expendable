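; BP_AutoDoorSml is a small automatic sliding door driven by actor overlaps.
; Server-named open event calls a local event that plays a hydraulic sound and toggles the door via a position-lerping Timeline.
; Both overlap events fire that toggle; begin also pauses the timer or toggles again, depending on door state.
; End overlap starts or resumes a looping timer that prints elapsed seconds and toggles the door after five.
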(event `Server_OpenDoor`
  (`self.Local_OpenDoor`))

(event `Local_OpenDoor`
  (`GameplayStatics.PlaySoundAtLocation` "/Game/SFX/echoey_hatch-hydrolic.echoey_hatch-hydrolic" (`SceneComponent.K2_GetComponentLocation` (`self.ARch`)) (struct) 0.7 1.0 0.0 "/Game/SFX/SA_Test.SA_Test" null null null)
  (if (not (`self.IsDoorOpen?`))
    (set `self.IsDoorOpen?` true)
    (bind (_direction _slidetrack) (`Timeline|SlideDoor` :!label _label)
      (:`Update`
        (`SceneComponent.K2_SetRelativeLocation` (`self.Door`) (`KismetMathLibrary.VLerp` (90.0 0.0 0.0) (240.0 0.0 0.0) _slidetrack) false true)))
    (else
      (set `self.IsDoorOpen?` false)
      (goto _label :!via `Reverse`))))

(event `self.ReceiveActorBeginOverlap`
  (params (OtherActor :type "Actor Object Reference"))
  (`self.Server_OpenDoor`)
  (if (`self.IsDoorOpen?`)
    (`self.PauseTime`)
    (else
      (`self.Server_OpenDoor`))))

(event `self.ReceiveActorEndOverlap`
  (params (OtherActor :type "Actor Object Reference"))
  (`self.Server_OpenDoor`)
  (if (`KismetSystemLibrary.K2_IsTimerPausedHandle` (`self.Timer`))
    (`self.ResumeTimer`)
    (else
      (`self.Start Timer`))))

(event `Start Timer`
  (set `self.Seconds` 0.0)
  (bind _returnvalue (`KismetSystemLibrary.K2_SetTimerDelegate` (delegate `DeltaSec`) 1.0 true))
  (set `self.Timer` _returnvalue))

(event `DeltaSec`
  (bind _result (`/Engine/EditorBlueprintResources/StandardMacros.IncrementFloat` (`self.Seconds`))
    (:`  `
      (`KismetSystemLibrary.PrintString` (`KismetStringLibrary.Conv_DoubleToString` _result))
      (if (>= _result 5.0)
        (`self.Server_OpenDoor`)
        (`KismetSystemLibrary.K2_ClearAndInvalidateTimerHandle` (`self.Timer`))))))

(event `PauseTime`
  (`KismetSystemLibrary.K2_PauseTimerHandle` (`self.Timer`)))

(event `ResumeTimer`
  (`KismetSystemLibrary.K2_UnPauseTimerHandle` (`self.Timer`)))

(fn `UserConstructionScript`)