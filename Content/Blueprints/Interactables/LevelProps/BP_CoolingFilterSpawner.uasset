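; Level prop cabinet that dispenses a cooling filter when its referenced disposal object signals that a filter was disposed.
; On authority it spawns a core equipment pickup at the spawner point and sets FilterSpawned.
; The OnRep for that flag switches the indicator sphere to its active material, updates the GameState cooler filter status and swings the cabinet door open with a timeline.
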(event `Server_CoolerReady`
  (`/Engine/EditorBlueprintResources/ActorMacros.Switch Has Authority`
    (:`Authority`
      (`|SpawnActorFromClass` "/Game/Blueprints/EquipmentSystem/BP_CoreEquipmentPickup.BP_CoreEquipmentPickup_C" (`KismetMathLibrary.MakeTransform` (`SceneComponent.K2_GetComponentLocation` (`self.FilterSpawner`)) (struct :`Yaw` 180.0)) "AdjustIfPossibleButAlwaysSpawn" "MultiplyWithRoot" null "6" null)
      (set `self.FilterSpawned?` true))
    (:`Remote`
      (`self.Server_CoolerReady`))))

(event `Local_CoolerReady`
  (bind (_direction _newtrack_0) (`Timeline|CabinetDoor`)
    (:`Update`
      (`SceneComponent.K2_SetRelativeRotation` (`self.SM_Prop_Cabinet_03_Door`) (`KismetMathLibrary.RLerp` (struct) (struct :`Yaw` -120.0) _newtrack_0 true) false false))))

(event `self.ReceiveBeginPlay`
  (add `/Game/Blueprints/Interactables/LevelProps/BP_FilterDisposal.CoolingFilterDispossed` (`self.DisposalRef`) (delegate `SpawnFilter`)))

(event `SpawnFilter`
  (`self.Server_CoolerReady`))

(fn `GetCanBePickedUp`
  (returns (CanBePickedUp :type Boolean))
  (return false))

(fn `GetCoolerFilterStatus`
  (returns (`InAC?` :type Boolean) (`InDispenser?` :type Boolean) (`Broken?` :type Boolean))
  (return false false false))

(fn `GetItemToSpawn`
  (returns (Item :type "/Game/Blueprints/Interactables/Weapons/BP_WeaponComponentMaster Class Reference"))
  (return null))

(fn `OnRep_FilterSpawned?`
  (if (`self.FilterSpawned?`)
    (`PrimitiveComponent.SetMaterial` (`self.Sphere`) 0 "/Game/Assets/Props/Lightswitch/ActiveOn.ActiveOn")
    (message `/Game/Blueprints/Interfaces/BPI_FilterStats.SetCoolerFilterStatus` (`GameplayStatics.GetGameState`) false true false)
    (`self.Local_CoolerReady`)))

(fn `UserConstructionScript`)