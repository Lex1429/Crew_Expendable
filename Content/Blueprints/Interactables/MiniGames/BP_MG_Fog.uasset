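; BP_MG_Fog is a minigame fog effect that clears once the referenced AC filter is repaired.
; On BeginPlay it binds its FansOnline event to the AC filter's repaired notification, which triggers ClearFog.
; A timeline then lerps the Niagara SpawnRate parameter down to zero and destroys the Niagara component when it finishes.
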(event `self.ReceiveBeginPlay`
  (add `/Game/Blueprints/Interactables/MiniGames/BP_MG_AirVent.ACRepaired` (`self.ACFilterRef`) (delegate `FansOnline`)))

(event `FansOnline`
  (`self.ClearFog`))

(event `ClearFog`
  (bind (_direction _newtrack_0) (`Timeline|FogClear`)
    (:`Update`
      (`FXSystemComponent.SetFloatParameter` (`self.Niagara`) "SpawnRate" (`KismetMathLibrary.Lerp` 50.0 0.0 _newtrack_0)))
    (:`Finished`
      (`ActorComponent.K2_DestroyComponent` (`self.Niagara`)))))

(fn `UserConstructionScript`)