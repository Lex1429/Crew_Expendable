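; BP_TunnelVent is a level-prop vent that teleports the BP_SAL actor to a linked station vent.
; On overlap it waits three seconds, then casts the overlapping actor to BP_SAL and its VentTarget to BP_StationVent.
; It moves SAL to that vent's SpawnPoint with zeroed rotation and turns off the game state's can-vent message.
; The construction script caches its own SpawnPoint relative location as SpawnLocation.
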(event `self.ReceiveActorBeginOverlap`
  (params (OtherActor :type "Actor Object Reference"))
  (`KismetSystemLibrary.Delay` 3.0)
  (bind _asbp_sal (cast `/Game/Blueprints/AI/Enemies/BP_SAL` OtherActor))
  (bind _asbp_station_vent (cast `/Game/Blueprints/Interactables/LevelProps/BP_StationVent` (`self.VentTarget`)))
  (`self.K2_TeleportTo` :`self` _asbp_sal :`DestLocation` (`SceneComponent.K2_GetComponentLocation` (`/Game/Blueprints/Interactables/LevelProps/BP_StationVent.SpawnPoint` _asbp_station_vent)))
  (message `/Game/Blueprints/Interfaces/BPI_SALStats.SetCanVent` (`GameplayStatics.GetGameState`) false))

(fn `UserConstructionScript`
  (set `self.SpawnLocation` (`SceneComponent.RelativeLocation` (`self.SpawnPoint`))))