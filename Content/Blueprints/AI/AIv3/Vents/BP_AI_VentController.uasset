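; BP_AI_VentController hands out vent locations for the AI in a randomized rotation.
; It shuffles its vent array on BeginPlay, then each SelectNextVent call stores the current vent's actor location in SelectedVentLocation and advances the index.
; After the fifth pick it resets the index and reshuffles, a shuffle-bag cycle that relies on a hard-coded last index rather than the array length.
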(event `self.ReceiveBeginPlay`
  (`self.ShuffleVentList`))

(event `SelectNextVent`
  (set `self.SelectedVentLocation` (`self.K2_GetActorLocation` (`|GetArrayItem` (`self.VentsArray`) (`self.VentIndex`))))
  (if (== (`self.VentIndex`) 4)
    (set `self.VentIndex` 0)
    (`self.ShuffleVentList`)
    (else
      (`/Engine/EditorBlueprintResources/StandardMacros.IncrementInt` (`self.VentIndex`)))))

(fn `ShuffleVentList`
  (`KismetArrayLibrary.Array_Shuffle` (`self.VentsArray`)))

(fn `UserConstructionScript`)