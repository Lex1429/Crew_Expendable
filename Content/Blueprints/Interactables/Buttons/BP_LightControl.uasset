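; BP_LightControl is an interactable touch panel that switches the lamps of a room on and off.
; Interact routes through server and local switch events, which toggle every BP_LampBase with a matching RoomTag via its server light calls, or force them off when the sector is unpowered.
; The panel's material follows the light state, and its box overlap adds or clears an outline overlay.
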(event `Local_Lightswitch`
  (bind _outactors (`GameplayStatics.GetAllActorsOfClass` "/Game/Blueprints/Interactables/CealingLights/BP_LampBase.BP_LampBase_C"))
  (for _array_element _outactors
    (if (== (`/Game/Blueprints/Interactables/CealingLights/BP_LampBase.RoomTag` _array_element) (`self.RoomTag`))
      (if (`self.SectorPowered`)
        (if (`/Game/Blueprints/Interactables/CealingLights/BP_LampBase.IsLightOn?` _array_element)
          (`/Game/Blueprints/Interactables/CealingLights/BP_LampBase.Server_LightOff` _array_element :!label _label)
          (`PrimitiveComponent.SetMaterial` (`self.TouchPanel`) 0 "/Game/PolygonSciFiSpace/Materials/Alternates/MI_PolygonSciFiSpace_01_A.MI_PolygonSciFiSpace_01_A")
          (else
            (`/Game/Blueprints/Interactables/CealingLights/BP_LampBase.Server_LightOn` _array_element)
            (`PrimitiveComponent.SetMaterial` (`self.TouchPanel`) 0 "/Game/PolygonSciFiSpace/Materials/Alternates/MI_PolygonSciFiSpace_01_B.MI_PolygonSciFiSpace_01_B")))
        (else
          (goto _label))))))

(event `Server_LightSwitch`
  (`self.Local_Lightswitch`))

(event `/Game/Blueprints/Interfaces/BPI_Interact.Interact`
  (params (Character :type "/Game/Blueprints/Characters/BP_BaseCharacter Object Reference"))
  (`self.Server_LightSwitch`))

(event `self.Box.OnComponentBeginOverlap`
  (params (OverlappedComponent :type "PrimitiveComponent Object Reference") (OtherActor :type "Actor Object Reference") (OtherComp :type "PrimitiveComponent Object Reference") (OtherBodyIndex :type Integer) (bFromSweep :type Boolean) (SweepResult :type "HitResult Structure (by ref)"))
  (`MeshComponent.SetOverlayMaterial` (`self.TouchPanel`) "/Game/Materials/M_Outline.M_Outline"))

(event `self.Box.OnComponentEndOverlap`
  (params (OverlappedComponent :type "PrimitiveComponent Object Reference") (OtherActor :type "Actor Object Reference") (OtherComp :type "PrimitiveComponent Object Reference") (OtherBodyIndex :type Integer))
  (`MeshComponent.SetOverlayMaterial` (`self.TouchPanel`) null))

(fn `UserConstructionScript`)