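; Modular furnished small-room building piece that switches between "On" and "Off" materials based on occupancy.
; RoomSensor overlaps raise and lower PersonCount, swapping the SmallRoom material on while occupied and off when empty.
; RoomTag selects the material set: Sector 1 for the eight Quarters tags, Sector 2 for Lockers.
; The construction script applies BuildingMaterial and sets the height of the four legs from LegLength.
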(event `self.RoomSensor.OnComponentBeginOverlap`
  (params (OverlappedComponent :type "PrimitiveComponent Object Reference") (OtherActor :type "Actor Object Reference") (OtherComp :type "PrimitiveComponent Object Reference") (OtherBodyIndex :type Integer) (bFromSweep :type Boolean) (SweepResult :type "HitResult Structure (by ref)"))
  (bind _smallroom (`self.SmallRoom`))
  (bind _result (`/Engine/EditorBlueprintResources/StandardMacros.IncrementInt` (`self.PersonCount`))
    (:`  `
      (if (> _result 0)
        (`|SwitchGameplayTagContainer` (`self.RoomTag`)
          (:`(GameplayTags=((TagName="Sector1.Quarters.1")))`
            (`PrimitiveComponent.SetMaterial` _smallroom 0 "/Game/Materials/CustomTextures/V1Materials/M_Sector1_On.M_Sector1_On" :!label _label))
          (:`(GameplayTags=((TagName="Sector1.Quarters.2")))`
            (goto _label))
          (:`(GameplayTags=((TagName="Sector1.Quarters.3")))`
            (goto _label))
          (:`(GameplayTags=((TagName="Sector1.Quarters.4")))`
            (goto _label))
          (:`(GameplayTags=((TagName="Sector1.Quarters.5")))`
            (goto _label))
          (:`(GameplayTags=((TagName="Sector1.Quarters.6")))`
            (goto _label))
          (:`(GameplayTags=((TagName="Sector1.Quarters.7")))`
            (goto _label))
          (:`(GameplayTags=((TagName="Sector1.Quarters.8")))`
            (goto _label))
          (:`(GameplayTags=((TagName="Sector2.Lockers")))`
            (`PrimitiveComponent.SetMaterial` _smallroom 0 "/Game/Materials/CustomTextures/V1Materials/M_Sector2_On.M_Sector2_On")))))))

(event `self.RoomSensor.OnComponentEndOverlap`
  (params (OverlappedComponent :type "PrimitiveComponent Object Reference") (OtherActor :type "Actor Object Reference") (OtherComp :type "PrimitiveComponent Object Reference") (OtherBodyIndex :type Integer))
  (bind _smallroom (`self.SmallRoom`))
  (bind _result (`/Engine/EditorBlueprintResources/StandardMacros.DecrementInt` (`self.PersonCount`))
    (:`  `
      (if (<= _result 0)
        (`|SwitchGameplayTagContainer` (`self.RoomTag`)
          (:`(GameplayTags=((TagName="Sector1.Quarters.1")))`
            (`PrimitiveComponent.SetMaterial` _smallroom 0 "/Game/Materials/CustomTextures/V1Materials/M_Sector1_OffRooms.M_Sector1_OffRooms" :!label _label_2))
          (:`(GameplayTags=((TagName="Sector1.Quarters.2")))`
            (goto _label_2))
          (:`(GameplayTags=((TagName="Sector1.Quarters.3")))`
            (goto _label_2))
          (:`(GameplayTags=((TagName="Sector1.Quarters.4")))`
            (goto _label_2))
          (:`(GameplayTags=((TagName="Sector1.Quarters.5")))`
            (goto _label_2))
          (:`(GameplayTags=((TagName="Sector1.Quarters.6")))`
            (goto _label_2))
          (:`(GameplayTags=((TagName="Sector1.Quarters.7")))`
            (goto _label_2))
          (:`(GameplayTags=((TagName="Sector1.Quarters.8")))`
            (goto _label_2))
          (:`(GameplayTags=((TagName="Sector2.Lockers")))`
            (`PrimitiveComponent.SetMaterial` _smallroom 0 "/Game/Materials/CustomTextures/V1Materials/M_Sector2_OffRooms.M_Sector2_OffRooms")))))))

(fn `UserConstructionScript`
  (bind _leglength (`self.LegLength`))
  (`PrimitiveComponent.SetMaterial` (`self.SmallRoom`) 0 (`self.BuildingMaterial`))
  (`SceneComponent.K2_SetRelativeLocation` (`self.Leg1`) (`KismetMathLibrary.MakeVector` 0.0 0.0 _leglength) false false)
  (`SceneComponent.K2_SetRelativeLocation` (`self.Leg2`) (`KismetMathLibrary.MakeVector` 0.0 0.0 _leglength) false false)
  (`SceneComponent.K2_SetRelativeLocation` (`self.Leg3`) (`KismetMathLibrary.MakeVector` 0.0 0.0 _leglength) false false)
  (`SceneComponent.K2_SetRelativeLocation` (`self.Leg4`) (`KismetMathLibrary.MakeVector` 0.0 0.0 _leglength) false false))