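; BP_SalvageDropOff is an interactable drop-off container where a character turns in the held item as salvage.
; A timeline swings the lid open on actor overlap and reverses when overlap ends.
; Interact looks up the current weapon's item name in DT_SalvageList and adds its value to the GameState's salvage amount.
; For valid items, it then spawns a half-scale pickup at ItemSpawnPoint and destroys the held item.
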(event `self.ReceiveActorBeginOverlap`
  (params (OtherActor :type "Actor Object Reference"))
  (bind (_direction _newtrack_0) (`Timeline|LidMovement` :!label _label)
    (:`Update`
      (`SceneComponent.K2_SetRelativeRotation` (`self.Lid`) (`KismetMathLibrary.RLerp` (struct) (struct :`Roll` -125.0) _newtrack_0) false false))))

(event `self.ReceiveActorEndOverlap`
  (params (OtherActor :type "Actor Object Reference"))
  (goto _label :!via `Reverse`))

(event `/Game/Blueprints/Interfaces/BPI_Interact.Interact`
  (params (Character :type "/Game/Blueprints/Characters/BP_BaseCharacter Object Reference"))
  (bind _returnvalue (`GameplayStatics.GetGameState`))
  (bind _output_get (set `self.DroppedItem` (`/Game/Blueprints/Interactables/Weapons/BP_WeaponComponentMaster.ItemName` (`/Game/Blueprints/Characters/BP_BaseCharacter.GetCurrentWeapon` Character))))
  (bind _returnvalue_2 (`|GetDataTableRow` "/Game/Blueprints/Salvage/DT_SalvageList.DT_SalvageList" _output_get)
    (:`then`
      (bind _salvage (message `/Game/Blueprints/Interfaces/BPI_Stats.GetSalvageAmount` _returnvalue))
      (message `/Game/Blueprints/Interfaces/BPI_Stats.SetSalvageAmount` _returnvalue (+ _salvage (`.Value_15_F222FCC64FCAB1A8F20AACB203483459` (break `/Game/Blueprints/Salvage/S_Salvage` _returnvalue_2))))
      (`self.Local_DropOff` Character))))

(event `Local_DropOff`
  (params (Character :type "/Game/Blueprints/Characters/BP_BaseCharacter Object Reference"))
  (`|SpawnActorFromClass` (`/Game/Blueprints/Interactables/Weapons/BP_WeaponComponentMaster.PickupClass` (`/Game/Blueprints/Characters/BP_BaseCharacter.GetCurrentWeapon` Character)) (`KismetMathLibrary.MakeTransform` (`SceneComponent.K2_GetComponentLocation` (`self.ItemSpawnPoint`)) (struct) (0.5 0.5 0.5)) "Undefined" "MultiplyWithRoot" null null)
  (`/Game/Blueprints/Characters/BP_BaseCharacter.DestroyCurrentItem` Character))

(fn `UserConstructionScript`)