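; Lobby player controller that handles the escape menu and a loading screen.
; Escape opens WB_EscapeMenu with UI-only input and a visible cursor, using a MenuUpMessage flag on the game instance to block duplicates.
; CreateLoadScreen shows WB_LoadingScreenSphere, creating the widget only when the cached reference is invalid.
; BeginPlay loads the "settings" save slot if it exists, but does not use the result.
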(event `CreateLoadScreen`
  (`self.LoadScreen`))

(event `self.ReceiveBeginPlay`
  (bind _returnvalue (`GameplayStatics.GetPlayerControllerID` (`GameplayStatics.GetPlayerController` 0)))
  (bind _returnvalue_2 (`GameplayStatics.DoesSaveGameExist` "settings" _returnvalue))
  (if _returnvalue_2
    (`GameplayStatics.LoadGameFromSlot` "settings" _returnvalue)))

(event `Key|Escape`
  (params (Key :type "Key Structure"))
  (:`Pressed`
    (bind _menuup (message `/Game/Blueprints/Interfaces/BPI_PlayerSettings.GetMenuUp` (`GameplayStatics.GetGameInstance`)))
    (if (not _menuup)
      (bind _returnvalue (`|CreateWidget` "/Game/UI/WB_EscapeMenu.WB_EscapeMenu_C" (`GameplayStatics.GetPlayerController` 0)))
      (`UserWidget.AddToPlayerScreen` _returnvalue 0)
      (`WidgetBlueprintLibrary.SetInputMode_UIOnlyEx` (`GameplayStatics.GetPlayerController` 0) _returnvalue "DoNotLock" true)
      (set `self.bShowMouseCursor` true)
      (message `/Game/Blueprints/Interfaces/BPI_PlayerSettings.SetMenuUp` (`GameplayStatics.GetGameInstance`) true))))

(fn `LoadScreen`
  (`/Engine/EditorBlueprintResources/StandardMacros.IsValid` (`self.LoadScreenRef`)
    (:`Is Valid`
      _)
    (:`Is Not Valid`
      (bind _returnvalue (`|CreateWidget` "/Game/UI/WB_LoadingScreenSphere.WB_LoadingScreenSphere_C" self))
      (bind _output_get (set `self.LoadScreenRef` _returnvalue))))
  (`UserWidget.AddToViewport` _output_get 0)
  (return))

(fn `UserConstructionScript`)