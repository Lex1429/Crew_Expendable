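; Test minigame interactable that cannot be picked up and opens a hacking test widget for the interacting player.
; It creates WB_HackTest at BeginPlay, then shows it on local interaction with UI-only input and a cursor until the game is complete.
; The widget's completion callback removes it, restores game input, marks completion and prints a debug string.
; A separate ServerCall event forwards to CallCompletedGame.
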(event `self.ReceiveBeginPlay`
  (bind _returnvalue (`|CreateWidget` "/Game/UI/HackerGame/WB_HackTest.WB_HackTest_C"))
  (bind _output_get (set `self.WidgetRef` _returnvalue))
  (add `/Game/UI/HackerGame/WB_HackTest.GameCompleted` _output_get (delegate `GameFinished`)))

(event `/Game/Blueprints/Interfaces/BPI_MGInteract.MGInteractLocal`
  (params (Player :type "/Game/Blueprints/Characters/BP_PlayerCharacterCore Object Reference"))
  (bind _returnvalue (`Pawn.GetLocalViewingPlayerController` Player))
  (bind _widgetref (`self.WidgetRef`))
  (if (not (`self.GameComplete?`))
    (`UserWidget.AddToViewport` _widgetref 0)
    (`WidgetBlueprintLibrary.SetInputMode_UIOnlyEx` _returnvalue _widgetref "LockOnCapture")
    (set `PlayerController.bShowMouseCursor` true _returnvalue)))

(event `GameFinished`
  (`Widget.RemoveFromParent` (`self.WidgetRef`))
  (`WidgetBlueprintLibrary.SetInputMode_GameOnly` (`Pawn.GetLocalViewingPlayerController` (stale `/Game/Blueprints/Interfaces/BPI_MGInteract.MGInteractLocal` Player)))
  (set `self.GameComplete?` true)
  (`KismetSystemLibrary.PrintString` "MGTestOwner" true true (struct :`G` 1.0 :`A` 1.0) 10.0))

(event `ServerCall`
  (`self.CompletedGame`))

(fn `GetCanBePickedUp`
  (returns (CanBePickedUp :type Boolean))
  (return false))

(fn `GetItemToSpawn`
  (returns (Item :type "/Game/Blueprints/Interactables/Weapons/BP_WeaponComponentMaster Class Reference"))
  (return null))

(fn `UserConstructionScript`)