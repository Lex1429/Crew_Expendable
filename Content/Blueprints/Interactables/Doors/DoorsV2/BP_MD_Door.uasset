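; BP_MD_Door is an interactable split door that slides top and bottom halves open or closed, and cannot be picked up.
; Interact routes through server and local activation events to a toggle that, unless locked, plays or reverses a timeline lerping both halves' relative locations.
; An automatic mode for the Corpo minigame sets a flag and starts StateTree logic.
; The construction script applies configurable door and frame materials.
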(event `SetDoorsToAutomatic`
  ;[1 0.5 0] Automatic door system for Corpo Minigame
  (set `self.Automatic?` true)
  (`BrainComponent.StartLogic` (`self.StateTree`)))

(event `/Game/Blueprints/Interfaces/BPI_Interact.Interact`
  (params (Character :type "/Game/Blueprints/Characters/BP_BaseCharacter Object Reference") (PlayerCharacter :type "/Game/Blueprints/Characters/BP_PlayerCharacterCore Object Reference"))
  (`self.Server_ActivateDoor`))

(event `Server_ActivateDoor`
  (`self.Local_ActivateDoor`))

(event `Local_ActivateDoor`
  (`self.ActivateDoor`))

(event `ActivateDoor`
  (if (not (`self.Locked?`))
    (if (not (`self.Open?`))
      (set `self.Open?` true)
      (bind (_direction _newtrack_0) (`Timeline|SplitDoor` :!label _label)
        (:`Update`
          (`SceneComponent.K2_SetRelativeLocation` (`self.DoorTop`) (`KismetMathLibrary.VLerp` (`self.TopClosed`) (`self.TopOpen`) _newtrack_0) false false)
          (`SceneComponent.K2_SetRelativeLocation` (`self.DoorBottom`) (`KismetMathLibrary.VLerp` (`self.BottomClosed`) (`self.BottomOpen`) _newtrack_0) false false)))
      (else
        (set `self.Open?` false)
        (goto _label :!via `Reverse`)))))

(fn `GetCanBePickedUp`
  (returns (CanBePickedUp :type Boolean))
  (return false))

(fn `GetItemToSpawn`
  (returns (Item :type "/Game/Blueprints/Interactables/Weapons/BP_WeaponComponentMaster Class Reference"))
  (return null))

(fn `UserConstructionScript`
  (bind _doormaterial (`self.DoorMaterial`))
  (`PrimitiveComponent.SetMaterial` (`self.DoorBottom`) 0 _doormaterial)
  (`PrimitiveComponent.SetMaterial` (`self.DoorTop`) 0 _doormaterial)
  (`PrimitiveComponent.SetMaterial` (`self.DoorFrame`) 0 (`self.FrameMaterial`))
  (`PrimitiveComponent.SetMaterial` (`self.DoorFrame`) 1 (`self.FrameMaterial2`))
  (`PrimitiveComponent.SetMaterial` (`self.DoorFrame`) 2 (`self.FrameMaterial3`)))