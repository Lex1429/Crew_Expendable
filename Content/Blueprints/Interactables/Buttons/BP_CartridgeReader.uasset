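; Interactable cartridge dock that unlocks a linked object when a player holding the cartridge item uses it.
; Insertion runs through the server, spawns a cartridge pickup in the dock, switches the screen material and clears the item from the player.
; Any end overlap on the box clears the inserted state, relocks and shows the error screen.
; The removal OnRep also re-equips the cartridge on the stored player; mission-log reporting is disconnected.
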(event `Server_InsertCartridge`
  (params (Player :type "/Game/Blueprints/Characters/BP_PlayerCharacterCore Object Reference"))
  (bind _cartridgespawn (`self.CartridgeSpawn`))
  (`|SpawnActorFromClass` "/Game/Blueprints/EquipmentSystem/BP_CoreEquipmentPickup.BP_CoreEquipmentPickup_C" (`KismetMathLibrary.MakeTransform` (`SceneComponent.K2_GetComponentLocation` _cartridgespawn) (`SceneComponent.K2_GetComponentRotation` _cartridgespawn)) "AdjustIfPossibleButAlwaysSpawn" "MultiplyWithRoot" null "15" null :!label _label)
  (`self.Local_InsertCartridge`)
  (`self.Owner_InsertCartridge` (`self.Player Ref`)))

(event `/Game/Blueprints/Interfaces/BPI_Interact.Interact`
  (params (Character :type "Object Object Reference") (PlayerCharacter :type "/Game/Blueprints/Characters/BP_PlayerCharacterCore Object Reference"))
  (bind _output_get (set `self.Player Ref` PlayerCharacter))
  (`/Engine/EditorBlueprintResources/StandardMacros.IsValid` _output_get
    (:`Is Valid`
      (if (not (`self.CartridgeInserted?`))
        (if (== (`/Game/Blueprints/Characters/BP_PlayerCharacterCore.CurrentEquipmentHeld` _output_get) "15")
          (`/Engine/EditorBlueprintResources/ActorMacros.Switch Has Authority`
            (:`Authority`
              (goto _label))
            (:`Remote`
              (`self.Server_InsertCartridge` (`self.Player Ref`)))))))
    (:`Is Not Valid`
      (`KismetSystemLibrary.PrintString` "NO PLAYER FOUND"))))

(event `self.Box.OnComponentEndOverlap`
  (params (OverlappedComponent :type "PrimitiveComponent Object Reference") (OtherActor :type "Actor Object Reference") (OtherComp :type "PrimitiveComponent Object Reference") (OtherBodyIndex :type Integer))
  (`self.Server_RemoveCartridge`)
  (`self.LockedObject`)
  (`PrimitiveComponent.SetMaterial` (`self.SM_Prop_Cartridge_Dock_01`) 1 "/Game/Synty/PolygonSciFiHorror/Materials/Misc/Screens/MI_PolygonSciFiHorror_Screens_Error_07.MI_PolygonSciFiHorror_Screens_Error_07"))

(event `Server_RemoveCartridge`
  (set `self.CartridgeInserted?` false))

(event `Local_InsertCartridge`
  (`PrimitiveComponent.SetMaterial` (`self.SM_Prop_Cartridge_Dock_01`) 1 "/Game/Synty/PolygonSciFiHorror/Materials/Misc/Screens/MI_PolygonSciFiHorror_Screens_01.MI_PolygonSciFiHorror_Screens_01")
  (`self.UnlockedObject`)
  (set `self.CartridgeInserted?` true))

(event `Owner_InsertCartridge`
  (params (Player :type "/Game/Blueprints/Characters/BP_PlayerCharacterCore Object Reference"))
  (`/Game/Blueprints/Characters/BP_PlayerCharacterCore.RemoveItemFromInventory` Player)
  (`/Game/Blueprints/Characters/BP_PlayerCharacterCore.Server_SetHeldEquipment` Player "1"))

(fn `GetCanBePickedUp`
  (returns (CanBePickedUp :type Boolean))
  (return false))

(fn `GetItemToSpawn`
  (returns (Item :type "/Game/Blueprints/Interactables/Weapons/BP_WeaponComponentMaster Class Reference"))
  (return null))

(fn `OnRep_CartridgeInserted?`
  (if (not (`self.CartridgeInserted?`))
    (`self.LockedObject`)
    (`PrimitiveComponent.SetMaterial` (`self.SM_Prop_Cartridge_Dock_01`) 1 "/Game/Synty/PolygonSciFiHorror/Materials/Misc/Screens/MI_PolygonSciFiHorror_Screens_Error_07.MI_PolygonSciFiHorror_Screens_Error_07")
    (`/Game/Blueprints/Characters/BP_PlayerCharacterCore.Server_SetHeldEquipment` (`self.Player Ref`) "15")))

(fn `QueryAsset`
  (returns (Asset :type "/Game/Blueprints/InventorySystem/Pickups/Data/PDA_Items Object Reference"))
  (return null))

(fn `QueryItem`
  (returns (Item :type Name))
  (return "None"))

(fn `UserConstructionScript`)