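; BP_MapTable is an interactable map table prop in the lobby that opens the lobby menu.
; Interact calls ToggleWBLobbyMenu on the BP_PC_Lobby player controller cached at BeginPlay.
; A looping timer steadily yaws the Destination component as an idle spin.
; Overlapping its Box applies the M_Outline overlay material to both table meshes, and leaving clears it.
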(event `self.ReceiveBeginPlay`
  (`|ExecutionSequence`
    (:`then_0`
      (bind _asbp_pc_lobby (cast `/Game/MBLS/Blueprints/Core/Lobby/Player/BP_PC_Lobby` (`GameplayStatics.GetPlayerController` 0)))
      (set `self.As BP PC Lobby` _asbp_pc_lobby))
    (:`then_1`
      (`KismetSystemLibrary.K2_SetTimerDelegate` (delegate `RotateDestination`) 0.1 true))))

(event `RotateDestination`
  (`SceneComponent.K2_AddRelativeRotation` (`self.Destination`) (`KismetMathLibrary.MakeRotator` 0.0 0.0 (`self.RotationRate`)) false false))

(event `/Game/Blueprints/Interfaces/BPI_Interact.Interact`
  (params (Character :type "/Game/Blueprints/Characters/BP_BaseCharacter Object Reference"))
  (`/Game/MBLS/Blueprints/Core/Lobby/Player/BP_PC_Lobby.Toggle_WB_Lobby_Menu` (`self.As BP PC Lobby`)))

(event `self.Box.OnComponentBeginOverlap`
  (params (OverlappedComponent :type "PrimitiveComponent Object Reference") (OtherActor :type "Actor Object Reference") (OtherComp :type "PrimitiveComponent Object Reference") (OtherBodyIndex :type Integer) (bFromSweep :type Boolean) (SweepResult :type "HitResult Structure (by ref)"))
  (`MeshComponent.SetOverlayMaterial` (`self.SM_Prop_MapTable_Top_01`) "/Game/Materials/M_Outline.M_Outline")
  (`MeshComponent.SetOverlayMaterial` (`self.SM_Prop_MapTable_01`) "/Game/Materials/M_Outline.M_Outline"))

(event `self.Box.OnComponentEndOverlap`
  (params (OverlappedComponent :type "PrimitiveComponent Object Reference") (OtherActor :type "Actor Object Reference") (OtherComp :type "PrimitiveComponent Object Reference") (OtherBodyIndex :type Integer))
  (`MeshComponent.SetOverlayMaterial` (`self.SM_Prop_MapTable_Top_01`) null)
  (`MeshComponent.SetOverlayMaterial` (`self.SM_Prop_MapTable_01`) null))

(fn `UserConstructionScript`)