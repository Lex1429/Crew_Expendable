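; BP_Offices_02 is a prebuilt office room actor whose left and right walls can be shown or hidden.
; Its construction script reads the LeftWallVisible and RightWallVisible booleans and sets visibility on each side's three wall meshes, along with that side's control panel and chair props.
; The event graph has no runtime logic, so the layout is determined only at construction.
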(fn `UserConstructionScript`
  (bind _sm_bld_base_wall_408_staticmeshcomponent0 (`self.SM_Bld_Base_Wall_408_StaticMeshComponent0`))
  (`|ExecutionSequence`
    (:`then_0`
      (if (`self.LeftWallVisible?`)
        (`SceneComponent.SetVisibility` _sm_bld_base_wall_408_staticmeshcomponent0 true false)
        (`SceneComponent.SetVisibility` (`self.SM_Bld_Base_Wall_372_StaticMeshComponent0`) true false)
        (`SceneComponent.SetVisibility` (`self.SM_Bld_Base_Wall_345_StaticMeshComponent0`) true false)
        (`SceneComponent.SetVisibility` (`self.SM_Prop_ControlPanel_06`) true false)
        (`SceneComponent.SetVisibility` (`self.SM_Prop_Chair_05`) true false)
        (else
          (`SceneComponent.SetVisibility` _sm_bld_base_wall_408_staticmeshcomponent0 false false)
          (`SceneComponent.SetVisibility` (`self.SM_Bld_Base_Wall_372_StaticMeshComponent0`) false false)
          (`SceneComponent.SetVisibility` (`self.SM_Bld_Base_Wall_345_StaticMeshComponent0`) false false)
          (`SceneComponent.SetVisibility` (`self.SM_Prop_ControlPanel_06`) false false)
          (`SceneComponent.SetVisibility` (`self.SM_Prop_Chair_05`) false false))))
    (:`then_1`
      (if (`self.RightWallVisible?`)
        (`SceneComponent.SetVisibility` (`self.SM_Bld_Base_Wall_501_StaticMeshComponent0`) true false)
        (`SceneComponent.SetVisibility` (`self.SM_Bld_Base_Wall_524_StaticMeshComponent0`) true false)
        (`SceneComponent.SetVisibility` (`self.SM_Bld_Base_Wall_552_StaticMeshComponent0`) true false)
        (`SceneComponent.SetVisibility` (`self.SM_Prop_ControlPanel_04`) true false)
        (`SceneComponent.SetVisibility` (`self.SM_Prop_Chair_03`) true false)
        (else
          (`SceneComponent.SetVisibility` (`self.SM_Bld_Base_Wall_552_StaticMeshComponent0`) false false)
          (`SceneComponent.SetVisibility` (`self.SM_Bld_Base_Wall_524_StaticMeshComponent0`) false false)
          (`SceneComponent.SetVisibility` (`self.SM_Bld_Base_Wall_501_StaticMeshComponent0`) false false)
          (`SceneComponent.SetVisibility` (`self.SM_Prop_ControlPanel_04`) false false)
          (`SceneComponent.SetVisibility` (`self.SM_Prop_Chair_03`) false false))))))