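; Main menu player controller that runs the game's intro sequence and hands off to the title screen.
; On BeginPlay it sets the game instance's server search message, plays 2D music and shows a splash screen widget for a fixed delay.
; It then swaps in the title screen widget, sets game-and-UI input focused on it and shows the mouse cursor.
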(event `self.ReceiveBeginPlay`
  (message `/Game/Blueprints/Interfaces/BPI_Server.SetServerSearch` (`GameplayStatics.GetGameInstance`) (struct))
  (`GameplayStatics.PlaySound2D` "/Game/SFX/apocalypse-153277.apocalypse-153277" 1.0 1.0 0.0 null null)
  (bind _returnvalue (`|CreateWidget` "/Game/UI/WB_SplashScreens.WB_SplashScreens_C" (`GameplayStatics.GetPlayerController` 0)))
  (`UserWidget.AddToViewport` _returnvalue 0)
  (`KismetSystemLibrary.Delay` 15.0)
  (`Widget.RemoveFromParent` _returnvalue)
  (bind _returnvalue_2 (`|CreateWidget` "/Game/UI/WB_TitleScreen.WB_TitleScreen_C" (`GameplayStatics.GetPlayerController` 0) "" "Expendable"))
  (`UserWidget.AddToViewport` _returnvalue_2 0)
  (`WidgetBlueprintLibrary.SetInputMode_GameAndUIEx` (`GameplayStatics.GetPlayerController` 0) _returnvalue_2)
  (set `self.bShowMouseCursor` true))

(fn `UserConstructionScript`)