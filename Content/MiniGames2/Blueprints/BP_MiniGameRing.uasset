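; Interactive ring-puzzle mini-game: on action in its trigger box, the camera blends to a screen where the player aligns four rings with a randomized base ring.
; A looping timer polls latched axis input to select a ring or step it one of 48 sectors, checking indices for success.
; Tick and decor updates drive a dynamic material that renders the puzzle.
; Starting also overrides TAA frame weight; success or cancel returns the camera.
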(event `self.ReceiveBeginPlay`
  ;[1 1 1] Init
  (`parent.ReceiveBeginPlay`)
  (bind _returnvalue (`KismetSystemLibrary.K2_SetTimer` null "CheckContorls" 0.05 true))
  (bind _output_get (set `self.TimeHandle` _returnvalue))
  (`KismetSystemLibrary.K2_UnPauseTimerHandle` _output_get)
  (bind _returnvalue_2 (`KismetSystemLibrary.K2_SetTimer` null "UpdateDecor" 0.15 true))
  (set `self.DecorTimeHandle` _returnvalue_2)
  ;;[1 1 1] Create Dynamic Material Instance
  (bind _returnvalue_3 (`KismetMaterialLibrary.CreateDynamicMaterialInstance` "/Game/MiniGames2/Materials/MI_MiniGamesRing_Inst.MI_MiniGamesRing_Inst"))
  (set `self.DMI` _returnvalue_3)
  (set `self.InputEnable` false)
  (set `self.IsMiniGameActivated` false))

(event `InitGame`
  (bind _dmi (`self.DMI`))
  ;[1 1 1] ReInit game
  (bind _returnvalue (`KismetSystemLibrary.GetConsoleVariableFloatValue` "r.TemporalAACurrentFrameWeight"))
  (set `self.GameTAACurrFrameWeight` _returnvalue)
  (`KismetSystemLibrary.ExecuteConsoleCommand` (`GameplayStatics.GetPlayerController` 0) "r.TemporalAACurrentFrameWeight 0.15" null)
  (set `self.Selector` 0)
  (set `self.RotAngle` (/ 1.0 48.0))
  ;;[1 1 1] Randomize ring segments
  (`MaterialInstanceDynamic.SetScalarParameterValue` (`self.DMI`) "TopLeft" (`KismetMathLibrary.SelectFloat` 0.0 1.0 (>= (`KismetMathLibrary.RandomIntegerInRange` 0 10) 5)))
  (`MaterialInstanceDynamic.SetScalarParameterValue` (`self.DMI`) "TopRight" (`KismetMathLibrary.SelectFloat` 0.0 1.0 (>= (`KismetMathLibrary.RandomIntegerInRange` 0 10) 5)))
  (`MaterialInstanceDynamic.SetScalarParameterValue` (`self.DMI`) "BottomRight" (`KismetMathLibrary.SelectFloat` 0.0 1.0 (>= (`KismetMathLibrary.RandomIntegerInRange` 0 10) 5)))
  (`MaterialInstanceDynamic.SetScalarParameterValue` (`self.DMI`) "BottomLeft" (`KismetMathLibrary.SelectFloat` 0.0 1.0 (>= (`KismetMathLibrary.RandomIntegerInRange` 0 10) 5)))
  ;;[1 1 1] Randomize rings rotation
  (bind _output_get (set `self.BaseRing_index` (`|GetArrayItem` (`self.NaturalRandomMap`) (`KismetMathLibrary.RandomIntegerInRange` 0 23))))
  (bind _output_get_2 (set `self.RingBaseAngle` (* _output_get (`self.RotAngle`))))
  (`MaterialInstanceDynamic.SetScalarParameterValue` _dmi "RotationRingBase" _output_get_2)
  (bind _output_get_3 (set `self.Ring1_Index` (`KismetMathLibrary.RandomIntegerInRange` 0 47)))
  (bind _output_get_4 (set `self.Ring01_Angle` (* _output_get_3 (`self.RotAngle`))))
  (`MaterialInstanceDynamic.SetScalarParameterValue` _dmi "RotationRing1" _output_get_4)
  (bind _output_get_5 (set `self.Ring2_Index` (`KismetMathLibrary.RandomIntegerInRange` 0 47)))
  (bind _output_get_6 (set `self.Ring02_Angle` (* _output_get_5 (`self.RotAngle`))))
  (`MaterialInstanceDynamic.SetScalarParameterValue` _dmi "RotationRing2" _output_get_6)
  (bind _output_get_7 (set `self.Ring3_Index` (`KismetMathLibrary.RandomIntegerInRange` 0 47)))
  (bind _output_get_8 (set `self.Ring03_Angle` (* _output_get_7 (`self.RotAngle`))))
  (`MaterialInstanceDynamic.SetScalarParameterValue` _dmi "RotationRing3" _output_get_8)
  (bind _output_get_9 (set `self.Ring4_Index` (`KismetMathLibrary.RandomIntegerInRange` 0 47)))
  (bind _output_get_10 (set `self.Ring04_Angle` (* _output_get_9 (`self.RotAngle`))))
  (`MaterialInstanceDynamic.SetScalarParameterValue` _dmi "RotationRing4" _output_get_10)
  (`MaterialInstanceDynamic.SetScalarParameterValue` (`self.DMI`) "ShowGranted" 0.0))

(event `CheckContorls`
  (bind _rightaxis (`self.RightAxis`))
  (bind _forwardaxis (`self.ForwardAxis`))
  (bind _basering_index (`self.BaseRing_index`))
  ;[1 1 1] Controls
  (if (`self.InputEnable`)
    (if (`self.IsMiniGameActivated`)
      (`|ExecutionSequence`
        (:`then_0`
          (if (!= _rightaxis 0.0)
            (if (`self.RightAxisEnable`)
              (set `self.RightAxisEnable` false)
              (set `self.RotationDirection` (* (`KismetMathLibrary.SignOfFloat` _rightaxis) -1.0))
              (`self.UpdateDecor2`)
              (switch `int` (`self.Selector`)
                (:`0`
                  (bind _result (`self.GetClamedAngle` (+ (`self.Ring01_Angle`) (* (`self.RotationDirection`) (`self.RotAngle`)))))
                  (set `self.Ring01_Angle` _result)
                  (bind _result_2 (`self.GetClampedIndex` (+ (`self.Ring1_Index`) (`KismetMathLibrary.FTrunc` (* (`self.RotationDirection`) 1.0)))))
                  (set `self.Ring1_Index` _result_2))
                (:`1`
                  (bind _result_3 (`self.GetClamedAngle` (+ (`self.Ring02_Angle`) (* (`self.RotationDirection`) (`self.RotAngle`)))))
                  (set `self.Ring02_Angle` _result_3)
                  (bind _result_4 (`self.GetClampedIndex` (+ (`self.Ring2_Index`) (`KismetMathLibrary.FTrunc` (* (`self.RotationDirection`) 1.0)))))
                  (set `self.Ring2_Index` _result_4))
                (:`2`
                  (bind _result_5 (`self.GetClamedAngle` (+ (`self.Ring03_Angle`) (* (`self.RotationDirection`) (`self.RotAngle`)))))
                  (set `self.Ring03_Angle` _result_5)
                  (bind _result_6 (`self.GetClampedIndex` (+ (`self.Ring3_Index`) (`KismetMathLibrary.FTrunc` (* (`self.RotationDirection`) 1.0)))))
                  (set `self.Ring3_Index` _result_6))
                (:`3`
                  (bind _result_7 (`self.GetClamedAngle` (+ (`self.Ring04_Angle`) (* (`self.RotationDirection`) (`self.RotAngle`)))))
                  (set `self.Ring04_Angle` _result_7)
                  (bind _result_8 (`self.GetClampedIndex` (+ (`self.Ring4_Index`) (`KismetMathLibrary.FTrunc` (* (`self.RotationDirection`) 1.0)))))
                  (set `self.Ring4_Index` _result_8)))
              (if (and (== (`self.Ring1_Index`) _basering_index) (== (`self.Ring2_Index`) _basering_index) (== (`self.Ring3_Index`) _basering_index) (== (`self.Ring4_Index`) _basering_index))
                ;;[1 1 1] Success
                (set `self.InputEnable` false)
                (set `self.MiniGameEnabled` false)
                (set `self.IsMiniGameActivated` false)
                (`MaterialInstanceDynamic.SetScalarParameterValue` (`self.DMI`) "ShowGranted" 1.0)
                (`KismetSystemLibrary.Delay` (`self.DelayTimeWhenComplete`))
                (`self.SetOfflineMaterial`)
                (`self.OnMiniGameSuccess`)
                (`KismetSystemLibrary.ExecuteConsoleCommand` (`GameplayStatics.GetPlayerController` 0) (`KismetStringLibrary.Concat_StrStr` "r.TemporalAACurrentFrameWeight " (`KismetStringLibrary.Conv_DoubleToString` (`self.GameTAACurrFrameWeight`))) null)
                (`self.BlendCameraFromGameToPlayer` (`self.OverlappedActor`))))
            (else
              (set `self.RightAxisEnable` true))))
        (:`then_1`
          (if (!= _forwardaxis 0.0)
            (if (`self.ForwardAxisEnable`)
              (set `self.ForwardAxisEnable` false)
              (set `self.SelectorSign` (`KismetMathLibrary.FTrunc` (`KismetMathLibrary.SignOfFloat` _forwardaxis)))
              (set `self.Selector` (`KismetMathLibrary.Clamp` (+ (`self.SelectorSign`) (`self.Selector`)) 0 3)))
            (else
              (set `self.ForwardAxisEnable` true))))))))

(event `UpdateDecor`
  (bind _dmi (`self.DMI`))
  ;[1 1 1] Update decor
  (`MaterialInstanceDynamic.SetScalarParameterValue` _dmi "Dec_Text1" 0.0)
  (`MaterialInstanceDynamic.SetScalarParameterValue` _dmi "Dec_Text2" 0.0)
  (`MaterialInstanceDynamic.SetScalarParameterValue` _dmi "Dec_Text3" 0.0)
  (`MaterialInstanceDynamic.SetScalarParameterValue` _dmi "Dec_Text4" 0.0)
  (`MaterialInstanceDynamic.SetScalarParameterValue` _dmi (`KismetStringLibrary.Conv_StringToName` (`KismetStringLibrary.Concat_StrStr` "Dec_Text" (`KismetStringLibrary.Conv_IntToString` (`KismetMathLibrary.RandomIntegerInRange` 1 4)))) 1.0))

(event `self.ForceExit`
  ;[1 1 1] Cancel
  (if (and (`self.MiniGameEnabled`) (`self.IsMiniGameActivated`))
    (set `self.IsMiniGameActivated` false)
    (set `self.InputEnable` false)
    (`KismetSystemLibrary.ExecuteConsoleCommand` (`GameplayStatics.GetPlayerController` 0) (`KismetStringLibrary.Concat_StrStr` "r.TemporalAACurrentFrameWeight " (`KismetStringLibrary.Conv_DoubleToString` (`self.GameTAACurrFrameWeight`))) null)
    (`self.OnMiniGameCanceled`)
    (`self.BlendCameraFromGameToPlayer` (`self.OverlappedActor`))))

(event `self.ForceAction`
  ;[1 1 1] Action button
  (if (`self.PlayerOverlapped`)
    (if (not (`self.IsMiniGameActivated`))
      (`self.InitGame`)
      (`PrimitiveComponent.SetMaterial` (`self.MiniGameScreen`) 0 (`self.DMI`))
      (`self.BlendCameraFromPlayerToGame` self (`self.OverlappedActor`))
      (set `self.IsMiniGameActivated` true)
      (set `self.InputEnable` true))))

(event `self.InteractionBoundBox.OnComponentBeginOverlap`
  (params (OverlappedComponent :type "PrimitiveComponent Object Reference") (OtherActor :type "Actor Object Reference") (OtherComp :type "PrimitiveComponent Object Reference") (OtherBodyIndex :type Integer) (bFromSweep :type Boolean) (SweepResult :type "HitResult Structure (by ref)"))
  ;[1 1 1] PLayer overlapping
  (`self.CheckBeginOverlap` OtherActor))

(event `self.InteractionBoundBox.OnComponentEndOverlap`
  (params (OverlappedComponent :type "PrimitiveComponent Object Reference") (OtherActor :type "Actor Object Reference") (OtherComp :type "PrimitiveComponent Object Reference") (OtherBodyIndex :type Integer))
  ;[1 1 1] PLayer overlapping
  (`self.CheckEndOverlap` OtherActor))

(event `UpdateDecor2`
  (bind _dmi (`self.DMI`))
  ;[1 1 1] Update decor
  (`MaterialInstanceDynamic.SetScalarParameterValue` _dmi "Dec_Text2_1" 0.0)
  (`MaterialInstanceDynamic.SetScalarParameterValue` _dmi "Dec_Text2_2" 0.0)
  (`MaterialInstanceDynamic.SetScalarParameterValue` _dmi "Dec_Text2_3" 0.0)
  (`MaterialInstanceDynamic.SetScalarParameterValue` _dmi "Dec_Text2_4" 0.0)
  (`MaterialInstanceDynamic.SetScalarParameterValue` _dmi (`KismetStringLibrary.Conv_StringToName` (`KismetStringLibrary.Concat_StrStr` "Dec_Text2_" (`KismetStringLibrary.Conv_IntToString` (`KismetMathLibrary.RandomIntegerInRange` 1 4)))) 1.0))

(event `self.ReceiveTick`
  (params (DeltaSeconds :type "Float (single-precision)"))
  ;[1 1 1] Update material
  (bind _output_get (set `self.DeltaTime` DeltaSeconds))
  (`parent.ReceiveTick` _output_get)
  (`self.UpdateMaterial`))

(fn `GetClamedAngle`
  (params (Angle :type "Float (double-precision)"))
  (returns (Result :type "Float (double-precision)"))
  (locals (OutAngle :type "Float (double-precision)"))
  ;[1 1 1] Get clamped 0...1 angle value
  (bind _output_get (set `local.OutAngle` Angle))
  (if (< _output_get 0.0)
    (set `local.OutAngle` (+ _output_get 1.0))
    (elif (> _output_get 1.0)
      (set `local.OutAngle` (- _output_get 1.0))))
  (return (`local.OutAngle`)))

(fn `GetClampedIndex`
  (params (Index :type Integer))
  (returns (Result :type Integer))
  (locals (OutIndex :type Integer))
  ;[1 1 1] Get clamped index for sector 0...47
  (set `local.OutIndex` Index)
  (if (> Index 47)
    (set `local.OutIndex` 0)
    (elif (< Index 0)
      (set `local.OutIndex` 47)))
  (return (`local.OutIndex`)))

(fn `GetRandomRotation`
  (params (Angle :type "Float (double-precision)"))
  (returns (Result :type "Float (double-precision)"))
  ;[1 1 1] Get random rotation value. 24 sectors max
  (return (* (`KismetMathLibrary.RandomIntegerInRange` 0 23) (* Angle 2.0))))

(fn `UpdateMaterial`
  (locals (MatSelector1 :type "Float (double-precision)") (MatSelector2 :type "Float (double-precision)") (MatSelector3 :type "Float (double-precision)") (MatSelector4 :type "Float (double-precision)"))
  (bind _dmi (`self.DMI`))
  (bind _dmi_2 (`self.DMI`))
  ;[1 1 1] Send parameters to material
  (`MaterialInstanceDynamic.SetScalarParameterValue` _dmi_2 "RotationRing1" (`self.Ring01_Angle`))
  (`MaterialInstanceDynamic.SetScalarParameterValue` _dmi_2 "RotationRing2" (`self.Ring02_Angle`))
  (`MaterialInstanceDynamic.SetScalarParameterValue` _dmi_2 "RotationRing3" (`self.Ring03_Angle`))
  (`MaterialInstanceDynamic.SetScalarParameterValue` _dmi_2 "RotationRing4" (`self.Ring04_Angle`))
  (set `local.MatSelector1` 0.0)
  (set `local.MatSelector2` 0.0)
  (set `local.MatSelector3` 0.0)
  (set `local.MatSelector4` 0.0)
  (switch `int` (`self.Selector`)
    (:`0`
      (set `local.MatSelector1` 1.0))
    (:`1`
      (set `local.MatSelector2` 1.0))
    (:`2`
      (set `local.MatSelector3` 1.0))
    (:`3`
      (set `local.MatSelector4` 1.0)))
  (`MaterialInstanceDynamic.SetScalarParameterValue` _dmi "Selector1" (`local.MatSelector1`))
  (`MaterialInstanceDynamic.SetScalarParameterValue` _dmi "Selector2" (`local.MatSelector2`))
  (`MaterialInstanceDynamic.SetScalarParameterValue` _dmi "Selector3" (`local.MatSelector3`))
  (`MaterialInstanceDynamic.SetScalarParameterValue` _dmi "Selector4" (`local.MatSelector4`)))

(fn `UserConstructionScript`
  (`parent.UserConstructionScript`))