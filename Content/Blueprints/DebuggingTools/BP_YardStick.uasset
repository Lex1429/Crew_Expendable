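; BP_YardStick is a debugging actor that visualizes a sphere of configurable Radius as a measuring aid.
; The construction script runs a short upward sphere trace with timed debug drawing, and BeginPlay repeats it with persistent drawing.
; Both traces start at the static mesh's relative location, not its world location, and their results are unused, so only the debug shapes matter.
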(event `self.ReceiveBeginPlay`
  (bind _relativelocation (`SceneComponent.RelativeLocation` (`self.StaticMesh`)))
  (`KismetSystemLibrary.SphereTraceSingleByProfile` :`Start` _relativelocation :`End` (+ _relativelocation (0.0 0.0 25.0)) :`Radius` (`self.Radius`) :`DrawDebugType` "Persistent"))

(fn `UserConstructionScript`
  (bind _relativelocation (`SceneComponent.RelativeLocation` (`self.StaticMesh`)))
  (`KismetSystemLibrary.SphereTraceSingleByProfile` :`Start` _relativelocation :`End` (+ _relativelocation (0.0 0.0 25.0)) :`Radius` (`self.Radius`) :`DrawDebugType` "ForDuration"))