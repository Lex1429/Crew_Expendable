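; Interactable vault door that toggles open and closed unless locked, with an automatic mode for the Corpo minigame that starts its StateTree.
; Interaction routes through server and local events to a timeline that rotates the door and calls the vault light activation.
; An optional linked reader drives the lock state through bound events.
; The construction script applies configurable door and frame materials.
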(event `SetDoorsToAutomatic`
  ;[1 0.5 0] Automatic door system for Corpo Minigame
  (set `self.Automatic?` true)
  (`BrainComponent.StartLogic` (`self.StateTree`)))

(event `self.Interact`
  (params (Character :type "/Game/Blueprints/Characters/BP_BaseCharacter Object Reference") (PlayerCharacter :type "/Game/Blueprints/Characters/BP_PlayerCharacterCore Object Reference"))
  (`self.Server_ActivateDoor`))

(event `Server_ActivateDoor`
  (`self.Local_ActivateDoor`))

(event `Local_ActivateDoor`
  (`self.ActivateDoor`))

(event `ActivateDoor`
  (if (not (`self.Locked?`))
    (if (not (`self.Open?`))
      (set `self.Open?` true)
      (bind (_direction _newtrack_0) (`Timeline|SplitDoor` :!label _label)
        (:`Update`
          (`SceneComponent.K2_SetRelativeRotation` (`self.VaultDoor`) (`KismetMathLibrary.RLerp` (struct) (struct :`Yaw` -90.0) _newtrack_0) false false)
          (`self.ActivateVaultLight`)))
      (else
        (set `self.Open?` false)
        (goto _label :!via `Reverse`)))))

(event `self.ReceiveBeginPlay`
  (bind _readerref (`self.ReaderRef`)
    (:`then`
      (add `/Game/Blueprints/Interactables/Buttons/BP_CartridgeReader.UnlockedObject` _readerref (delegate `UnlockDoor`))
      (add `/Game/Blueprints/Interactables/Buttons/BP_CartridgeReader.LockedObject` _readerref (delegate `LockDoor`)))
    (:`else`)))

(event `LockDoor`
  (set `self.Locked?` true))

(event `UnlockDoor`
  (set `self.Locked?` false))

(fn `GetCanBePickedUp`
  (returns (CanBePickedUp :type Boolean))
  (return false))

(fn `GetItemToSpawn`
  (returns (Item :type "/Game/Blueprints/Interactables/Weapons/BP_WeaponComponentMaster Class Reference"))
  (return null))

(fn `UserConstructionScript`
  (`PrimitiveComponent.SetMaterial` (`self.VaultDoor`) 0 (`self.DoorMaterial`))
  (`PrimitiveComponent.SetMaterial` (`self.DoorFrame`) 0 (`self.FrameMaterial`))
  (`PrimitiveComponent.SetMaterial` (`self.DoorFrame`) 1 (`self.FrameMaterial2`))
  (`PrimitiveComponent.SetMaterial` (`self.DoorFrame`) 2 (`self.FrameMaterial3`)))