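; BP_DoorConsole is an interactable console that triggers the doors of the room matching its tag.
; Interact calls a server switch event, which passes to a local event that searches all BP_DoorBase actors.
; Each door whose RoomTag equals ConsoleTag receives ServerOpenDoor.
; Overlapping InteractRadius applies an outline overlay material to the console mesh, and ending the overlap clears it.
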(event `Server_DoorSwitch`
  (`self.Local_DoorSwitch`))

(event `Local_DoorSwitch`
  (bind _outactors (`GameplayStatics.GetAllActorsOfClass` "/Game/Blueprints/Interactables/Doors/BP_DoorBase.BP_DoorBase_C"))
  (for _array_element _outactors
    (if (== (`/Game/Blueprints/Interactables/Doors/BP_DoorBase.RoomTag` _array_element) (`self.ConsoleTag`))
      (`/Game/Blueprints/Interactables/Doors/BP_DoorBase.Server_OpenDoor` _array_element))))

(event `/Game/Blueprints/Interfaces/BPI_Interact.Interact`
  (params (Character :type "/Game/Blueprints/Characters/BP_BaseCharacter Object Reference"))
  (`self.Server_DoorSwitch`))

(event `self.InteractRadius.OnComponentBeginOverlap`
  (params (OverlappedComponent :type "PrimitiveComponent Object Reference") (OtherActor :type "Actor Object Reference") (OtherComp :type "PrimitiveComponent Object Reference") (OtherBodyIndex :type Integer) (bFromSweep :type Boolean) (SweepResult :type "HitResult Structure (by ref)"))
  (`MeshComponent.SetOverlayMaterial` (`self.DoorConsole`) "/Game/Materials/M_Outline.M_Outline"))

(event `self.InteractRadius.OnComponentEndOverlap`
  (params (OverlappedComponent :type "PrimitiveComponent Object Reference") (OtherActor :type "Actor Object Reference") (OtherComp :type "PrimitiveComponent Object Reference") (OtherBodyIndex :type Integer))
  (`MeshComponent.SetOverlayMaterial` (`self.DoorConsole`) null))

(fn `UserConstructionScript`)