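; BP_CealingLights is a ceiling light interactable that toggles on and off unless a power outage is active.
; Local_ToggleLights checks PowerOutage, flips IsLightOn, sets the LightStrength material parameter on the ceiling mesh and prints the new state.
; Server_ToggleLights forwards to the local toggle.
; The visible change is driven purely through the material parameter, with no light component touched.
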(event `Local_ToggleLights`
  (if (`self.PowerOutage`)
    _
    (elif (`self.IsLightOn?`)
      (`MeshComponent.SetScalarParameterValueOnMaterials` (`self.SM_Bld_Ceiling_03`) "LightStrength" 0.0)
      (set `self.IsLightOn?` false)
      (`KismetSystemLibrary.PrintString` "Lights off")
      (else
        (`MeshComponent.SetScalarParameterValueOnMaterials` (`self.SM_Bld_Ceiling_03`) "LightStrength" 2.0)
        (set `self.IsLightOn?` true)
        (`KismetSystemLibrary.PrintString` "Lights On")))))

(event `Server_ToggleLights`
  (`self.Local_ToggleLights`))

(fn `UserConstructionScript`)