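; BP_Lightswitch is an interactable, damageable switch that toggles every BP_LampBase sharing its RoomTag.
; Interact routes through a server event to the local toggle, which flips each matching lamp by its own state, swaps indicator materials, animates the button via timeline and calls LightSwitchToggle.
; Damage depletes HP until it breaks, spawning looping electric Niagara effects and blocking further toggles.
; Viewing and InRange events drive the player UI prompt and a temporary outline overlay.
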(event `Local_Lightswitch`
  (if (not (`self.Broken?`))
    (bind _outactors (`GameplayStatics.GetAllActorsOfClass` "/Game/Blueprints/Interactables/CealingLights/BP_LampBase.BP_LampBase_C"))
    (for _array_element _outactors
      (if (== (`/Game/Blueprints/Interactables/CealingLights/BP_LampBase.RoomTag` _array_element) (`self.RoomTag`))
        (if (`/Game/Blueprints/Interactables/CealingLights/BP_LampBase.IsLightOn?` _array_element)
          (`/Game/Blueprints/Interactables/CealingLights/BP_LampBase.Server_LightOff` _array_element)
          (`PrimitiveComponent.SetMaterial` (`self.OffLight`) 0 (`self.OffLightOn`))
          (`PrimitiveComponent.SetMaterial` (`self.OnLight`) 0 (`self.OnLightOff`))
          (`self.LightSwitchToggle` false)
          (bind (_direction _newtrack_0) (`Timeline|Switch` :!via `Reverse` :!label _label)
            (:`Update`
              (`SceneComponent.K2_SetRelativeLocation` (`self.Button`) (`KismetMathLibrary.VLerp` (0.0 0.0 0.0) (0.0 0.0 7.0) _newtrack_0) false false)))
          (else
            (`/Game/Blueprints/Interactables/CealingLights/BP_LampBase.Server_LightOn` _array_element)
            (`PrimitiveComponent.SetMaterial` (`self.OffLight`) 0 (`self.OffLightOff`))
            (`PrimitiveComponent.SetMaterial` (`self.OnLight`) 0 (`self.OnLightOn`))
            (`self.LightSwitchToggle` true)
            (goto _label)))))))

(event `Server_LightSwitch`
  (`self.Local_Lightswitch`))

(event `/Game/Blueprints/Interfaces/BPI_Interact.Interact`
  (params (Character :type "/Game/Blueprints/Characters/BP_BaseCharacter Object Reference"))
  (`self.Server_LightSwitch`))

(event `self.ReceiveAnyDamage`
  (params (Damage :type "Float (single-precision)") (DamageType :type "DamageType Object Reference") (InstigatedBy :type "Controller Object Reference") (DamageCauser :type "Actor Object Reference"))
  (bind _output_get (set `self.HP` (- (`self.HP`) Damage)))
  (if (<= _output_get 0.0)
    (`PrimitiveComponent.SetMaterial` (`self.AcitvityLight`) 0 (`self.OffLightOn`))
    (`NiagaraFunctionLibrary.SpawnSystemAtLocation` "/Game/AllShadesofVFXBundle/EnvironmentVFX/VFX/Electricity/Systems/N_ElectricLoop.N_ElectricLoop" (`SceneComponent.K2_GetComponentLocation` (`self.SwitchCase`)) (struct) (1.0 1.0 1.0) false)
    (set `self.Broken?` true)))

(event `self.ReceiveBeginPlay`
  (`KismetSystemLibrary.Delay` 2.0)
  (bind _foundwidgets (`WidgetBlueprintLibrary.GetAllWidgetsOfClass` "/Game/UI/WB_PlayerUI.WB_PlayerUI_C"))
  (set `self.PlayerUIRef` (`|GetArrayItem` _foundwidgets)))

(event `/Game/Blueprints/Interfaces/BPI_Interact.Viewing`
  (params (State :type Boolean))
  (bind _playeruiref (`self.PlayerUIRef`))
  (if State
    (message `/Game/Blueprints/Interfaces/BPI_CombatUI.InteractElement` _playeruiref "Light Switch" "" "Toggle" true)
    (else
      (message `/Game/Blueprints/Interfaces/BPI_CombatUI.InteractElement` _playeruiref "" "" "" false))))

(event `/Game/Blueprints/Interfaces/BPI_Interact.InRange`
  (params (State :type Boolean))
  (bind _switchcase (`self.SwitchCase`))
  (if State
    (`MeshComponent.SetOverlayMaterial` _switchcase "/Game/Materials/M_Outline.M_Outline")
    (`KismetSystemLibrary.Delay` 1.5)
    (`MeshComponent.SetOverlayMaterial` _switchcase null)))

(fn `UserConstructionScript`)