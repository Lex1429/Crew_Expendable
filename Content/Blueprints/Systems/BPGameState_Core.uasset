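; Core game state Blueprint that stores shared match data: research points, server and living player counts, player list, sector power and reactor status.
; Setter events and getter functions expose this data, while other player and server getters are empty or default-value stubs.
; SetAbletoExit tells the first BP_ExitSignal found to update its research message.
; BeginPlay loops endlessly, starting the space ambience 2D sound again every 0.2 seconds.
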(event `self.ReceiveBeginPlay`
  (`|ExecutionSequence`
    (:`then_0`
      (`GameplayStatics.PlaySound2D` "/Game/SFX/Music/space-ambience_03.space-ambience_03" 1.0 1.0 0.0 null null false :!label _label)
      (`KismetSystemLibrary.Delay` 0.2)
      (goto _label))))

(event `/Game/Blueprints/Interfaces/BPI_Stats.SetResearchPoints`
  (params (ResearchPoints :type Integer))
  (set `self.ResearchPoints` ResearchPoints))

(event `/Game/Blueprints/Interfaces/BPI_Stats.SetAbleToExit`
  (bind _outactors (`GameplayStatics.GetAllActorsOfClass` "/Game/Blueprints/Interactables/LevelProps/BP_ExitSignal.BP_ExitSignal_C"))
  (message `/Game/Blueprints/Interfaces/BPI_ResearchUpdate.UpdateResearch` (`|GetArrayItem` _outactors)))

(event `/Game/Blueprints/Interfaces/BPI_Server.SetPlayerCount`
  (params (PlayerCount :type Integer))
  (set `self.ServerPlayerCount` PlayerCount))

(event `/Game/Blueprints/Interfaces/BPI_Server.SetLivePlayers`
  (params (LivePlayerCount :type Integer))
  (set `self.LivePlayers` LivePlayerCount))

(event `/Game/Blueprints/Interfaces/BPI_Stats.SetSectorPower`
  (params (SectorsWithPower :type "GameplayTagContainer Structure"))
  (set `self.SectorsWithPower` SectorsWithPower))

(event `/Game/Blueprints/Interfaces/BPI_Stats.SetReactorOn`
  (params (`ReactorOn?` :type Boolean))
  (set `self.ReactorOn?` `ReactorOn?`))

(event `AddToPlayerList`
  (params (Players :type "Character Object Reference"))
  (`KismetArrayLibrary.Array_Add` (`self.Players`) Players))

(event `RemoveFromPlayerList`
  (params (Players :type "Character Object Reference"))
  (`KismetArrayLibrary.Array_RemoveItem` (`self.Players`) Players))

(fn `GetCanSprint`
  (returns (CanSprint :type Boolean))
  (return false))

(fn `GetCurrentPlayerCount`
  (returns (Players :type "Array of Character Object Reference"))
  (return))

(fn `GetIsDead`
  (returns (IsDead :type Boolean))
  (return false))

(fn `GetLivePlayers`
  (returns (LivePalyerCount :type Integer))
  (return (`self.LivePlayers`)))

(fn `GetPlayerCount`
  (returns (PlayerCount :type Integer))
  (return (`self.ServerPlayerCount`)))

(fn `GetPlayerID`
  (returns (PlayerID :type Integer))
  (return 0))

(fn `GetPlayerMaxStamina`
  (returns (MaxStamina :type Integer))
  (return 0))

(fn `GetPlayerStamina`
  (returns (Stamina :type Integer))
  (return 0))

(fn `GetReactorOn`
  (returns (`ReactorOn?` :type Boolean))
  (return (`self.ReactorOn?`)))

(fn `GetResearchPoints`
  (returns (ResearchPoints :type Integer))
  (return (`self.ResearchPoints`)))

(fn `GetSectorPower`
  (returns (SectorsWithPower :type "GameplayTagContainer Structure"))
  (return (`self.SectorsWithPower`)))

(fn `GetServerCreator`
  (returns (Creator :type Text))
  (return ""))

(fn `GetServerSearch`
  (returns (SearchResult :type "BlueprintSessionResult Structure"))
  (return))

(fn `UserConstructionScript`)