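; BP_InfectionManager is a manager Blueprint that starts the alien infection when play begins.
; BeginPlay calls a server event that forwards to a local event, which picks a random BP_RoomAlienSpawnPoint, spawns an alien there and prints its room tag for debugging.
; A disconnected branch would, after a delay, assign the Corpo role to a random BP_BaseCharacter, but it never runs.
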(event `self.ReceiveBeginPlay`
  (`self.Server_InfectionController`))

(event `Server_InfectionController`
  (`self.Local_InfectionController`))

(event `Local_InfectionController`
  (`|ExecutionSequence`
    (:`then_0`
      (bind _outactors (`GameplayStatics.GetAllActorsOfClass` "/Game/Blueprints/Interactables/LevelProps/BP_RoomAlienSpawnPoint.BP_RoomAlienSpawnPoint_C"))
      (bind _output_get (set `self.RandomInt` (`KismetMathLibrary.RandomIntegerInRange` 0 (- (`KismetArrayLibrary.Array_Length` _outactors) 1))))
      (bind _output (`|GetArrayItem` _outactors _output_get))
      (`/Game/Blueprints/Interactables/LevelProps/BP_RoomAlienSpawnPoint.SpawnAlien` _output)
      (`KismetSystemLibrary.PrintString` (`BlueprintGameplayTagLibrary.GetDebugStringFromGameplayTag` (`/Game/Blueprints/Interactables/LevelProps/BP_RoomAlienSpawnPoint.RoomTag` _output)) true true (struct :`G` 0.66 :`B` 1.0 :`A` 1.0) 10.0))))

(fn `UserConstructionScript`)