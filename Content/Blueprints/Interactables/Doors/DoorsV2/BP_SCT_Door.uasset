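; BP_SCT_Door is an interactable, non-pickup sliding door that can switch to automatic operation for the Corpo minigame.
; Interact routes through server and local events to ActivateDoor, which toggles the Open state unless the door is locked.
; The SplitDoor timeline plays or reverses to lerp DoorTop between closed and open positions, calling the warning light on each update.
; SetDoorsToAutomatic flags the door as automatic and starts its StateTree logic.
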(event `SetDoorsToAutomatic`
  ;[1 0.5 0] Automatic door system for Corpo Minigame
  (set `self.Automatic?` true)
  (`BrainComponent.StartLogic` (`self.StateTree`)))

(event `self.Interact`
  (params (Character :type "/Game/Blueprints/Characters/BP_BaseCharacter Object Reference") (PlayerCharacter :type "/Game/Blueprints/Characters/BP_PlayerCharacterCore Object Reference"))
  (`self.Server_ActivateDoor`))

(event `Server_ActivateDoor`
  (`self.Local_ActivateDoor`))

(event `Local_ActivateDoor`
  (`self.ActivateDoor`))

(event `ActivateDoor`
  (if (not (`self.Locked?`))
    (if (not (`self.Open?`))
      (set `self.Open?` true)
      (bind (_direction _newtrack_0) (`Timeline|SplitDoor` :!label _label)
        (:`Update`
          (`SceneComponent.K2_SetRelativeLocation` (`self.DoorTop`) (`KismetMathLibrary.VLerp` (`self.TopClosed`) (`self.TopOpen`) _newtrack_0) false false)
          (`self.ActivateWarningLight`)))
      (else
        (set `self.Open?` false)
        (goto _label :!via `Reverse`)))))

(fn `GetCanBePickedUp`
  (returns (CanBePickedUp :type Boolean))
  (return false))

(fn `GetItemToSpawn`
  (returns (Item :type "/Game/Blueprints/Interactables/Weapons/BP_WeaponComponentMaster Class Reference"))
  (return null))

(fn `UserConstructionScript`)