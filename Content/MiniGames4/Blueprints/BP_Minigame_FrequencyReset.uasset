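; Minigame actor where the player matches a solver sine wave's period and phase to a moving sample wave on a decoder screen.
; Tick applies axis input, drifts and periodically retargets the sample, then tests for a match to finish the game.
; CalculatePoints packs each wave's points in pairs into Material Parameter Collection vectors, while a dynamic material handles decorative text and success display.
; Activation and exit blend the camera between player and game.
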(event `self.ReceiveBeginPlay`
  ;[1 1 1] Begin play
  (`parent.ReceiveBeginPlay`)
  (bind _returnvalue (`KismetMaterialLibrary.CreateDynamicMaterialInstance` "/Game/MiniGames4/Materials/MI_MG_WaveDecoder_Inst.MI_MG_WaveDecoder_Inst"))
  (set `self.DMI` _returnvalue))

(event `InitGame`
  ;[1 1 1] Init game
  (bind _output_get (set `self.SampleAmp` (`KismetMathLibrary.RandomFloatInRange` 0.025 0.1)))
  (set `self.TargetSampletAmp` _output_get)
  (bind _output_get_2 (set `self.SamplePeriod` (`KismetMathLibrary.RandomFloatInRange` 7.0 24.0)))
  (set `self.TargetSamplePeriod` _output_get_2)
  (bind _output_get_3 (set `self.SampleOffset` (`KismetMathLibrary.RandomFloatInRange` 0.0 (`KismetMathLibrary.GetPI`))))
  (set `self.TargetSampleOffset` _output_get_3)
  (set `self.SolverPeriod` (+ (`self.SamplePeriod`) (`KismetMathLibrary.RandomFloatInRange` 3.0 7.0)))
  (set `self.SolverOffset` (+ (`KismetMathLibrary.RandomFloatInRange` (/ (`KismetMathLibrary.GetPI`) 8.0) (`KismetMathLibrary.GetPI`)) (`self.SampleOffset`)))
  (bind _output_get_4 (set `self.StartChangeTime` (`KismetSystemLibrary.GetGameTimeInSeconds`)))
  (set `self.DecorTime` _output_get_4))

(event `CheckContorls`
  (bind _forwardaxis (`self.ForwardAxis`))
  (bind _rightaxis (`self.RightAxis`))
  ;[1 1 1] Controls
  (if (`self.InputEnable`)
    (if (`self.IsMiniGameActivated`)
      (`|ExecutionSequence`
        (:`then_0`
          (if (!= _rightaxis 0.0)
            (bind _result (`self.ClampDelta` (+ (`self.SolverOffset`) (`KismetMathLibrary.SelectFloat` -0.05 0.05 (> _rightaxis 0.0)))))
            (set `self.SolverOffset` _result)))
        (:`then_1`
          (if (!= _forwardaxis 0.0)
            (set `self.SolverPeriod` (`KismetMathLibrary.FClamp` (+ (`self.SolverPeriod`) (`KismetMathLibrary.SelectFloat` -0.07 0.07 (> _forwardaxis 0.0))) 7.0 24.0))))))))

(event `UpdateDecor`
  (bind _dmi (`self.DMI`))
  ;[1 1 1] Update Decor
  (if (>= (- (`KismetSystemLibrary.GetGameTimeInSeconds`) (`self.DecorTime`)) 0.15)
    (`MaterialInstanceDynamic.SetScalarParameterValue` _dmi "DecorText4" (`KismetMathLibrary.Conv_IntToDouble` (`KismetMathLibrary.RandomIntegerInRange` 0 31)))
    (`MaterialInstanceDynamic.SetScalarParameterValue` _dmi "DecorText1" (`KismetMathLibrary.Conv_IntToDouble` (`KismetMathLibrary.RandomIntegerInRange` 0 31)))
    (`MaterialInstanceDynamic.SetScalarParameterValue` _dmi "DecorText2" (`KismetMathLibrary.Conv_IntToDouble` (`KismetMathLibrary.RandomIntegerInRange` 0 31)))
    (`MaterialInstanceDynamic.SetScalarParameterValue` _dmi "DecorText3" (`KismetMathLibrary.Conv_IntToDouble` (`KismetMathLibrary.RandomIntegerInRange` 0 31)))
    (set `self.DecorTime` (`KismetSystemLibrary.GetGameTimeInSeconds`))))

(event `self.ForceExit`
  ;[1 1 1] Cancel
  (if (and (`self.MiniGameEnabled`) (`self.IsMiniGameActivated`))
    (set `self.IsMiniGameActivated` false)
    (set `self.InputEnable` false)
    (`self.OnMiniGameCanceled`)
    (`self.BlendCameraFromGameToPlayer` (`self.OverlappedActor`))))

(event `self.ForceAction`
  (params (Player :type "/Game/Blueprints/Characters/BP_PlayerCharacterCore Object Reference"))
  ;[1 1 1] Action
  (if (`self.PlayerOverlapped`)
    (if (not (`self.IsMiniGameActivated`))
      (`self.InitGame`)
      (`PrimitiveComponent.SetMaterial` (`self.MiniGameScreen`) 0 (`self.DMI`))
      (`self.BlendCameraFromPlayerToGame` self (`self.OverlappedActor`))
      (set `self.IsMiniGameActivated` true)
      (set `self.InputEnable` true))))

(event `self.InteractionBoundBox.OnComponentBeginOverlap`
  (params (OverlappedComponent :type "PrimitiveComponent Object Reference") (OtherActor :type "Actor Object Reference") (OtherComp :type "PrimitiveComponent Object Reference") (OtherBodyIndex :type Integer) (bFromSweep :type Boolean) (SweepResult :type "HitResult Structure (by ref)"))
  ;[1 1 1] Overlap events
  (`self.CheckBeginOverlap` OtherActor))

(event `self.InteractionBoundBox.OnComponentEndOverlap`
  (params (OverlappedComponent :type "PrimitiveComponent Object Reference") (OtherActor :type "Actor Object Reference") (OtherComp :type "PrimitiveComponent Object Reference") (OtherBodyIndex :type Integer))
  ;[1 1 1] Overlap events
  (`self.CheckEndOverlap` OtherActor))

(event `self.ReceiveTick`
  (params (DeltaSeconds :type "Float (single-precision)"))
  ;[1 0 0] Tick
  (bind _output_get (set `self.DeltaTime` DeltaSeconds))
  (`parent.ReceiveTick` _output_get)
  (if (`self.IsMiniGameActivated`)
    (`self.UpdateDecor`)
    (`self.CheckContorls`)
    (if (and (`KismetMathLibrary.NearlyEqual_FloatFloat` (`self.SolverPeriod`) (`self.SamplePeriod`) 0.2) (`KismetMathLibrary.NearlyEqual_FloatFloat` (/ (`self.SampleOffset`) (`self.SamplePeriod`)) (/ (`self.SolverOffset`) (`self.SolverPeriod`)) 0.004))
      ;[1 1 1] Success
      (set `self.MiniGameEnabled` false)
      (set `self.IsMiniGameActivated` false)
      (set `self.InputEnable` false)
      (`MaterialInstanceDynamic.SetScalarParameterValue` (`self.DMI`) "ShowUnblocked" 1.0)
      (`KismetSystemLibrary.Delay` (`self.DelayTimeWhenComplete`))
      (`self.SetOfflineMaterial`)
      (`self.GameFinished` self)
      (`self.BlendCameraFromGameToPlayer` (`self.OverlappedActor`))
      (else
        ;[1 1 1] Solver points
        (`self.CalculatePoints` 1 (/ (`KismetMathLibrary.GetPI`) (`self.SolverPeriod`)) (`self.SampleAmp`) (`self.SolverOffset`))
        ;[1 1 1] Sample points
        (`self.CalculatePoints` 25 (/ (`KismetMathLibrary.GetPI`) (`self.SamplePeriod`)) (`self.SampleAmp`) (`self.SampleOffset`))
        (bind _output_get_2 (set `self.SampleOffset` (+ (`self.SampleOffset`) (* (/ (`self.MovementSpeed`) 1000.0) (`KismetMathLibrary.SelectFloat` 1.0 -1.0 (`self.SampleDirection`))))))
        (bind _result (`self.ClampDelta` _output_get_2))
        (set `self.SampleOffset` _result)
        (set `self.SamplePeriod` (`KismetMathLibrary.FInterpTo` (`self.SamplePeriod`) (`self.TargetSamplePeriod`) (`self.DeltaTime`) 2.0))
        (set `self.SampleAmp` (`KismetMathLibrary.FInterpTo` (`self.SampleAmp`) (`self.TargetSampletAmp`) (`self.DeltaTime`) 2.0))
        ;[1 1 1] Create new sample data
        (if (>= (- (`KismetSystemLibrary.GetGameTimeInSeconds`) (`self.StartChangeTime`)) (`self.IntervalTime`))
          (set `self.StartChangeTime` (`KismetSystemLibrary.GetGameTimeInSeconds`))
          (set `self.TargetSampletAmp` (`KismetMathLibrary.RandomFloatInRange` 0.025 0.1))
          (set `self.TargetSamplePeriod` (`KismetMathLibrary.RandomFloatInRange` 7.0 24.0))
          (set `self.SampleDirection` (`KismetMathLibrary.RandomBool`)))))))

(fn `CalculatePoints`
  (params (MPCIndex :type Integer) (Period :type "Float (double-precision)") (Amplitude :type "Float (double-precision)") (Offset :type "Float (double-precision)"))
  (locals (Rvalue :type "Float (double-precision)") (Gvalue :type "Float (double-precision)") (MPC_Index :type Integer) (Period_Loc :type "Float (double-precision)") (Amp_Loc :type "Float (double-precision)") (Offset_loc :type "Float (double-precision)") (S2 :type "Float (double-precision)") (S :type "Float (double-precision)"))
  (bind _s2 (`local.S2`))
  (bind _returnvalue (* (`KismetMathLibrary.Sin` (+ (`local.S`) (`local.Offset_loc`))) (`local.Amp_Loc`)))
  ;[1 1 1] Calculating sinusoidal curve points and pass into a material
  (set `local.MPC_Index` MPCIndex)
  (set `local.Period_Loc` Period)
  (set `local.Amp_Loc` Amplitude)
  (set `local.Offset_loc` Offset)
  (set `local.S2` -0.5)
  (for _index (range 48)
    (if (== (mod (+ _index 1) 2) 0)
      (`KismetMaterialLibrary.SetVectorParameterValue` "/Game/MiniGames4/Materials/MPC_MG_WaveDecoder.MPC_MG_WaveDecoder" (`KismetStringLibrary.Conv_StringToName` (`KismetStringLibrary.Concat_StrStr` "Vector" (`KismetStringLibrary.Conv_IntToString` (`local.MPC_Index`)))) (make `LinearColor` (`local.Rvalue`) (`local.Gvalue`) _s2 _returnvalue))
      (`/Engine/EditorBlueprintResources/StandardMacros.IncrementInt` (`local.MPC_Index`)
        (:`  `
          _))
      (else
        (set `local.Rvalue` _s2)
        (set `local.Gvalue` _returnvalue)))
    (set `local.S2` (+ (`local.S2`) (/ 1.0 48.0)))
    (set `local.S` (+ (`local.S`) (`local.Period_Loc`)))))

(fn `ClampDelta`
  (params (Value :type "Float (double-precision)"))
  (returns (Result :type "Float (double-precision)"))
  (bind _returnvalue (* (`KismetMathLibrary.GetPI`) 2.0))
  ;[1 1 1] Clamp value from 0 to 2*PI
  (return (`KismetMathLibrary.SelectFloat` (- Value _returnvalue) (`KismetMathLibrary.SelectFloat` (+ Value _returnvalue) Value (< Value 0.0)) (> Value _returnvalue))))

(fn `UserConstructionScript`
  (`parent.UserConstructionScript`))