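; Interactable breaker primer that players pump to charge, then press to signal the reactor is on.
; Interact routes through server and local events; four successive pumps each animate the lever by timeline and light an indicator, the last setting SystemCharged.
; A further interaction animates the button, turns it green, sets the GameState reactor message and updates every BP_BreakerPanelV2's status.
; Collision overlap toggles the lever outline and prompt widget.
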(event `Local_PrimerHandle`
  (if (not (`self.SystemOn?`))
    (if (not (`self.SystemCharged?`))
      (switch `int` (`self.PrimerPumpCount`)
        (:`0`
          (`/Engine/EditorBlueprintResources/StandardMacros.IncrementInt` (`self.PrimerPumpCount`)
            (:`  `
              (bind (_direction _pump1) (`Timeline|Timeline` :!label _label)
                (:`Update`
                  (`SceneComponent.K2_SetRelativeRotation` (`self.PrimerLever`) (`KismetMathLibrary.RLerp` (struct) (struct :`Pitch` -160.0) _pump1) false true)
                  (`/Engine/EditorBlueprintResources/StandardMacros.DoOnce` false
                    (:`Completed`
                      (`MeshComponent.SetScalarParameterValueOnMaterials` (`self.ReadyLight1`) "LightStrength" 2.0)
                      (`KismetSystemLibrary.Delay` 0.5)
                      (goto _label :!via `Reverse`))))))))
        (:`1`
          (`/Engine/EditorBlueprintResources/StandardMacros.IncrementInt` (`self.PrimerPumpCount`)
            (:`  `
              (bind (_direction_2 _pump1_2 _pump2) (`Timeline|Timeline_0` :!label _label_2)
                (:`Update`
                  (`SceneComponent.K2_SetRelativeRotation` (`self.PrimerLever`) (`KismetMathLibrary.RLerp` (struct) (struct :`Pitch` -160.0) _pump2) false true)
                  (`/Engine/EditorBlueprintResources/StandardMacros.DoOnce` false
                    (:`Completed`
                      (`MeshComponent.SetScalarParameterValueOnMaterials` (`self.ReadyLight2`) "LightStrength" 2.0)
                      (`KismetSystemLibrary.Delay` 1.0)
                      (goto _label_2 :!via `Reverse`))))))))
        (:`2`
          (`/Engine/EditorBlueprintResources/StandardMacros.IncrementInt` (`self.PrimerPumpCount`)
            (:`  `
              (bind (_direction_3 _pump1_3 _pump2_2 _pump3) (`Timeline|Timeline_1` :!label _label_3)
                (:`Update`
                  (`SceneComponent.K2_SetRelativeRotation` (`self.PrimerLever`) (`KismetMathLibrary.RLerp` (struct) (struct :`Pitch` -160.0) _pump3) false true)
                  (`/Engine/EditorBlueprintResources/StandardMacros.DoOnce` false
                    (:`Completed`
                      (`MeshComponent.SetScalarParameterValueOnMaterials` (`self.ReadyLight3`) "LightStrength" 2.0)
                      (`KismetSystemLibrary.Delay` 1.5)
                      (goto _label_3 :!via `Reverse`))))))))
        (:`3`
          (`/Engine/EditorBlueprintResources/StandardMacros.IncrementInt` (`self.PrimerPumpCount`)
            (:`  `
              (bind (_direction_4 _pump1_4 _pump2_3 _pump3_2 _pump4) (`Timeline|Timeline_2` :!label _label_4)
                (:`Update`
                  (`SceneComponent.K2_SetRelativeRotation` (`self.PrimerLever`) (`KismetMathLibrary.RLerp` (struct) (struct :`Pitch` -160.0) _pump4) false true)
                  (`KismetSystemLibrary.Delay` 2.5)
                  (`MeshComponent.SetScalarParameterValueOnMaterials` (`self.ReadyLight4`) "LightStrength" 2.0)
                  (`|ExecutionSequence`
                    (:`then_0`
                      (goto _label_4 :!via `Reverse`))
                    (:`then_1`
                      (set `self.SystemCharged?` true)
                      (`PrimitiveComponent.SetMaterial` (`self.PrimerButton1`) 0 "/Game/PolygonSciFiWorlds/Materials/FX/M_YellowGlow.M_YellowGlow")))))))))
      (else
        (bind (_direction_5 _newtrack_0) (`Timeline|PrimerButtonTime`)
          (:`Update`
            (`SceneComponent.K2_SetRelativeLocation` (`self.PrimerButton1`) (`KismetMathLibrary.VLerp` (1.0 -25.0 5.0) (0.0 -25.0 5.0) _newtrack_0) false false)
            (`|ExecutionSequence`
              (:`then_0`
                (`PrimitiveComponent.SetMaterial` (`self.PrimerButton1`) 0 "/Game/PolygonSciFiWorlds/Materials/FX/M_FX_Green_Glow.M_FX_Green_Glow")
                (message `/Game/Blueprints/Interfaces/BPI_Stats.SetReactorOn` (`GameplayStatics.GetGameState`) true)
                (`self.SetPanelReady`)))))))))

(event `Server_PrimerHandle`
  (`self.Local_PrimerHandle`))

(event `self.Interact`
  (params (Character :type "/Game/Blueprints/Characters/BP_BaseCharacter Object Reference"))
  (`self.Server_PrimerHandle`))

(event `self.PrimerCollision.OnComponentBeginOverlap`
  (params (OverlappedComponent :type "PrimitiveComponent Object Reference") (OtherActor :type "Actor Object Reference") (OtherComp :type "PrimitiveComponent Object Reference") (OtherBodyIndex :type Integer) (bFromSweep :type Boolean) (SweepResult :type "HitResult Structure (by ref)"))
  (`MeshComponent.SetOverlayMaterial` (`self.PrimerLever`) "/Game/Materials/M_Outline.M_Outline")
  (`SceneComponent.SetVisibility` (`self.Widget`) true false))

(event `self.PrimerCollision.OnComponentEndOverlap`
  (params (OverlappedComponent :type "PrimitiveComponent Object Reference") (OtherActor :type "Actor Object Reference") (OtherComp :type "PrimitiveComponent Object Reference") (OtherBodyIndex :type Integer))
  (`MeshComponent.SetOverlayMaterial` (`self.PrimerLever`) null)
  (`SceneComponent.SetVisibility` (`self.Widget`) false false))

(fn `OnRep_SystemOn?`)

(fn `SetPanelReady`
  (bind _outactors (`GameplayStatics.GetAllActorsOfClass` "/Game/Blueprints/Interactables/Buttons/BP_BreakerPanelV2.BP_BreakerPanelV2_C"))
  (for _array_element _outactors
    (`/Game/Blueprints/Interactables/Buttons/BP_BreakerPanelV2.SetPanelStatus` _array_element)))

(fn `UserConstructionScript`)