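; Interactable breaker panel that toggles power for the lights in its tagged sector, showing that sector's number on a sign.
; Interact routes through a server event to the toggle, which works only while the game state reports the reactor on.
; It updates matching BP_LightControl actors, calling their light switch only on power-off, and swaps the switch material.
; Box overlap outlines the switch, and SetPanelStatus sets its material from reactor state.
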(event `self.ReceiveBeginPlay`
  (`|SwitchGameplayTagContainer` (`self.SectorTag`)
    (:`(GameplayTags=((TagName="Sector1")))`
      (`StaticMeshComponent.SetStaticMesh` (`self.SectorSign`) "/Game/PolygonSciFiSpace/Meshes/Signs/SM_SignBorder_Number_01.SM_SignBorder_Number_01"))
    (:`(GameplayTags=((TagName="Sector2")))`
      (`StaticMeshComponent.SetStaticMesh` (`self.SectorSign`) "/Game/PolygonSciFiSpace/Meshes/Signs/SM_SignBorder_Number_02.SM_SignBorder_Number_02"))
    (:`(GameplayTags=((TagName="Sector3")))`
      (`StaticMeshComponent.SetStaticMesh` (`self.SectorSign`) "/Game/PolygonSciFiSpace/Meshes/Signs/SM_SignBorder_Number_03.SM_SignBorder_Number_03"))
    (:`(GameplayTags=((TagName="Sector4")))`
      (`StaticMeshComponent.SetStaticMesh` (`self.SectorSign`) "/Game/PolygonSciFiSpace/Meshes/Signs/SM_SignBorder_Number_04.SM_SignBorder_Number_04"))
    (:`(GameplayTags=((TagName="Sector5")))`
      (`StaticMeshComponent.SetStaticMesh` (`self.SectorSign`) "/Game/PolygonSciFiSpace/Meshes/Signs/SM_SignBorder_Number_05.SM_SignBorder_Number_05"))
    (:`(GameplayTags=((TagName="Sector6")))`
      (`StaticMeshComponent.SetStaticMesh` (`self.SectorSign`) "/Game/PolygonSciFiSpace/Meshes/Signs/SM_SignBorder_Number_06.SM_SignBorder_Number_06"))
    (:`(GameplayTags=((TagName="Sector7")))`
      (`StaticMeshComponent.SetStaticMesh` (`self.SectorSign`) "/Game/PolygonSciFiSpace/Meshes/Signs/SM_SignBorder_Number_07.SM_SignBorder_Number_07"))))

(event `Local_SectorPower`
  (bind _reactoron_ (message `/Game/Blueprints/Interfaces/BPI_Stats.GetReactorOn` (`GameplayStatics.GetGameState`)))
  (if _reactoron_
    (if (`self.SectorPowerOn?`)
      (set `self.SectorPowerOn?` false)
      (else
        (set `self.SectorPowerOn?` true)))
    (bind _outactors (`GameplayStatics.GetAllActorsOfClass` "/Game/Blueprints/Interactables/Buttons/BP_LightControl.BP_LightControl_C"))
    (for _array_element _outactors
      (if (== (`/Game/Blueprints/Interactables/Buttons/BP_LightControl.SectorTag` _array_element) (`self.SectorTag`))
        (if (`self.SectorPowerOn?`)
          (set `/Game/Blueprints/Interactables/Buttons/BP_LightControl.SectorPowered` true _array_element)
          (`PrimitiveComponent.SetMaterial` (`self.PanelSwitch`) 0 "/Game/PolygonSciFiSpace/Materials/Alternates/MI_PolygonSciFiSpace_01_B.MI_PolygonSciFiSpace_01_B")
          (else
            (set `/Game/Blueprints/Interactables/Buttons/BP_LightControl.SectorPowered` false _array_element)
            (`/Game/Blueprints/Interactables/Buttons/BP_LightControl.Server_LightSwitch` _array_element)
            (`PrimitiveComponent.SetMaterial` (`self.PanelSwitch`) 0 "/Game/PolygonSciFiSpace/Materials/Alternates/MI_PolygonSciFiSpace_01_A.MI_PolygonSciFiSpace_01_A")))))))

(event `/Game/Blueprints/Interfaces/BPI_Interact.Interact`
  (params (Character :type "/Game/Blueprints/Characters/BP_BaseCharacter Object Reference"))
  (`self.Server_SectorPower`))

(event `Server_SectorPower`
  (`self.Local_SectorPower`))

(event `self.Box.OnComponentBeginOverlap`
  (params (OverlappedComponent :type "PrimitiveComponent Object Reference") (OtherActor :type "Actor Object Reference") (OtherComp :type "PrimitiveComponent Object Reference") (OtherBodyIndex :type Integer) (bFromSweep :type Boolean) (SweepResult :type "HitResult Structure (by ref)"))
  (`MeshComponent.SetOverlayMaterial` (`self.PanelSwitch`) "/Game/Materials/M_Outline.M_Outline"))

(event `self.Box.OnComponentEndOverlap`
  (params (OverlappedComponent :type "PrimitiveComponent Object Reference") (OtherActor :type "Actor Object Reference") (OtherComp :type "PrimitiveComponent Object Reference") (OtherBodyIndex :type Integer))
  (`MeshComponent.SetOverlayMaterial` (`self.PanelSwitch`) null))

(fn `SetPanelStatus`
  (bind _reactoron_ (message `/Game/Blueprints/Interfaces/BPI_Stats.GetReactorOn` (`GameplayStatics.GetGameState`)))
  (if _reactoron_
    (`PrimitiveComponent.SetMaterial` (`self.PanelSwitch`) 0 "/Game/PolygonSciFiSpace/Materials/Alternates/MI_PolygonSciFiSpace_01_A.MI_PolygonSciFiSpace_01_A")
    (else
      (`PrimitiveComponent.SetMaterial` (`self.PanelSwitch`) 0 "/Game/PolygonSciFiSpace/Materials/Alternates/MI_PolygonSciFiSpace_01_A_Inst.MI_PolygonSciFiSpace_01_A_Inst"))))

(fn `UserConstructionScript`)