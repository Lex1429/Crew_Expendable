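; Core player controller that toggles the escape menu and switches input modes between gameplay and UI.
; Escape creates or removes WB_EscapeMenu, setting cursor visibility and input mode, with menu-open state read and written through GameInstance messages.
; BeginPlay loads the "settings" save slot if present, without using the result, and caches the player's BP_BaseCharacter.
; Possession restores game-only input.
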(event `self.ReceiveBeginPlay`
  (bind _returnvalue (`GameplayStatics.GetPlayerControllerID` (`GameplayStatics.GetPlayerController` 0)))
  (`|ExecutionSequence`
    (:`then_0`
      (bind _returnvalue_2 (`GameplayStatics.DoesSaveGameExist` "settings" _returnvalue))
      (if _returnvalue_2
        (`GameplayStatics.LoadGameFromSlot` "settings" _returnvalue)))
    (:`then_1`
      (bind _asbp_base_character (cast `/Game/Blueprints/Characters/BP_BaseCharacter` (`GameplayStatics.GetPlayerCharacter` 0)))
      (set `self.CharacterRef` _asbp_base_character))))

(event `Key|Escape`
  (params (Key :type "Key Structure"))
  (:`Pressed`
    (bind _menuup (message `/Game/Blueprints/Interfaces/BPI_PlayerSettings.GetMenuUp` (`GameplayStatics.GetGameInstance`)))
    (if (not _menuup)
      (bind _returnvalue (`|CreateWidget` "/Game/UI/WB_EscapeMenu.WB_EscapeMenu_C" (`GameplayStatics.GetPlayerController` 0)))
      (bind _output_get (set `self.MenuRef` _returnvalue))
      (`UserWidget.AddToPlayerScreen` _output_get 0)
      (`WidgetBlueprintLibrary.SetInputMode_GameAndUIEx` (`GameplayStatics.GetPlayerController` 0) _output_get "DoNotLock" true true)
      (set `self.bShowMouseCursor` true)
      (message `/Game/Blueprints/Interfaces/BPI_PlayerSettings.SetMenuUp` (`GameplayStatics.GetGameInstance`) true)
      (else
        (`Widget.RemoveFromParent` (`self.MenuRef`))
        (`WidgetBlueprintLibrary.SetInputMode_GameOnly` (`GameplayStatics.GetPlayerController` 0) true)
        (set `self.bShowMouseCursor` false)
        (message `/Game/Blueprints/Interfaces/BPI_PlayerSettings.SetMenuUp` (`GameplayStatics.GetGameInstance`) false)))))

(event `self.ReceivePossess`
  (params (PossessedPawn :type "Pawn Object Reference"))
  (`WidgetBlueprintLibrary.SetInputMode_GameOnly` (`GameplayStatics.GetPlayerController` 0) true))

(fn `UserConstructionScript`)