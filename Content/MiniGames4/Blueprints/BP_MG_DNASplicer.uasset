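; DNA splicer minigame: a player in the interaction box rotates blocks of a spinning DNA strand until their angles match randomized reference angles.
; InitGame randomizes the blocks; the action toggles between selecting and rotating, easing the spin to a stop while rotating.
; Tick projects block endpoints in simple perspective and writes them, with match indicators, to a parameter collection driving the screen material.
; Enough matches show the unblocked screen, finish the game and return the camera.
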(event `self.ReceiveBeginPlay`
  ;[1 1 1] Init
  (`parent.ReceiveBeginPlay`)
  (bind _returnvalue (`KismetMaterialLibrary.CreateDynamicMaterialInstance` "/Game/MiniGames4/Materials/MI_MG_DNADecryptor.MI_MG_DNADecryptor"))
  (set `self.DMI` _returnvalue))

(event `InitGame`
  (bind _returnvalue (`KismetMathLibrary.RandomFloatInRange` 90.0 270.0))
  (bind _linelenght (`self.LineLenght`))
  (bind _dataindices (`self.DataIndices`))
  (bind _equaltolerance (`self.EqualTolerance`))
  (bind _returnvalue_2 (- (`self.BlocksCount`) 1))
  ;[1 1 1] Init game. Prepare DNA structure with random blocks rotation
  (set `self.Selected` false)
  (set `self.SelectorIndex` 0)
  (bind _output_get (set `self.TargetRotSpeed` (`self.DNARotationSpeed`)))
  (set `self.CurrRotSpeed` _output_get)
  (`KismetArrayLibrary.Array_Clear` (`self.Data`))
  (`KismetArrayLibrary.Array_Clear` (`self.DataIndices`))
  (for _index (range (+ _returnvalue_2 1))
    (`KismetArrayLibrary.Array_Add` _dataindices _index))
  (`KismetArrayLibrary.Array_Shuffle` _dataindices)
  (for (_array_element _array_index) (`self.DataIndices`)
    (`KismetArrayLibrary.Array_Add` (`self.Data`) (make `/Game/MiniGames4/Blueprints/Data/F_MG_DNADecryptorData` _returnvalue (+ _returnvalue (`KismetMathLibrary.SelectFloat` (`KismetMathLibrary.RandomFloatInRange` -70.0 (* _equaltolerance -2.0)) (`KismetMathLibrary.RandomFloatInRange` 70.0 (* _equaltolerance 2.0)) (`KismetMathLibrary.RandomBool`))) (`KismetMathLibrary.SelectInt` -1 _array_element (== _array_element _returnvalue_2)) (+ (`KismetMathLibrary.Abs` (* (`KismetMathLibrary.Sin` (* _array_index (* (/ (`KismetMathLibrary.GetPI`) (`KismetMathLibrary.Conv_IntToDouble` (- (`self.BlocksCount`) 1))) 2.0))) (* _linelenght 0.75))) (* _linelenght 0.25)))))
  (for _index_2 (range 1 16)
    (`KismetMaterialLibrary.SetScalarParameterValue` "/Game/MiniGames4/Materials/MPC_MG_DNADecryptor.MPC_MG_DNADecryptor" (`KismetStringLibrary.Conv_StringToName` (`KismetStringLibrary.Concat_StrStr` "Line" (`KismetStringLibrary.Conv_IntToString` _index_2))))))

(event `self.InteractionBoundBox.OnComponentBeginOverlap`
  (params (OverlappedComponent :type "PrimitiveComponent Object Reference") (OtherActor :type "Actor Object Reference") (OtherComp :type "PrimitiveComponent Object Reference") (OtherBodyIndex :type Integer) (bFromSweep :type Boolean) (SweepResult :type "HitResult Structure (by ref)"))
  ;[1 1 1] Overlap events
  (`self.CheckBeginOverlap` OtherActor))

(event `self.InteractionBoundBox.OnComponentEndOverlap`
  (params (OverlappedComponent :type "PrimitiveComponent Object Reference") (OtherActor :type "Actor Object Reference") (OtherComp :type "PrimitiveComponent Object Reference") (OtherBodyIndex :type Integer))
  ;[1 1 1] Overlap events
  (`self.CheckEndOverlap` OtherActor))

(event `self.ForceAction`
  (params (Player :type "/Game/Blueprints/Characters/BP_PlayerCharacterCore Object Reference"))
  ;[1 1 1] Action
  (if (`self.PlayerOverlapped`)
    (if (`self.IsMiniGameActivated`)
      (bind _output_get (set `self.Selected` (not (`self.Selected`))))
      (if _output_get
        (set `self.TargetRotSpeed` 0.0)
        (else
          (set `self.TargetRotSpeed` (`self.DNARotationSpeed`))))
      (else
        (`self.InitGame`)
        (`PrimitiveComponent.SetMaterial` (`self.MiniGameScreen`) 0 (`self.DMI`))
        (`self.BlendCameraFromPlayerToGame` self (`self.OverlappedActor`))
        (set `self.IsMiniGameActivated` true)
        (set `self.InputEnable` true)))))

(event `CheckControls`
  (bind _rightaxis (`self.RightAxis`))
  (bind _selectorindex (`self.SelectorIndex`))
  (bind _data (`self.Data`))
  (bind (_output_angle _output_refangle _output_firstindex _output_lenght) (break `/Game/MiniGames4/Blueprints/Data/F_MG_DNADecryptorData` (`|GetArrayItem` _data _selectorindex)))
  ;[1 1 1] Controls
  (if (`self.Selected`)
    (if (!= (`self.ForwardAxis`) 0.0)
      (bind _output_get (set `self.CurrRotation Speed` (`KismetMathLibrary.FInterpTo` (`self.CurrRotation Speed`) (`self.BlockRotationSpeed`) (`self.DeltaTime`) 2.0)))
      (`KismetArrayLibrary.Array_Set` _data _selectorindex (make `/Game/MiniGames4/Blueprints/Data/F_MG_DNADecryptorData` (`self.ClampAngle` (+ (* _output_get (`self.ForwardAxis`)) _output_angle)) _output_refangle _output_firstindex _output_lenght))
      (else
        (set `self.CurrRotation Speed` 0.0)))
    (elif (!= _rightaxis 0.0)
      (if (!= (`KismetMathLibrary.SignOfFloat` _rightaxis) (`KismetMathLibrary.SignOfFloat` (`self.PrevRigthAxis`)))
        (set `self.PrevRigthAxis` _rightaxis)
        (set `self.SelectorIndex` (`KismetMathLibrary.Clamp` (+ (`self.SelectorIndex`) (`KismetMathLibrary.SelectInt` 1 -1 (> _rightaxis 0.0))) 0 (- (`self.BlocksCount`) 1))))
      (else
        (set `self.PrevRigthAxis` 0.0)))))

(event `self.ForceExit`
  ;[1 1 1] Cancel
  (if (and (`self.MiniGameEnabled`) (`self.IsMiniGameActivated`))
    (set `self.IsMiniGameActivated` false)
    (set `self.InputEnable` false)
    (`self.OnMiniGameCanceled`)
    (`self.BlendCameraFromGameToPlayer` (`self.OverlappedActor`))))

(event `self.ReceiveTick`
  (params (DeltaSeconds :type "Float (single-precision)"))
  ;[1 0 0] Tick
  (bind _output_get (set `self.DeltaTime` DeltaSeconds))
  (`parent.ReceiveTick` _output_get)
  (if (`self.IsMiniGameActivated`)
    (set `self.CurrRotation` (`self.ClampAngle` (+ (`self.CurrRotation`) (`self.CurrRotSpeed`))))
    (`self.CheckControls`)
    ;[1 1 1] Update material
    (`self.UpdateMaterial` (`self.BlocksCount`) (`self.DNADist`) (`self.SelectorIndex`) (`self.CurrRotation`))
    (set `self.CurrRotSpeed` (`KismetMathLibrary.FInterpTo` (`self.CurrRotSpeed`) (`self.TargetRotSpeed`) (`self.DeltaTime`) 4.0))
    (set `self.Solved` 0)
    (for (_array_element _array_index) (`self.Data`)
      (if (>= _array_index 0)
        (set `self.Solved` (+ (`KismetMathLibrary.SelectInt` 1 0 (`KismetMathLibrary.NearlyEqual_FloatFloat` (break `/Game/MiniGames4/Blueprints/Data/F_MG_DNADecryptorData` _array_element) (`.RefAngle_11_3187CBCF40C4079349CD568E59414C26` (break `/Game/MiniGames4/Blueprints/Data/F_MG_DNADecryptorData` _array_element)) (`self.EqualTolerance`))) (`self.Solved`)))))
    ;[1 1 1] If all blocks are rotated correctly
    (if (>= (`self.Solved`) (- (`self.BlocksCount`) 1))
      ;[1 1 1] Success
      (set `self.MiniGameEnabled` false)
      (set `self.IsMiniGameActivated` false)
      (set `self.InputEnable` false)
      (`KismetSystemLibrary.Delay` 1.0)
      (`MaterialInstanceDynamic.SetScalarParameterValue` (`self.DMI`) "ShowUnblocked" 1.0)
      (`KismetSystemLibrary.Delay` (`self.DelayTimeWhenComplete`))
      (`self.SetOfflineMaterial`)
      (`self.GameFinished` self)
      (`self.BlendCameraFromGameToPlayer` (`self.OverlappedActor`)))))

(fn `CalcLinePoints`
  (params (Angle :type "Float (double-precision)") (XOffset :type "Float (double-precision)") (Lenght :type "Float (double-precision)") (FOV :type "Float (double-precision)"))
  (returns (Result :type "LinearColor Structure") (BulbScale1 :type "Float (double-precision)") (BulbScale2 :type "Float (double-precision)"))
  (bind (_returnvalue_x _returnvalue_y _returnvalue_z) (`KismetMathLibrary.BreakVector` (`KismetMathLibrary.GreaterGreater_VectorRotator` (`KismetMathLibrary.MakeVector` XOffset Lenght) (`KismetMathLibrary.MakeRotator` Angle))))
  (bind _linelenght (`self.LineLenght`))
  (bind _linelenght_2 (`self.LineLenght`))
  (bind (_returnvalue_x_2 _returnvalue_y_2 _returnvalue_z_2) (`KismetMathLibrary.BreakVector` (`KismetMathLibrary.GreaterGreater_VectorRotator` (`KismetMathLibrary.MakeVector` XOffset (* Lenght -1.0)) (`KismetMathLibrary.MakeRotator` Angle))))
  ;[1 1 1] Calculating simple perspective projection
  (return (make `LinearColor` (+ (/ (* _returnvalue_x FOV) (+ _returnvalue_z FOV)) 0.5) (+ (/ (* _returnvalue_y FOV) (+ _returnvalue_z FOV)) 0.5) (+ (/ (* _returnvalue_x_2 FOV) (+ _returnvalue_z_2 FOV)) 0.5) (+ (/ (* _returnvalue_y_2 FOV) (+ _returnvalue_z_2 FOV)) 0.5)) (`KismetMathLibrary.MapRangeClamped` _returnvalue_z (* _linelenght_2 -1.0) _linelenght_2 1.0) (`KismetMathLibrary.MapRangeClamped` _returnvalue_z_2 (* _linelenght -1.0) _linelenght 1.0)))

(fn `ClampAngle`
  (params (Value :type "Float (double-precision)"))
  (returns (Result :type "Float (double-precision)"))
  ;[1 1 1] Clamp value 0 to 360
  (return (`KismetMathLibrary.SelectFloat` (- Value 360.0) (`KismetMathLibrary.SelectFloat` (+ Value 360.0) Value (< Value 0.0)) (> Value 360.0))))

(fn `UpdateMaterial`
  (params (Count :type Integer) (DNADist :type "Float (double-precision)") (SelectorIndex :type Integer) (Rotation :type "Float (double-precision)"))
  (locals (Rvalue :type "Float (double-precision)") (Gvalue :type "Float (double-precision)") (Count_loc :type Integer) (XOffset :type "Float (double-precision)") (DNADist_Loc :type "Float (double-precision)") (Index_loc :type Integer) (Rot_Loc :type "Float (double-precision)"))
  ;[1 1 1] Pass DNA structure data to the material
  (set `local.Count_loc` Count)
  (set `local.Index_loc` SelectorIndex)
  (set `local.DNADist_Loc` DNADist)
  (set `local.Rot_Loc` Rotation)
  (set `local.XOffset` (* (* (`local.DNADist_Loc`) -1.0) (/ (`KismetMathLibrary.Conv_IntToDouble` (- (`local.Count_loc`) 1)) 2.0)))
  (for _index (range (`local.Count_loc`))
    (bind (_output_angle _output_refangle _output_firstindex _output_lenght) (break `/Game/MiniGames4/Blueprints/Data/F_MG_DNADecryptorData` (`|GetArrayItem` (`self.Data`) _index)))
    (bind (_result _bulbscale1 _bulbscale2) (`self.CalcLinePoints` (`self.ClampAngle` (+ (`local.Rot_Loc`) _output_angle)) (`local.XOffset`) _output_lenght (`self.CamDist`)))
    (`KismetMaterialLibrary.SetVectorParameterValue` "/Game/MiniGames4/Materials/MPC_MG_DNADecryptor.MPC_MG_DNADecryptor" (`KismetStringLibrary.Conv_StringToName` (`KismetStringLibrary.Concat_StrStr` "Vector" (`KismetStringLibrary.Conv_IntToString` (+ _index 1)))) _result)
    (bind _returnvalue (* _index 2))
    (`KismetMaterialLibrary.SetScalarParameterValue` "/Game/MiniGames4/Materials/MPC_MG_DNADecryptor.MPC_MG_DNADecryptor" (`KismetStringLibrary.Conv_StringToName` (`KismetStringLibrary.Concat_StrStr` "Scalar" (`KismetStringLibrary.Conv_IntToString` (+ _returnvalue 1)))) _bulbscale1)
    (`KismetMaterialLibrary.SetScalarParameterValue` "/Game/MiniGames4/Materials/MPC_MG_DNADecryptor.MPC_MG_DNADecryptor" (`KismetStringLibrary.Conv_StringToName` (`KismetStringLibrary.Concat_StrStr` "Scalar" (`KismetStringLibrary.Conv_IntToString` (+ _returnvalue 2)))) _bulbscale2)
    (if (== _index (`local.Index_loc`))
      ;;[1 1 1] Selector
      (`KismetMaterialLibrary.SetVectorParameterValue` "/Game/MiniGames4/Materials/MPC_MG_DNADecryptor.MPC_MG_DNADecryptor" "Vector48" _result)
      (`KismetMaterialLibrary.SetScalarParameterValue` "/Game/MiniGames4/Materials/MPC_MG_DNADecryptor.MPC_MG_DNADecryptor" "Scalar33" _bulbscale1)
      (`KismetMaterialLibrary.SetScalarParameterValue` "/Game/MiniGames4/Materials/MPC_MG_DNADecryptor.MPC_MG_DNADecryptor" "Scalar34" _bulbscale2))
    (set `local.XOffset` (+ (`local.XOffset`) (`local.DNADist_Loc`)))
    (if (>= _output_firstindex 0)
      (`KismetMaterialLibrary.SetScalarParameterValue` "/Game/MiniGames4/Materials/MPC_MG_DNADecryptor.MPC_MG_DNADecryptor" (`KismetStringLibrary.Conv_StringToName` (`KismetStringLibrary.Concat_StrStr` "Line" (`KismetStringLibrary.Conv_IntToString` (+ _output_firstindex 1)))) (`KismetMathLibrary.SelectFloat` 1.0 0.0 (`KismetMathLibrary.NearlyEqual_FloatFloat` _output_angle _output_refangle (`self.EqualTolerance`)))))))

(fn `UserConstructionScript`
  (`parent.UserConstructionScript`))