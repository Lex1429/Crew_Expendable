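; Base GameState Blueprint that holds shared match state: player count, live players, player list, reactor status and which sectors have power.
; Simple events write these values or add and remove list entries, and getters expose the counts, reactor and sector power.
; Other getters for sprint, stamina, death, research points and server info are stubs returning default or empty values, likely from a shared interface.
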(event `/Game/Blueprints/Interfaces/BPI_Server.SetPlayerCount`
  (params (PlayerCount :type Integer))
  (set `self.ServerPlayerCount` PlayerCount))

(event `/Game/Blueprints/Interfaces/BPI_Server.SetLivePlayers`
  (params (LivePlayerCount :type Integer))
  (set `self.LivePlayers` LivePlayerCount))

(event `/Game/Blueprints/Interfaces/BPI_Stats.SetSectorPower`
  (params (SectorsWithPower :type "GameplayTagContainer Structure"))
  (set `self.SectorsWithPower` SectorsWithPower))

(event `/Game/Blueprints/Interfaces/BPI_Stats.SetReactorOn`
  (params (`ReactorOn?` :type Boolean))
  (set `self.ReactorOn?` `ReactorOn?`))

(event `AddToPlayerList`
  (params (Players :type "Character Object Reference (by ref)"))
  (`KismetArrayLibrary.Array_Add` (`self.Players`) Players))

(event `RemoveFromPlayerList`
  (params (Players :type "Character Object Reference (by ref)"))
  (`KismetArrayLibrary.Array_RemoveItem` (`self.Players`) Players))

(fn `GetCanSprint`
  (returns (CanSprint :type Boolean))
  (return false))

(fn `GetIsDead`
  (returns (IsDead :type Boolean))
  (return false))

(fn `GetLivePlayers`
  (returns (LivePalyerCount :type Integer))
  (return (`self.LivePlayers`)))

(fn `GetPlayerCount`
  (returns (PlayerCount :type Integer))
  (return (`self.ServerPlayerCount`)))

(fn `GetPlayerMaxStamina`
  (returns (MaxStamina :type Integer))
  (return 0))

(fn `GetPlayerStamina`
  (returns (Stamina :type Integer))
  (return 0))

(fn `GetReactorOn`
  (returns (`ReactorOn?` :type Boolean))
  (return (`self.ReactorOn?`)))

(fn `GetResearchPoints`
  (returns (ResearchPoints :type Integer))
  (return 0))

(fn `GetSectorPower`
  (returns (SectorsWithPower :type "GameplayTagContainer Structure"))
  (return (`self.SectorsWithPower`)))

(fn `GetServerCreator`
  (returns (Creator :type Text))
  (return ""))

(fn `GetServerSearch`
  (returns (SearchResult :type "BlueprintSessionResult Structure"))
  (return))

(fn `UserConstructionScript`)