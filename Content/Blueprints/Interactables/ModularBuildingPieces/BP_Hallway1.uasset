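; Modular hallway building piece whose main mesh changes look with a linked light switch.
; The construction script applies a master material to hallway, supports and legs, positions the legs from LegLength, and passes RoomTag to the overhead lamp child actor.
; At BeginPlay it binds to the light switch's toggle event, then swaps the hallway material to the on or off variant for the sector in RoomTag.
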(event `self.ReceiveBeginPlay`
  (bind _lightswitchref (`self.LightSwitchRef`))
  (`/Engine/EditorBlueprintResources/StandardMacros.IsValid` _lightswitchref
    (:`Is Valid`
      (add `/Game/Blueprints/Interactables/Buttons/BP_Lightswitch.LightSwitchToggle` _lightswitchref (`|CreateDelegate` :!event `LightSwitchToggle`)))))

(event `LightSwitchToggle`
  (params (`IsOn?` :type Boolean))
  (bind _hallway (`self.Hallway`))
  (bind _hallway_2 (`self.Hallway`))
  (if `IsOn?`
    (`|SwitchGameplayTagContainer` (`self.RoomTag`)
      (:`(GameplayTags=((TagName="Sector1.Hallways")))`
        (`PrimitiveComponent.SetMaterial` _hallway 0 "/Game/Materials/CustomTextures/V1Materials/M_Sector1_On.M_Sector1_On"))
      (:`(GameplayTags=((TagName="Sector2.Hallways")))`
        (`PrimitiveComponent.SetMaterial` _hallway 0 "/Game/Materials/CustomTextures/V1Materials/M_Sector2_On.M_Sector2_On"))
      (:`(GameplayTags=((TagName="Sector3.Hallways")))`
        (`PrimitiveComponent.SetMaterial` _hallway 0 "/Game/Materials/CustomTextures/V1Materials/M_Sector3_On.M_Sector3_On"))
      (:`(GameplayTags=((TagName="Sector4.Hallways")))`
        (`PrimitiveComponent.SetMaterial` _hallway 0 "/Game/Materials/CustomTextures/V1Materials/M_Sector4_On.M_Sector4_On"))
      (:`(GameplayTags=((TagName="Sector5.Hallways")))`
        (`PrimitiveComponent.SetMaterial` _hallway 0 "/Game/Materials/CustomTextures/V1Materials/M_Sector5_On.M_Sector5_On")))
    (else
      (`|SwitchGameplayTagContainer` (`self.RoomTag`)
        (:`(GameplayTags=((TagName="Sector1.Hallways")))`
          (`PrimitiveComponent.SetMaterial` _hallway_2 0 "/Game/Materials/CustomTextures/V1Materials/M_Sector1_Off.M_Sector1_Off"))
        (:`(GameplayTags=((TagName="Sector2.Hallways")))`
          (`PrimitiveComponent.SetMaterial` _hallway_2 0 "/Game/Materials/CustomTextures/V1Materials/M_Sector2_Off.M_Sector2_Off"))
        (:`(GameplayTags=((TagName="Sector3.Hallways")))`
          (`PrimitiveComponent.SetMaterial` _hallway_2 0 "/Game/Materials/CustomTextures/V1Materials/M_Sector3_Off.M_Sector3_Off"))
        (:`(GameplayTags=((TagName="Sector4.Hallways")))`
          (`PrimitiveComponent.SetMaterial` _hallway_2 0 "/Game/Materials/CustomTextures/V1Materials/M_Sector4_Off.M_Sector4_Off"))
        (:`(GameplayTags=((TagName="Sector5.Hallways")))`
          (`PrimitiveComponent.SetMaterial` _hallway_2 0 "/Game/Materials/CustomTextures/V1Materials/M_Sector5_Off.M_Sector5_Off"))))))

(fn `UserConstructionScript`
  (bind _leglength (`self.LegLength`))
  (`PrimitiveComponent.SetMaterial` (`self.Hallway`) 0 (`self.MasterMaterial`))
  (`PrimitiveComponent.SetMaterial` (`self.Support1`) 0 (`self.MasterMaterial`))
  (`PrimitiveComponent.SetMaterial` (`self.Leg1`) 0 (`self.MasterMaterial`))
  (`PrimitiveComponent.SetMaterial` (`self.Support2`) 0 (`self.MasterMaterial`))
  (`PrimitiveComponent.SetMaterial` (`self.Leg2`) 0 (`self.MasterMaterial`))
  (`SceneComponent.K2_SetRelativeLocation` (`self.Leg1`) (`KismetMathLibrary.MakeVector` 0.0 155.0 _leglength) false false)
  (`SceneComponent.K2_SetRelativeLocation` (`self.Leg2`) (`KismetMathLibrary.MakeVector` 0.0 155.0 _leglength) false false)
  (bind _asbp_lamp_base (cast `/Game/Blueprints/Interactables/CealingLights/BP_LampBase` (`ChildActorComponent.ChildActor` (`self.OverheadLight1`))))
  (set `/Game/Blueprints/Interactables/CealingLights/BP_LampBase.RoomTag` (`self.RoomTag`) _asbp_lamp_base))