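; Switch-panel minigame actor where the player toggles the right combination of 5–7 pins to reach full power.
; SetupPins shuffles solver pins, normalized to total one, among negative or high-value decoys.
; A looping timer polls axis input for selection; action toggles animate pins and recompute power, all displayed through a dynamic screen material.
; Overload flags an error and re-randomizes the puzzle; enabling exactly the solver pins reports success.
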(event `self.ReceiveBeginPlay`
  ;[1 1 1] Init
  (`parent.ReceiveBeginPlay`)
  (set `self.IsMiniGameActivated` false)
  (set `self.InputEnable` false)
  (bind _returnvalue (`KismetSystemLibrary.K2_SetTimer` null "CheckContorls" 0.05 true))
  (bind _output_get (set `self.TimeHandle` _returnvalue))
  (`KismetSystemLibrary.K2_UnPauseTimerHandle` _output_get)
  (bind _returnvalue_2 (`KismetMaterialLibrary.CreateDynamicMaterialInstance` "/Game/MiniGames2/Materials/MI_MiniGameSwitcher_Inst.MI_MiniGameSwitcher_Inst"))
  (set `self.DMI` _returnvalue_2))

(event `ReInitGame`
  (bind _dmi (`self.DMI`))
  (bind _dmi_2 (`self.DMI`))
  (bind _dmi_3 (`self.DMI`))
  ;[1 1 1] ReInit
  (set `self.ResultPower` 0.0)
  (`KismetArrayLibrary.Array_Clear` (`self.PinData`))
  (set `self.Reinit` false)
  (bind _output_get (set `self.SolversCount` (select `/Game/MiniGames2/Blueprints/Data/E_MG_SwitcherCount` (`self.PinsCount`) :`NewEnumerator0` (`KismetMathLibrary.RandomIntegerInRange` 1 2) :`NewEnumerator1` (`KismetMathLibrary.RandomIntegerInRange` 2 3) :`NewEnumerator2` (`KismetMathLibrary.RandomIntegerInRange` 3 4))))
  (`self.SetupPins` (select `/Game/MiniGames2/Blueprints/Data/E_MG_SwitcherCount` (`self.PinsCount`) :`NewEnumerator0` 4 :`NewEnumerator1` 5 :`NewEnumerator2` 6) _output_get)
  (`MaterialInstanceDynamic.SetScalarParameterValue` (`self.DMI`) "PowerProgress" 0.0)
  (`MaterialInstanceDynamic.SetScalarParameterValue` (`self.DMI`) "ShowError" 0.0)
  (`MaterialInstanceDynamic.SetScalarParameterValue` (`self.DMI`) "ShowEnabled" 0.0)
  (switch `/Game/MiniGames2/Blueprints/Data/E_MG_SwitcherCount` (`self.PinsCount`)
    (:`NewEnumerator0`
      (`MaterialInstanceDynamic.SetScalarParameterValue` _dmi "Pin6_Vis" 0.0)
      (`MaterialInstanceDynamic.SetScalarParameterValue` _dmi "Pin7_Vis" 0.0)
      (`MaterialInstanceDynamic.SetScalarParameterValue` _dmi "Pin1_OX" 0.2)
      (`MaterialInstanceDynamic.SetScalarParameterValue` _dmi "Pin2_OX" 0.1)
      (`MaterialInstanceDynamic.SetScalarParameterValue` _dmi "Pin3_OX" 0.0)
      (`MaterialInstanceDynamic.SetScalarParameterValue` _dmi "Pin4_OX" -0.1)
      (`MaterialInstanceDynamic.SetScalarParameterValue` _dmi "Pin5_OX" -0.2)
      (`MaterialInstanceDynamic.SetScalarParameterValue` _dmi "Pin6_OX" -0.25)
      (`MaterialInstanceDynamic.SetScalarParameterValue` _dmi "Pin7_OX" -0.3))
    (:`NewEnumerator1`
      (`MaterialInstanceDynamic.SetScalarParameterValue` _dmi_2 "Pin6_Vis" 1.0)
      (`MaterialInstanceDynamic.SetScalarParameterValue` _dmi_2 "Pin7_Vis" 0.0)
      (`MaterialInstanceDynamic.SetScalarParameterValue` _dmi_2 "Pin1_OX" 0.25)
      (`MaterialInstanceDynamic.SetScalarParameterValue` _dmi_2 "Pin2_OX" 0.15)
      (`MaterialInstanceDynamic.SetScalarParameterValue` _dmi_2 "Pin3_OX" 0.05)
      (`MaterialInstanceDynamic.SetScalarParameterValue` _dmi_2 "Pin4_OX" -0.05)
      (`MaterialInstanceDynamic.SetScalarParameterValue` _dmi_2 "Pin5_OX" -0.15)
      (`MaterialInstanceDynamic.SetScalarParameterValue` _dmi_2 "Pin6_OX" -0.25)
      (`MaterialInstanceDynamic.SetScalarParameterValue` _dmi_2 "Pin7_OX" -0.3))
    (:`NewEnumerator2`
      (`MaterialInstanceDynamic.SetScalarParameterValue` _dmi_3 "Pin6_Vis" 1.0)
      (`MaterialInstanceDynamic.SetScalarParameterValue` _dmi_3 "Pin7_Vis" 1.0)
      (`MaterialInstanceDynamic.SetScalarParameterValue` _dmi_3 "Pin1_OX" 0.3)
      (`MaterialInstanceDynamic.SetScalarParameterValue` _dmi_3 "Pin2_OX" 0.2)
      (`MaterialInstanceDynamic.SetScalarParameterValue` _dmi_3 "Pin3_OX" 0.1)
      (`MaterialInstanceDynamic.SetScalarParameterValue` _dmi_3 "Pin4_OX" 0.0)
      (`MaterialInstanceDynamic.SetScalarParameterValue` _dmi_3 "Pin5_OX" -0.1)
      (`MaterialInstanceDynamic.SetScalarParameterValue` _dmi_3 "Pin6_OX" -0.2)
      (`MaterialInstanceDynamic.SetScalarParameterValue` _dmi_3 "Pin7_OX" -0.3)))
  (set `self.Value` 0.0)
  (`self.ResetPins`)
  (for _index (range 7)
    (set `self.PinIndex` _index)
    (`self.ForceUpdatePins`))
  (set `self.PinIndex` 0)
  (`MaterialInstanceDynamic.SetScalarParameterValue` (`self.DMI`) "Fold1_Sel" 1.0))

(event `ResetPins`
  (bind _dmi (`self.DMI`))
  ;[1 1 1] Controls
  (`MaterialInstanceDynamic.SetScalarParameterValue` _dmi "Fold1_Sel" 0.0)
  (`MaterialInstanceDynamic.SetScalarParameterValue` _dmi "Fold2_Sel" 0.0)
  (`MaterialInstanceDynamic.SetScalarParameterValue` _dmi "Fold3_Sel" 0.0)
  (`MaterialInstanceDynamic.SetScalarParameterValue` _dmi "Fold4_Sel" 0.0)
  (`MaterialInstanceDynamic.SetScalarParameterValue` _dmi "Fold5_Sel" 0.0)
  (`MaterialInstanceDynamic.SetScalarParameterValue` _dmi "Fold6_Sel" 0.0)
  (`MaterialInstanceDynamic.SetScalarParameterValue` _dmi "Fold7_Sel" 0.0))

(event `CheckContorls`
  (bind _dmi (`self.DMI`))
  (bind _rightaxis (`self.RightAxis`))
  ;[1 1 1] Controls
  (if (`self.InputEnable`)
    (if (`self.IsMiniGameActivated`)
      (if (!= _rightaxis 0.0)
        (if (`self.RightAxisEnable`)
          (set `self.RightAxisEnable` false)
          (set `self.SelectorSign` (`KismetMathLibrary.FTrunc` (`KismetMathLibrary.SignOfFloat` _rightaxis)))
          (bind _output_get (set `self.PinIndex` (`KismetMathLibrary.Clamp` (+ (`self.PinIndex`) (`self.SelectorSign`)) 0 (select `/Game/MiniGames2/Blueprints/Data/E_MG_SwitcherCount` (`self.PinsCount`) :`NewEnumerator0` 4 :`NewEnumerator1` 5 :`NewEnumerator2` 6))))
          ;;[1 1 1] For debug
          (if (`self.DebugPins`)
            (bind (_pinvalue _enabled _issolver) (break `/Game/MiniGames2/Blueprints/Data/F_MG_SwitcherPin` (`|GetArrayItem` (`self.PinData`) _output_get)))
            (`KismetSystemLibrary.PrintString` (`KismetTextLibrary.Conv_TextToString` (select `bool` _issolver :`false` "Wrong pin" :`true` "Correct pin" :!type "Text")) true true (`KismetMathLibrary.SelectColor` (make `LinearColor` 0.0 1.0 0.0 1.0) (make `LinearColor` 1.0 0.0 0.0 1.0) _issolver)))
          (`self.ResetPins`)
          (switch `int` _output_get
            (:`0`
              (`MaterialInstanceDynamic.SetScalarParameterValue` _dmi "Fold1_Sel" 1.0))
            (:`1`
              (`MaterialInstanceDynamic.SetScalarParameterValue` _dmi "Fold2_Sel" 1.0))
            (:`2`
              (`MaterialInstanceDynamic.SetScalarParameterValue` _dmi "Fold3_Sel" 1.0))
            (:`3`
              (`MaterialInstanceDynamic.SetScalarParameterValue` _dmi "Fold4_Sel" 1.0))
            (:`4`
              (`MaterialInstanceDynamic.SetScalarParameterValue` _dmi "Fold5_Sel" 1.0))
            (:`5`
              (`MaterialInstanceDynamic.SetScalarParameterValue` _dmi "Fold6_Sel" 1.0))
            (:`6`
              (`MaterialInstanceDynamic.SetScalarParameterValue` _dmi "Fold7_Sel" 1.0))))
        (else
          (set `self.RightAxisEnable` true))))))

(event `ForceUpdatePins`
  (bind _dmi (`self.DMI`))
  (bind _value (`self.Value`))
  ;[1 1 1] Action button
  (switch `int` (`self.PinIndex`) :!label _label
    (:`0`
      (`MaterialInstanceDynamic.SetScalarParameterValue` _dmi "Pin1_Ypos" _value))
    (:`1`
      (`MaterialInstanceDynamic.SetScalarParameterValue` _dmi "Pin2_Ypos" _value))
    (:`2`
      (`MaterialInstanceDynamic.SetScalarParameterValue` _dmi "Pin3_Ypos" _value))
    (:`3`
      (`MaterialInstanceDynamic.SetScalarParameterValue` _dmi "Pin4_Ypos" _value))
    (:`4`
      (`MaterialInstanceDynamic.SetScalarParameterValue` _dmi "Pin5_Ypos" _value))
    (:`5`
      (`MaterialInstanceDynamic.SetScalarParameterValue` _dmi "Pin6_Ypos" _value))
    (:`6`
      (`MaterialInstanceDynamic.SetScalarParameterValue` _dmi "Pin7_Ypos" _value))))

(event `self.ForceAction`
  (bind _limitpinypos (`self.LimitPinYpos`))
  (bind _output (`|GetArrayItem` (`self.PinData`) (`self.PinIndex`)))
  ;[1 1 1] Action button
  (if (`self.PlayerOverlapped`)
    (if (`self.IsMiniGameActivated`)
      (if (`self.InputEnable`)
        (set `self.InputEnable` false)
        (bind _output_get (set `self.IsPinEnabled` (`.Enabled_5_DE2A55DD40E3C576F49FAE85F166C401` (break `/Game/MiniGames2/Blueprints/Data/F_MG_SwitcherPin` _output))))
        (setmembers `/Game/MiniGames2/Blueprints/Data/F_MG_SwitcherPin` :`StructRef` _output :`Enabled` (not _output_get))
        (bind (_direction _newtrack_0) (`Timeline|Timeline_0` :!via `PlayFromStart`)
          (:`Update`
            (set `self.Value` (`KismetMathLibrary.SelectFloat` (`KismetMathLibrary.Lerp` _limitpinypos 0.0 _newtrack_0) (`KismetMathLibrary.Lerp` 0.0 _limitpinypos _newtrack_0) (`self.IsPinEnabled`)))
            (goto _label))
          (:`Finished`
            (set `self.InputEnable` true)
            (`self.UpdateCheckPins`))))
      (else
        (`self.ReInitGame`)
        (`PrimitiveComponent.SetMaterial` (`self.MiniGameScreen`) 0 (`self.DMI`))
        (set `self.IsMiniGameActivated` true)
        (set `self.InputEnable` true)))))

(event `UpdateCheckPins`
  (bind _errorsound (`self.ErrorSound`))
  (bind _powerval (`self.PowerVal`))
  (bind _downpin (`self.DownPin`))
  (bind _returnvalue (+ (`self.SolversCount`) 1))
  ;[1 1 1] Update pins and power. Check value
  (set `self.PowerVal` 0.0)
  (set `self.EnabledPins` 0)
  (set `self.SolversEnabled` 0)
  (set `self.DownPin` 0)
  (for _array_element (`self.PinData`)
    (bind (_pinvalue _enabled _issolver) (break `/Game/MiniGames2/Blueprints/Data/F_MG_SwitcherPin` _array_element))
    (if _enabled
      (`/Engine/EditorBlueprintResources/StandardMacros.IncrementInt` (`self.EnabledPins`)
        (:`  `
          (if _issolver
            (`/Engine/EditorBlueprintResources/StandardMacros.IncrementInt` (`self.SolversEnabled`)
              (:`  `
                (set `self.PowerVal` (+ _pinvalue (`self.PowerVal`)) :!label _label_2)))
            (elif (> _pinvalue 0.0)
              (goto _label_2)
              (else
                (`/Engine/EditorBlueprintResources/StandardMacros.IncrementInt` (`self.DownPin`)))))))))
  (if (`KismetMathLibrary.NearlyEqual_FloatFloat` _powerval 2.0 0.01)
    (set `self.ResultPower` 2.5)
    (else
      (set `self.ResultPower` (/ _powerval (`KismetMathLibrary.SelectFloat` (`KismetMathLibrary.Conv_IntToDouble` (* _downpin 2)) 1.0 (> _downpin 0))))))
  (`MaterialInstanceDynamic.SetScalarParameterValue` (`self.DMI`) "PowerProgress" (`KismetMathLibrary.FClamp` (`self.ResultPower`)))
  ;;[0.01729 0.9203 1] Check power value
  (if (> (`self.ResultPower`) 1.05)
    ;;[1 1 1] Error
    (set `self.StartTime` (`KismetSystemLibrary.GetGameTimeInSeconds`))
    (set `self.Counter_0` 0)
    (`MaterialInstanceDynamic.SetScalarParameterValue` (`self.DMI`) "ShowError" 1.0)
    (set `self.InputEnable` false)
    (set `self.Reinit` true)
    (`/Engine/EditorBlueprintResources/StandardMacros.IsValid` _errorsound
      (:`Is Valid`
        (`GameplayStatics.PlaySoundAtLocation` _errorsound (`self.K2_GetActorLocation` self) (struct) 1.0 1.0 0.0 null null null null)))
    (else
      ;;[1 1 1] Success
      (if (and (== _returnvalue (`self.SolversEnabled`)) (== _returnvalue (`self.EnabledPins`)))
        (set `self.MiniGameEnabled` false)
        (set `self.IsMiniGameActivated` false)
        (set `self.InputEnable` false)
        (`MaterialInstanceDynamic.SetScalarParameterValue` (`self.DMI`) "ShowEnabled" 1.0)
        (`KismetSystemLibrary.Delay` (`self.DelayTimeWhenComplete`))
        (`self.SetOfflineMaterial`)
        (`self.OnMiniGameSuccess`)))))

(event `self.ReceiveTick`
  (params (DeltaSeconds :type "Float (single-precision)"))
  ;[1 1 1] Reinit game if wrong power value is calculated
  (`parent.ReceiveTick` DeltaSeconds)
  (if (`self.IsMiniGameActivated`)
    (if (`self.Reinit`)
      (if (>= (`self.Counter_0`) 35)
        (set `self.Reinit` false)
        (`MaterialInstanceDynamic.SetScalarParameterValue` (`self.DMI`) "ShowError" 0.0)
        (`KismetSystemLibrary.Delay` 0.2)
        (bind (_direction _newtrack_0) (`Timeline|Timeline_1` :!via `PlayFromStart`)
          (:`Update`
            (for (_array_element _array_index) (`self.PinData`)
              (set `self.PinIndex` _array_index)
              (set `self.Value` (`KismetMathLibrary.SelectFloat` (`KismetMathLibrary.Lerp` (`self.LimitPinYpos`) 0.0 _newtrack_0) 0.0 (`.Enabled_5_DE2A55DD40E3C576F49FAE85F166C401` (break `/Game/MiniGames2/Blueprints/Data/F_MG_SwitcherPin` _array_element))))
              (`self.ForceUpdatePins`)))
          (:`Finished`
            (`self.ReInitGame`)
            (set `self.InputEnable` true)))
        (elif (>= (- (`KismetSystemLibrary.GetGameTimeInSeconds`) (`self.StartTime`)) 0.035)
          (set `self.StartTime` (`KismetSystemLibrary.GetGameTimeInSeconds`))
          (`/Engine/EditorBlueprintResources/StandardMacros.IncrementInt` (`self.Counter_0`)))))))

(event `self.InteractionBoundBox.OnComponentBeginOverlap`
  (params (OverlappedComponent :type "PrimitiveComponent Object Reference") (OtherActor :type "Actor Object Reference") (OtherComp :type "PrimitiveComponent Object Reference") (OtherBodyIndex :type Integer) (bFromSweep :type Boolean) (SweepResult :type "HitResult Structure (by ref)"))
  ;[1 1 1] Check Player overlapping
  (`self.CheckBeginOverlap` OtherActor))

(event `self.InteractionBoundBox.OnComponentEndOverlap`
  (params (OverlappedComponent :type "PrimitiveComponent Object Reference") (OtherActor :type "Actor Object Reference") (OtherComp :type "PrimitiveComponent Object Reference") (OtherBodyIndex :type Integer))
  ;[1 1 1] Check Player overlapping
  (`self.CheckEndOverlap` OtherActor))

(event `self.ForceExit`
  ;[1 1 1] Cancel
  (if (and (`self.MiniGameEnabled`) (`self.IsMiniGameActivated`))
    (set `self.IsMiniGameActivated` false)
    (set `self.InputEnable` false)
    (`self.OnMiniGameCanceled`)))

(fn `SetupPins`
  (params (TotalCount :type Integer) (SolverCount :type Integer))
  (locals (PinValueArray :type "Array of Integer") (Summ :type Integer) (Val :type Integer) (FinalVal :type "Float (double-precision)") (IsSolver :type Boolean) (MinSolverValue :type "Float (double-precision)") (Ind1 :type Integer) (Ind2 :type Integer) (Val1 :type "/Game/MiniGames2/Blueprints/Data/F_MG_SwitcherPin Structure") (Val2 :type "/Game/MiniGames2/Blueprints/Data/F_MG_SwitcherPin Structure"))
  (bind _pindata (`self.PinData`))
  (bind _pinvaluearray (`local.PinValueArray`))
  ;[1 1 1] Set randomized values for pins. Then normalize values based on active pins count
  (set `local.Summ` 0)
  (`KismetArrayLibrary.Array_Clear` _pinvaluearray)
  (for _index (range (+ TotalCount 1))
    (bind _output_get (set `local.Val` (`KismetMathLibrary.RandomIntegerInRange` 10 70)))
    (`KismetArrayLibrary.Array_Add` _pinvaluearray _output_get)
    (if (<= _index SolverCount)
      (set `local.Summ` (+ (`local.Summ`) _output_get))))
  (for _index_2 (range (+ TotalCount 1))
    (if (<= _index_2 SolverCount)
      (set `local.FinalVal` (/ (* (`KismetMathLibrary.Conv_IntToDouble` (`|GetArrayItem` (`local.PinValueArray`) _index_2)) (/ 100.0 (`KismetMathLibrary.Conv_IntToDouble` (`local.Summ`)))) 100.0))
      (set `local.IsSolver` true)
      (else
        (set `local.FinalVal` (`KismetMathLibrary.SelectFloat` (`KismetMathLibrary.RandomFloatInRange` -0.1 -0.5) 0.95 (>= (`KismetMathLibrary.RandomIntegerInRange` 0 10) 6)))
        (set `local.IsSolver` false)))
    (`KismetArrayLibrary.Array_Add` (`self.PinData`) (make `/Game/MiniGames2/Blueprints/Data/F_MG_SwitcherPin` (`local.FinalVal`) false (`local.IsSolver`))))
  (for _ (range 6)
    ;;[1 0.07657 0] For Nativization compatibility
    (set `local.Ind1` (`KismetMathLibrary.RandomIntegerInRange` 0 TotalCount))
    (set `local.Ind2` (`KismetMathLibrary.RandomIntegerInRange` 0 TotalCount))
    (set `local.Val1` (`|GetArrayItem` _pindata (`local.Ind1`)))
    (set `local.Val2` (`|GetArrayItem` _pindata (`local.Ind2`)))
    (`KismetArrayLibrary.Array_Set` _pindata (`local.Ind1`) (`local.Val2`))
    (`KismetArrayLibrary.Array_Set` _pindata (`local.Ind2`) (`local.Val1`))))

(fn `UserConstructionScript`
  (`parent.UserConstructionScript`))