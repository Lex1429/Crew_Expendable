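; Minigame vent Actor with a lid that toggles open or closed on both begin and end overlap, through a Server-to-Local event pair.
; Timelines drive the lid rotation and slide the cooling filter from seated to removed position.
; Overlap also binds to the cooling filter pickup's pull event, which animates removal when it is pickable and in the AC.
; Unfinished: Interact routes to an empty local pull event, and filter selection and pickup getters are stubs.
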(event `self.ReceiveBeginPlay`
  (`|ExecutionSequence`
    (:`then_0`
      (bind _returnvalue (`GameplayStatics.GetActorOfClass` "/Game/Blueprints/Interactables/MiniGames/Pickups/BP_MG_HeatFilterPickup.BP_MG_HeatFilterPickup_C"))
      (set `self.HeatRef` _returnvalue))
    (:`then_1`
      (bind _returnvalue_2 (`GameplayStatics.GetActorOfClass` "/Game/Blueprints/Interactables/MiniGames/Pickups/BP_MG_CoolingFilterPickup.BP_MG_CoolingFilterPickup_C"))
      (set `self.CoolRef` _returnvalue_2))))

(event `Server_OpenVent`
  ;[0 0.03425 1] Baseline works. Need to add in logic.
  (`self.Local_OpenVent`))

(event `Local_OpenVent`
  ;[0 0.03425 1] Baseline works. Need to add in logic.
  (if (not (`self.VentOpen?`))
    (set `self.VentOpen?` true)
    (bind (_direction _newtrack_0) (`Timeline|VentOpen` :!label _label)
      (:`Update`
        (`SceneComponent.K2_SetRelativeRotation` (`self.VentLid`) (`KismetMathLibrary.RLerp` (`self.VentLidOpen`) (`self.VentLidClosed`) _newtrack_0) false true)))
    (else
      (set `self.VentOpen?` false)
      (goto _label :!via `Reverse`))))

(event `self.ReceiveActorBeginOverlap`
  (params (OtherActor :type "Actor Object Reference"))
  (`self.Server_OpenVent` :!label _label_2)
  (bind _coolref (`self.CoolRef`)
    (:`then`
      (add `/Game/Blueprints/Interactables/MiniGames/Pickups/BP_MG_CoolingFilterPickup.PullingFilter` _coolref (delegate `Test_PullFilter`)))
    (:`else`)))

(event `self.ReceiveActorEndOverlap`
  (params (OtherActor :type "Actor Object Reference"))
  (goto _label_2))

(event `Test_PullFilter`
  (bind _coolref (`self.CoolRef`))
  (if (and (`/Game/Blueprints/Interactables/Pickups/BP_PrimaryWeaponPickup.CanBePickedUp?` _coolref) (`/Game/Blueprints/Interactables/MiniGames/Pickups/BP_MG_CoolingFilterPickup.InAC?` _coolref))
    (bind (_direction _newtrack_0) (`Timeline|FilterRemove`)
      (:`Update`
        (`SceneComponent.K2_SetRelativeLocation` (`self.FilterCool`) (`KismetMathLibrary.VLerp` (`self.CoolingSeatedPos`) (`self.CoolingRemovePos`) _newtrack_0) false true)))))

(event `Local_PullFilter`
  (params (Character :type "/Game/Blueprints/Characters/BP_BaseCharacter Object Reference")))

(event `/Game/Blueprints/Interfaces/BPI_Interact.Interact`
  (params (Character :type "/Game/Blueprints/Characters/BP_BaseCharacter Object Reference"))
  (`self.Server_PullFilter` Character))

(event `Server_PullFilter`
  (params (Character :type "/Game/Blueprints/Characters/BP_BaseCharacter Object Reference"))
  (`self.Local_PullFilter` Character))

(fn `FilterSelect`
  (bind _selectedfilter (`self.SelectedFilter`)
    (:`then`
      _)
    (:`else`
      _))
  (bind _item (message `/Game/Blueprints/Interfaces/BPI_Interact.GetItemToSpawn` _selectedfilter))
  (bind _output_get (set `self.FilterToSpawn` _item))
  (if (== _output_get "/Game/Blueprints/Interactables/MiniGames/Components/BP_MG_HeatFilter.BP_MG_HeatFilter_C")
    (set `self.SelectedFilter` null)
    (else
      (set `self.SelectedFilter` null))))

(fn `GetCanBePickedUp`
  (returns (CanBePickedUp :type Boolean))
  (return false))

(fn `GetItemToSpawn`
  (returns (Item :type "/Game/Blueprints/Interactables/Weapons/BP_WeaponComponentMaster Class Reference"))
  (return null))

(fn `UserConstructionScript`)