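; BP_UtilityPickup is an interactable pickup that gives the interacting character an item and then removes itself.
; Interact passes the character and the ItemToSpawn variable to the Server_SpawnItem event.
; That event calls SpawnPrimaryWeapon on the character, leaving the ItemToSpawn argument unused, then destroys the pickup.
; BeginPlay, overlap and Tick are disabled stubs, so pickup happens only through interaction.
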(event `/Game/Blueprints/Interfaces/BPI_Interact.Interact`
  (params (Character :type "/Game/Blueprints/Characters/BP_BaseCharacter Object Reference"))
  (`self.Server_SpawnItem` Character (`self.ItemToSpawn`)))

(event `Server_SpawnItem`
  (params (Target :type "/Game/Blueprints/Characters/BP_BaseCharacter Object Reference") (ItemToSpawn :type "/Game/Blueprints/Interactables/Weapons/BP_WeaponComponentMaster Class Reference"))
  (`/Game/Blueprints/Characters/BP_BaseCharacter.SpawnPrimaryWeapon` Target null)
  (`self.K2_DestroyActor`))

(fn `UserConstructionScript`
  (`parent.UserConstructionScript`))