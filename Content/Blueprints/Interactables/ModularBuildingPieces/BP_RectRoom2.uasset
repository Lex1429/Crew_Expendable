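; Modular rectangular room building piece with four optional end caps and a light-switch-driven material.
; The construction script applies the building material to the room and caps, then shows or hides each cap and its window, moving hidden caps upward.
; On BeginPlay it binds to an optional referenced light switch.
; Toggling swaps only the room's material between on and off variants chosen by the room's sector gameplay tag.
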(event `self.ReceiveBeginPlay`
  (bind _lightswitchref (`self.LightSwitchRef`))
  (`/Engine/EditorBlueprintResources/StandardMacros.IsValid` _lightswitchref
    (:`Is Valid`
      (add `/Game/Blueprints/Interactables/Buttons/BP_Lightswitch.LightSwitchToggle` _lightswitchref (`|CreateDelegate` :!event `LightSwitchToggle`)))))

(event `LightSwitchToggle`
  (params (`IsOn?` :type Boolean))
  (bind _room (`self.Room`))
  (if `IsOn?`
    (`|SwitchGameplayTagContainer` (`self.RoomTag`)
      (:`(GameplayTags=((TagName="Sector2.Servers")))`
        (`PrimitiveComponent.SetMaterial` _room 0 "/Game/Materials/CustomTextures/V1Materials/M_Sector2_On.M_Sector2_On"))
      (:`(GameplayTags=((TagName="Sector3.Engineering")))`
        (`PrimitiveComponent.SetMaterial` _room 0 "/Game/Materials/CustomTextures/V1Materials/M_Sector3_On.M_Sector3_On"))
      (:`(GameplayTags=((TagName="Sector5.CargoBay")))`
        (`PrimitiveComponent.SetMaterial` _room 0 "/Game/Materials/CustomTextures/V1Materials/M_Sector5_On.M_Sector5_On")))
    (else
      (`|SwitchGameplayTagContainer` (`self.RoomTag`)
        (:`(GameplayTags=((TagName="Sector2.Servers")))`
          (`PrimitiveComponent.SetMaterial` _room 0 "/Game/Materials/CustomTextures/V1Materials/M_Sector2_Off.M_Sector2_Off"))
        (:`(GameplayTags=((TagName="Sector3.Engineering")))`
          (`PrimitiveComponent.SetMaterial` _room 0 "/Game/Materials/CustomTextures/V1Materials/M_Sector3_Off.M_Sector3_Off"))
        (:`(GameplayTags=((TagName="Sector5.CargoBay")))`
          (`PrimitiveComponent.SetMaterial` _room 0 "/Game/Materials/CustomTextures/V1Materials/M_Sector5_Off.M_Sector5_Off"))))))

(fn `UserConstructionScript`
  (bind _endcap1 (`self.EndCap1`))
  (bind _endcap4 (`self.EndCap4`))
  (bind _endcap4_2 (`self.EndCap4`))
  (bind _endcap1_2 (`self.EndCap1`))
  (`PrimitiveComponent.SetMaterial` (`self.Room`) 0 (`self.BuildingMaterial`))
  (`PrimitiveComponent.SetMaterial` (`self.EndCap1`) 0 (`self.BuildingMaterial`))
  (`PrimitiveComponent.SetMaterial` (`self.EndCap2`) 0 (`self.BuildingMaterial`))
  (`PrimitiveComponent.SetMaterial` (`self.EndCap3`) 0 (`self.BuildingMaterial`))
  (`PrimitiveComponent.SetMaterial` (`self.EndCap4`) 0 (`self.BuildingMaterial`))
  (`|ExecutionSequence`
    (:`then_0`
      (if (`self.Endcap1On?`)
        (`SceneComponent.SetVisibility` _endcap1 true false)
        (`SceneComponent.SetVisibility` (`self.Window1`) true false)
        (`SceneComponent.K2_SetRelativeLocation` _endcap1 (0.0 -480.0 0.0) false false)
        (else
          (`SceneComponent.SetVisibility` _endcap1_2 false false)
          (`SceneComponent.SetVisibility` (`self.Window1`) false false)
          (`SceneComponent.K2_SetRelativeLocation` _endcap1_2 (-0.0 -480.0 400.0) false false))))
    (:`then_1`
      (if (`self.Endcap2On?`)
        (`SceneComponent.SetVisibility` (`self.Window2`) true false)
        (`SceneComponent.SetVisibility` (`self.EndCap2`) true false)
        (`SceneComponent.K2_SetRelativeLocation` (`self.EndCap2`) (0.0 480.0 0.0) false false)
        (else
          (`SceneComponent.SetVisibility` (`self.Window2`) false false)
          (`SceneComponent.SetVisibility` (`self.EndCap2`) false false)
          (`SceneComponent.K2_SetRelativeLocation` (`self.EndCap2`) (0.0 480.0 400.0) false false))))
    (:`then_2`
      (if (`self.EndCap3On?`)
        (`SceneComponent.SetVisibility` (`self.Window3`) true false)
        (`SceneComponent.SetVisibility` (`self.EndCap3`) true false)
        (`SceneComponent.K2_SetRelativeLocation` (`self.EndCap3`) (980.0 0.0 0.0) false false)
        (else
          (`SceneComponent.SetVisibility` (`self.Window3`) false false)
          (`SceneComponent.SetVisibility` (`self.EndCap3`) false false)
          (`SceneComponent.K2_SetRelativeLocation` (`self.EndCap3`) (980.0 0.0 400.0) false false))))
    (:`then_3`
      (if (`self.EndCap4On?`)
        (`SceneComponent.SetVisibility` _endcap4_2 true false)
        (`SceneComponent.SetVisibility` (`self.Window4`) true false)
        (`SceneComponent.K2_SetRelativeLocation` _endcap4_2 (-980.0 0.0 0.0) false false)
        (else
          (`SceneComponent.SetVisibility` _endcap4 false false)
          (`SceneComponent.SetVisibility` (`self.Window4`) false false)
          (`SceneComponent.K2_SetRelativeLocation` _endcap4 (-980.0 0.0 400.0) false false))))))