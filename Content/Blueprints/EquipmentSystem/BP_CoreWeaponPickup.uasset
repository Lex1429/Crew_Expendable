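; Weapon pickup actor that shows an interaction prompt and hands its weapon ID to the player character when used.
; SetUpPickUp, run at construction and BeginPlay, reads the DT_WeaponDetails row for WeaponID to set the mesh and display name.
; SetFocused shows the "Pick Up" prompt on WB_PlayerUI, using a retriggerable delay to clear it once focus calls stop.
; Interact passes the ID to HandlePickupMessage, destroys the actor and clears the prompt.
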(event `self.ReceiveBeginPlay`
  (`parent.ReceiveBeginPlay`)
  (`|ExecutionSequence`
    (:`then_0`
      (`KismetSystemLibrary.Delay` 0.3)
      (bind _foundwidgets (`WidgetBlueprintLibrary.GetAllWidgetsOfClass` "/Game/UI/WB_PlayerUI.WB_PlayerUI_C"))
      (set `self.PlayerUIRef` (`|GetArrayItem` _foundwidgets)))
    (:`then_1`
      (`self.SetUpPickUp`))))

(event `/Game/Blueprints/Interfaces/BPI_Interact.SetFocused`
  (bind _playeruiref (`self.PlayerUIRef`))
  (message `/Game/Blueprints/Interfaces/BPI_CombatUI.InteractElement` _playeruiref (`KismetTextLibrary.Conv_StringToText` (`self.Dispaly Name`)) "" "Pick Up" true "")
  (`KismetSystemLibrary.RetriggerableDelay` 0.1)
  (message `/Game/Blueprints/Interfaces/BPI_CombatUI.InteractElement` _playeruiref "" "" "" false ""))

(event `/Game/Blueprints/Interfaces/BPI_Interact.Interact`
  (params (Character :type "/Game/Blueprints/Characters/BP_BaseCharacter Object Reference") (PlayerCharacter :type "/Game/Blueprints/Characters/BP_PlayerCharacterCore Object Reference"))
  (message `/Game/Blueprints/Interfaces/BPI_Equipables.HandlePickup` PlayerCharacter (`KismetStringLibrary.Conv_NameToString` (`self.WeaponID`)))
  (`self.K2_DestroyActor`)
  (message `/Game/Blueprints/Interfaces/BPI_CombatUI.InteractElement` (`self.PlayerUIRef`) "" "" "" false ""))

(fn `GetCanBePickedUp`
  (returns (CanBePickedUp :type Boolean))
  (return false))

(fn `GetItemToSpawn`
  (returns (Item :type "/Game/Blueprints/Interactables/Weapons/BP_WeaponComponentMaster Class Reference"))
  (return null))

(fn `SetUpPickUp`
  (`parent.UserConstructionScript`)
  (bind _returnvalue (`|GetDataTableRow` "/Game/Blueprints/EquipmentSystem/DT_WeaponDetails.DT_WeaponDetails" (`self.WeaponID`))
    (:`then`
      (bind (_dispalyname _animationtype _weapontag _startingammo _rateoffire _firerange _throwingrange _damage _staticmesh) (break `/Game/Blueprints/EquipmentSystem/ST_Weapons` _returnvalue))
      (`StaticMeshComponent.SetStaticMesh` (`self.ObjectPickUp`) _staticmesh)
      (set `self.Dispaly Name` _dispalyname))))

(fn `UserConstructionScript`
  (`self.SetUpPickUp`))