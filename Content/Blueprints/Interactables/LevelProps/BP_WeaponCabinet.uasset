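; BP_WeaponCabinet is a level-prop weapon cabinet that opens its lid when a linked minigame's assignment completes.
; On BeginPlay it binds its unlock event to the mission log component of the referenced minigame, if that reference is valid.
; Unlocking calls a server event that sets the replicated Open flag.
; The flag's OnRep plays a timeline locally that rotates the lid mesh open.
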(event `Server_OpenCabinet`
  (set `self.Open?` true))

(event `Local_OpenCabinet`
  (bind (_direction _newtrack_0) (`Timeline|Open`)
    (:`Update`
      (`SceneComponent.K2_SetRelativeRotation` (`self.SM_Prop_Weapon_Rack_02_Lid`) (`KismetMathLibrary.RLerp` (struct) (struct :`Roll` -110.0) _newtrack_0) false false))))

(event `self.ReceiveBeginPlay`
  (bind _minigameref (`self.MinigameRef`)
    (:`then`
      (add `/Game/Blueprints/MissionLog/BP_MissionLogComponent.AssignmentCompleted` (`/Game/Blueprints/Interactables/MiniGames/BP_AssignmentsBase.BP_MissionLogComponent` _minigameref) (delegate `UnlockCabinet`)))
    (:`else`)))

(event `UnlockCabinet`
  (`self.Server_OpenCabinet`))

(fn `OnRep_Open?`
  (if (`self.Open?`)
    (`self.Local_OpenCabinet`)))

(fn `UserConstructionScript`)