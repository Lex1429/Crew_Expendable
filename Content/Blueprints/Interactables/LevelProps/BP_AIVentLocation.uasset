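; BP_AIVentLocation is an AI vent trigger that relocates the monster to a random room spawn point.
; When anything begins overlapping its box, it finds the BP_MonsterBase actor and checks whether it is chasing.
; If not, it gathers all BP_RoomAlienSpawnPoint actors, picks one at random and moves the monster to that point's SpawnPoint location.
; The overlapping actor is not filtered.
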(event `self.Box.OnComponentBeginOverlap`
  (params (OverlappedComponent :type "PrimitiveComponent Object Reference") (OtherActor :type "Actor Object Reference") (OtherComp :type "PrimitiveComponent Object Reference") (OtherBodyIndex :type Integer) (bFromSweep :type Boolean) (SweepResult :type "HitResult Structure (by ref)"))
  (bind _returnvalue (`GameplayStatics.GetActorOfClass` "/Game/Blueprints/AI/Enemies/BP_MonsterBase.BP_MonsterBase_C"))
  (bind _chasing (message `/Game/Blueprints/Interfaces/BPI_EnemyAI.GetISChasing` _returnvalue))
  (if (not _chasing)
    (bind _outactors (`GameplayStatics.GetAllActorsOfClass` "/Game/Blueprints/Interactables/LevelProps/BP_RoomAlienSpawnPoint.BP_RoomAlienSpawnPoint_C"))
    (bind _output_get (set `self.TeleportPoint` (`KismetMathLibrary.RandomIntegerInRange` 0 (- (`KismetArrayLibrary.Array_Length` _outactors) 1))))
    (`self.K2_SetActorLocation` _returnvalue (`SceneComponent.K2_GetComponentLocation` (`/Game/Blueprints/Interactables/LevelProps/BP_RoomAlienSpawnPoint.SpawnPoint` (`|GetArrayItem` _outactors _output_get))) false false)))

(fn `UserConstructionScript`)