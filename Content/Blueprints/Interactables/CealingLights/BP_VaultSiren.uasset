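; BP_VaultSiren is a rotating warning light that runs when its linked vault door signals it.
; On BeginPlay it binds ActivateLight to the door's event, which makes the prop material glow and enables Tick for a few seconds, then switches both lights off.
; Tick holds the spotlight intensity up and spins it one turn per second.
; The construction script applies SirenColor and starts the glow dark.
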(event `self.ReceiveBeginPlay`
  (add `/Game/Blueprints/Interactables/Doors/DoorsV2/BP_MD_Vault.ActivateVaultLight` (`self.LinkedDoor`) (delegate `ActivateLight`)))

(event `ActivateLight`
  (`self.SetActorTickEnabled` true)
  (`MeshComponent.SetScalarParameterValueOnMaterials` (`self.SM_Prop_Light_Small_08`) "LightStrength" 2.0)
  (`KismetSystemLibrary.Delay` 5.0)
  (`self.SetActorTickEnabled` false)
  (`LightComponent.SetIntensity` (`self.SpotLight`) 0.0)
  (`MeshComponent.SetScalarParameterValueOnMaterials` (`self.SM_Prop_Light_Small_08`) "LightStrength" 0.0))

(event `self.ReceiveTick`
  (params (DeltaSeconds :type "Float (single-precision)"))
  (`LightComponent.SetIntensity` (`self.SpotLight`) 5000.0)
  (`SceneComponent.K2_AddLocalRotation` (`self.SpotLight`) (* (`KismetMathLibrary.MakeRotator` 0.0 0.0 360.0) DeltaSeconds) false false))

(fn `UserConstructionScript`
  (`LightComponent.SetLightColor` (`self.SpotLight`) (`self.SirenColor`) true)
  (`MeshComponent.SetScalarParameterValueOnMaterials` (`self.SM_Prop_Light_Small_08`) "LightStrength" 0.0))