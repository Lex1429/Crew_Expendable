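; BP_ExitSignal is a level exit actor that triggers the crew victory when something overlaps it with the game state's research points at exactly 6.
; The overlap shows WB_GameOverCrew, plays victory audio, then server-travels to ResearchShip_Level after a delay.
; UpdateResearch sets AbleToExit and hides the actor's widget, but the live overlap path ignores that flag.
; Older player-counting and lobby-travel logic remains disconnected.
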(event `/Game/Blueprints/Interfaces/BPI_ResearchUpdate.UpdateResearch`
  ; Start From Scratch
  (set `self.AbleToExit?` true)
  (`SceneComponent.SetVisibility` (`self.Widget`) false false))

(event `self.ReceiveActorEndOverlap`
  (params (OtherActor :type "Actor Object Reference"))
  ; Start From Scratch
)

(event `self.ReceiveActorBeginOverlap`
  (params (OtherActor :type "Actor Object Reference"))
  (bind _researchpoints (message `/Game/Blueprints/Interfaces/BPI_Stats.GetResearchPoints` (`GameplayStatics.GetGameState`)))
  (if (== _researchpoints 6)
    (bind _returnvalue (`|CreateWidget` "/Game/UI/WB_GameOverCrew.WB_GameOverCrew_C"))
    (`UserWidget.AddToViewport` _returnvalue 0)
    (`GameplayStatics.PlaySound2D` "/Game/SFX/Music/tactics_victory.tactics_victory" 1.0 1.0 0.0 null null)
    (`KismetSystemLibrary.Delay` 8.0)
    (`AdvancedSessionsLibrary.ServerTravel` "ResearchShip_Level")))

(fn `GetIsDead`
  (returns (IsDead :type Boolean))
  (return false))

(fn `GetResearchPoints`
  (returns (ResearchPoints :type Integer))
  (return 0))

(fn `UpdateResearchFunc`
  (bind _researchpoints (message `/Game/Blueprints/Interfaces/BPI_Stats.GetResearchPoints` (`GameplayStatics.GetGameState`)))
  (if (== _researchpoints 6)
    (set `self.AbleToExit?` true)))

(fn `UserConstructionScript`)