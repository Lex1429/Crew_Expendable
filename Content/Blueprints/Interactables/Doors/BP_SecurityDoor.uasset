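; Interactable sliding security door that toggles open and closed, or only plays a sound when locked.
; Interact routes through a server event to a local event that plays or reverses a timeline.
; The timeline rotates the lock and slides it and both door panels via lerps.
; A box overlap toggles an outline overlay material on the arch.
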(event `/Game/Blueprints/Interfaces/BPI_Interact.Interact`
  (params (Character :type "/Game/Blueprints/Characters/BP_BaseCharacter Object Reference"))
  (`self.Server_OpenDoor`))

(event `Server_OpenDoor`
  (`self.Local_OpenDoor`))

(event `Local_OpenDoor`
  (if (not (`self.IsDoorLocked?`))
    (`GameplayStatics.PlaySoundAtLocation` null (`SceneComponent.K2_GetComponentLocation` (`self.Arch`)) (struct) 1.0 1.0 0.0 null null null null)
    (if (not (`self.IsDoorOpen?`))
      (set `self.IsDoorOpen?` true)
      (bind (_direction _locktime _doorstime) (`Timeline|SecurityDoorTimeline` :!label _label)
        (:`Update`
          (`SceneComponent.K2_SetRelativeRotation` (`self.Lock`) (`KismetMathLibrary.RLerp` (struct) (struct :`Pitch` 90.0) _locktime) false false)
          (`SceneComponent.K2_SetRelativeLocation` (`self.Lock`) (`KismetMathLibrary.VLerp` (3.0 0.0 151.0) (-147.0 0.0 151.0) _doorstime) false true)
          (`SceneComponent.K2_SetRelativeLocation` (`self.LeftDoor`) (`KismetMathLibrary.VLerp` (-166.0 0.0 0.0) (-313.0 0.0 0.0) _doorstime) false true)
          (`SceneComponent.K2_SetRelativeLocation` (`self.RightDoor`) (`KismetMathLibrary.VLerp` (172.0 0.0 0.0) (316.0 0.0 0.0) _doorstime) false true)))
      (else
        (set `self.IsDoorOpen?` false)
        (goto _label :!via `Reverse`)))
    (else
      (`GameplayStatics.PlaySoundAtLocation` null (`SceneComponent.K2_GetComponentLocation` (`self.Arch`)) (struct) 1.0 1.0 0.0 null null null null))))

(event `self.Box.OnComponentBeginOverlap`
  (params (OverlappedComponent :type "PrimitiveComponent Object Reference") (OtherActor :type "Actor Object Reference") (OtherComp :type "PrimitiveComponent Object Reference") (OtherBodyIndex :type Integer) (bFromSweep :type Boolean) (SweepResult :type "HitResult Structure (by ref)"))
  (`MeshComponent.SetOverlayMaterial` (`self.Arch`) "/Game/Materials/M_Outline.M_Outline"))

(event `self.Box.OnComponentEndOverlap`
  (params (OverlappedComponent :type "PrimitiveComponent Object Reference") (OtherActor :type "Actor Object Reference") (OtherComp :type "PrimitiveComponent Object Reference") (OtherBodyIndex :type Integer))
  (`MeshComponent.SetOverlayMaterial` (`self.Arch`) null))

(fn `UserConstructionScript`)