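; BP_RectRoom1 is a modular rectangular room piece for assembling buildings, configured per instance in the editor.
; Its construction script applies a shared building material to the room and both end caps, then uses four booleans to toggle each end cap with its window and each emergency door with its frame.
; Disabled parts are hidden and have collision turned off; the event graph has no active logic.
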(fn `UserConstructionScript`
  (bind _window2 (`self.Window2`))
  (bind _door1 (`self.Door1`))
  (bind _doorframe2 (`self.Doorframe2`))
  (bind _endcap1 (`self.EndCap1`))
  (`PrimitiveComponent.SetMaterial` (`self.Room`) 0 (`self.BuildingMaterial`))
  (`PrimitiveComponent.SetMaterial` (`self.EndCap2`) 0 (`self.BuildingMaterial`))
  (`PrimitiveComponent.SetMaterial` (`self.EndCap1`) 0 (`self.BuildingMaterial`))
  (`|ExecutionSequence`
    (:`then_0`
      (if (`self.Endcap1On?`)
        (`SceneComponent.SetVisibility` (`self.EndCap1`) true false)
        (`SceneComponent.SetVisibility` (`self.Window1`) true false)
        (else
          (`SceneComponent.SetVisibility` _endcap1 false false)
          (`SceneComponent.SetVisibility` (`self.Window1`) false false)
          (`PrimitiveComponent.SetCollisionEnabled` _endcap1 "NoCollision")
          (`PrimitiveComponent.SetCollisionEnabled` (`self.Window1`) "NoCollision"))))
    (:`then_1`
      (if (`self.Endcap2On?`)
        (`SceneComponent.SetVisibility` (`self.Window2`) true false)
        (`SceneComponent.SetVisibility` (`self.EndCap2`) true false)
        (else
          (`SceneComponent.SetVisibility` _window2 false false)
          (`SceneComponent.SetVisibility` (`self.EndCap2`) false false)
          (`PrimitiveComponent.SetCollisionEnabled` _window2 "NoCollision")
          (`PrimitiveComponent.SetCollisionEnabled` (`self.EndCap2`) "NoCollision"))))
    (:`then_2`
      (if (`self.EmergencyDoor1?`)
        (`SceneComponent.SetVisibility` (`self.Doorframe1`) true false)
        (`SceneComponent.SetVisibility` (`self.Door1`) true false)
        (else
          (`SceneComponent.SetVisibility` _door1 false false)
          (`SceneComponent.SetVisibility` (`self.Doorframe1`) false false)
          (`PrimitiveComponent.SetCollisionEnabled` _door1 "NoCollision")
          (`PrimitiveComponent.SetCollisionEnabled` (`self.Doorframe1`) "NoCollision"))))
    (:`then_3`
      (if (`self.EmergencyDoor2?`)
        (`SceneComponent.SetVisibility` (`self.Doorframe2`) true false)
        (`SceneComponent.SetVisibility` (`self.Door2`) true false)
        (else
          (`SceneComponent.SetVisibility` _doorframe2 false false)
          (`SceneComponent.SetVisibility` (`self.Door2`) false false)
          (`PrimitiveComponent.SetCollisionEnabled` _doorframe2 "NoCollision")
          (`PrimitiveComponent.SetCollisionEnabled` (`self.Door2`) "NoCollision"))))))