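; Timed padlock minigame on a 3x3 screen grid, started by a nearby player with a camera blend.
; Axis input, polled by timer, moves a selector; action toggles that cell's pattern, and toggled patterns XOR together until all nine buttons are set.
; CreatePatterns splits shuffled buttons across a few patterns to guarantee a solution, then adds random decoys.
; A dynamic material shows grid, countdown and result; timeout cancels the game.
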(event `self.ReceiveBeginPlay`
  ;[1 1 1] Begin play
  (`parent.ReceiveBeginPlay`)
  (set `self.IsMiniGameActivated` false)
  (set `self.InputEnable` false)
  (bind _returnvalue (`KismetMaterialLibrary.CreateDynamicMaterialInstance` "/Game/MiniGames4/Materials/MI_MG_PadLock_Inst.MI_MG_PadLock_Inst"))
  (set `self.DMI` _returnvalue)
  (bind _returnvalue_2 (`KismetSystemLibrary.K2_SetTimer` null "CheckContorls" 0.05 true))
  (set `self.ControlsTimeHandle` _returnvalue_2)
  (bind _returnvalue_3 (`KismetSystemLibrary.K2_SetTimer` null "UpdateBar" 1.0 true))
  (bind _output_get (set `self.BarTimer` _returnvalue_3))
  (`KismetSystemLibrary.K2_PauseTimerHandle` _output_get))

(event `Init`
  ;[1 1 1] Init
  (set `self.SelectorIndexX` 0)
  (set `self.SelectorIndexY` 0)
  (set `self.PrevRightAxis` 0.0)
  (set `self.PrevForwAxis` 0.0)
  (`KismetArrayLibrary.Array_Clear` (`self.Patterns`))
  (`KismetArrayLibrary.Array_Clear` (`self.SelectorPattern`))
  (`KismetArrayLibrary.Array_Clear` (`self.FinalPattern`))
  (`self.CreatePatterns`)
  (set `self.CurrentBarValue` (`self.MaterialMaxBarValue`))
  (set `self.BarDelta` (/ (`self.MaterialMaxBarValue`) (`self.Timer`)))
  (`MaterialInstanceDynamic.SetScalarParameterValue` (`self.DMI`) "ShowError" 0.0)
  (`MaterialInstanceDynamic.SetScalarParameterValue` (`self.DMI`) "ShowUnlocked" 0.0)
  (`MaterialInstanceDynamic.SetScalarParameterValue` (`self.DMI`) "Progress" (`self.MaterialMaxBarValue`))
  (`KismetArrayLibrary.Array_Clear` (`self.SelectorPattern`))
  (`KismetArrayLibrary.Array_Clear` (`self.FinalPattern`))
  (`KismetSystemLibrary.K2_UnPauseTimerHandle` (`self.BarTimer`))
  (`self.UpdateSelector`)
  (`self.UpdatePattern`)
  (for _ (range 9)
    (`KismetArrayLibrary.Array_Add` (`self.SelectorPattern`)))
  (for _ (range 9)
    (`KismetArrayLibrary.Array_Add` (`self.FinalPattern`)))
  (set `self.InputEnable` true))

(event `UpdateSelector`
  (bind _dmi (`self.DMI`))
  ;[1 1 1] Controls
  (`MaterialInstanceDynamic.SetScalarParameterValue` _dmi "SelectorIndexX" (`KismetMathLibrary.Conv_IntToDouble` (`self.SelectorIndexX`)) :!label _label)
  (`MaterialInstanceDynamic.SetScalarParameterValue` _dmi "SelectorIndexY" (`KismetMathLibrary.Conv_IntToDouble` (`self.SelectorIndexY`))))

(event `CheckContorls`
  (bind _rightaxis (`self.RightAxis`))
  (bind _forwardaxis (`self.ForwardAxis`))
  (bind _returnvalue (`KismetMathLibrary.SignOfFloat` _rightaxis))
  (bind _returnvalue_2 (* _forwardaxis -1.0))
  (bind _returnvalue_3 (`KismetMathLibrary.SignOfFloat` _returnvalue_2))
  ;[1 1 1] Controls
  (if (`self.InputEnable`)
    (if (`self.IsMiniGameActivated`)
      (`|ExecutionSequence`
        (:`then_0`
          (if (!= _rightaxis 0.0)
            (if (!= _rightaxis (`self.PrevRightAxis`))
              (set `self.PrevRightAxis` _returnvalue)
              (set `self.SelectorIndexX` (`KismetMathLibrary.Clamp` (+ (`KismetMathLibrary.FTrunc` _returnvalue) (`self.SelectorIndexX`)) 0 2))
              (`self.UpdatePattern` :!label _label_2)
              (goto _label))
            (else
              (set `self.PrevRightAxis` 0.0))))
        (:`then_1`
          (if (!= _forwardaxis 0.0)
            (if (!= _returnvalue_2 (`self.PrevForwAxis`))
              (set `self.PrevForwAxis` _returnvalue_3)
              (set `self.SelectorIndexY` (`KismetMathLibrary.Clamp` (+ (`KismetMathLibrary.FTrunc` _returnvalue_3) (`self.SelectorIndexY`)) 0 2))
              (goto _label_2))
            (else
              (set `self.PrevForwAxis` 0.0))))))))

(event `self.ForceExit`
  ;[1 1 1] Cancel
  (if (and (`self.MiniGameEnabled`) (`self.IsMiniGameActivated`))
    (set `self.IsMiniGameActivated` false)
    (set `self.InputEnable` false)
    (`self.OnMiniGameCanceled`)
    (`KismetSystemLibrary.K2_PauseTimerHandle` (`self.BarTimer`))
    (`self.BlendCameraFromGameToPlayer` (`self.OverlappedActor`))))

(event `self.InteractionBoundBox.OnComponentBeginOverlap`
  (params (OverlappedComponent :type "PrimitiveComponent Object Reference") (OtherActor :type "Actor Object Reference") (OtherComp :type "PrimitiveComponent Object Reference") (OtherBodyIndex :type Integer) (bFromSweep :type Boolean) (SweepResult :type "HitResult Structure (by ref)"))
  ;[1 1 1] Overlap events
  (`self.CheckBeginOverlap` OtherActor))

(event `self.ForceAction`
  (params (Player :type "/Game/Blueprints/Characters/BP_PlayerCharacterCore Object Reference"))
  (bind _selectorpattern (`self.SelectorPattern`))
  (bind _finalpattern (`self.FinalPattern`))
  (bind _returnvalue (+ (`self.SelectorIndexX`) (* (`self.SelectorIndexY`) 3)))
  ;[1 1 1] Action
  (if (`self.PlayerOverlapped`)
    (if (`self.IsMiniGameActivated`)
      (`KismetArrayLibrary.Array_Set` _selectorpattern _returnvalue (not (`|GetArrayItem` _selectorpattern _returnvalue)))
      (`self.UpdatePattern`)
      (if (and (`|GetArrayItem` _finalpattern) (`|GetArrayItem` _finalpattern 1) (`|GetArrayItem` _finalpattern 2) (`|GetArrayItem` _finalpattern 3) (`|GetArrayItem` _finalpattern 4) (`|GetArrayItem` _finalpattern 5) (`|GetArrayItem` _finalpattern 6) (`|GetArrayItem` _finalpattern 7) (`|GetArrayItem` _finalpattern 8))
        ;[1 1 1] Success
        (set `self.MiniGameEnabled` false)
        (set `self.IsMiniGameActivated` false)
        (set `self.InputEnable` false)
        (`KismetSystemLibrary.K2_PauseTimerHandle` (`self.BarTimer`))
        (`MaterialInstanceDynamic.SetScalarParameterValue` (`self.DMI`) "ShowUnlocked" 1.0)
        (`KismetSystemLibrary.Delay` (`self.DelayTimeWhenComplete`))
        (`self.SetOfflineMaterial`)
        (`self.OnMiniGameSuccess`)
        (`self.BlendCameraFromGameToPlayer` (`self.OverlappedActor`)))
      (else
        (`self.Init`)
        (`PrimitiveComponent.SetMaterial` (`self.MiniGameScreen`) 0 (`self.DMI`))
        (`self.BlendCameraFromPlayerToGame` self (`self.OverlappedActor`))
        (set `self.IsMiniGameActivated` true)))))

(event `self.InteractionBoundBox.OnComponentEndOverlap`
  (params (OverlappedComponent :type "PrimitiveComponent Object Reference") (OtherActor :type "Actor Object Reference") (OtherComp :type "PrimitiveComponent Object Reference") (OtherBodyIndex :type Integer))
  ;[1 1 1] Overlap events
  (`self.CheckEndOverlap` OtherActor))

(event `UpdatePattern`
  (bind _finalpattern (`self.FinalPattern`))
  (bind _finalpattern_2 (`self.FinalPattern`))
  (bind _returnvalue (+ (`self.SelectorIndexX`) (* (`self.SelectorIndexY`) 3)))
  (bind _output_buttons (break `/Game/MiniGames4/Blueprints/Data/F_MG_PadLockPattern` (`|GetArrayItem` (`self.Patterns`) _returnvalue)))
  ;[1 1 1] Update pattern (do XOR between selected and pressed patterns)
  (for (_ _array_index) _finalpattern_2
    (`KismetArrayLibrary.Array_Set` _finalpattern_2 _array_index))
  (for (_array_element _array_index_2) (`self.SelectorPattern`)
    (if _array_element
      (bind _output_buttons_2 (break `/Game/MiniGames4/Blueprints/Data/F_MG_PadLockPattern` (`|GetArrayItem` (`self.Patterns`) _array_index_2)))
      (for (_array_element_2 _array_index_3) _output_buttons_2
        (`KismetArrayLibrary.Array_Set` _finalpattern _array_index_3 (xor _array_element_2 (`|GetArrayItem` _finalpattern _array_index_3))))))
  (for (_array_element_3 _array_index_4) _output_buttons
    (bind _returnvalue_2 (`KismetStringLibrary.Conv_IntToString` (+ _array_index_4 1)))
    (bind _output (`|GetArrayItem` (`self.FinalPattern`) _array_index_4))
    (`MaterialInstanceDynamic.SetScalarParameterValue` (`self.DMI`) (`KismetStringLibrary.Conv_StringToName` (`KismetStringLibrary.Concat_StrStr` "ButtonSet" _returnvalue_2)) (`KismetMathLibrary.SelectFloat` (`KismetMathLibrary.SelectFloat` 1.0 0.0 _output) (`KismetMathLibrary.SelectFloat` 1.0 0.0 (xor _array_element_3 _output)) (`|GetArrayItem` (`self.SelectorPattern`) _returnvalue)))
    (`MaterialInstanceDynamic.SetScalarParameterValue` (`self.DMI`) (`KismetStringLibrary.Conv_StringToName` (`KismetStringLibrary.Concat_StrStr` "ButtonPressed" _returnvalue_2)) (`KismetMathLibrary.SelectFloat` 1.0 0.0 (`|GetArrayItem` (`self.SelectorPattern`) _array_index_4)))
    (`MaterialInstanceDynamic.SetScalarParameterValue` (`self.DMI`) (`KismetStringLibrary.Conv_StringToName` (`KismetStringLibrary.Concat_StrStr` "ButtonPressed" _returnvalue_2)) (`KismetMathLibrary.SelectFloat` 1.0 0.0 (`|GetArrayItem` (`self.SelectorPattern`) _array_index_4)))))

(event `UpdateBar`
  (bind _errorsound (`self.ErrorSound`))
  ;[1 1 1] Update time bar
  (bind _output_get (set `self.CurrentBarValue` (`KismetMathLibrary.FClamp` (- (`self.CurrentBarValue`) (`self.BarDelta`)) 0.0 (`self.MaterialMaxBarValue`))))
  (`MaterialInstanceDynamic.SetScalarParameterValue` (`self.DMI`) "Progress" _output_get)
  (if (<= _output_get 0.0)
    (set `self.InputEnable` false)
    (`KismetSystemLibrary.K2_PauseTimerHandle` (`self.BarTimer`))
    (`MaterialInstanceDynamic.SetScalarParameterValue` (`self.DMI`) "ShowError" 1.0)
    (`/Engine/EditorBlueprintResources/StandardMacros.IsValid` _errorsound
      (:`Is Valid`
        (`GameplayStatics.PlaySoundAtLocation` _errorsound (`self.K2_GetActorLocation` self) (struct) 1.0 1.0 0.0 null null null null))
      (:`Is Not Valid`
        _))
    (`KismetSystemLibrary.Delay` 1.0)
    (`PrimitiveComponent.SetMaterial` (`self.MiniGameScreen`) 0 (`self.DMI_Idle`))
    (`self.ForceExit`)))

(fn `CreatePatterns`
  (locals (RandomIndices :type "Array of Integer") (CurrPattern :type Integer) (LastIndex :type Integer))
  (bind _randomindices (`local.RandomIndices`))
  (bind _lastindex (`local.LastIndex`))
  (bind _lastindex_2 (`local.LastIndex`))
  (bind _lastindex_3 (`local.LastIndex`))
  ;[1 1 1] Setup patterns
  (`KismetArrayLibrary.Array_Clear` (`local.RandomIndices`))
  (for _index (range 9)
    (`KismetArrayLibrary.Array_Add` _randomindices _index))
  (`KismetArrayLibrary.Array_Shuffle` _randomindices)
  (set `local.CurrPattern` 0)
  (`KismetArrayLibrary.Array_Add` (`self.Patterns`) (make `/Game/MiniGames4/Blueprints/Data/F_MG_PadLockPattern` (`|MakeArray` false false false false false false false false false)))
  (for _index_2 (range (+ (`KismetMathLibrary.RandomIntegerInRange` 1 3) 1))
    (`KismetArrayLibrary.Array_Set` (`.Buttons_43_4EFB4C1F47EB58D33A7A4DB0337FA5D8` (break `/Game/MiniGames4/Blueprints/Data/F_MG_PadLockPattern` (`|GetArrayItem` (`self.Patterns`) (`local.CurrPattern`)))) (`|GetArrayItem` (`local.RandomIndices`) _index_2) true))
  (set `local.LastIndex` _index_2)
  (`/Engine/EditorBlueprintResources/StandardMacros.IncrementInt` (`local.CurrPattern`)
    (:`  `
      (`KismetArrayLibrary.Array_Add` (`self.Patterns`) (make `/Game/MiniGames4/Blueprints/Data/F_MG_PadLockPattern` (`|MakeArray` false false false false false false false false false)))
      (for _index_3 (range _lastindex (+ (+ _lastindex (`KismetMathLibrary.RandomIntegerInRange` 1 3)) 1))
        (`KismetArrayLibrary.Array_Set` (`.Buttons_43_4EFB4C1F47EB58D33A7A4DB0337FA5D8` (break `/Game/MiniGames4/Blueprints/Data/F_MG_PadLockPattern` (`|GetArrayItem` (`self.Patterns`) (`local.CurrPattern`)))) (`|GetArrayItem` (`local.RandomIndices`) _index_3) true))
      (set `local.LastIndex` _index_3)
      (`KismetArrayLibrary.Array_Add` (`self.Patterns`) (make `/Game/MiniGames4/Blueprints/Data/F_MG_PadLockPattern` (`|MakeArray` false false false false false false false false false)))
      (`/Engine/EditorBlueprintResources/StandardMacros.IncrementInt` (`local.CurrPattern`)
        (:`  `
          (for _index_4 (range _lastindex_2 (+ (+ _lastindex_2 (`KismetMathLibrary.RandomIntegerInRange` 0 (- 8 (`local.LastIndex`)))) 1))
            (`KismetArrayLibrary.Array_Set` (`.Buttons_43_4EFB4C1F47EB58D33A7A4DB0337FA5D8` (break `/Game/MiniGames4/Blueprints/Data/F_MG_PadLockPattern` (`|GetArrayItem` (`self.Patterns`) (`local.CurrPattern`)))) (`|GetArrayItem` (`local.RandomIndices`) _index_4) true))
          (bind _output_get (set `local.LastIndex` _index_4))
          (if (< _output_get 9)
            (`KismetArrayLibrary.Array_Add` (`self.Patterns`) (make `/Game/MiniGames4/Blueprints/Data/F_MG_PadLockPattern` (`|MakeArray` false false false false false false false false false)))
            (`/Engine/EditorBlueprintResources/StandardMacros.IncrementInt` (`local.CurrPattern`)
              (:`  `
                (for _index_5 (range _lastindex_3 (+ (+ _lastindex_3 (- 8 (`local.LastIndex`))) 1))
                  (`KismetArrayLibrary.Array_Set` (`.Buttons_43_4EFB4C1F47EB58D33A7A4DB0337FA5D8` (break `/Game/MiniGames4/Blueprints/Data/F_MG_PadLockPattern` (`|GetArrayItem` (`self.Patterns`) (`local.CurrPattern`)))) (`|GetArrayItem` (`local.RandomIndices`) _index_5) true)))))
          (for _ (range (+ (- 8 (+ (`local.CurrPattern`) 1)) 1))
            (`KismetArrayLibrary.Array_Add` (`self.Patterns`) (make `/Game/MiniGames4/Blueprints/Data/F_MG_PadLockPattern` (`|MakeArray` (`KismetMathLibrary.RandomBoolWithWeight` 0.6) (`KismetMathLibrary.RandomBoolWithWeight` 0.5) (`KismetMathLibrary.RandomBoolWithWeight` 0.5) (`KismetMathLibrary.RandomBoolWithWeight` 0.6) (`KismetMathLibrary.RandomBoolWithWeight` 0.6) (`KismetMathLibrary.RandomBoolWithWeight` 0.6) (`KismetMathLibrary.RandomBoolWithWeight` 0.5) (`KismetMathLibrary.RandomBoolWithWeight` 0.5) (`KismetMathLibrary.RandomBoolWithWeight` 0.5)))))
          (if (not (`self.TestMode`))
            (`KismetArrayLibrary.Array_Shuffle` (`self.Patterns`))))))))

(fn `UserConstructionScript`
  (`parent.UserConstructionScript`))