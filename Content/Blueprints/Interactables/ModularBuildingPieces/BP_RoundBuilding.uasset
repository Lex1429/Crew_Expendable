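; Modular round building piece whose pod material follows the room's light switch, with an optional emergency door.
; The construction script passes RoomTag to the overhead BP_LampBase child actor, applies BuildingMaterial, then shows or hides and repositions the door via UseEmergencyDoor.
; On BeginPlay it binds to the referenced light switch's toggle, then swaps between per-sector on and off materials selected by RoomTag, with both Sector 4 rooms sharing materials.
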(event `self.ReceiveBeginPlay`
  (bind _lightswitchref (`self.LightSwitchRef`))
  (`/Engine/EditorBlueprintResources/StandardMacros.IsValid` _lightswitchref
    (:`Is Valid`
      (add `/Game/Blueprints/Interactables/Buttons/BP_Lightswitch.LightSwitchToggle` _lightswitchref (`|CreateDelegate` :!event `LightSwitchToggle`)))))

(event `LightSwitchToggle`
  (params (`IsOn?` :type Boolean))
  (bind _sm_bld_pod_research_03 (`self.SM_Bld_Pod_Research_03`))
  (if `IsOn?`
    (`|SwitchGameplayTagContainer` (`self.RoomTag`)
      (:`(GameplayTags=((TagName="Sector1.MessHall")))`
        (`PrimitiveComponent.SetMaterial` _sm_bld_pod_research_03 0 "/Game/Materials/CustomTextures/V1Materials/M_Sector1_On.M_Sector1_On"))
      (:`(GameplayTags=((TagName="Sector3.MedBay")))`
        (`PrimitiveComponent.SetMaterial` _sm_bld_pod_research_03 0 "/Game/Materials/CustomTextures/V1Materials/M_Sector3_On.M_Sector3_On"))
      (:`(GameplayTags=((TagName="Sector4.LifeSupport")))`
        (`PrimitiveComponent.SetMaterial` _sm_bld_pod_research_03 0 "/Game/Materials/CustomTextures/V1Materials/M_Sector4_On.M_Sector4_On" :!label _label))
      (:`(GameplayTags=((TagName="Sector4.PowerControl")))`
        (goto _label)))
    (else
      (`|SwitchGameplayTagContainer` (`self.RoomTag`)
        (:`(GameplayTags=((TagName="Sector1.MessHall")))`
          (`PrimitiveComponent.SetMaterial` _sm_bld_pod_research_03 0 "/Game/Materials/CustomTextures/V1Materials/M_Sector1_Off.M_Sector1_Off"))
        (:`(GameplayTags=((TagName="Sector3.MedBay")))`
          (`PrimitiveComponent.SetMaterial` _sm_bld_pod_research_03 0 "/Game/Materials/CustomTextures/V1Materials/M_Sector3_Off.M_Sector3_Off"))
        (:`(GameplayTags=((TagName="Sector4.LifeSupport")))`
          (`PrimitiveComponent.SetMaterial` _sm_bld_pod_research_03 0 "/Game/Materials/CustomTextures/V1Materials/M_Sector4_Off.M_Sector4_Off" :!label _label_2))
        (:`(GameplayTags=((TagName="Sector4.PowerControl")))`
          (goto _label_2))))))

(fn `UserConstructionScript`
  (bind _asbp_lamp_base (cast `/Game/Blueprints/Interactables/CealingLights/BP_LampBase` (`ChildActorComponent.ChildActor` (`self.OverheadLight1`))))
  (set `/Game/Blueprints/Interactables/CealingLights/BP_LampBase.RoomTag` (`self.RoomTag`) _asbp_lamp_base)
  (`PrimitiveComponent.SetMaterial` (`self.SM_Bld_Pod_Research_03`) 0 (`self.BuildingMaterial`))
  (if (`self.UseEmergencyDoor?`)
    (`SceneComponent.SetVisibility` (`self.DoorFrame`) true false)
    (`SceneComponent.SetVisibility` (`self.InnerFrame`) true false)
    (`SceneComponent.SetVisibility` (`self.EmergencyDoor`) true false)
    (`SceneComponent.K2_SetRelativeLocation` (`self.EmergencyDoor`) (-75.0 0.0 0.0) false false)
    (else
      (`SceneComponent.SetVisibility` (`self.DoorFrame`) false false)
      (`SceneComponent.SetVisibility` (`self.InnerFrame`) false false)
      (`SceneComponent.SetVisibility` (`self.EmergencyDoor`) false false)
      (`SceneComponent.K2_SetRelativeLocation` (`self.EmergencyDoor`) (-75.0 0.0 400.0) false false))))