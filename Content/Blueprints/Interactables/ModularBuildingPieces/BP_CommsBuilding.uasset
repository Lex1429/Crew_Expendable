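; Modular comms building with radar and satellite dish meshes that respond to a light switch.
; On BeginPlay it binds to the toggle event of a referenced light switch, if one is set.
; Toggling swaps the first material slot on the radar, swivel and dish meshes between Sector 2 on and off materials.
; The construction script copies the building's RoomTag to the child lamp actor of its overhead light.
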(event `self.ReceiveBeginPlay`
  (bind _lightswitchref (`self.LightSwitchRef`))
  (`/Engine/EditorBlueprintResources/StandardMacros.IsValid` _lightswitchref
    (:`Is Valid`
      (add `/Game/Blueprints/Interactables/Buttons/BP_Lightswitch.LightSwitchToggle` _lightswitchref (`|CreateDelegate` :!event `LightSwitchToggle`)))))

(event `LightSwitchToggle`
  (params (`IsOn?` :type Boolean))
  (bind _sm_bld_corp_radar_01 (`self.SM_Bld_Corp_Radar_01`))
  (if `IsOn?`
    (`PrimitiveComponent.SetMaterial` _sm_bld_corp_radar_01 0 "/Game/Materials/CustomTextures/V1Materials/M_Sector2_On.M_Sector2_On")
    (`PrimitiveComponent.SetMaterial` (`self.SM_Prop_Satellite_04_Swivel_02`) 0 "/Game/Materials/CustomTextures/V1Materials/M_Sector2_On.M_Sector2_On")
    (`PrimitiveComponent.SetMaterial` (`self.SM_Prop_Satellite_04_Dish_01`) 0 "/Game/Materials/CustomTextures/V1Materials/M_Sector2_On.M_Sector2_On")
    (else
      (`PrimitiveComponent.SetMaterial` _sm_bld_corp_radar_01 0 "/Game/Materials/CustomTextures/V1Materials/M_Sector2_Off.M_Sector2_Off")
      (`PrimitiveComponent.SetMaterial` (`self.SM_Prop_Satellite_04_Swivel_02`) 0 "/Game/Materials/CustomTextures/V1Materials/M_Sector2_Off.M_Sector2_Off")
      (`PrimitiveComponent.SetMaterial` (`self.SM_Prop_Satellite_04_Dish_01`) 0 "/Game/Materials/CustomTextures/V1Materials/M_Sector2_Off.M_Sector2_Off"))))

(fn `UserConstructionScript`
  (bind _asbp_lamp_base (cast `/Game/Blueprints/Interactables/CealingLights/BP_LampBase` (`ChildActorComponent.ChildActor` (`self.OverheadLight1`))))
  (set `/Game/Blueprints/Interactables/CealingLights/BP_LampBase.RoomTag` (`self.RoomTag`) _asbp_lamp_base))