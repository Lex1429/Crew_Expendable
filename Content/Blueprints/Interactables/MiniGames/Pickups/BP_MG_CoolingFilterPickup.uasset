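; Cooling filter pickup for a minigame, which begins inside the AC and is handed to the player as a primary weapon.
; When ServerSpawnWeapon runs on a pickable filter still in the AC, it calls PullingFilter, waits briefly, marks the filter broken and updates player pawn 0's filter status.
; It then spawns the weapon on the target, destroys itself and triggers the interaction UI message.
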(event `self.ReceiveBeginPlay`
  (`parent.ReceiveBeginPlay`)
  (set `self.InAC?` true))

(event `self.Server_SpawnWeapon`
  (params (Target :type "/Game/Blueprints/Characters/BP_BaseCharacter Object Reference") (WeaponToSpawn :type "/Game/Blueprints/Interactables/Weapons/BP_WeaponComponentMaster Class Reference"))
  (if (`self.CanBePickedUp?`)
    (if (`self.InAC?`)
      (`self.PullingFilter`)
      (`KismetSystemLibrary.Delay` 0.5)
      (bind _output_get (set `self.Broken?` true))
      (message `/Game/Blueprints/Interfaces/BPI_FilterStats.SetCoolerFilterStatus` (`GameplayStatics.GetPlayerPawn` 0) false false _output_get)
      (set `self.InAC?` false))
    (`/Game/Blueprints/Characters/BP_BaseCharacter.SpawnPrimaryWeapon` Target WeaponToSpawn)
    (`self.K2_DestroyActor`)
    (message `/Game/Blueprints/Interfaces/BPI_CombatUI.InteractElement` (`self.PlayerUIRef`) "" "" "" false "")))

(fn `UserConstructionScript`
  (`parent.UserConstructionScript`))