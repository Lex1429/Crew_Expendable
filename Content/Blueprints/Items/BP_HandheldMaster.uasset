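; BP_HandheldMaster is the base Blueprint for handheld, ammo-limited weapons.
; Setup pulls its skeletal mesh from DT_SalvageList by ItemName and binds to the player character's fire and release events.
; Server fire events start or clear a looping RateOfFire timer, using a negative start delay for an immediate first shot.
; Each tick checks and decrements ammo, plays the attached shot sound and debug-prints the count, with no projectile or hit logic.
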(event `SetUpActor`
  (bind _as_bp_player_character_core (`self.As BP Player Character Core`))
  (`self.Setup`)
  (add `/Game/Blueprints/Characters/BP_PlayerCharacterCore.FireWeapon` _as_bp_player_character_core (delegate `PrimaryFire`))
  (add `/Game/Blueprints/Characters/BP_PlayerCharacterCore.ReleaseWeapon` _as_bp_player_character_core (delegate `ReleaseFire`)))

(event `PrimaryFire`
  (`self.HandlePrimaryFire`))

(event `ReleaseFire`
  (`self.HandleWeaponRelease`))

(event `HandlePrimaryFire`
  (`self.Server_PrimaryFire` true))

(event `HandleWeaponRelease`
  (`self.Server_PrimaryFire` false))

(event `Server_PrimaryFire`
  (params (`Pressed?` :type Boolean))
  (bind _rateoffire (`self.RateOfFire`))
  (if `Pressed?`
    (bind _returnvalue (`KismetSystemLibrary.K2_SetTimerDelegate` (delegate `Shooting`) _rateoffire true false (* _rateoffire -1.0)))
    (set `self.THShooting` _returnvalue)
    (else
      (`KismetSystemLibrary.K2_ClearAndInvalidateTimerHandle` (`self.THShooting`)))))

(event `Shooting`
  (`self.CanShoot?`
    (:`true`
      (bind _result (`/Engine/EditorBlueprintResources/StandardMacros.DecrementInt` (`self.CurrentAmmo`))
        (:`  `
          (`self.Local_Shoot`)
          (`KismetSystemLibrary.PrintString` (`KismetStringLibrary.Conv_IntToString` _result)))))))

(event `Local_Shoot`
  (`GameplayStatics.SpawnSoundAttached` (`self.ShotSound`) (`self.SkeletalMesh`) "None" (0.0 0.0 0.0) (struct) "KeepRelativeOffset" false 1.0 1.0 0.0 null null))

(fn `Setup`
  (bind _returnvalue (`|GetDataTableRow` "/Game/Blueprints/Salvage/DT_SalvageList.DT_SalvageList" (`self.ItemName`))
    (:`then`
      (`SkeletalMeshComponent.SetSkeletalMeshAsset` (`self.SkeletalMesh`) (`.SkeletalMesh_48_8CA639C24B0AE43C51762786A566C6D9` (break `/Game/Blueprints/Salvage/S_Salvage` _returnvalue))))))

(fn `UserConstructionScript`)