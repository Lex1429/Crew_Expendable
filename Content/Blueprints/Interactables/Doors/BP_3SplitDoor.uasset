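; Interactable three-piece split door that toggles open and closed, either on interact or automatically on overlap, with an optional keycard lock.
; Interaction routes through server and local open events; a successful keycard check clears the character's keycard flag and unlocks the door.
; A timeline slides the top, left and right pieces with sound.
; Overlap outlines the arch, while a pausable looping timer re-triggers automatic doors about five seconds after exit.
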(event `/Game/Blueprints/Interfaces/BPI_Interact.Interact`
  (params (Character :type "Object Object Reference") (PlayerCharacter :type "/Game/Blueprints/Characters/BP_PlayerCharacterCore Object Reference"))
  (`self.Server_OpenDoor` PlayerCharacter))

(event `Server_OpenDoor`
  (params (Character :type "/Game/Blueprints/Characters/BP_PlayerCharacterCore Object Reference"))
  (`self.Local_OpenDoor` Character))

(event `Local_OpenDoor`
  (params (Character :type "/Game/Blueprints/Characters/BP_PlayerCharacterCore Object Reference"))
  (bind _returnvalue (`SceneComponent.K2_GetComponentLocation` (`self.Arch`)))
  (if (`self.RequiresKeyCard?`)
    (bind _haskeycard (message `/Game/Blueprints/Interfaces/BPI_SelectedWeapons.GetHasKeycard` Character))
    (if _haskeycard
      (`GameplayStatics.PlaySoundAtLocation` null (`SceneComponent.K2_GetComponentLocation` (`self.Arch`)) (struct) 1.0 1.0 0.0 null null null null :!label _label)
      (message `/Game/Blueprints/Interfaces/BPI_SelectedWeapons.SetHasKeycard` Character false)
      (if (not (`self.IsDoorOpen?`))
        (set `self.IsDoorOpen?` true)
        (`GameplayStatics.PlaySoundAtLocation` "/Game/SFX/Doors/SC_DoorOpen.SC_DoorOpen" _returnvalue (struct) 1.0 1.0 0.0 null null null null)
        (bind (_direction _3waytrack) (`Timeline|3WayDoor` :!label _label_2)
          (:`Update`
            (`SceneComponent.K2_SetRelativeLocation` (`self.TopPiece`) (`KismetMathLibrary.VLerp` (-5.0 0.0 310.0) (-5.0 0.0 400.0) _3waytrack) false true)
            (`SceneComponent.K2_SetRelativeLocation` (`self.LeftPiece`) (`KismetMathLibrary.VLerp` (-185.0 0.0 0.0) (-335.0 0.0 0.0) _3waytrack) false true)
            (`SceneComponent.K2_SetRelativeLocation` (`self.RightPiece`) (`KismetMathLibrary.VLerp` (175.0 0.0 0.0) (335.0 0.0 0.0) _3waytrack) false true)
            (set `self.RequiresKeyCard?` false)))
        (else
          (set `self.IsDoorOpen?` false)
          (`GameplayStatics.PlaySoundAtLocation` "/Game/SFX/Doors/SC_DoorClose.SC_DoorClose" _returnvalue (struct) 1.0 1.0 0.0 null null null null)
          (goto _label_2 :!via `Reverse`)))
      (else
        (`GameplayStatics.PlaySoundAtLocation` null (`SceneComponent.K2_GetComponentLocation` (`self.Arch`)) (struct) 1.0 1.0 0.0 null null null null)))
    (else
      (goto _label))))

(event `self.ReceiveActorBeginOverlap`
  (params (OtherActor :type "Actor Object Reference"))
  (`MeshComponent.SetOverlayMaterial` (`self.Arch`) "/Game/Materials/M_Outline.M_Outline")
  (if (`self.IsDoorOpen?`)
    (`self.PauseTime`)
    (elif (`self.Automatic?`)
      (`self.Server_OpenDoor` null))))

(event `self.ReceiveActorEndOverlap`
  (params (OtherActor :type "Actor Object Reference"))
  (`MeshComponent.SetOverlayMaterial` (`self.Arch`) null)
  (if (`KismetSystemLibrary.K2_IsTimerPausedHandle` (`self.Timer`))
    (`self.ResumeTimer`)
    (elif (`self.Automatic?`)
      (`self.Start Timer`))))

(event `Start Timer`
  (set `self.Seconds` 0.0)
  (bind _returnvalue (`KismetSystemLibrary.K2_SetTimerDelegate` (delegate `DeltaSec`) 1.0 true))
  (set `self.Timer` _returnvalue))

(event `DeltaSec`
  (bind _result (`/Engine/EditorBlueprintResources/StandardMacros.IncrementFloat` (`self.Seconds`))
    (:`  `
      (`KismetSystemLibrary.PrintString` (`KismetStringLibrary.Conv_DoubleToString` _result))
      (if (>= _result 5.0)
        (`self.Server_OpenDoor` null)
        (`KismetSystemLibrary.K2_ClearAndInvalidateTimerHandle` (`self.Timer`))))))

(event `PauseTime`
  (`KismetSystemLibrary.K2_PauseTimerHandle` (`self.Timer`)))

(event `ResumeTimer`
  (`KismetSystemLibrary.K2_UnPauseTimerHandle` (`self.Timer`)))

(fn `GetCanBePickedUp`
  (returns (CanBePickedUp :type Boolean))
  (return false))

(fn `GetItemToSpawn`
  (returns (Item :type "/Game/Blueprints/Interactables/Weapons/BP_WeaponComponentMaster Class Reference"))
  (return null))

(fn `UserConstructionScript`)