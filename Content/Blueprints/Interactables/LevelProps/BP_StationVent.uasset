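; BP_StationVent is a level prop vent that teleports an overlapping BP_SAL to a linked tunnel vent.
; Beginning an overlap starts a five-second timer that ending the overlap cancels.
; When it fires, a further short delay precedes the teleport to the SpawnPoint of the VentTarget BP_TunnelVent, with zero rotation.
; The construction script caches its own SpawnPoint's relative location in SpawnLocation.
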(event `self.ReceiveActorEndOverlap`
  (params (OtherActor :type "Actor Object Reference"))
  (`KismetSystemLibrary.K2_ClearAndInvalidateTimerHandle` (`self.VentTimer`)))

(event `self.ReceiveActorBeginOverlap`
  (params (OtherActor :type "Actor Object Reference"))
  (bind _returnvalue (`KismetSystemLibrary.K2_SetTimerDelegate` (delegate `VentToTunnels`) 5.0))
  (set `self.VentTimer` _returnvalue))

(event `VentToTunnels`
  (`KismetSystemLibrary.Delay` 2.0)
  (bind _asbp_sal (cast `/Game/Blueprints/AI/Enemies/BP_SAL` (stale `self.ReceiveActorBeginOverlap` OtherActor)))
  (bind _asbp_tunnel_vent (cast `/Game/Blueprints/Interactables/LevelProps/BP_TunnelVent` (`self.VentTarget`)))
  (`self.K2_TeleportTo` :`self` _asbp_sal :`DestLocation` (`SceneComponent.K2_GetComponentLocation` (`/Game/Blueprints/Interactables/LevelProps/BP_TunnelVent.SpawnPoint` _asbp_tunnel_vent))))

(fn `UserConstructionScript`
  (set `self.SpawnLocation` (`SceneComponent.RelativeLocation` (`self.SpawnPoint`))))