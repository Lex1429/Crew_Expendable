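; BP_GhostMode is a player-controlled character with Enhanced Input movement, look and jump, adding IMC_Characters on BeginPlay.
; Look pitch follows an inversion flag in the game instance, which ToggleInverted flips.
; Holster events route from server to local to attach a weapon to its mesh socket.
; The GhostMode function is an empty stub, with unconnected spawn-and-possess nodes that have no class set.
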(event `self.ReceiveBeginPlay`
  ;[1 1 1] Initialize Controller
  (`|ExecutionSequence`
    (:`then_0`
      (bind _asbp_player_controller_core (cast `/Game/Blueprints/Systems/BP_PlayerController_Core` (`self.GetController`)))
      (bind _returnvalue (pcsubsystem `EnhancedInputLocalPlayerSubsystem` _asbp_player_controller_core))
      (`/Engine/EditorBlueprintResources/StandardMacros.IsValid` _returnvalue
        (:`Is Valid`
          (`EnhancedInputSubsystemInterface.AddMappingContext` _returnvalue "/Game/Blueprints/Inputs/IMC_Characters.IMC_Characters" 0 (struct)))))))

(event `EnhancedInput|/Game/Blueprints/Inputs/IA_Look`
  (params (ActionValue :type "Vector2D Structure") (ElapsedSeconds :type "Float (double-precision)") (TriggeredSeconds :type "Float (double-precision)") (InputAction :type "InputAction Object Reference" :default "/Game/Blueprints/Inputs/IA_Look.IA_Look"))
  (bind (_x _y) (`KismetMathLibrary.BreakVector2D` ActionValue))
  ;[1 1 1] Camera Control
  (:`Triggered`
    (bind _inversionpitch (`self.MouseInversion`))
    (`self.AddControllerYawInput` _x)
    (`self.AddControllerPitchInput` (* _y _inversionpitch))))

(event `EnhancedInput|/Game/Blueprints/Inputs/IA_Jump`
  (params (ActionValue :type Boolean) (ElapsedSeconds :type "Float (double-precision)") (TriggeredSeconds :type "Float (double-precision)") (InputAction :type "InputAction Object Reference" :default "/Game/Blueprints/Inputs/IA_Jump.IA_Jump"))
  ;[0.8854 0.8854 0.8854] Jumping
  (:`Triggered`
    (`self.Jump`))
  (:`Completed`
    (`self.StopJumping`)))

(event `ToggleInverted`
  (bind _returnvalue (`GameplayStatics.GetGameInstance`))
  ;[1 1 1] Toggle Invert
  (`/Engine/EditorBlueprintResources/StandardMacros.FlipFlop`
    (:`A`
      (message `/Game/Blueprints/Interfaces/BPI_PlayerSettings.SetMouseInversion` _returnvalue true))
    (:`B`
      (message `/Game/Blueprints/Interfaces/BPI_PlayerSettings.SetMouseInversion` _returnvalue false))))

(event `EnhancedInput|/Game/Blueprints/Inputs/IA_Move`
  (params (ActionValue :type "Vector2D Structure") (ElapsedSeconds :type "Float (double-precision)") (TriggeredSeconds :type "Float (double-precision)") (InputAction :type "InputAction Object Reference" :default "/Game/Blueprints/Inputs/IA_Move.IA_Move"))
  (bind (_x _y) (`KismetMathLibrary.BreakVector2D` ActionValue))
  (bind (_returnvalue_roll _returnvalue_pitch _returnvalue_yaw) (`KismetMathLibrary.BreakRotator` (`self.GetControlRotation`)))
  (bind (_returnvalue_roll_2 _returnvalue_pitch_2 _returnvalue_yaw_2) (`KismetMathLibrary.BreakRotator` (`self.GetControlRotation`)))
  ;[1 1 1] Player Movement
  (:`Triggered`
    (`self.AddMovementInput` (`KismetMathLibrary.GetRightVector` (`KismetMathLibrary.MakeRotator` _returnvalue_roll 0.0 _returnvalue_yaw)) _x)
    (`self.AddMovementInput` (`KismetMathLibrary.GetForwardVector` (`KismetMathLibrary.MakeRotator` 0.0 0.0 _returnvalue_yaw_2)) _y)))

(event `Server_HolsterWeapon`
  (params (Target :type "/Game/Blueprints/Interactables/Weapons/BP_WeaponComponentMaster Object Reference"))
  ;[0 0.1464 1 0.5] Holsters Weapons when new weapon is picked up
  (`self.Local_HolsterWeapon` Target))

(event `Local_HolsterWeapon`
  (params (Target :type "/Game/Blueprints/Interactables/Weapons/BP_WeaponComponentMaster Object Reference"))
  ;[0 0.1464 1 0.5] Holsters Weapons when new weapon is picked up
  (`SceneComponent.K2_AttachToComponent` Target (`self.Mesh`) (`/Game/Blueprints/Interactables/Weapons/BP_WeaponComponentMaster.HolsterSocketName` Target) "KeepRelative" "KeepRelative" "KeepRelative" true))

(fn `GetMouseInversion`
  (returns (MouseInverted :type Boolean))
  (return false))

(fn `GhostMode`
  (params (SpawnTransform :type "Transform Structure")))

(fn `MouseInversion`
  (returns (InversionPitch :type "Float (double-precision)"))
  (bind _mouseinverted (message `/Game/Blueprints/Interfaces/BPI_PlayerSettings.GetMouseInversion` (`GameplayStatics.GetGameInstance`)))
  (if _mouseinverted
    (bind _output_get (set `self.InversionPitch` 1.0))
    (return _output_get)
    (else
      (bind _output_get_2 (set `self.InversionPitch` -1.0))
      (return _output_get_2))))

(fn `UserConstructionScript`)